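; Utility function collection for HUD widgets, covering material-driven images, screen positioning and view-model access.
; Helpers create and cache dynamic material instances, push progress-bar parameters into them, and convert widget-local coordinates to scale-multiplied viewport positions.
; Others look up the gameflow view-model actor and bind or unbind blackboard added/removed delegates on the game-state view model.
; A trailer-mode query reads the cheat manager, returning false when it is invalid.
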(fn `AssignDMI`
  (params (Material :type "MaterialInterface Object Reference") (Image :type "Image Object Reference") (Cache :type "MaterialInstanceDynamic Object Reference (by ref)"))
  (bind _returnvalue (`KismetMaterialLibrary.CreateDynamicMaterialInstance` null Material))
  (`Image.SetBrushFromMaterial` (`local.image`) _returnvalue)
  (`|VariableSetRef` (`local.cache`) _returnvalue))

(fn `BindGameBlackboard`
  (params (AddDelegate :type "Delegate (by ref)") (RemoveDelegate :type "Delegate (by ref)"))
  (returns (OutViewModel :type "/Game/Blueprints/Gameflow/ViewModel/B_VM_GameState Object Reference"))
  (locals (vm_gameState :type "/Game/Blueprints/Gameflow/ViewModel/B_VM_GameState Object Reference"))
  (bind _output_get (set `local.vm_gameState` (`/Game/Blueprints/Gameflow/GS_GameStateCustom.GetViewModel` (`/Game/Blueprints/Core/Utilities/BP_Utils.Game State` null))))
  (add `/Game/Blueprints/Gameflow/ViewModel/B_VM_GameState.OnNotifyBlackboardAdded` _output_get AddDelegate)
  (add `/Game/Blueprints/Gameflow/ViewModel/B_VM_GameState.OnNotifyBlackboardRemoved` _output_get RemoveDelegate)
  (return (`local.vm_gameState`)))

(fn `GetViewportPosition`
  (params (InWidget :type "Widget Object Reference") (LocalCoordinate :type "Vector2D Structure"))
  (returns (ViewportPosition :type "Vector2D Structure"))
  (return (* (`.ViewportPosition` (`SlateBlueprintLibrary.LocalToViewport` null (`Widget.GetCachedGeometry` InWidget) LocalCoordinate)) (`WidgetLayoutLibrary.GetViewportScale` null))))

(fn `GlobalViewModelSystem`
  (returns (OutGlobalVM :type "/Game/Blueprints/Core/ViewModel/BP_Gameflow_ViewModel Object Reference"))
  (bind _returnvalue (`GameplayStatics.GetActorOfClass` null "/Game/Blueprints/Core/ViewModel/BP_Gameflow_ViewModel.BP_Gameflow_ViewModel_C"))
  (return _returnvalue))

(fn `IsTrailerMode`
  (returns (OutValid :type Boolean))
  (locals (vm_playerState :type "/Game/Blueprints/Player/ViewModel/B_VM_PlayerState Object Reference"))
  (bind (_outvalid _outcheats) (`/Game/Blueprints/Core/Debug/B_Utilities_Cheats.IsCheatManagerValid` null))
  (if _outvalid
    (return (`/Game/Blueprints/Core/Debug/B_CheatManager_Uncertified.IsTrailerTemporaryMode` _outcheats))
    (else
      (return false))))

(fn `SetProgressBarInfo`
  (params (info :type "/Game/Blueprints/HUD/Utilities/GlobalStruct/STR_UI_ProgressBar Structure") (DMI :type "MaterialInstanceDynamic Object Reference"))
  (bind _dmi (`local.DMI`))
  (bind (_percent _startangle _thickness _bflipdirection) (break `/Game/Blueprints/HUD/Utilities/GlobalStruct/STR_UI_ProgressBar` (`local.info`)))
  (`MaterialInstanceDynamic.SetScalarParameterValue` _dmi "Percent" _percent)
  (`MaterialInstanceDynamic.SetScalarParameterValue` _dmi "StartAngle" _startangle)
  (`MaterialInstanceDynamic.SetScalarParameterValue` _dmi "Thickness" _thickness)
  (`MaterialInstanceDynamic.SetScalarParameterValue` _dmi "FlipDirection" (select `bool` _bflipdirection :`true` 1.0 :!type "Float (single-precision)")))

(fn `UnbindGameBlackboard`
  (params (AddDelegate :type "Delegate (by ref)") (RemoveDelegate :type "Delegate (by ref)"))
  (returns (OutViewModel :type "/Game/Blueprints/Gameflow/ViewModel/B_VM_GameState Object Reference"))
  (locals (vm_gameState :type "/Game/Blueprints/Gameflow/ViewModel/B_VM_GameState Object Reference"))
  (bind _output_get (set `local.vm_gameState` (`/Game/Blueprints/Gameflow/GS_GameStateCustom.GetViewModel` (`/Game/Blueprints/Core/Utilities/BP_Utils.Game State` null))))
  (remove `/Game/Blueprints/Gameflow/ViewModel/B_VM_GameState.OnNotifyBlackboardAdded` _output_get AddDelegate)
  (remove `/Game/Blueprints/Gameflow/ViewModel/B_VM_GameState.OnNotifyBlackboardRemoved` _output_get RemoveDelegate)
  (return (`local.vm_gameState`)))