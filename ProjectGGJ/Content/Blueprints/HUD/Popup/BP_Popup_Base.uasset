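; BP_Popup_Base is a base popup actor that shows a supplied widget in a focused interaction mode.
; BeginPlay switches the game mode's focus and input mappings and hides the custom HUD.
; StartWidget creates and adds the popup to the viewport; GetPopup exposes it and its class.
; OnBeginPress restores input and, if the HUD exists, shows it and destroys the actor, without explicitly removing the popup widget.
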(event `self.ReceiveBeginPlay`
  (`/Game/Blueprints/Gameflow/GM_GGJ2024_Base.SetInteractFocusMode` (`/Game/Blueprints/Gameflow/BP_Utils.Game Mode`) true "/Game/Inputs/IM_LockInteractionMap.IM_LockInteractionMap" "/Game/Inputs/IM_CustomInputMap.IM_CustomInputMap")
  ;[1 1 1] to move to player view
  (bind _foundwidgets (`WidgetBlueprintLibrary.GetAllWidgetsOfClass` "/Game/Blueprints/HUD/BP_Widget_HUDCustom.BP_Widget_HUDCustom_C"))
  (if (`KismetArrayLibrary.Array_IsNotEmpty` _foundwidgets)
    (`Widget.SetVisibility` (`|GetArrayItem` _foundwidgets) "Hidden") ; only hides it
  ))

(event `StartWidget`
  (params (widget :type "UserWidget Class Reference") (controller :type "Controller Object Reference"))
  (bind _output_get (set `self.widgetClass` widget))
  (bind _asplayer_controller (cast `PlayerController` controller))
  (bind _returnvalue (`|CreateWidget` _output_get _asplayer_controller))
  (bind _output_get_2 (set `self.widgetPopup` _returnvalue))
  (`UserWidget.AddToViewport` _output_get_2 0))

(event `OnBeginPress`
  (`/Game/Blueprints/Gameflow/GM_GGJ2024_Base.SetInteractFocusMode` (`/Game/Blueprints/Gameflow/BP_Utils.Game Mode`) false "/Game/Inputs/IM_CustomInputMap.IM_CustomInputMap" "/Game/Inputs/IM_LockInteractionMap.IM_LockInteractionMap")
  (bind _foundwidgets (`WidgetBlueprintLibrary.GetAllWidgetsOfClass` "/Game/Blueprints/HUD/BP_Widget_HUDCustom.BP_Widget_HUDCustom_C"))
  (if (`KismetArrayLibrary.Array_IsNotEmpty` _foundwidgets)
    (`Widget.SetVisibility` (`|GetArrayItem` _foundwidgets) "Visible")
    (`self.K2_DestroyActor`)))

(fn `GetPopup`
  (returns (popup :type "UserWidget Object Reference") (class :type "UserWidget Class Reference"))
  (return (`self.widgetPopup`) (`self.widgetClass`)))

(fn `UserConstructionScript`)