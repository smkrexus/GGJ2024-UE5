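; BP_Reflector_Overlay_InfluenceLevel is an overlay actor that presents the influence level celebration on the HUD.
; Display creates the default widget from its celebration view model, adds it to the viewport and forces a refresh.
; When the view model notifies the common button Select tag, Clear removes the view and destroys the actor.
; GetViewModel exposes the view model to callers.
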(event `self.B_VM_Celebration_InfluenceLevel.OnNotifyEvent`
  (params (tag :type "GameplayTag Structure"))
  (`|SwitchGameplayTag` tag
    (:`ViewModel.Common.Button.Select`
      (`self.Clear`))))

(fn `Clear`
  (`/Game/Blueprints/Core/ViewModel/B_VM_BaseComponent.RemoveView` (`self.B_VM_Celebration_InfluenceLevel`))
  (`self.K2_DestroyActor`))

(fn `Display`
  (bind _b_vm_celebration_influencelevel (`self.B_VM_Celebration_InfluenceLevel`))
  (bind _view (`/Game/Blueprints/Core/ViewModel/B_VM_BaseComponent.CreateView` _b_vm_celebration_influencelevel (`/Game/Blueprints/Core/ViewModel/B_VM_BaseComponent.GetDefaultWidget` _b_vm_celebration_influencelevel)))
  (`UserWidget.AddToViewport` _view 0)
  (`/Game/Blueprints/Core/ViewModel/B_VM_BaseComponent.ForceRefresh` _b_vm_celebration_influencelevel))

(fn `GetViewModel`
  (returns (OutViewModel :type "/Game/Blueprints/HUD/Celebration/B_VM_Celebration_InfluenceLevel Object Reference"))
  (return (`self.B_VM_Celebration_InfluenceLevel`)))

(fn `UserConstructionScript`
  (`parent.UserConstructionScript`))