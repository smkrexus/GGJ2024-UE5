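; Emote manager for the HUD that queues emote requests and feeds them to its emote view model.
; QueueEmoteRequest wraps a handle in a B_QueueItem_Emote and adds it to the queue component.
; OnNext passes the handle to the view model and attaches that view model to the global player view model's emote slot.
; The view model's timer-clear notify tag advances the queue.
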(event `self.B_QueueItemComponent.OnNext`
  (params (Item :type "/Game/Blueprints/Core/UI/B_QueueItem_Base Object Reference (by ref)"))
  (bind _asb_queue_item_emote (cast `/Game/Blueprints/HUD/Emotes/B_QueueItem_Emote` Item))
  (`KismetSystemLibrary.PrintString` "OnNext")
  (`/Game/Blueprints/HUD/Emotes/B_VM_EmoteManager.VM_AddEmote` (`self.B_VM_EmoteManager`) (`/Game/Blueprints/HUD/Emotes/B_QueueItem_Emote.GetHandle` _asb_queue_item_emote))
  (bind _asviewmodel_player (cast `/Game/Blueprints/Player/ViewModel/B_VM_Player` (`/Game/Blueprints/Core/ViewModel/BP_Gameflow_ViewModel.GetViewModel` (`/Game/Blueprints/HUD/Utilities/BP_Utilities_Widget.GlobalViewModelSystem`) "/Game/Blueprints/Player/ViewModel/B_VM_Player.B_VM_Player_C")))
  (`/Game/Blueprints/Player/ViewModel/B_VM_Player.VM_AddExtension` _asviewmodel_player "emote_01" (`self.B_VM_EmoteManager`)))

(event `self.B_VM_EmoteManager.OnNotifyEvent`
  (params (tag :type "GameplayTag Structure"))
  (`|SwitchGameplayTag` tag
    (:`ViewModel.Common.Refresh.Timer.Clear`
      (`/Game/Blueprints/Core/UI/B_QueueItemComponent.MoveQueue` (`self.B_QueueItemComponent`)))))

(fn `GetViewModel`
  (returns (OutViewModel :type "/Game/Blueprints/HUD/Emotes/B_VM_EmoteManager Object Reference"))
  (return (`self.B_VM_EmoteManager`)))

(fn `QueueEmoteRequest`
  (params (InHandle :type "/Game/Blueprints/HUD/Emotes/STR_EmoteHandle Structure"))
  (bind _returnvalue (`|GenericCreateObject` "/Game/Blueprints/HUD/Emotes/B_QueueItem_Emote.B_QueueItem_Emote_C" InHandle))
  (`/Game/Blueprints/Core/UI/B_QueueItemComponent.Add` (`self.B_QueueItemComponent`) _returnvalue))

(fn `UserConstructionScript`)