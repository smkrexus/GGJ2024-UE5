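; BP_PickableItem_DebugItemB is a debug pickable item Blueprint for observing item capacity changes.
; When its ItemCapacityComponent fires OnCapacityChange, it prints the delta and the component's current capacity as formatted text.
; It adds no other logic: BeginPlay, overlap and Tick are disabled stubs, and the construction script only calls the parent.
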(event `self.ItemCapacityComponent.OnCapacityChange`
  (params (delta :type "Float (double-precision)"))
  (`KismetSystemLibrary.PrintText` (`|FormatText` "Capacity Change {delta} : current {c}" delta (`/Game/Blueprints/Interactables/Extensions/Items/B_ItemCapacityComponent.current` (`self.ItemCapacityComponent`)))))

(fn `UserConstructionScript`
  (`parent.UserConstructionScript`))