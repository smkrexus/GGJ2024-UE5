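; BP_PlacementItem_Base is a base actor for an interactable spot where a player places their active equipment item.
; On Interact, if its ItemDefinitionComponent has a valid item, it drops the full active stack from the controlled BP_PawnCustom's equipment component.
; The drop uses BP_EquipmentAction_Drop_Placement with this actor as instigator.
; A successful drop destroys the actor, marked as temporary behavior.
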(event `/Game/Blueprints/Interactables/BPI_Interactable.Interact`
  (params (controller :type "Controller Object Reference"))
  (if (`/Game/Blueprints/Items/B_ItemDefinitionComponent.HasValidItem` (`self.ItemDefinitionComponent`))
    (bind _asbp_pawn_custom (cast `/Game/Blueprints/BP_PawnCustom` (`Controller.K2_GetPawn` controller)))
    (`|ExecutionSequence`
      (:`then_0`
        (bind _returnvalue (`self.GetComponentByClass` _asbp_pawn_custom "/Game/Blueprints/Pawn/B_PawnEquipmentComponent.B_PawnEquipmentComponent_C"))
        (bind (_activeitem _handle) (`/Game/Blueprints/Pawn/B_PawnEquipmentComponent.GetActiveItem` _returnvalue))
        (bind _itemdropped (`/Game/Blueprints/Pawn/B_PawnEquipmentComponent.DropItem` _returnvalue _activeitem (`.stackCount_10_17932609405E05092F7DF690CEF9C84C` (break `/Game/Blueprints/Items/STR_ItemHandle` _handle)) "/Game/Blueprints/Pawn/Equipment/BP_EquipmentAction_Drop_Placement.BP_EquipmentAction_Drop_Placement_C" self))
        (if _itemdropped
          (`self.K2_DestroyActor`) ; temp version
        )))))

(fn `UserConstructionScript`
  (`parent.UserConstructionScript`))