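; Item utility Blueprint that finds item definitions in the DT_ItemList data table matching a gameplay tag filter.
; FindItemsByFilter loads each row's definition class synchronously and checks tags from its class defaults, without spawning items.
; Items need an exact match with any valid tag, or pass if none are specified, and are excluded by any exact blocked-tag match.
; It returns the unique matching definitions and whether any exist.
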(fn `FindItemsByFilter`
  (params (filter :type "/Game/Blueprints/Interactables/Requirements/STR_InteractRequirement_TagSettings Structure"))
  (returns (items :type "Array of /Game/Blueprints/Items/Definitions/B_ItemDefinition_Base Soft Class Reference") (hasItems :type Boolean))
  (locals (foundItems :type "Array of /Game/Blueprints/Items/Definitions/B_ItemDefinition_Base Soft Class Reference"))
  (bind _founditems (`local.foundItems`))
  (bind (_validtags _blockedtags) (break `/Game/Blueprints/Interactables/Requirements/STR_InteractRequirement_TagSettings` (`local.filter`)))
  (bind _outrownames (`DataTableFunctionLibrary.GetDataTableRowNames` "/Game/Blueprints/Items/List/DT_ItemList.DT_ItemList"))
  (for _array_element _outrownames
    (bind _returnvalue (`|GetDataTableRow` "/Game/Blueprints/Items/List/DT_ItemList.DT_ItemList" _array_element)
      (:`then`
        (bind ((`definition_14_4466125D4906A351F095EC90E9362479` _definition)) (break `/Game/Blueprints/Items/List/STR_ItemList` _returnvalue))
        (bind _returnvalue_2 (`KismetSystemLibrary.LoadClassAsset_Blocking` _definition))
        (bind _tags (defaults `Object` (castclass `/Game/Blueprints/Items/Definitions/B_ItemDefinition_Base` _returnvalue_2 :!pure true)))
        (if (and (or (`BlueprintGameplayTagLibrary.HasAnyTags` _tags _validtags true) (== (`BlueprintGameplayTagLibrary.GetNumGameplayTagsInContainer` _validtags) 0)) (not (`BlueprintGameplayTagLibrary.HasAnyTags` _tags _blockedtags true)))
          (`KismetArrayLibrary.Array_AddUnique` (`local.foundItems`) _definition)))))
  (return _founditems (`KismetArrayLibrary.Array_IsNotEmpty` _founditems)))