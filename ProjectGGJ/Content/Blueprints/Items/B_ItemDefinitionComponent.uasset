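; Item definition component that links its owner to an item row in a data table and supplies that item's data.
; HasValidItem confirms that the Definition row handle points to a valid table and an existing row.
; RetrieveDataFromDefinition lazily blocking-loads the row's definition class, constructs and caches it as a B_ItemDefinition_Base object, then returns its GetData result.
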(event `self.ReceiveBeginPlay`)

(fn `HasValidItem`
  (returns (valid :type Boolean))
  (bind (_datatable _rowname) (break `DataTableRowHandle` (`self.definition`)))
  (if (`KismetSystemLibrary.IsValid` _datatable)
    (bind _returnvalue (`|GetDataTableRow` _datatable _rowname)
      (:`then`
        (return true))
      (:`RowNotFound`
        (return false)))
    (else
      (return false))))

(fn `RetrieveDataFromDefinition`
  (returns (item :type "/Game/Blueprints/Items/ItemInfoData Object Reference"))
  (bind (_datatable _rowname) (break `DataTableRowHandle` (`self.definition`)))
  (if (`self.HasValidItem`)
    (bind _returnvalue (`|GetDataTableRow` _datatable _rowname)
      (:`then`
        (bind _itemdefinition (`self.itemDefinition`)
          (:`then`
            (return (`/Game/Blueprints/Items/Definitions/B_ItemDefinition_Base.GetData` _itemdefinition)))
          (:`else`
            (bind _returnvalue_2 (`KismetSystemLibrary.LoadClassAsset_Blocking` (`.definition_14_4466125D4906A351F095EC90E9362479` (break `/Game/Blueprints/Items/List/STR_ItemList` _returnvalue))))
            (bind _returnvalue_3 (`|GenericCreateObject` _returnvalue_2))
            (bind _output_get (set `self.itemDefinition` (cast `/Game/Blueprints/Items/Definitions/B_ItemDefinition_Base` _returnvalue_3 :!pure true)))
            (return (`/Game/Blueprints/Items/Definitions/B_ItemDefinition_Base.GetData` _output_get)))))
      (:`RowNotFound`
        (return null)))
    (else
      (return null))))