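; Base Blueprint for world items that a player can pick up through interaction.
; On Interact with a valid item definition, it builds an item handle from the definition data, its own class and its unequip/drop behaviours.
; It passes that handle to the controlled BP_PawnCustom's equipment component as a single-item stack.
; It then plays the interact definition's 2D sound and destroys itself.
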(event `/Game/Blueprints/Interactables/BPI_Interactable.Interact`
  (params (controller :type "Controller Object Reference"))
  (if (`/Game/Blueprints/Items/B_ItemDefinitionComponent.HasValidItem` (`self.ItemDefinitionComponent`))
    (bind _asbp_pawn_custom (cast `/Game/Blueprints/BP_PawnCustom` (`Controller.K2_GetPawn` controller)))
    (`|ExecutionSequence`
      (:`then_0`
        (`/Game/Blueprints/Pawn/B_PawnEquipmentComponent.PickupItem` (`self.GetComponentByClass` _asbp_pawn_custom "/Game/Blueprints/Pawn/B_PawnEquipmentComponent.B_PawnEquipmentComponent_C") (make `/Game/Blueprints/Items/STR_ItemHandle` (`|ConvertAsset` (`/Game/Blueprints/Items/B_ItemDefinitionComponent.RetrieveDataFromDefinition` (`self.ItemDefinitionComponent`))) (`|ConvertAsset` (`GameplayStatics.GetObjectClass` self)) 1 (make `/Game/Blueprints/Items/STR_ItemEquipActionHandle` (`self.UnequipBehaviour`) (`self.DropBehaviour`)))))
      (:`then_1`
        (`GameplayStatics.PlaySound2D` (`/Game/Blueprints/Interactables/InteractableInfoData.sound` (`/Game/Blueprints/Interactables/B_InteractDefinitionComponent.RetrieveDataFromDefinition` (`self.InteractDefinitionComponent`))) 1.0 1.0 0.0 null null))
      (:`then_2`
        (`self.K2_DestroyActor`)))))

(fn `ChildFunction`)

(fn `UserConstructionScript`
  (`parent.UserConstructionScript`))