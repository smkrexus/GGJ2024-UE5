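; Component that posts simulated social media notifications to the game's social media notification channel.
; DisplayNotification shuffles the NotificationData table, sends the first message whose tags exactly match the requested tag, and plays a pop sound.
; An empty title gets a generated name, and a delay timer blocks further messages unless overridden.
; An optional looping timer calls a test-notification dispatcher.
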(event `self.ReceiveBeginPlay`
  (if (> (`self.TestMessageLoopDuration`) 0.0)
    (`KismetSystemLibrary.K2_SetTimerDelegate` (delegate `TestNotification`) (`self.TestMessageLoopDuration`) true)))

(event `TestNotification`
  (`self.OnTestNotification`))

(event `ClearMessageRestrictions`
  (`KismetSystemLibrary.K2_ClearAndInvalidateTimerHandle` (`self._messageTimer`)))

(fn `AddCustomInfo`
  (params (InfoClass :type "/Game/Blueprints/Core/Notification/Channels/B_NotificationChannelMessageInfo_Base Class Reference"))
  (returns (OutInfo :type "/Game/Blueprints/Core/Notification/Channels/B_NotificationChannelMessageInfo_Base Object Reference"))
  (bind _returnvalue (`|GenericCreateObject` InfoClass))
  (return _returnvalue))

(fn `DisplayNotification`
  (params (InTitle :type Text) (InDuration :type "Float (double-precision)") (InTag :type "GameplayTag Structure") (InMessageType :type "/Game/Blueprints/Core/Notification/Channels/B_NotificationChannelMessage_Base Class Reference") (ShouldOverride :type Boolean) (InCustomInfo :type "Object Object Reference"))
  (locals (allNames :type "Array of Name"))
  (if (`local.ShouldOverride`)
    _
    (elif (`KismetSystemLibrary.K2_IsValidTimerHandle` (`self._messageTimer`))
      (return)
      (else
        _)))
  (bind _notificationdata (`self.NotificationData`)
    (:`then`
      (bind _outrownames (`DataTableFunctionLibrary.GetDataTableRowNames` _notificationdata))
      (bind _output_get (set `local.allNames` _outrownames))
      (`KismetArrayLibrary.Array_Shuffle` _output_get)
      (for _array_element (`local.allNames`)
        (bind _returnvalue (`|GetDataTableRow` (`self.NotificationData`) _array_element)
          (:`then`
            (bind (_message _collectiontags) (break `/Game/Blueprints/SocialMedia/Messages/STR_SocialMediaMessage` _returnvalue))
            ;[1 1 1] Tag match then add
            (if (`BlueprintGameplayTagLibrary.HasTag` _collectiontags (`local.InTag`) true)
              (if (`KismetTextLibrary.TextIsEmpty` (`local.InTitle`))
                (bind _outtext (`/Game/Blueprints/SocialMedia/B_SocialMediaNameGeneratorComponent.GenerateName` (`/Game/Blueprints/Gameflow/GS_GameStateCustom.SocialMediaNameGeneratorComponent` (`/Game/Blueprints/Core/Utilities/BP_Utils.Game State`))))
                (`/Game/Blueprints/Core/Notification/Channels/B_NotificationChannelManager.AddMessageToChannel` (`/Game/Blueprints/Gameflow/GS_GameStateCustom.NotificationChannelManager` (`/Game/Blueprints/Core/Utilities/BP_Utils.Game State`)) "/Game/Blueprints/SocialMedia/Channel/B_NotificationChannel_SocialMedia.B_NotificationChannel_SocialMedia_C" _outtext _message (`local.InDuration`) (`local.InMessageType`) (`local.InCustomInfo`))
                (else
                  (`/Game/Blueprints/Core/Notification/Channels/B_NotificationChannelManager.AddMessageToChannel` (`/Game/Blueprints/Gameflow/GS_GameStateCustom.NotificationChannelManager` (`/Game/Blueprints/Core/Utilities/BP_Utils.Game State`)) "/Game/Blueprints/SocialMedia/Channel/B_NotificationChannel_SocialMedia.B_NotificationChannel_SocialMedia_C" (`local.InTitle`) _message (`local.InDuration`) (`local.InMessageType`) (`local.InCustomInfo`))))
              (bind _returnvalue_2 (`KismetSystemLibrary.K2_SetTimerDelegate` (`|CreateDelegate` :!event `ClearMessageRestrictions`) (`self.MessageDelay`)))
              (set `self._messageTimer` _returnvalue_2)
              (`GameplayStatics.PlaySound2D` "/Game/Assets/Audio/SC_Notif_pop.SC_Notif_pop" 1.0 1.0 0.0 null null)
              (return))))))
    (:`else`)))