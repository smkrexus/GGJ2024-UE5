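; Component that simulates a social media donator, holding a donor name and amount, and distributing rewards on donation.
; GenerateDonation optionally resets, then, unless a donator is registered, takes a generated name and random amount, gives rewards and fires a donator-found callback.
; Notification functions push banner messages, optionally carrying a reward, through the notification channel manager, optionally mirrored to chat with a pop sound.
; Donator messages are picked randomly from a gameplay-tagged data table.
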(event `self.ReceiveBeginPlay`
  (set `self._notificationManager` (`/Game/Blueprints/Gameflow/GS_GameStateCustom.NotificationChannelManager` (`/Game/Blueprints/Core/Utilities/BP_Utils.Game State`))))

(event `/Game/Blueprints/Core/Rewards/BPI_Rewarder.GiveRewards`
  (params (InGameState :type "GameStateBase Object Reference"))
  (bind _bsuccess (`/Game/Blueprints/Core/Objective/Utilities/B_Utilities_Objective_Rewards.DistributeReward` (`self.Rewards`) self))
  (`KismetSystemLibrary.PrintText` (`|FormatText` "Rewards given from donator: {a}" _bsuccess)))

(fn `GenerateDonation`
  (params (bShouldReset :type Boolean))
  (`|ExecutionSequence`
    (:`then_0`
      (if (`local.bShouldReset`)
        (`self.Reset`)))
    (:`then_1`
      (if (`self.bIsRegistered`)
        (return)
        (else
          (bind _outtext (`/Game/Blueprints/SocialMedia/B_SocialMediaNameGeneratorComponent.GenerateName` (`/Game/Blueprints/Gameflow/GS_GameStateCustom.SocialMediaNameGeneratorComponent` (`/Game/Blueprints/Core/Utilities/BP_Utils.Game State`))))
          (`self.SetDonator` (`KismetStringLibrary.Conv_StringToName` (`KismetTextLibrary.Conv_TextToString` _outtext)) (`KismetMathLibrary.RandomIntegerInRange` 10 50))
          (`/Game/Blueprints/Core/Rewards/BPI_Rewarder.GiveRewards` (`GameplayStatics.GetGameState`))
          (`self.OnDonatorFound`))))))

(fn `GenerateNotification`
  (params (InRequestName :type Name) (InMessage :type Text) (InType :type "/Game/Blueprints/Core/Notification/Channels/B_NotificationChannelMessage_Base Class Reference") (bReplicateInChat :type Boolean))
  (locals (info :type "/Game/Blueprints/SocialMedia/Channel/Banner/B_NotificationChannelMessageInfo_SocialMediaBanner Object Reference"))
  (`|ExecutionSequence`
    (:`then_0`
      (bind _returnvalue (`|GenericCreateObject` "/Game/Blueprints/SocialMedia/Channel/Banner/B_NotificationChannelMessageInfo_SocialMediaBanner.B_NotificationChannelMessageInfo_SocialMediaBanner_C" (`self._donatorName`) (`self._donationAmount`) (`local.InRequestName`) (`local.InMessage`)))
      (set `local.info` _returnvalue)
      (`/Game/Blueprints/Core/Notification/Channels/B_NotificationChannelManager.AddMessageToChannel` (`self._notificationManager`) "/Game/Blueprints/SocialMedia/Channel/Banner/B_NotificationChannel_SocialMediaBanner.B_NotificationChannel_SocialMediaBanner_C" "" "" 0.0 (`local.InType`) (`local.info`)))
    (:`then_1`
      (if (`local.bReplicateInChat`)
        (`/Game/Blueprints/Core/Notification/Channels/B_NotificationChannelManager.AddMessageToChannel` (`self._notificationManager`) "/Game/Blueprints/SocialMedia/Channel/B_NotificationChannel_SocialMedia.B_NotificationChannel_SocialMedia_C" "" "" 0.0 "/Game/Blueprints/SocialMedia/Channel/B_NotificationChannelMessage_SocialMedia_Donator.B_NotificationChannelMessage_SocialMedia_Donator_C" (`local.info`))
        (`GameplayStatics.PlaySound2D` "/Game/Assets/Audio/SC_Notif_pop.SC_Notif_pop" 1.0 1.0 0.0 null null)))))

(fn `GenerateRewardNotification`
  (params (InRequestName :type Name) (InMessage :type Text) (InType :type "/Game/Blueprints/Core/Notification/Channels/B_NotificationChannelMessage_Base Class Reference") (InReward :type "/Game/Blueprints/Core/Rewards/STR_RewardHandle Structure") (bReplicateInChat :type Boolean))
  (locals (info :type "/Game/Blueprints/SocialMedia/Channel/Banner/B_NotificationChannelMessageInfo_SocialMediaBanner Object Reference"))
  (`|ExecutionSequence`
    (:`then_0`
      (bind _returnvalue (`|GenericCreateObject` "/Game/Blueprints/SocialMedia/Channel/Banner/B_NotificationChannelMessageInfo_SocialMediaBanner.B_NotificationChannelMessageInfo_SocialMediaBanner_C" (`self._donatorName`) (`self._donationAmount`) (`local.InRequestName`) (`local.InMessage`)))
      (bind _output_get (set `local.info` _returnvalue))
      (`/Game/Blueprints/SocialMedia/Channel/Banner/B_NotificationChannelMessageInfo_SocialMediaBanner.SetReward` _output_get (`local.InReward`))
      (`/Game/Blueprints/Core/Notification/Channels/B_NotificationChannelManager.AddMessageToChannel` (`self._notificationManager`) "/Game/Blueprints/SocialMedia/Channel/Banner/B_NotificationChannel_SocialMediaBanner.B_NotificationChannel_SocialMediaBanner_C" "" "" 0.0 (`local.InType`) (`local.info`)))
    (:`then_1`
      (if (`local.bReplicateInChat`)
        (`/Game/Blueprints/Core/Notification/Channels/B_NotificationChannelManager.AddMessageToChannel` (`self._notificationManager`) "/Game/Blueprints/SocialMedia/Channel/B_NotificationChannel_SocialMedia.B_NotificationChannel_SocialMedia_C" "" "" 0.0 "/Game/Blueprints/SocialMedia/Channel/B_NotificationChannelMessage_SocialMedia_Donator.B_NotificationChannelMessage_SocialMedia_Donator_C" (`local.info`))
        (`GameplayStatics.PlaySound2D` "/Game/Assets/Audio/SC_Notif_pop.SC_Notif_pop" 1.0 1.0 0.0 null null)))))

(fn `GetDonator`
  (returns (OutName :type Name) (OutAmount :type Integer))
  (return (`self._donatorName`) (`self._donationAmount`)))

(fn `GetDonatorMessage`
  (params (InTag :type "GameplayTag Structure"))
  (returns (OutText :type Text))
  (locals (data :type "Array of Name"))
  (bind _messages (`self.Messages`))
  (bind _outrownames (`DataTableFunctionLibrary.GetDataTableRowNames` _messages))
  (bind _output_get (set `local.data` _outrownames))
  (`KismetArrayLibrary.Array_Shuffle` _output_get)
  (for _array_element (`local.data`)
    (bind _returnvalue (`|GetDataTableRow` _messages _array_element)
      (:`then`
        (bind (_message _collectiontags) (break `/Game/Blueprints/SocialMedia/Messages/STR_SocialMediaMessage` _returnvalue))
        (if (`BlueprintGameplayTagLibrary.HasTag` _collectiontags (`local.InTag`) true)
          (return _message)))))
  (return "Missing Donator Message"))

(fn `Reset`
  (set `self.bIsRegistered` false))

(fn `SetDonator`
  (params (InName :type Name) (InAmount :type Integer))
  (set `self._donatorName` InName)
  (set `self._donationAmount` InAmount)
  (set `self.bIsRegistered` true))