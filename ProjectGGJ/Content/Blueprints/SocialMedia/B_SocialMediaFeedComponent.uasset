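; Actor component that controls whether a social media feed is displayed.
; On BeginPlay it adds a B_VM_SocialMediaFeed view model to its owning actor and stores the reference.
; DisplayFeed and HideFeed set a display flag, then RefreshFeedDisplay pushes that flag to the view model through VMSetDisplayFeed.
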(event `self.ReceiveBeginPlay`
  (bind _returnvalue (`|AddComponentByClass` (`self.GetOwner`) "/Game/Blueprints/SocialMedia/B_VM_SocialMediaFeed.B_VM_SocialMediaFeed_C"))
  (set `self.vm_feed` _returnvalue))

(fn `DisplayFeed`
  (set `self.bIsDisplayFeed` true)
  (`self.RefreshFeedDisplay`))

(fn `GetViewModel`
  (returns (OutViewModel :type "/Game/Blueprints/SocialMedia/B_VM_SocialMediaFeed Object Reference"))
  (return (`self.vm_feed`)))

(fn `HideFeed`
  (set `self.bIsDisplayFeed` false)
  (`self.RefreshFeedDisplay`))

(fn `RefreshFeedDisplay`
  (`/Game/Blueprints/SocialMedia/B_VM_SocialMediaFeed.VM_SetDisplayFeed` (`self.GetViewModel`) (`self.bIsDisplayFeed`)))