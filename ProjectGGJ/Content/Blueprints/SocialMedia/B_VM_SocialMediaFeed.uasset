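; View model Blueprint for the social media feed, holding its display flag, controls-enabled flag, toggle description and input actions.
; Setters store each value and broadcast a named change through CallOnNotifyVariable, while getters expose the flags and description.
; Input actions accumulate by appending.
; Two validators compare supplied actions against them, returning registered matches when the newest action is registered, or registered actions now missing.
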(fn `VM_GetToggleDescription`
  (returns (OutText :type Text))
  (return (`self._toggleDescription`)))

(fn `VM_HasEnabledControls`
  (returns (OutValid :type Boolean))
  (return (`self.bControlsEnabled`)))

(fn `VM_SetDisplayFeed`
  (params (InDisplay :type Boolean))
  (set `self.bIsDisplayFeed` InDisplay)
  (`self.OnNotifyVariable` "displayFeed"))

(fn `VM_SetEnableControls`
  (params (InEnable :type Boolean))
  (set `self.bControlsEnabled` InEnable)
  (`self.OnNotifyVariable` "controlsEnabled"))

(fn `VM_SetInputActions`
  (params (InActions :type "Array of InputAction Soft Object Reference"))
  (`KismetArrayLibrary.Array_Append` (`self._inputActions`) (`local.InActions`))
  (`self.OnNotifyVariable` "inputActions"))

(fn `VM_SetToggleDescription`
  (params (InDescription :type Text))
  (set `self._toggleDescription` InDescription)
  (`self.OnNotifyVariable` "toggleDescription"))

(fn `VM_ShouldDisplayFeed`
  (returns (OutValid :type Boolean))
  (return (`self.bIsDisplayFeed`)))

(fn `VM_ValidateNewAction`
  (params (InActions :type "Array of InputAction Soft Object Reference"))
  (returns (OutValidActions :type "Array of InputAction Soft Object Reference"))
  (locals (validActions :type "Array of InputAction Soft Object Reference"))
  (bind _inactions (`local.InActions`))
  (`|ExecutionSequence`
    (:`then_0`
      ;[0.625 0.1327 0] Ignore if latest action is not part of actions to validate
      (if (not (`KismetArrayLibrary.Array_Contains` (`self._inputActions`) (`|GetArrayItem` _inactions (`KismetArrayLibrary.Array_LastIndex` _inactions))))
        (return (`local.validActions`))))
    (:`then_1`
      (for _array_element (`self._inputActions`)
        (if (`KismetArrayLibrary.Array_Contains` (`local.InActions`) _array_element)
          (`KismetArrayLibrary.Array_AddUnique` (`local.validActions`) _array_element)))
      (return (`local.validActions`)))))

(fn `VM_ValidateRemoveAction`
  (params (InActions :type "Array of InputAction Soft Object Reference"))
  (returns (OutRemoveActions :type "Array of InputAction Soft Object Reference"))
  (locals (removeActions :type "Array of InputAction Soft Object Reference"))
  (for _array_element (`self._inputActions`)
    (if (not (`KismetArrayLibrary.Array_Contains` (`local.InActions`) _array_element))
      (`KismetArrayLibrary.Array_AddUnique` (`local.removeActions`) _array_element)))
  (return (`local.removeActions`)))