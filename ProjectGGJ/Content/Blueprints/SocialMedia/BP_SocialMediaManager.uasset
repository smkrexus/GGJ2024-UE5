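; Social media manager Blueprint whose only logic registers a dynamic objective list view model with the player's UI.
; On BeginPlay, Initialize asks the first player controller to validate its initialization message.
; On success it adds the view model to the controller's B_VM_Player component as an extension in the first objectives slot.
; Otherwise it sets a short timer, apparently to retry until the controller is ready.
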(event `self.ReceiveBeginPlay`
  (`self.Initialize`))

(event `Initialize`
  (bind _outvalidated (message `/Game/Blueprints/Gameflow/Components/BPI_Gameflow_Validator.ValidateInitialization` (`GameplayStatics.GetPlayerController` 0)))
  (if _outvalidated
    (`/Game/Blueprints/Player/ViewModel/B_VM_Player.VM_AddExtension` (`self.GetComponentByClass` (`GameplayStatics.GetPlayerController` 0) "/Game/Blueprints/Player/ViewModel/B_VM_Player.B_VM_Player_C") "objectives_01" (`self.ViewModel_DynamicObjectiveList`))
    (else
      (`KismetSystemLibrary.K2_SetTimerDelegate` (`|CreateDelegate` :!event `Initialize`) 0.5))))

(fn `UserConstructionScript`)