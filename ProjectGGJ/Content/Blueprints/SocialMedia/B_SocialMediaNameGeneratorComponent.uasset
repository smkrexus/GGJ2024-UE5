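; Component that generates random social media names in a hyphenated "left-right" format.
; GenerateName draws one element each from the LeftNames and RightNames data tables and joins them with FormatText.
; GetRandomNameElement shuffles the table's row names and returns the first row's Name field, or an empty string if that row is not found.
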(fn `GenerateName`
  (returns (OutText :type Text))
  (locals (selectedLeft :type Text) (selectedRight :type Text))
  (set `local.selectedLeft` (`self.GetRandomNameElement` (`self._leftNames`)))
  (set `local.selectedRight` (`self.GetRandomNameElement` (`self._rightNames`)))
  (return (`|FormatText` "{left}-{right}" (`local.selectedLeft`) (`local.selectedRight`))))

(fn `GetRandomNameElement`
  (params (InData :type "DataTable Object Reference"))
  (returns (OutName :type Text))
  (locals (allNames :type "Array of Name"))
  (bind _outrownames (`DataTableFunctionLibrary.GetDataTableRowNames` InData))
  (bind _output_get (set `local.allNames` _outrownames))
  (`KismetArrayLibrary.Array_Shuffle` _output_get)
  (bind _returnvalue (`|GetDataTableRow` (`local.InData`) (`|GetArrayItem` (`local.allNames`)))
    (:`then`
      (return (`.name_3_C1164CE24A3810C4F2D62ABCC3E3AB7B` (break `/Game/Blueprints/SocialMedia/Names/STR_SocialMediaName` _returnvalue))))
    (:`RowNotFound`
      (return ""))))