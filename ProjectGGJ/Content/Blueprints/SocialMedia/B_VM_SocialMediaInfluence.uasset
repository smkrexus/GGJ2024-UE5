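; View model for social media influence, holding the Views and Followers values shown in the player's UI.
; Each setter stores its value and fires a named variable notification for bound views, with matching getters for reads.
; CreateAllViews builds the view and follower widgets and manually registers them as extensions in two social media slots on the player view model.
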(fn `CreateAllViews`
  (params (PlayerViewModel :type "/Game/Blueprints/Player/ViewModel/B_VM_Player Object Reference"))
  (`|ExecutionSequence`
    (:`then_0`
      (bind _view (`self.CreateView` (`self._viewWidget`)))
      (`/Game/Blueprints/Player/ViewModel/B_VM_Player.VM_AddExtensionManual` (`local.PlayerViewModel`) "socialmedia_01" _view))
    (:`then_1`
      (bind _view_2 (`self.CreateView` (`self._followerWidget`)))
      (`/Game/Blueprints/Player/ViewModel/B_VM_Player.VM_AddExtensionManual` (`local.PlayerViewModel`) "socialmedia_02" _view_2))))

(fn `VM_GetFollowers`
  (returns (OutFollowers :type Integer))
  (return (`self._followers`)))

(fn `VM_GetViews`
  (returns (OutViews :type Integer))
  (return (`self._views`)))

(fn `VM_SetFollowers`
  (params (InFollowers :type Integer))
  (set `self._followers` InFollowers)
  (`self.OnNotifyVariable` "followers"))

(fn `VM_SetViews`
  (params (InViews :type Integer))
  (set `self._views` InViews)
  (`self.OnNotifyVariable` "views"))