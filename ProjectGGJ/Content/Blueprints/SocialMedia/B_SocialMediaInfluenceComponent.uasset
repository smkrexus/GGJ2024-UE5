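; Social media influence component that simulates livestreaming, tracking views, followers and interest, with save and load through the game instance.
; While streaming, timers drive engagement and view gains, with views scaling by followers and influence level; full interest also adds followers.
; View gains pass through modifiers keyed by active game-event tags.
; Changes feed a view model and scenario counters, while stream state reaches subscribers through an observer pattern with disposable unsubscribers.
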(event `self.ReceiveBeginPlay`
  (`|ExecutionSequence`
    (:`then_0`
      (bind _returnvalue (`|GenericCreateObject` "/Game/Blueprints/SocialMedia/Stats/B_Stat_SocialMedia_Views.B_Stat_SocialMedia_Views_C"))
      (set `self._statViews` _returnvalue)
      (bind _returnvalue_2 (`|GenericCreateObject` "/Game/Blueprints/SocialMedia/Stats/B_Stat_SocialMedia_ViewInterval.B_Stat_SocialMedia_ViewInterval_C"))
      (set `self._statViewRateInterval` _returnvalue_2)
      (bind _returnvalue_3 (`|GenericCreateObject` "/Game/Blueprints/SocialMedia/Stats/B_Stat_SocialMedia_EngagementInterval.B_Stat_SocialMedia_EngagementInterval_C"))
      (set `self._statEngagementInterval` _returnvalue_3)
      (`/Game/Blueprints/Core/Stats/B_Stat.Initialize` (`self._statViewRateInterval`) "View Rate Interval" (make `/Game/Blueprints/Core/Stats/STR_StatDef` :`Initial` (`self.ViewRateInterval`)))
      (`/Game/Blueprints/Core/Stats/B_Stat.Initialize` (`self._statEngagementInterval`) "Engagement Interval" (make `/Game/Blueprints/Core/Stats/STR_StatDef` :`Initial` (`self.EngagementInterval`))))
    (:`then_1`
      (`self.Load`)
      (`self.ConstructViewModel`) ; only constructs if nothing else calls ViewModel before begin play
      (`self.ListenToGameEvents`))
    (:`then_2`
      (set `self.bInitialized` true))))

(event `EngagementUpdate`
  (`self.AddFollowers` 1) ; should be variable amount
  (`self.OnFollowersUpdated`))

(event `BroadcastFollowerAlert`
  (`self.AddFollowers` 1) ; should be variable amount
  (`self.OnFollowersUpdated`))

(event `ViewRateUpdate`
  (if (<= (`self._followers`) 0)
    (`KismetSystemLibrary.K2_ClearAndInvalidateTimerHandle` (`self._viewRateIntervalTimer`))
    (else
      (`self.AddViews` (`self.CalculateViewRate`)))))

(event `/Game/Blueprints/Gameflow/Save/BPI_SaveGame.Save`
  (bind _asgi_uncertified (cast `/Game/Blueprints/Gameflow/GI_Uncertified` (`GameplayStatics.GetGameInstance`)))
  (bind _globalsave (`/Game/Blueprints/Gameflow/GI_Uncertified.GlobalSave` _asgi_uncertified))
  (bind _structout (setmembers `/Game/Blueprints/Gameflow/Save/STR_Save_Influence` :`StructRef` (`/Game/Blueprints/Gameflow/Save/B_SaveGame_Global.SocialMedia` _globalsave) :`followers` (`self._followers`) :`views` (`self.GET_VIEWS`)))
  (set `/Game/Blueprints/Gameflow/Save/B_SaveGame_Global.SocialMedia` _structout _globalsave))

(event `/Game/Blueprints/Gameflow/Save/BPI_SaveGame.Load`
  (bind _asgi_uncertified (cast `/Game/Blueprints/Gameflow/GI_Uncertified` (`GameplayStatics.GetGameInstance`)))
  (bind (_influencelevel _followers _views) (break `/Game/Blueprints/Gameflow/Save/STR_Save_Influence` (`/Game/Blueprints/Gameflow/Save/B_SaveGame_Global.SocialMedia` (`/Game/Blueprints/Gameflow/GI_Uncertified.GlobalSave` _asgi_uncertified))))
  (set `self._influenceLevel` _influencelevel)
  (set `self._followers` _followers)
  (`/Game/Blueprints/Core/Stats/B_Stat.Change` (`self._statViews`) (`KismetMathLibrary.Conv_IntToDouble` _views)))

(event `/Game/Blueprints/Core/Objective/Interface/ScenarioEvent/BPI_ObserverScenarioEvent.Update`
  (params (InTag :type "GameplayTag Structure") (bEventActive :type Boolean) (Level :type Integer))
  (if bEventActive
    (`BlueprintMapLibrary.Map_Add` (`self._eventMap`) InTag Level)
    (else
      (`BlueprintMapLibrary.Map_Remove` (`self._eventMap`) InTag))))

(event `self.ReceiveEndPlay`
  (params (EndPlayReason :type "EEndPlayReason Enum" :default "Destroyed"))
  (bind __disposablelistener (`self._disposableListener`)
    (:`then`
      (message `/Game/Blueprints/Core/Objective/Interface/BPI_Disposable.Dispose` __disposablelistener))
    (:`else`)))

(event `/Game/Blueprints/SocialMedia/Source/Interface/SubjectObserver/BPI_ObservableSocialMediaStream.Unsubscribe`
  (params (InObserver :type "/Game/Blueprints/SocialMedia/Source/Interface/SubjectObserver/BPI_ObserverSocialMediaStream Interface"))
  (`KismetArrayLibrary.Array_RemoveItem` (`self._subscribers`) InObserver))

(event `ConstructViewModel`
  (`self.vm_influence`
    (:`then`)
    (:`else`
      (bind _returnvalue (`|AddComponentByClass` (`self.GetOwner`) "/Game/Blueprints/SocialMedia/B_VM_SocialMediaInfluence.B_VM_SocialMediaInfluence_C"))
      (set `self.vm_influence` _returnvalue)
      (`self.OnConstructViewModel`))))

(event `OnConstructViewModel`
  (bind _returnvalue (`GameplayStatics.GetPlayerController` 0))
  (`/Engine/EditorBlueprintResources/StandardMacros.IsValid` (`Actor.GetComponentByClass` _returnvalue "/Game/Blueprints/Player/ViewModel/B_VM_Player.B_VM_Player_C")
    (:`Is Valid`
      (`self.InitializeViewModel`))
    (:`Is Not Valid`
      (bind _asbp_pawn_controller_custom (cast `/Game/Blueprints/Pawn/BP_PawnControllerCustom` _returnvalue))
      (add `/Game/Blueprints/Pawn/BP_PawnControllerCustom.OnPlayerViewLoaded` _asbp_pawn_controller_custom (`|CreateDelegate` :!event `InitializeViewModel`)) ; controller has not initialized fully, so bind to that, should use component for loading issues in future\nOnLoaded (GameplayTag) seems better
    )))

(event `InitializeViewModel`
  (`/Game/Blueprints/SocialMedia/B_VM_SocialMediaInfluence.CreateAllViews` (`self.vm_influence`) (`Actor.GetComponentByClass` (`GameplayStatics.GetPlayerController` 0) "/Game/Blueprints/Player/ViewModel/B_VM_Player.B_VM_Player_C"))
  (`/Game/Blueprints/SocialMedia/B_VM_SocialMediaInfluence.VM_SetViews` (`self.vm_influence`) (`self.GET_VIEWS`))
  (`/Game/Blueprints/SocialMedia/B_VM_SocialMediaInfluence.VM_SetFollowers` (`self.vm_influence`) (`self._followers`))
  (`/Game/Blueprints/Core/ViewModel/B_VM_BaseComponent.ForceRefresh` (`self.vm_influence`)))

(event `ListenToGameEvents`
  (bind _outdisposable (message `/Game/Blueprints/Core/Objective/Interface/ScenarioEvent/BPI_ObservableScenarioEvent.Subscribe` (`/Game/Blueprints/Gameflow/GS_GameStateCustom.GetGameEvents` (`/Game/Blueprints/Core/Utilities/BP_Utils.Game State`)) self))
  (set `self._disposableListener` _outdisposable))

(fn `AddFollowers`
  (params (InAmount :type Integer))
  (locals (initialFollowers :type Integer :default 0))
  (bind _output_get (set `local.initialFollowers` (`self._followers`)))
  (set `self._followers` (+ _output_get (`local.InAmount`)))
  (`/Game/Blueprints/SocialMedia/B_VM_SocialMediaInfluence.VM_SetFollowers` (`self.GetInfluenceViewModel`) (`self._followers`))
  (`self.INITIALIZE_VIEWRATEINTERVAL`)
  (`/Game/Blueprints/Gameflow/Components/B_GameScenarioCounter.CountSubscriber` (`.OutCounter` (`/Game/Blueprints/Gameflow/GS_GameStateCustom.GetScenarioComponents` (`/Game/Blueprints/Core/Utilities/BP_Utils.Game State`))) (`local.InAmount`)))

(fn `AddInterest`
  (params (InAmount :type Integer))
  (`|ExecutionSequence`
    (:`then_0`
      (if (`self.bIsPaused`)
        (return)))
    (:`then_1`
      (bind _output_get (set `self._interest` (`KismetMathLibrary.Clamp` (+ InAmount (`self._interest`)) 0 (`self._interestMax`))))
      (if (== _output_get (`self._interestMax`))
        (`self.BroadcastFollowerAlert`)
        (set `self._interest` 0)))))

(fn `AddViews`
  (params (InAmount :type Integer))
  (returns (OutModified :type Boolean))
  (locals (viewsModified :type Integer) (viewsInitial :type Integer) (eventTags :type "GameplayTagContainer Structure") (selectedTagForModification :type "GameplayTag Structure"))
  (bind _output_get (set `local.viewsInitial` InAmount))
  (set `local.viewsModified` _output_get)
  (`|ExecutionSequence`
    (:`then_0`
      (if (`KismetArrayLibrary.Array_IsNotEmpty` (`self.Modifiers`))
        (bind _keys (`BlueprintMapLibrary.Map_Keys` (`self._eventMap`)))
        (set `local.eventTags` (`BlueprintGameplayTagLibrary.MakeGameplayTagContainerFromArray` _keys))
        ;[0.3364 0.5305 1 0.172] Modify values if applicable tags
        (for _array_element (`self.Modifiers`)
          (bind (_outvalid _outtag) (`self.SHOULD_APPLY_MODIFIERS` _array_element (`self._statViews`) (`local.eventTags`)))
          (if _outvalid
            (set `local.selectedTagForModification` _outtag)
            (bind _outmodified (`/StandardModifiers/Blueprints/PDA_StandardModifier.ModifyValue` _array_element (`KismetMathLibrary.Conv_IntToDouble` (`local.viewsModified`)) (- (`BlueprintMapLibrary.Map_Find` (`self._eventMap`) (`local.selectedTagForModification`)) 1)))
            (set `local.viewsModified` (`KismetMathLibrary.FTrunc` _outmodified))))
        (if (<= (`local.viewsModified`) 0)
          (return true))))
    (:`then_1`
      (`/Game/Blueprints/Core/Stats/B_Stat.Change` (`self._statViews`) (`KismetMathLibrary.Conv_IntToDouble` (`local.viewsModified`)))
      (`/Game/Blueprints/Gameflow/Components/B_GameScenarioCounter.CountViews` (`.OutCounter` (`/Game/Blueprints/Gameflow/GS_GameStateCustom.GetScenarioComponents` (`/Game/Blueprints/Core/Utilities/BP_Utils.Game State`))) (`local.InAmount`))
      (`/Game/Blueprints/SocialMedia/B_VM_SocialMediaInfluence.VM_SetViews` (`self.vm_influence`) (`self.GET_VIEWS`)))
    (:`then_2`
      (return (!= (`local.viewsModified`) (`local.viewsInitial`))))))

(fn `CalculateViewRate`
  (returns (ReturnValue :type Integer))
  (return (* (`self._followers`) (`KismetMathLibrary.Clamp` (`self._influenceLevel`) 1 9999))))

(fn `EndStream`
  (set `self.bIsStreaming` false)
  (`KismetSystemLibrary.K2_ClearAndInvalidateTimerHandle` (`self._viewRateIntervalTimer`))
  (`KismetSystemLibrary.K2_ClearAndInvalidateTimerHandle` (`self._followerIntervalTimer`))
  (`self.UPDATE_SUBSCRIBERS`))

(fn `GetInfluenceViewModel`
  (returns (OutViewModel :type "/Game/Blueprints/SocialMedia/B_VM_SocialMediaInfluence Object Reference"))
  (bind _vm_influence (`self.vm_influence`)
    (:`then`
      (return (`self.vm_influence`)))
    (:`else`
      (`self.ConstructViewModel`)
      (return _vm_influence))))

(fn `IsStreaming`
  (returns (OutValid :type Boolean))
  (return (`self.bIsStreaming`)))

(fn `PauseStream`
  (set `self.bIsPaused` true)
  (`KismetSystemLibrary.K2_ClearAndInvalidateTimerHandle` (`self._viewRateIntervalTimer`))
  (`KismetSystemLibrary.K2_ClearAndInvalidateTimerHandle` (`self._followerIntervalTimer`))
  (`self.UPDATE_SUBSCRIBERS`))

(fn `StartStream`
  (set `self.bIsStreaming` true)
  (set `self.bIsPaused` false)
  (`self.INITIALIZE_ENGAGEMENTINTERVAL`)
  (`self.INITIALIZE_VIEWRATEINTERVAL`)
  (`self.UPDATE_SUBSCRIBERS`))

(fn `Subscribe`
  (params (InObserver :type "/Game/Blueprints/SocialMedia/Source/Interface/SubjectObserver/BPI_ObserverSocialMediaStream Interface"))
  (returns (OutDisposable :type "/Game/Blueprints/SocialMedia/Source/Interface/SubjectObserver/B_SocialMediaUnsubscriberStream Object Reference"))
  (`KismetArrayLibrary.Array_Add` (`self._subscribers`) InObserver)
  (`/Game/Blueprints/SocialMedia/Source/Interface/SubjectObserver/BPI_ObserverSocialMediaStream.Update` (`local.InObserver`) (`self.bIsStreaming`) (`self.bIsPaused`)) ; pushes latest updates immediately without waiting for next broadcast
  (bind _returnvalue (`|GenericCreateObject` "/Game/Blueprints/SocialMedia/Source/Interface/SubjectObserver/B_SocialMediaUnsubscriberStream.B_SocialMediaUnsubscriberStream_C"))
  (`/Game/Blueprints/SocialMedia/Source/Interface/SubjectObserver/B_SocialMediaUnsubscriberStream.SetDisposables` _returnvalue self (`local.InObserver`))
  (return _returnvalue))

(fn `ValidateInitialization`
  (returns (OutValidated :type Boolean))
  (return (`self.bInitialized`)))