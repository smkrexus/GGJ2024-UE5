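; BP_ScoreTracker_Base is a base actor that tracks a score and publishes its values and grade pass state to a view model.
; TrackScore runs once, adding a view model component from a configurable class, taking a validator from EnableTracking and setting the condition display.
; Each score update refreshes the view model's scores and checks the validator against grades S through D to set the passed flag.
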(event `OnScoreUpdated`
  (params (InScore :type "/Game/Blueprints/Patient/Session/Scoring/B_SessionScore_Base Object Reference"))
  (`/Game/Blueprints/GameScenario/Score/B_VM_ScoreTracker_Base.VM_UpdateScores` (`self.GetScoreTrackerView`) InScore) ; update the values in vm
  (bind _outvalid (`self.ValidateScore`))
  (`/Game/Blueprints/GameScenario/Score/B_VM_ScoreTracker_Base.VM_SetGradePassed` (`self.GetScoreTrackerView`) _outvalid))

(fn `GetScore`
  (returns (OutScore :type "/Game/Blueprints/Patient/Session/Scoring/B_SessionScore_Base Object Reference"))
  (return (`self._score`)))

(fn `GetScoreTrackerView`
  (returns (OutTracker :type "/Game/Blueprints/GameScenario/Score/B_VM_ScoreTracker_Base Object Reference"))
  (return (`self.vm_scoreTracker`)))

(fn `TrackScore`
  (params (InScore :type "/Game/Blueprints/Patient/Session/Scoring/B_SessionScore_Base Object Reference"))
  (if (`KismetSystemLibrary.IsValid` (`self.vm_scoreTracker`))
    (return) ; tracking already begun
    (else
      (set `self._score` (`local.InScore`))
      (bind _returnvalue (`|AddComponentByClass` (`self.ViewModelClass`)))
      (bind _output_get (set `self.vm_scoreTracker` _returnvalue))
      (`/Game/Blueprints/GameScenario/Score/B_VM_ScoreTracker_Base.VM_SetTrackedScore` _output_get (`local.InScore`))
      (bind _outvalidator (`/Game/Blueprints/Patient/Session/Scoring/B_SessionScore_Base.EnableTracking` (`/Game/Blueprints/GameScenario/Score/B_VM_ScoreTracker_Base.VM_GetTrackedScore` (`self.vm_scoreTracker`)) 0)) ; ensure only the view model uses the tracker
      (set `self._scoreValidator` _outvalidator)
      (`self.OnScoreUpdated` (`local.InScore`))
      (`/Game/Blueprints/GameScenario/Score/B_VM_ScoreTracker_Base.VM_SetTrackedConditionDisplay` (`self.GetScoreTrackerView`) (`/Game/Blueprints/Core/Rewards/Validator/B_RewardValidator_Base.GetRewardDisplayFormat` (`self._scoreValidator`)))
      (add `/Game/Blueprints/Patient/Session/Scoring/B_SessionScore_Base.OnScoresUpdated` (`self._score`) (`|CreateDelegate` :!event `OnScoreUpdated`)))))

(fn `UserConstructionScript`)

(fn `ValidateScore`
  (returns (OutValid :type Boolean))
  (return (`/Game/Blueprints/Core/Rewards/Validator/B_RewardValidator_Base.IsGradeValid` (`self._scoreValidator`) (`|MakeArray` "S" "A" "B" "C" "D" :!type "Name"))))