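; Scenario event for latency that shows a screen glitch while the signal strength stat is at or below a threshold.
; A looping timer is set up for signal decay, and stat notifications from the events view model begin, escalate or clear the event.
; A dynamic post-process material scales glitch strength as the signal weakens.
; Cheat commands stop the timer and set the effect level directly.
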(event `self.ReceiveBeginPlay`
  (`parent.ReceiveBeginPlay`))

(event `OnNotifyReceived_EventStats`
  (params (InTag :type "GameplayTag Structure"))
  (`|SwitchGameplayTag` InTag
    (:`Stats.Event.Scenario.SignalStrength`
      (`self.CheckSignalStrength`)
      (`self.DisplaySignalStrength`))))

(event `self.OnEventBegin`
  ;[1 1 1] Standard events begin / clear / available
  (set `PostProcessComponent.bEnabled` true (`self.PostProcess_Glitch`)))

(event `self.OnEventClear`
  ;[1 1 1] Standard events begin / clear / available
  (set `PostProcessComponent.bEnabled` false (`self.PostProcess_Glitch`))
  (`KismetSystemLibrary.K2_ClearAndInvalidateTimerHandle` (`self.signalReductionTimer`))
  (`self.SAVE_SIGNAL_STRENGTH`))

(event `self.OnEventAvailable`
  ;[1 1 1] Standard events begin / clear / available
  (`self.SET_SIGNAL_REDUCTION_INTERVAL`))

(event `ReduceSignalStrength`
  (`/Game/Blueprints/Core/Stats/B_StatComponent.ChangeStatFromTag` (`/Game/Blueprints/Gameflow/Components/B_GameEvents.GetStats` (`self.GetEventsComponent`)) -1.0 (struct :`TagName` "Stats.Event.Scenario.SignalStrength")))

(event `self.OnCommand`
  (params (InCommand :type Name))
  ;[1 1 1] CHEATS
  (switch `name` InCommand
    (:`start`
      (`/Game/Blueprints/Core/Stats/B_StatComponent.ChangeStatFromTag` (`/Game/Blueprints/Gameflow/Components/B_GameEvents.GetStats` (`self.GetEventsComponent`)) -4.0 (struct :`TagName` "Stats.Event.Scenario.SignalStrength"))
      (`self.BeginEvent` 1)
      (`KismetSystemLibrary.K2_ClearAndInvalidateTimerHandle` (`self.signalReductionTimer`))
      (`self.SET_EFFECT_STRENGTH_DIRECT` 1))))

(event `self.OnCommandLevel`
  (params (InLevel :type Integer))
  ;[1 1 1] CHEATS
  (`KismetSystemLibrary.K2_ClearAndInvalidateTimerHandle` (`self.signalReductionTimer`))
  (`self.SET_EFFECT_STRENGTH_DIRECT` InLevel))

(event `self.OnCommandRemoved`
  ;[1 1 1] CHEATS
  (`self.ClearEvent`)
  (`self.SET_SIGNAL_REDUCTION_INTERVAL`))

(fn `CheckSignalStrength`
  (`|ExecutionSequence`
    (:`then_0`
      ;[1 1 1] Don't use event stats to trigger anything in command mode
      (if (`self.IsWaitingCommands`)
        (return)))
    (:`then_1`
      ;[1 1 1] increase event potency based on signal strength: only when event active
      (if (< (`/Game/Blueprints/GameScenario/Events/Stats/B_VM_StatGroup_Events.VM_GetSignalStrength` (`self.vm_eventStats`)) (`self._signalStrength`))
        (`self.SAVE_SIGNAL_STRENGTH`)
        (if (`self.IsEventActive`)
          (`/Game/Blueprints/Gameflow/Components/B_GameEvents.ActivateEvent` (`self.GetEventsComponent`) (`self.EventTag`) (- (`self.SignalThreshold`) (- (`self._signalStrength`) 1))))
        (else
          (`self.SET_SIGNAL_REDUCTION_INTERVAL`) ; if it was not reduced, reset this timer
        )))
    (:`then_2`
      (if (<= (`/Game/Blueprints/GameScenario/Events/Stats/B_VM_StatGroup_Events.VM_GetSignalStrength` (`self.vm_eventStats`)) (`self.SignalThreshold`))
        (if (not (`self.IsEventActive`))
          (`self.BeginEvent` 1)
          (return))))
    (:`then_3`
      (if (> (`/Game/Blueprints/GameScenario/Events/Stats/B_VM_StatGroup_Events.VM_GetSignalStrength` (`self.vm_eventStats`)) (`self.SignalThreshold`))
        (if (`self.IsEventActive`)
          (`self.ClearEvent`)
          (return))))))

(fn `DisplaySignalStrength`
  (`|ExecutionSequence`
    (:`then_0`
      (if (not (`self.IsEventActive`))
        (return)))
    (:`then_1`
      (if (<= (`/Game/Blueprints/GameScenario/Events/Stats/B_VM_StatGroup_Events.VM_GetSignalStrength` (`self.vm_eventStats`)) (`self.SignalThreshold`))
        (`self.SET_EFFECT_STRENGTH` (`KismetMathLibrary.Lerp` 0.3 0.07 (/ (`KismetMathLibrary.Conv_IntToDouble` (- (`/Game/Blueprints/GameScenario/Events/Stats/B_VM_StatGroup_Events.VM_GetSignalStrength` (`self.vm_eventStats`)) 1)) (`KismetMathLibrary.Conv_IntToDouble` (- (`self.SignalThreshold`) 1)))))))))

(fn `Initialize`
  (params (InEvents :type "/Game/Blueprints/Gameflow/Components/B_GameEvents Object Reference"))
  (`parent.Initialize` InEvents)
  (bind _asb_vm_stat_group_events (cast `/Game/Blueprints/GameScenario/Events/Stats/B_VM_StatGroup_Events` (`/Game/Blueprints/Core/Stats/B_StatComponent.GetViewModel` (`/Game/Blueprints/Gameflow/Components/B_GameEvents.GetStats` (`self.GetEventsComponent`)))))
  (bind _output_get (set `self.vm_eventStats` _asb_vm_stat_group_events))
  (add `/Game/Blueprints/Core/ViewModel/B_VM_BaseComponent.OnNotifyEvent` _output_get (`|CreateDelegate` :!event `OnNotifyReceived_EventStats`))
  (bind _returnvalue (`KismetMaterialLibrary.CreateDynamicMaterialInstance` "/Game/Assets/VFX/PostProcess/PPMI_ScreenGlitch_Default.PPMI_ScreenGlitch_Default"))
  (set `self._glitchEffect` _returnvalue)
  (setmembers `WeightedBlendables` :`StructRef` (`.WeightedBlendables` (break `PostProcessSettings` (`PostProcessComponent.Settings` (`self.PostProcess_Glitch`)))) :`Array` (`|MakeArray` (make `WeightedBlendable` 1.0 (`self._glitchEffect`))))
  (`self.DisplaySignalStrength`))

(fn `UserConstructionScript`
  (`parent.UserConstructionScript`))