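; Base actor for scenario events, with overridable hooks for begin, pause, resume, clear and availability.
; Start/End or level commands begin or clear the event, activating or deactivating its tag on an injected events component.
; A timer set on begin, intended for repeat reminders, pauses with the event and is cleared at the end.
; Clearing either starts a cooldown for restartable events or destroys the actor.
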(event `self.ReceiveBeginPlay`
  (if (`self.bStartAvailable`)
    (`self.OnEventAvailable`)))

(event `OnEventBegin`
  ;[1 1 1] Override in children
)

(event `OnEventPaused`
  ;[1 1 1] Override in children
)

(event `OnEventClear`
  ;[1 1 1] Override in children
)

(event `OnEventResume`
  ;[1 1 1] Override in children
)

(event `OnEventAvailable`
  ;[1 1 1] Override in children
)

(event `OnCommand`
  (params (InCommand :type Name))
  (switch `name` InCommand
    (:`start`
      (`self.BeginEvent` 1))
    (:`end`
      (`self.ClearEvent`))))

(event `OnCommandLevel`
  (params (InLevel :type Integer)))

(event `OnCommandRemoved`)

(fn `BeginEvent`
  (params (InLevel :type Integer :default 1))
  (set `self.bEventActive` true)
  (`|ExecutionSequence`
    (:`then_0`
      (`self.CREATE_REMINDER`))
    (:`then_1`
      (`/Game/Blueprints/Gameflow/Components/B_GameEvents.ActivateEvent` (`self.__EVENTS__`) (`self.EventTag`) (`local.InLevel`))
      (`self.OnEventBegin`))))

(fn `ClearEvent`
  (set `self.bEventActive` false)
  (`KismetSystemLibrary.K2_ClearAndInvalidateTimerHandle` (`self._eventReminderTimer`))
  (`/Game/Blueprints/Gameflow/Components/B_GameEvents.DeactivateEvent` (`self.__EVENTS__`) (`self.EventTag`))
  (`self.OnEventClear`)
  (if (`self.bCanRestart`)
    (`self.CooldownEvent`)
    (else
      (`self.K2_DestroyActor`))))

(fn `CooldownEvent`
  (bind _cooldown (`self.Cooldown`))
  (if (> _cooldown 0.0)
    (`KismetSystemLibrary.K2_SetTimerDelegate` (`|CreateDelegate` :!event `OnEventAvailable`) _cooldown)
    (else
      (`self.OnEventAvailable`))))

(fn `GetEventsComponent`
  (returns (OutEvents :type "/Game/Blueprints/Gameflow/Components/B_GameEvents Object Reference"))
  (return (`self.__EVENTS__`)))

(fn `Initialize`
  (params (InEvents :type "/Game/Blueprints/Gameflow/Components/B_GameEvents Object Reference"))
  (set `self.__EVENTS__` InEvents))

(fn `IsEventActive`
  (returns (OutActive :type Boolean))
  (return (`self.bEventActive`)))

(fn `IsEventPaused`
  (returns (OutPaused :type Boolean))
  (return (`self.bIsPaused`)))

(fn `IsWaitingCommands`
  (returns (OutValid :type Boolean))
  (return (`self.bWaitingCommands`)))

(fn `PauseEvent`
  (set `self.bIsPaused` true)
  (`self.TOGGLE_REMINDER`)
  (`self.OnEventPaused`)
  (`self.OnPause` (`self.EventTag`)))

(fn `PushNotificationReminder`
  (`/Game/Blueprints/Gameflow/Components/B_GameEvents.OnEventReminder` (`self.GetEventsComponent`) (`self.EventTag`)))

(fn `ResumeEvent`
  (set `self.bIsPaused` false)
  (`self.TOGGLE_REMINDER`)
  (`self.OnEventResume`)
  (`self.OnResume` (`self.EventTag`)))

(fn `SendCommand`
  (params (InCommand :type Name))
  (bind _output_get (set `self.bWaitingCommands` (!= InCommand "None")))
  (if _output_get
    (`self.OnCommand` InCommand)
    (else
      (`self.OnCommandRemoved`))))

(fn `SendCommandLevel`
  (params (InLevel :type Integer))
  (bind _inlevel (`local.InLevel`))
  (bind _output_get (set `self.bWaitingCommands` (> InLevel 0)))
  (if _output_get
    (`self.BeginEvent` _inlevel)
    (`self.OnCommandLevel` _inlevel)
    (else
      (`self.OnCommandRemoved`))))

(fn `UserConstructionScript`)