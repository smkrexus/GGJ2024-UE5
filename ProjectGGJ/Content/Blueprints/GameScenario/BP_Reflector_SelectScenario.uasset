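; BP_Reflector_SelectScenario presents one selectable scenario through a scenario definition view model and reports when it is chosen.
; SetScenarioDefinition stores the name, definition and save summary, passes them to the view model, then creates its default widget.
; A notify event carrying the common Select button gameplay tag calls the OnSelectScenario dispatcher with itself, and GetViewModel exposes the view model.
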(event `self.B_VM_ScenarioDefintion.OnNotifyEvent`
  (params (tag :type "GameplayTag Structure"))
  (`|SwitchGameplayTag` tag
    (:`ViewModel.Common.Button.Select`
      (`self.OnSelectScenario` self))))

(fn `GetViewModel`
  (returns (OutViewModel :type "/Game/Blueprints/GameScenario/B_VM_ScenarioDefintion Object Reference"))
  (return (`self.B_VM_ScenarioDefintion`)))

(fn `SetScenarioDefinition`
  (params (InName :type Name) (InDefinition :type "/Game/Blueprints/GameScenario/STR_ScenarioDefinition Structure") (InSaveSummary :type "/Game/Blueprints/Gameflow/Save/STR_Save_Scenario_Summary Structure"))
  (bind _b_vm_scenariodefintion (`self.B_VM_ScenarioDefintion`))
  (set `self._scenarioName` InName)
  (set `self._scenarioDefintion` InDefinition)
  (set `self._scenarioSummary` InSaveSummary)
  (`/Game/Blueprints/GameScenario/B_VM_ScenarioDefintion.VM_SetScenarioDefinition` _b_vm_scenariodefintion (`self._scenarioName`) (`self._scenarioDefintion`) (`self._scenarioSummary`))
  (`/Game/Blueprints/Core/ViewModel/B_VM_BaseComponent.CreateView` _b_vm_scenariodefintion (`/Game/Blueprints/Core/ViewModel/B_VM_BaseComponent.GetDefaultWidget` _b_vm_scenariodefintion)))

(fn `UserConstructionScript`)