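; View model Blueprint for a game scenario, likely backing a selectable entry in a scenario selection UI.
; It stores the scenario's name, definition and save summary through one setter and exposes them through two getters.
; Selecting the scenario fires a notify event tagged as the common Select button, leaving the response to listeners.
; The event graph holds no active logic.
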(fn `VM_GetScenarioDefinition`
  (returns (OutName :type Name) (OutDefinition :type "/Game/Blueprints/GameScenario/STR_ScenarioDefinition Structure"))
  (return (`self._scenarioName`) (`self._scenarioDefinition`)))

(fn `VM_GetScenarioSummary`
  (returns (OutSummary :type "/Game/Blueprints/Gameflow/Save/STR_Save_Scenario_Summary Structure"))
  (return (`self._scenarioSummary`)))

(fn `VM_SelectScenario`
  (`self.OnNotifyEvent` (struct :`TagName` "ViewModel.Common.Button.Select")))

(fn `VM_SetScenarioDefinition`
  (params (InName :type Name) (InDefinition :type "/Game/Blueprints/GameScenario/STR_ScenarioDefinition Structure") (InSaveSummary :type "/Game/Blueprints/Gameflow/Save/STR_Save_Scenario_Summary Structure"))
  (set `self._scenarioName` InName)
  (set `self._scenarioDefinition` InDefinition)
  (set `self._scenarioSummary` InSaveSummary))