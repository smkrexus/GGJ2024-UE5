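; Custom player controller that sets up local player input and view models and switches controls by player mode.
; BeginPlay registers the input cache, adds context-menu and cheat input controllers, creates the player view model and binds to PlayerState view-model notifications.
; Gameplay-tag modes toggle menu interaction and character inputs; possession registers the pawn and sets Game mode, using a timer when initialization is pending.
; Helper functions add or remove Enhanced Input mapping contexts with optional caching.
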(event `self.ReceiveBeginPlay`
  (if (`self.IsLocalPlayerController`)
    (`WidgetBlueprintLibrary.SetInputMode_GameOnly` self)
    (`|ExecutionSequence`
      (:`then_0`
        (`/Game/Blueprints/Core/Inputs/B_InputCacheComponent.RegisterInputController` (`self.InputCacheComponent`) self)
        (bind _outinputcontroller (`/Game/Blueprints/Core/Utilities/BP_Utils.AddInputController` self "/Game/Blueprints/Core/Contexts/B_InputController_Menu_Context.B_InputController_Menu_Context_C" (`self.PlayerState`)))
        (set `self._contextOptionsController` _outinputcontroller))
      (:`then_3`
        (bind _returnvalue (`|AddComponentByClass` "/Game/Blueprints/Player/ViewModel/B_VM_Player.B_VM_Player_C")) ; main view, initialize HUD through controller\nmay want to split mini game to its own VM / interact to its own VM later
        (set `self.vm_playerView` _returnvalue)
        (`self.OnPlayerViewLoaded`))
      (:`then_4`
        (bind _output_get (set `self.vm_playerState` (`self.GetComponentByClass` (`self.PlayerState`) "/Game/Blueprints/Player/ViewModel/B_VM_PlayerState.B_VM_PlayerState_C"))) ; bind to this to get the current state of player, use notify event
        (add `/Game/Blueprints/Core/ViewModel/B_VM_BaseComponent.OnNotifyEvent` _output_get (`|CreateDelegate` :!event `OnNotifyReceivedEvent_PlayerState`)))
      (:`then_5`
        ;[1 1 1] Skip for non-shipping builds
        (`/Engine/EditorBlueprintResources/StandardMacros.IsValid` (`self.CheatManager`)
          (:`Is Valid`
            (`/Game/Blueprints/Core/Utilities/BP_Utils.AddInputController` self "/Game/Blueprints/Core/Debug/B_InputController_Cheats.B_InputController_Cheats_C" self))))
      (:`then_6`
        (set `self.bHasInitialized` true)))))

(event `OnNotifyReceivedEvent_PlayerState`
  (params (tag :type "GameplayTag Structure"))
  ;[1 0.8206 0 1 36] KEY INPUT CHANGES FROM PLAYER
  (`|SwitchGameplayTag` tag
    (:`ViewModel.PlayerState.StateHasChanged`
      (`|SwitchGameplayTag` (`/Game/Blueprints/Player/ViewModel/B_VM_PlayerState.VM_GetCurrentMode` (`self.vm_playerState`))
        (:`ViewModel.PlayerState.Modes.Game`
          (`/Game/Blueprints/Core/Utilities/BP_Utils.DisableMenuInteraction` self)
          (`/Game/Blueprints/Core/Inputs/B_InputController_Base.ActivateInputs` (`self._contextOptionsController`) self)
          (`/Game/Blueprints/Core/Inputs/B_InputController_Base.ActivateInputs` (`self.B_InputController_Character_Default`) self))
        (:`ViewModel.PlayerState.Modes.Menu`
          (`/Game/Blueprints/Core/Utilities/BP_Utils.EnableMenuInteraction` self)
          (`/Game/Blueprints/Core/Inputs/B_InputController_Base.RemoveInputs` (`self._contextOptionsController`) false)
          (`/Game/Blueprints/Core/Inputs/B_InputController_Base.RemoveInputs` (`self.B_InputController_Character_Default`) false))
        (:`ViewModel.PlayerState.Modes.Menu.QuickAccess`
          (`/Game/Blueprints/Core/Utilities/BP_Utils.EnableMenuInteraction` self :!label _label)
          (`/Game/Blueprints/Core/Inputs/B_InputController_Base.RemoveInputs` (`self.B_InputController_Character_Default`) false))
        (:`ViewModel.PlayerState.Modes.Menu.Popup`
          (goto _label))
        (:`ViewModel.PlayerState.Modes.MiniGame`
          (`/Game/Blueprints/Core/Inputs/B_InputController_Base.RemoveInputs` (`self.B_InputController_Character_Default`) false :!label _label_2))
        (:`ViewModel.PlayerState.Modes.Respawn`
          (goto _label_2))))))

(event `self.ReceiveUnPossess`
  (params (UnpossessedPawn :type "Pawn Object Reference")))

(event `self.ReceivePossess`
  (params (PossessedPawn :type "Pawn Object Reference"))
  (`self.RegisterPawn`))

(event `RegisterPawn`
  (bind _outvalidated (`self.ValidateInitialization`))
  (if _outvalidated
    (`/Game/Blueprints/Core/Inputs/B_InputController_Base.RegisterTargetForInput` (`self.B_InputController_Character_Default`) (`self.K2_GetPawn`))
    (`/Game/Blueprints/Player/ViewModel/B_VM_PlayerState.VM_SetCurrentMode` (`self.vm_playerState`) (struct :`TagName` "ViewModel.PlayerState.Modes.Game"))
    (else
      (`KismetSystemLibrary.K2_SetTimerDelegate` (`|CreateDelegate` :!event `RegisterPawn`) 0.5))))

(fn `DisableMappingContext`
  (params (MappingContext :type "InputMappingContext Object Reference") (ShouldClearInputCache :type Boolean :default true))
  (`EnhancedInputSubsystemInterface.RemoveMappingContext` (subsystem `EnhancedInputLocalPlayerSubsystem`) MappingContext (struct))
  (`|ExecutionSequence`
    (:`then_0`
      (if (`local.ShouldClearInputCache`)
        (`/Game/Blueprints/Core/Inputs/B_InputCacheComponent.RemoveInputFromCache` (`self.InputCacheComponent`) (`local.MappingContext`))))
    (:`then_1`
      (`self.ShowInputCacheDebug`)
      (`KismetSystemLibrary.PrintText` (`|FormatText` "Disable Input: {name} Clear cache {valid}" (`KismetSystemLibrary.GetDisplayName` (`local.MappingContext`)) (`local.ShouldClearInputCache`)) true true (struct :`G` 0.66 :`B` 1.0 :`A` 1.0) 10.0))))

(fn `GetContextController`
  (returns (OutInputController :type "/Game/Blueprints/Core/Inputs/B_InputController_Base Object Reference"))
  (return (`self._contextOptionsController`)))

(fn `GetInputSubsystem`
  (returns (inputSubsystem :type "EnhancedInputLocalPlayerSubsystem Object Reference"))
  (return (subsystem `EnhancedInputLocalPlayerSubsystem`)))

(fn `SetMappingContext`
  (params (MappingContext :type "InputMappingContext Object Reference") (ShouldCacheInput :type Boolean :default true) (InPriority :type Integer))
  (if (`.ReturnValue` (`EnhancedInputSubsystemInterface.HasMappingContext` (subsystem `EnhancedInputLocalPlayerSubsystem`) (`local.MappingContext`)))
    (`self.ShowInputCacheDebug`)
    (`KismetSystemLibrary.PrintText` (`|FormatText` "Existing Input Map found: {map} - Skipping" (`KismetSystemLibrary.GetDisplayName` (`local.MappingContext`))) true true (struct :`G` 0.66 :`B` 1.0 :`A` 1.0) 10.0)
    (return)
    (else
      (`EnhancedInputSubsystemInterface.AddMappingContext` (subsystem `EnhancedInputLocalPlayerSubsystem`) (`local.MappingContext`) (`local.InPriority`) (struct))
      (`|ExecutionSequence`
        (:`then_0`
          (if (`local.ShouldCacheInput`)
            (`/Game/Blueprints/Core/Inputs/B_InputCacheComponent.AddInputToCache` (`self.InputCacheComponent`) (`|MakeArray` (`local.MappingContext`)))))
        (:`then_1`
          (`self.ShowInputCacheDebug`)
          (`KismetSystemLibrary.PrintText` (`|FormatText` "Enable Input: {name}" (`KismetSystemLibrary.GetDisplayName` (`local.MappingContext`))) true true (struct :`G` 0.66 :`B` 1.0 :`A` 1.0) 10.0))))))

(fn `UserConstructionScript`)

(fn `ValidateInitialization`
  (returns (OutValidated :type Boolean))
  (return (`self.bHasInitialized`)))