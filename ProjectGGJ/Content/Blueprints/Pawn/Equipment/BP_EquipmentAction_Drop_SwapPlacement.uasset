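; Equipment action that, judging by its name, drops an item as a placement swap, by requesting its placement at a pickable item's holder.
; On activation it takes the Instigator as the pickable item and the controller of the equipment owner's pawn as the requestor.
; It passes the inventory item's handle to the holder's RequestPlacement, then ends the action.
; The validity check also calls EndAction but does not stop the later placement step in the sequence.
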(fn `OnActivateAction`
  (params (inventoryItem :type "/Game/Blueprints/Pawn/Inventory/B_InventoryItem_Base Object Reference") (equipmentComponent :type "/Game/Blueprints/Pawn/B_PawnEquipmentComponent Object Reference") (instigator :type "Actor Object Reference"))
  (locals (pickableItem :type "/Game/Blueprints/Items/BP_PickableItem_Base Object Reference") (requestController :type "Controller Object Reference"))
  (`|ExecutionSequence`
    (:`then_0`
      (bind _asbp_pickable_item_base (cast `/Game/Blueprints/Items/BP_PickableItem_Base` (`local.instigator`)))
      (set `local.pickableItem` _asbp_pickable_item_base))
    (:`then_1`
      (bind _aspawn (cast `Pawn` (`ActorComponent.GetOwner` (`local.equipmentComponent`))))
      (set `local.requestController` (`Pawn.GetController` _aspawn)))
    (:`then_2`
      (if (`KismetMathLibrary.BooleanNAND` (`KismetSystemLibrary.IsValid` (`local.pickableItem`)) (`KismetSystemLibrary.IsValid` (`local.requestController`)))
        (`self.EndAction`)))
    (:`then_3`
      (`/Game/Blueprints/Interactables/Extensions/Items/B_ItemHolder.RequestPlacement` (`/Game/Blueprints/Items/BP_PickableItem_Base.GetHolder` (`local.pickableItem`)) (`.handle` (`/Game/Blueprints/Pawn/Inventory/B_InventoryItem_Base.GetItem` (`local.inventoryItem`))) (`local.requestController`))
      (`self.EndAction`))))

(fn `UserConstructionScript`
  (`parent.UserConstructionScript`))