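; Standard equip action that puts an item's first-person held actor into the instigating pawn's right hand.
; It synchronously loads the item's soft HoldClass, spawns it at the component tagged FP.SocketRight, attaches it and registers it as the equipment component's active first-person item.
; If the handle's SaveData is valid, it loads that data onto the actor before calling BeginEquip.
; The action then ends through a Sequence node.
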(fn `OnActivateAction`
  (params (item :type "/Game/Blueprints/Items/ItemInfoData Object Reference") (itemHandle :type "/Game/Blueprints/Items/STR_ItemHandle Structure") (equipmentComponent :type "/Game/Blueprints/Pawn/B_PawnEquipmentComponent Object Reference") (instigator :type "Actor Object Reference"))
  (bind ((`saveData_22_AAC9F4C24D176FF2C97BAFA00FE7E4EB` _savedata)) (break `/Game/Blueprints/Items/STR_ItemHandle` (`local.itemHandle`)))
  (bind _holdclass (`/Game/Blueprints/Items/ItemInfoData.holdClass` (`local.item`)))
  (`|ExecutionSequence`
    (:`then_0`
      (bind _asbp_pawn_custom (cast `/Game/Blueprints/BP_PawnCustom` (`local.instigator`)))
      (if (`KismetSystemLibrary.IsValidSoftClassReference` _holdclass)
        (bind _returnvalue (`KismetSystemLibrary.LoadClassAsset_Blocking` _holdclass))
        (bind _asscene_component (cast `SceneComponent` (`|GetArrayItem` (`self.GetComponentsByTag` _asbp_pawn_custom "/Script/Engine.ActorComponent" "FP.SocketRight")) :!pure true))
        (bind (_returnvalue_location _returnvalue_rotation) (`KismetMathLibrary.BreakTransform` (`SceneComponent.K2_GetComponentToWorld` _asscene_component)))
        (bind _returnvalue_2 (`|SpawnActorFromClass` (castclass `/Game/Blueprints/Items/BP_Item_FirstPerson_Base` _returnvalue :!pure true) (`KismetMathLibrary.MakeTransform` _returnvalue_location _returnvalue_rotation) "Undefined" "MultiplyWithRoot" null _asbp_pawn_custom))
        (`self.K2_AttachToComponent` _returnvalue_2 _asscene_component "None" "KeepWorld" "KeepWorld" "KeepWorld" true)
        (bind _output_get (set `/Game/Blueprints/Pawn/B_PawnEquipmentComponent.activeFirstPersonItem` _returnvalue_2 (`local.equipmentComponent`)))
        (add `/Game/Blueprints/Items/MetaData/B_ItemMetaState_Base.OnLoadComplete` _savedata (`|CreateDelegate` _output_get :!event `OnLoaded`))
        (if (`KismetSystemLibrary.IsValid` _savedata)
          (`/Game/Blueprints/Items/MetaData/B_ItemMetaState_Base.LoadDataOnItem` _savedata (`/Game/Blueprints/Pawn/B_PawnEquipmentComponent.activeFirstPersonItem` (`local.equipmentComponent`)))
          (`/Game/Blueprints/Items/BP_Item_FirstPerson_Base.BeginEquip` _returnvalue_2) ; load data must complete first before equip
        )))
    (:`then_1`
      (`self.EndAction`))))

(fn `UserConstructionScript`
  (`parent.UserConstructionScript`))