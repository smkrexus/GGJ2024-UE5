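; Equipment action that drops an inventory item into the world as a thrown item actor.
; On activation it blocking-loads the item's class, spawns it at the owning pawn's camera transform and applies a forward impulse to its mesh.
; If the item handle holds valid save data, it binds a load-complete event and loads that data onto the spawned actor, then ends the action.
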(fn `OnActivateAction`
  (params (inventoryItem :type "/Game/Blueprints/Pawn/Inventory/B_InventoryItem_Base Object Reference") (equipmentComponent :type "/Game/Blueprints/Pawn/B_PawnEquipmentComponent Object Reference") (instigator :type "Actor Object Reference"))
  (bind ((`definition_26_917AB3E64853692B5840979E99D76636` _definition) (`saveData_22_AAC9F4C24D176FF2C97BAFA00FE7E4EB` _savedata)) (break `/Game/Blueprints/Items/STR_ItemHandle` (`.handle` (`/Game/Blueprints/Pawn/Inventory/B_InventoryItem_Base.GetItem` (`local.inventoryItem`)))))
  (`|ExecutionSequence`
    (:`then_0`
      (bind _returnvalue (`KismetSystemLibrary.LoadClassAsset_Blocking` (`.class_12_C91158A64EE1BB336321798171CF6EE8` (break `/Game/Blueprints/Items/STR_ItemHandle` (`.handle` (`/Game/Blueprints/Pawn/Inventory/B_InventoryItem_Base.GetItem` (`local.inventoryItem`)))))))
      (bind _returnvalue_2 (`|SpawnActorFromClass` (castclass `/Game/Blueprints/Items/BP_Item_Base` _returnvalue :!pure true) (`SceneComponent.K2_GetComponentToWorld` (`/Game/Blueprints/Pawn/BP_PawnCustom.Camera` (cast `/Game/Blueprints/Pawn/BP_PawnCustom` (`ActorComponent.GetOwner` (`local.equipmentComponent`)) :!pure true))) "AlwaysSpawn" "MultiplyWithRoot" null null))
      (`PrimitiveComponent.AddImpulse` (`/Game/Blueprints/Items/BP_Item_Base.StaticMesh` _returnvalue_2) (* (`self.GetActorForwardVector`) 500.0) "None" false))
    (:`then_1`
      (`/Engine/EditorBlueprintResources/StandardMacros.IsValid` _savedata
        (:`Is Valid`
          (add `/Game/Blueprints/Items/MetaData/B_ItemMetaState_Base.OnLoadComplete` _savedata (`|CreateDelegate` _returnvalue_2 :!event `OnLoaded`))
          (`/Game/Blueprints/Items/MetaData/B_ItemMetaState_Base.LoadDataOnItem` _savedata _returnvalue_2))))
    (:`then_2`
      (`self.EndAction`))))

(fn `UserConstructionScript`
  (`parent.UserConstructionScript`))