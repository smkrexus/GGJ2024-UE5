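; BP_EquipmentAction_Drop_Placement is an equipment action that hands an inventory item to the instigator's B_ItemHolder component for placement.
; With AutoPlace set, the holder places the item immediately at the instigator's transform.
; Otherwise it requests placement on behalf of the controller of the pawn owning the equipment component.
; The action then ends without waiting for a placement result.
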(fn `OnActivateAction`
  (params (inventoryItem :type "/Game/Blueprints/Pawn/Inventory/B_InventoryItem_Base Object Reference") (equipmentComponent :type "/Game/Blueprints/Pawn/B_PawnEquipmentComponent Object Reference") (instigator :type "Actor Object Reference"))
  (locals (itemHolder :type "/Game/Blueprints/Interactables/Extensions/Items/B_ItemHolder Object Reference"))
  (`|ExecutionSequence`
    (:`then_0`
      (set `local.itemHolder` (`self.GetComponentByClass` (`local.instigator`) "/Game/Blueprints/Interactables/Extensions/Items/B_ItemHolder.B_ItemHolder_C")))
    (:`then_1`
      (bind _itemholder (`local.itemHolder`)
        (:`then`
          (if (`/Game/Blueprints/Interactables/Extensions/Items/B_ItemHolder.bAutoPlace` _itemholder)
            (`/Game/Blueprints/Interactables/Extensions/Items/B_ItemHolder.PlaceItem` (`local.itemHolder`) (`.handle` (`/Game/Blueprints/Pawn/Inventory/B_InventoryItem_Base.GetItem` (`local.inventoryItem`))) (`self.GetTransform` (`local.instigator`)))
            (else
              (bind _aspawn (cast `Pawn` (`ActorComponent.GetOwner` (`local.equipmentComponent`))))
              (`/Game/Blueprints/Interactables/Extensions/Items/B_ItemHolder.RequestPlacement` (`local.itemHolder`) (`.handle` (`/Game/Blueprints/Pawn/Inventory/B_InventoryItem_Base.GetItem` (`local.inventoryItem`))) (`Pawn.GetController` _aspawn)))))
        (:`else`)))
    (:`then_2`
      (`self.EndAction`))))

(fn `UserConstructionScript`
  (`parent.UserConstructionScript`))