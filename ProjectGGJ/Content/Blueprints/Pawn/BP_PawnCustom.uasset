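; Player character pawn with visible hands, handling movement, look, timeline-driven crouch, equipment and camera-raycast interaction.
; Player-state view model mode changes toggle interaction and hand visibility for game, menu, mini-game and cinematic states.
; Look input rescales interaction reach by pitch, extending it when aiming downward.
; Registered rooms forward decibel immunity thresholds to GameState, and unpossession shuts down components, collision and visuals.
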(event `self.ReceiveBeginPlay`
  (bind _asbp_player_state_custom (cast `/Game/Blueprints/Player/BP_PlayerStateCustom` (`GameplayStatics.GetPlayerState` 0)))
  (bind _output_get (set `self.vm_playerState` (`/Game/Blueprints/Player/BP_PlayerStateCustom.GetViewModel` _asbp_player_state_custom)))
  (add `/Game/Blueprints/Core/ViewModel/B_VM_BaseComponent.OnNotifyEvent` _output_get (`|CreateDelegate` :!event `OnNotifyEventReceived_PlayerState`)))

(event `self.ReceiveTick`
  (params (DeltaSeconds :type "Float (single-precision)"))
  (bind _camera (`self.Camera`))
  (`/Game/Blueprints/Pawn/BP_PawnInteractionComponent.Raycast Interaction` (`self.BP_PawnInteractionComponent`) (`SceneComponent.K2_GetComponentLocation` _camera) (`SceneComponent.GetForwardVector` _camera)))

(event `OnNotifyEventReceived_PlayerState`
  (params (tag :type "GameplayTag Structure"))
  (`|SwitchGameplayTag` tag
    (:`ViewModel.PlayerState.StateHasChanged`
      (`|SwitchGameplayTag` (`/Game/Blueprints/Player/ViewModel/B_VM_PlayerState.VM_GetCurrentMode` (`self.vm_playerState`))
        (:`ViewModel.PlayerState.Modes.Game`
          (`SceneComponent.SetVisibility` (`self.Hand_L`) true true)
          (`SceneComponent.SetVisibility` (`self.Hand_R`) true true)
          (`/Game/Blueprints/Pawn/BP_PawnInteractionComponent.Enable` (`self.BP_PawnInteractionComponent`)))
        (:`ViewModel.PlayerState.Modes.Menu`
          (`self.DISABLE_INTERACTION_QUERY` :!label _label))
        (:`ViewModel.PlayerState.Modes.MiniGame`
          (goto _label))
        (:`ViewModel.PlayerState.Modes.Cinematic`
          (`self.DISABLE_INTERACTION_QUERY`)
          (`SceneComponent.SetVisibility` (`self.Hand_L`) false true)
          (`SceneComponent.SetVisibility` (`self.Hand_R`) false true))
        (:`ViewModel.PlayerState.Modes.Menu.Popup`
          (goto _label))))))

(event `OnRoomImmunityLevelChanged`
  (params (InThreshold :type Integer))
  (bind _gamedecibels (`/Game/Blueprints/Gameflow/GS_GameStateCustom.GameDecibels` (`/Game/Blueprints/Core/Utilities/BP_Utils.Game State`)))
  ;[1 1 1] Set Immunity if there is decibel immunity in the room (eg. playing radio)
  (if (!= InThreshold -1)
    (`/Game/Blueprints/Gameflow/Components/B_GameDecibels.SetImmunityThreshold` _gamedecibels InThreshold)
    (else
      (`/Game/Blueprints/Gameflow/Components/B_GameDecibels.RemoveImmunity` _gamedecibels))))

(event `self.ReceivePossessed`
  (params (NewController :type "Controller Object Reference"))
  ;[0 0 0] INIT & CLEANUP
  (`/Game/Blueprints/Pawn/BP_PawnInteractionComponent.Initialize` (`self.BP_PawnInteractionComponent`) self)
  (`/Game/Blueprints/Pawn/B_PawnEquipmentComponent.Initialize` (`self.PawnEquipmentComponent`) self))

(event `self.ReceiveUnpossessed`
  (params (OldController :type "Controller Object Reference"))
  ;[0 0 0] INIT & CLEANUP
  (`/Game/Blueprints/Pawn/B_PawnEquipmentComponent.Cleanup` (`self.PawnEquipmentComponent`))
  (`/Game/Blueprints/Pawn/BP_PawnInteractionComponent.Cleanup` (`self.BP_PawnInteractionComponent`))
  (`self.Cleanup`))

(event `self.B_RoomItemComponent.OnRegisterRoom`
  (params (RegisteredRoom :type "/Game/Blueprints/Room/BP_Room_Base Object Reference"))
  (bind _roomdecibelscomponent (`/Game/Blueprints/Room/BP_Room_Base.RoomDecibelsComponent` RegisteredRoom))
  (add `/Game/Blueprints/Room/B_RoomDecibelsComponent.OnImmunityThresholdChanged` _roomdecibelscomponent (`|CreateDelegate` :!event `OnRoomImmunityLevelChanged`))
  (`self.OnRoomImmunityLevelChanged` (`/Game/Blueprints/Room/B_RoomDecibelsComponent.GetImmunityThreshold` _roomdecibelscomponent)))

(event `self.B_RoomItemComponent.OnUnregisterRoom`
  (params (UnregisteredRoom :type "/Game/Blueprints/Room/BP_Room_Base Object Reference"))
  (remove `/Game/Blueprints/Room/B_RoomDecibelsComponent.OnImmunityThresholdChanged` (`/Game/Blueprints/Room/BP_Room_Base.RoomDecibelsComponent` UnregisteredRoom) (`|CreateDelegate` :!event `OnRoomImmunityLevelChanged`))
  (`/Game/Blueprints/Gameflow/Components/B_GameDecibels.RemoveImmunity` (`/Game/Blueprints/Gameflow/GS_GameStateCustom.GameDecibels` (`/Game/Blueprints/Core/Utilities/BP_Utils.Game State`))))

(event `self.K2_OnStartCrouch`
  (params (HalfHeightAdjust :type "Float (single-precision)") (ScaledHalfHeightAdjust :type "Float (single-precision)"))
  (bind (_direction _crouchoffset) (`Timeline|CrouchTimeline` :!label _label)
    (:`Update`
      (bind _returnvalue (* _crouchoffset -1.0))
      (set `SpringArmComponent.TargetOffset` (select `bool` (`self.bIsCrouched`) :`false` (`KismetMathLibrary.MakeVector` 0.0 0.0 _returnvalue) :`true` (`KismetMathLibrary.MakeVector` 0.0 0.0 _returnvalue) :!type "Vector Structure") (`self.SpringArm`)))))

(event `self.K2_OnEndCrouch`
  (params (HalfHeightAdjust :type "Float (single-precision)") (ScaledHalfHeightAdjust :type "Float (single-precision)"))
  (goto _label :!via `ReverseFromEnd`))

(event `UpdateBoost`
  (params (InEnabled :type Boolean)))

(event `UpdateMoveDirection`
  (params (InDirection :type "Vector2D Structure"))
  (bind (_x _y) (`KismetMathLibrary.BreakVector2D` InDirection))
  (bind _returnvalue (`KismetMathLibrary.MakeRotator` 0.0 0.0 (.yaw (`self.GetControlRotation`))))
  (`|ExecutionSequence`
    (:`then_0`
      (if (!= _x 0.0)
        (`self.AddMovementInput` (`KismetMathLibrary.GetForwardVector` _returnvalue) (`KismetMathLibrary.SignOfFloat` _x))))
    (:`then_1`
      (if (!= _y 0.0)
        (`self.AddMovementInput` (`KismetMathLibrary.GetRightVector` _returnvalue) (`KismetMathLibrary.SignOfFloat` _y))))))

(event `UpdateLookDirection`
  (params (InDirection :type "Vector2D Structure"))
  (bind (_x _y) (`KismetMathLibrary.BreakVector2D` InDirection))
  (bind _bp_pawninteractioncomponent (`self.BP_PawnInteractionComponent`))
  (bind _looksensitivity (`self.LookSensitivity`))
  (bind _returnvalue (`KismetMathLibrary.DegAsin` (`KismetMathLibrary.Dot_VectorVector` (`KismetMathLibrary.Normal` (`SceneComponent.GetForwardVector` (`self.Camera`))) (`KismetMathLibrary.MakeVector` 0.0 0.0 1.0))))
  (`self.AddControllerYawInput` (* _x (`KismetMathLibrary.Abs` _looksensitivity)))
  (`self.AddControllerPitchInput` (* (* _y (`KismetMathLibrary.Abs` _looksensitivity)) -1.0))
  (if (< (`KismetMathLibrary.SignOfFloat` _returnvalue) 0.0)
    (set `/Game/Blueprints/Pawn/BP_PawnInteractionComponent.raycastDistance` (`KismetMathLibrary.Lerp` 150.0 200.0 (/ (`KismetMathLibrary.FClamp` (- (`KismetMathLibrary.Abs` _returnvalue) (- 80.0 45.0)) 0.0 45.0) 45.0)) _bp_pawninteractioncomponent)
    (else
      (set `/Game/Blueprints/Pawn/BP_PawnInteractionComponent.raycastDistance` 120.0 _bp_pawninteractioncomponent))))

(fn `Cleanup`
  (remove `/Game/Blueprints/Core/ViewModel/B_VM_BaseComponent.OnNotifyEvent` (`self.vm_playerState`) (`|CreateDelegate` :!event `OnNotifyEventReceived_PlayerState`))
  (`self.SetActorTickEnabled` false)
  (`PrimitiveComponent.SetCollisionEnabled` (`self.CapsuleComponent`) "NoCollision")
  (`SceneComponent.SetVisibility` (`self.Mesh`) false false)
  (`SceneComponent.SetVisibility` (`self.Hand_R`) false true)
  (`SceneComponent.SetVisibility` (`self.Hand_L`) false true)
  (`ActorComponent.K2_DestroyComponent` (`self.Camera`))
  (`ActorComponent.Deactivate` (`self.CharacterMovement`))
  (`ActorComponent.Deactivate` (`self.BP_PawnInteractionComponent`))
  (`ActorComponent.Deactivate` (`self.PawnEquipmentComponent`))
  (`KismetSystemLibrary.K2_SetTimerDelegate` (`|CreateDelegate` :!event `K2_DestroyActor`) 3.0))

(fn `UserConstructionScript`)