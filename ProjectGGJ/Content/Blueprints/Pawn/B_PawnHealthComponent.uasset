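; Pawn health component that handles kill and respawn sequences with a screen fade, broadcasting OnKill and OnRespawnComplete events.
; Kill and Respawn both fade to black through a lazily created overlay widget, then start a delay timer.
; MoveToPlayerStart fades back, teleports player 0's pawn to the first PlayerStart found and aligns control rotation.
; Despite its name, it tracks no health value.
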(event `KillEvent`
  (`self.OnKill`))

(fn `Kill`
  (`self.FADE_TO_BLACK`)
  (`KismetSystemLibrary.K2_SetTimerDelegate` (`|CreateDelegate` :!event `KillEvent`) 3.0))

(fn `MoveToPlayerStart`
  (bind _returnvalue (`GameplayStatics.GetPlayerPawn` 0))
  (`/Game/Blueprints/Core/UI/Transition/WBP_Transition_Base.Apply Transition` (`self._fader`) true 1.0)
  (bind _outactors (`GameplayStatics.GetAllActorsOfClass` "/Script/Engine.PlayerStart"))
  (bind _rotation (.rotation (`Actor.GetTransform` (`|GetArrayItem` _outactors))))
  (`Actor.K2_TeleportTo` _returnvalue (.location (`Actor.GetTransform` (`|GetArrayItem` _outactors))) _rotation)
  (`Controller.SetControlRotation` (`Pawn.GetController` _returnvalue) _rotation)
  (`self.OnRespawnComplete`))

(fn `Respawn`
  (`self.FADE_TO_BLACK`)
  (`KismetSystemLibrary.K2_SetTimerDelegate` (`|CreateDelegate` :!event `MoveToPlayerStart`) 3.0))