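; Pawn component that finds the interactable under a raycast and forwards interaction requests to it, set up for local controllers.
; RaycastInteraction checks tag-matched interact area components first, then falls back to a Visibility trace for actors implementing BPI_Interactable.
; Focus changes notify the interactable, fire detect/end/empty dispatchers and clear the interaction view model when empty.
; That view model links to crosshair and equipment view models, waiting on global registration when they are missing.
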(event `OnDetectStart`
  (params (interactable :type "/Game/Blueprints/Interactables/BPI_Interactable Interface"))
  ;[1 1 1] Interaction object in focus
  (`|ExecutionSequence`
    (:`then_0`
      (bind _output_get (set `self.interactableObject` interactable))
      (`self.OnDetectInteractable` _output_get))
    (:`then_1`
      (`/Game/Blueprints/Interactables/BPI_Interactable.OnComponentFound` (`self.interactableObject`) (`self.vm_interaction`) (`self._controller`)) ; component based interaction
    )))

(event `self.ReceiveBeginPlay`)

(event `OnDetectClear`
  ;[1 1 1] Interaction object fully out of focus
  (set `self.interactableObject` null)
  (`/Game/Blueprints/Pawn/Interaction/ViewModel/B_VM_InteractionComponent.VM_ClearInteraction` (`self.vm_interaction`))
  (`self.OnEmptyInteractable`))

(event `LinkToCrosshair`
  (bind _outviewmodel (`/Game/Blueprints/Core/ViewModel/BP_Gameflow_ViewModel.GetViewModel` (`self._globalVM`) "/Game/Blueprints/Player/ViewModel/B_VM_Crosshair_Default.B_VM_Crosshair_Default_C"))
  (bind _outvalidated (message `/Game/Blueprints/Gameflow/Components/BPI_Gameflow_Validator.ValidateInitialization` (`self._globalVM`)))
  (if _outvalidated
    (`/Engine/EditorBlueprintResources/StandardMacros.IsValid` _outviewmodel
      (:`Is Valid`
        (message `/Game/Blueprints/Core/ViewModel/BPI_Widget_ViewModel.AddViewModel` (`/Game/Blueprints/Core/ViewModel/B_VM_BaseComponent.GetWidgetObject` _outviewmodel) (`self.vm_interaction`))
        (`/Engine/EditorBlueprintResources/StandardMacros.IsValid` (`KismetSystemLibrary.Conv_InterfaceToObject` (`self.interactableObject`))
          (:`Is Valid`
            (`/Game/Blueprints/Pawn/Interaction/ViewModel/B_VM_InteractionComponent.VM_DetectInteractable` (`self.vm_interaction`) (`self.interactableObject`)))
          (:`Is Not Valid`
            (`/Game/Blueprints/Pawn/Interaction/ViewModel/B_VM_InteractionComponent.VM_ClearInteraction` (`self.vm_interaction`))))))
    (else
      (`KismetSystemLibrary.K2_SetTimerDelegate` (`|CreateDelegate` :!event `LinkToCrosshair`) 0.5))))

(event `OnDetectStop`
  (params (interactable :type "/Game/Blueprints/Interactables/BPI_Interactable Interface"))
  ;[1 1 1] Interaction object out of focus when changing to new interaction object
  (`/Engine/EditorBlueprintResources/StandardMacros.IsValid` (`KismetSystemLibrary.Conv_InterfaceToObject` interactable)
    (:`Is Valid`
      (`self.OnDetectInteractableEnd` interactable) ; call end on previous object
      (`/Game/Blueprints/Interactables/BPI_Interactable.OnComponentClear` (`self.interactableObject`)))))

(event `LinkToEquipment`
  (bind _outviewmodel (`/Game/Blueprints/Core/ViewModel/BP_Gameflow_ViewModel.GetViewModel` (`self._globalVM`) "/Game/Blueprints/Player/ViewModel/B_VM_EquipmentComponent.B_VM_EquipmentComponent_C"))
  (bind _outvalidated (message `/Game/Blueprints/Gameflow/Components/BPI_Gameflow_Validator.ValidateInitialization` (`self._globalVM`)))
  (if _outvalidated
    (`/Engine/EditorBlueprintResources/StandardMacros.IsValid` _outviewmodel
      (:`Is Valid`
        (`/Game/Blueprints/Pawn/Interaction/ViewModel/B_VM_InteractionComponent.VM_AddExtension` (`self.vm_interaction`) "requirements" _outviewmodel) ; adds equipment view model to interaction widget extension so that\nit can reflect requirements based on equipment properly
      ))
    (else
      (`KismetSystemLibrary.K2_SetTimerDelegate` (`|CreateDelegate` :!event `LinkToEquipment`) 0.5))))

(event `WaitVMDependencies`
  (`|ExecutionSequence`
    (:`then_0`
      (`/Engine/EditorBlueprintResources/StandardMacros.IsValid` (`/Game/Blueprints/Core/ViewModel/BP_Gameflow_ViewModel.GetViewModel` (`self._globalVM`) "/Game/Blueprints/Player/ViewModel/B_VM_Crosshair_Default.B_VM_Crosshair_Default_C")
        (:`Is Valid`
          (if (not (`self.bCrosshairLinked`))
            (`self.LinkToCrosshair`)
            (set `self.bCrosshairLinked` true)))))
    (:`then_1`
      (`/Engine/EditorBlueprintResources/StandardMacros.IsValid` (`/Game/Blueprints/Core/ViewModel/BP_Gameflow_ViewModel.GetViewModel` (`self._globalVM`) "/Game/Blueprints/Player/ViewModel/B_VM_EquipmentComponent.B_VM_EquipmentComponent_C")
        (:`Is Valid`
          (if (not (`self.bEquipmentLinked`))
            (`self.LinkToEquipment`)
            (set `self.bEquipmentLinked` true)))))
    (:`then_2`
      (if (and (`self.bEquipmentLinked`) (`self.bCrosshairLinked`))
        (remove `/Game/Blueprints/Core/ViewModel/BP_Gameflow_ViewModel.OnRegisterViewModel` (`self._globalVM`) (`|CreateDelegate` :!event `WaitVMDependencies`))))))

(fn `Cleanup`
  (`/Game/Blueprints/Core/ViewModel/B_VM_BaseComponent.RemoveView` (`self.vm_interaction`)))

(fn `Disable`
  (set `self.enabled` false)
  (`self.OnDetectClear`))

(fn `Enable`
  (set `self.enabled` true))

(fn `GetInteractable`
  (returns (interactableObject :type "/Game/Blueprints/Interactables/BPI_Interactable Interface"))
  (return (`self.interactableObject`)))

(fn `HasInteractable`
  (returns (valid :type Boolean))
  (return (`KismetSystemLibrary.IsValid` (`KismetSystemLibrary.Conv_InterfaceToObject` (`self.interactableObject`)))))

(fn `Initialize`
  (params (InPawn :type "Pawn Object Reference"))
  (locals (WaitForVMFramework :type Boolean))
  (bind _output_get (set `self._controller` (`Pawn.GetController` (`local.InPawn`))))
  (if (`Controller.IsLocalController` _output_get)
    (`|ExecutionSequence`
      (:`then_0`
        (bind _returnvalue (`|AddComponentByClass` (`local.InPawn`) "/Game/Blueprints/Pawn/Interaction/ViewModel/B_VM_InteractionComponent.B_VM_InteractionComponent_C"))
        (set `self.vm_interaction` _returnvalue)
        (set `self.enabled` true)
        (set `self._globalVM` (`/Game/Blueprints/HUD/Utilities/BP_Utilities_Widget.GlobalViewModelSystem`)))
      (:`then_1`
        (`/Engine/EditorBlueprintResources/StandardMacros.IsValid` (`/Game/Blueprints/Core/ViewModel/BP_Gameflow_ViewModel.GetViewModel` (`self._globalVM`) "/Game/Blueprints/Player/ViewModel/B_VM_Crosshair_Default.B_VM_Crosshair_Default_C")
          (:`Is Valid`
            (`self.LinkToCrosshair`))
          (:`Is Not Valid`
            (set `local.WaitForVMFramework` true))))
      (:`then_2`
        (`/Engine/EditorBlueprintResources/StandardMacros.IsValid` (`/Game/Blueprints/Core/ViewModel/BP_Gameflow_ViewModel.GetViewModel` (`self._globalVM`) "/Game/Blueprints/Player/ViewModel/B_VM_EquipmentComponent.B_VM_EquipmentComponent_C")
          (:`Is Valid`
            (`self.LinkToEquipment`))
          (:`Is Not Valid`
            (set `local.WaitForVMFramework` true))))
      (:`then_3`
        (if (`local.WaitForVMFramework`)
          (add `/Game/Blueprints/Core/ViewModel/BP_Gameflow_ViewModel.OnRegisterViewModel` (`self._globalVM`) (`|CreateDelegate` :!event `WaitVMDependencies`)))))))

(fn `Raycast Interaction`
  (params (start :type "Vector Structure") (forward :type "Vector Structure"))
  (bind _start (`local.start`))
  (bind _returnvalue (+ _start (* (`local.forward`) (`self.raycastDistance`))))
  (`|ExecutionSequence`
    (:`then_0`
      (if (not (`self.enabled`))
        ;[0.01044 0.2188 0.01118] New interaction, uses interact area component, returns immediately if available
        (return)))
    (:`then_1`
      (bind (_outhit _returnvalue_2) (`KismetSystemLibrary.LineTraceSingle` :`Start` _start :`End` _returnvalue :`TraceChannel` "TraceTypeQuery3" :`DrawTime` 0.5))
      (if _returnvalue_2
        (bind (_bblockinghit _binitialoverlap _time _distance _location _impactpoint _normal _impactnormal _physmat _hitactor _hitcomponent) (`GameplayStatics.BreakHitResult` _outhit))
        (bind _componenttags (`ActorComponent.ComponentTags` _hitcomponent))
        (if (`KismetArrayLibrary.Array_IsNotEmpty` _componenttags)
          (bind _output (`|GetArrayItem` (`Actor.GetComponentsByTag` _hitactor "/Game/Blueprints/Interactables/B_InteractAreaComponent.B_InteractAreaComponent_C" (`|GetArrayItem` _componenttags))))
          (if (`/Game/Blueprints/Interactables/B_InteractAreaComponent.IsInteractable` _output)
            (bind _asbpi_interactable (cast `/Game/Blueprints/Interactables/BPI_Interactable` _output))
            (`self.SetInteractable` _asbpi_interactable
              (:`valid`
                (set `self.requestClear` true)
                (`self.OnDetectStop` (`self.interactableObject`)) ; call end on previous object
                (`self.OnDetectStart` _asbpi_interactable)
                (return))
              (:`default`
                (return) ; new interaction, no need clear
              ))))))
    (:`then_2`
      ;[0.00444 0.005208 0.000712] Default Interaction (by object), may be deprecated later
      (bind (_outhit_2 _returnvalue_3) (`KismetSystemLibrary.LineTraceSingle` :`Start` _start :`End` _returnvalue :`TraceChannel` "TraceTypeQuery1" :`DrawTime` 0.5))
      (if _returnvalue_3
        ;;[1 1 1] Check for invalid or same data
        (bind _asbpi_interactable_2 (cast `/Game/Blueprints/Interactables/BPI_Interactable` (`.HitActor` (`GameplayStatics.BreakHitResult` _outhit_2)))
          (:`then`
            (`self.SetInteractable` _asbpi_interactable_2
              (:`valid`
                (set `self.requestClear` true)
                (`self.OnDetectStop` (`self.interactableObject`)) ; call end on previous object
                (`self.OnDetectStart` _asbpi_interactable_2)
                (return))))
          (:`CastFailed`
            _)))
      ;;[1 1 1] Check if data exists then empty it
      (`self.ClearInteractable`
        (:`clearRequest`
          (`self.OnDetectStop` (`self.interactableObject`)) ; call end on previous object
          (`self.OnDetectClear`))))))

(fn `RequestInteraction`
  (params (InController :type "Controller Object Reference"))
  (returns (OutSuccess :type Boolean))
  (if (`self.HasInteractable`)
    (`/Game/Blueprints/Interactables/BPI_Interactable.Interact` (`self.GetInteractable`) (`local.InController`))
    (return true)
    (else
      (return false))))