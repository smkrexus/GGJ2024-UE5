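; Pawn equipment component that tracks picked-up items, their stack counts and the active item.
; PickupItem blocking-loads the item data, activates it if nothing is active, and merges stacks into ItemHandles or adds a new handle.
; DropItem spawns the item class at the owner's transform, reduces or removes the stack, then revalidates the active item.
; A debug B key drops one active item; spawned drops do not yet receive their stack count.
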(event EventBeginPlay
  (Input|EnableInput (Components|GetOwner) (Game|GetPlayerController 0)))

(event EventTick
  (params (DeltaSeconds :type Float%20%28single-precision%29)))

(event Input|KeyboardEvents|DebugKeyB
  (params (Key :type Key%20Structure :default "None") (ActionValue :type Input%20Action%20Value%20Structure))
  (:Pressed
    (CallFunction|DropItem (CallFunction|GetActiveItem) 1)))

(fn PickupItem
  (params (itemToPickup :type STR%20Item%20Handle%20Structure))
  (Utilities|FlowControl|Sequence
    (:then_0
      (bind _returnvalue (Utilities|LoadAssetBlocking (.data itemToPickup)))
      (Development|PrintText (Utilities|Text|FormatText "Picked item {tag}" (GameplayTags|GetTagName (Variables|/Game/Blueprints/Items/ItemInfoData.ItemInfoData_C|Getdescriptor (.AsItem%20Info%20Data (Utilities|Casting|CastToItemInfoData _returnvalue))))) false))
    (:then_1
      (Utilities|Array|AddUnique (Variables|Default|GetavailableItems) (.AsItem%20Info%20Data (Utilities|Casting|CastToItemInfoData _returnvalue))))
    (:then_2
      (Variables|Default|GetactiveItem
        (:then)
        (:else
          (CallFunction|SetActiveItem (.AsItem%20Info%20Data (Utilities|Casting|CastToItemInfoData _returnvalue))))))
    (:then_3
      (for _array_element (Variables|Default|GetitemHandles)
        (if (== (.data (Utilities|Struct|BreakSTR_ItemHandle _array_element)) (.data itemToPickup))
          (bind _structout (Utilities|Struct|SetmembersinSTR_ItemHandle _array_element (+ (.stackCount (Utilities|Struct|BreakSTR_ItemHandle _array_element)) (.stackcount itemToPickup))))
          (|SetBy-RefVar _array_element _structout)
          (return) ; already exists no need to add item to list
        ))
      (Utilities|Array|Add (Variables|Default|GetitemHandles) itemToPickup) ; new item, add to list
    )))

(fn DropItem
  (params (itemToDrop :type Item%20Info%20Data%20Object%20Reference) (dropQuantity :type Integer))
  (Utilities|FlowControl|Sequence ; valid checks
    (:then_0
      (if (not (Utilities|IsValid itemToDrop))
        (Development|PrintText "Undefined item for dropping, skipping" false)
        (return false 0)))
    (:then_1
      (if (== (Utilities|Array|FindItem (Variables|Default|GetavailableItems) itemToDrop) -1)
        (Development|PrintText (Utilities|Text|FormatText "Unable to drop item {tag} as does not exist in equipment list" (GameplayTags|GetTagName (Variables|/Game/Blueprints/Items/ItemInfoData.ItemInfoData_C|Getdescriptor itemToDrop))) false)
        (return false 0)))
    (:then_2
      (Utilities|FlowControl|Sequence
        (:then_0
          (bind (_array_element _array_index) (Utilities|Array|ForEachLoopwithBreak (Variables|Default|GetitemHandles) :!label _label)
            (:LoopBody
              (if (== (.data (Utilities|Struct|BreakSTR_ItemHandle _array_element)) (Utilities|ResolveSoftReference itemToDrop))
                (LocalVariables|SetstacksRemaining (- (.stackCount (Utilities|Struct|BreakSTR_ItemHandle _array_element)) dropQuantity))
                (LocalVariables|SethandleIndex _array_index)
                (LocalVariables|SetstacksToDrop (Math|Integer|Clamp(Integer) dropQuantity 1 (.stackCount (Utilities|Struct|BreakSTR_ItemHandle _array_element))))
                (goto _label Break)))))
        (:then_1
          (if (Utilities|Array|IsValidIndex (Variables|Default|GetitemHandles) (LocalVariables|GethandleIndex))
            (bind _returnvalue (Utilities|LoadClassAssetBlocking (.class (Utilities|Struct|BreakSTR_ItemHandle (Utilities|Array|Get(acopy) (Variables|Default|GetitemHandles) (LocalVariables|GethandleIndex))))))
            (bind _returnvalue_2 (Game|SpawnActorfromClass (.AsBP%20Item%20Base (Utilities|Casting|CastToBP_Item_BaseClass _returnvalue)) (Transformation|GetActorTransform (Components|GetOwner)) "Undefined" "MultiplyWithRoot" 0 0)) ; then set stacks to drop once implemented
            (LocalVariables|SetdroppedActor _returnvalue_2)
            (Development|PrintText (Utilities|Text|FormatText "Dropping item {tag} count {c}" (GameplayTags|GetTagName (Variables|/Game/Blueprints/Items/ItemInfoData.ItemInfoData_C|Getdescriptor itemToDrop)) (LocalVariables|GetstacksToDrop)) false)))
        (:then_2
          (if (> (LocalVariables|GetstacksRemaining) 0)
            (Utilities|Struct|SetmembersinSTR_ItemHandle (Utilities|Array|Get(acopy) (Variables|Default|GetitemHandles) (LocalVariables|GethandleIndex)) (LocalVariables|GetstacksRemaining))
            (else
              (Utilities|Array|RemoveIndex (Variables|Default|GetitemHandles) (LocalVariables|GethandleIndex))
              (Utilities|Array|RemoveItem (Variables|Default|GetavailableItems) itemToDrop))))
        (:then_3
          (CallFunction|CheckActiveItem)
          (return true (LocalVariables|GetdroppedActor)))))))

(fn SetActiveItem
  (params (item :type Item%20Info%20Data%20Object%20Reference))
  (bind _output_get (Variables|Default|SetactiveItem item))
  (Development|PrintText (Utilities|Text|FormatText "Setting item active {tag}" (GameplayTags|GetTagName (Variables|/Game/Blueprints/Items/ItemInfoData.ItemInfoData_C|Getdescriptor _output_get)))))

(fn GetActiveItem
  (return (Variables|Default|GetactiveItem)))

(fn CheckActiveItem
  (if (== (Utilities|Array|FindItem (Variables|Default|GetavailableItems) (Variables|Default|GetactiveItem)) -1)
    (Variables|Default|SetactiveItem 0) ; active item is now null
  ))