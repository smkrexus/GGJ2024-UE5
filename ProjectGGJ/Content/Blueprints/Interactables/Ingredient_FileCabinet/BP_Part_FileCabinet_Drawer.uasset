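; Interactable file cabinet drawer part that slides its mesh via a transition component and holds spawned items for the player to review.
; Interacting starts the transition, and SetTransform applies only the relative location to the mesh.
; Place spawns actors at the Placement socket, tracks them until destroyed, and enables a scene-tracker locator until the drawer empties.
; Tracker events toggle the "items available" interact status and the range-based locator display.
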(event `self.ReceiveBeginPlay`
  (`/Game/Blueprints/Interactables/B_InteractAreaComponent.AssignArea` (`self.InteractAreaComponent`) (`self.Area_Interaction`)))

(event `self.InteractAreaComponent.OnInteracted`
  (params (controller :type "Controller Object Reference"))
  (`/Game/Blueprints/Interactables/Extensions/Ingredients/B_InteractTransitionComponent.StartTransition` (`self.InteractTransitionComponent`) controller))

(event `/Game/Blueprints/Interactables/Extensions/Interfaces/BPI_Ingredient_Transform.SetTransform`
  (params (transform :type "Transform Structure"))
  (`SceneComponent.K2_SetRelativeLocation` (`self.StaticMesh`) (.location transform) false false))

(event `RemovePlacedActor`
  (params (DestroyedActor :type "Actor Object Reference"))
  (`KismetArrayLibrary.Array_RemoveItem` (`self._placedActors`) DestroyedActor)
  (if (`KismetArrayLibrary.Array_IsEmpty` (`self._placedActors`))
    (`/ActorTracker/Blueprints/B_SceneTracker_Base.SetTrackingEnabled` (`self.B_SceneTracker_InteractableLocator`) false)))

(event `self.B_SceneTracker_InteractableLocator.OnTrackingEnabled`
  ;[1 1 1] Display items for review prompt, then hide when nothing available
  (`/Game/Blueprints/Interactables/B_InteractAreaComponent.SetStatus` (`self.InteractAreaComponent`) (make `/Game/Blueprints/Interactables/Status/STR_InteractStatus` true "Items available for review")))

(event `self.B_SceneTracker_InteractableLocator.OnRangeDetected`
  (params (player :type "Pawn Object Reference"))
  ;[1 1 1] Standard show/hide indicator if tracking is enabled
  (`self.IS_TRACKING_PROMPT`)
  (`/Game/Blueprints/Interactables/Locator/ViewModel/B_VM_InteractableLocator.VM_SetShouldDisplayLocator` (`/Game/Blueprints/Interactables/Locator/B_SceneTracker_InteractableLocator.GetViewModel` (`self.B_SceneTracker_InteractableLocator`)) true))

(event `self.B_SceneTracker_InteractableLocator.OnTrackingDisabled`
  ;[1 1 1] Display items for review prompt, then hide when nothing available
  (`/Game/Blueprints/Interactables/B_InteractAreaComponent.SetStatus` (`self.InteractAreaComponent`) (make `/Game/Blueprints/Interactables/Status/STR_InteractStatus` false)))

(event `self.B_SceneTracker_InteractableLocator.OnRangeExceeded`
  (params (player :type "Pawn Object Reference") (inMaxRange :type Boolean))
  ;[1 1 1] Standard show/hide indicator if tracking is enabled
  (`self.IS_TRACKING_PROMPT`)
  (`/Game/Blueprints/Interactables/Locator/ViewModel/B_VM_InteractableLocator.VM_SetShouldDisplayLocator` (`/Game/Blueprints/Interactables/Locator/B_SceneTracker_InteractableLocator.GetViewModel` (`self.B_SceneTracker_InteractableLocator`)) (select `bool` inMaxRange :`true` true)))

(fn `GetTransitionSettings`
  (returns (start :type "Transform Structure") (end :type "Transform Structure") (duration :type "Float (double-precision)"))
  (bind (_start _end _duration) (`/Game/Blueprints/Interactables/Extensions/Ingredients/B_InteractTransitionComponent.GetTransitionSettingsByState` (`self.InteractTransitionComponent`)))
  (return _start _end _duration))

(fn `Place`
  (params (InClass :type "Actor Class Reference"))
  (returns (OutActor :type "Actor Object Reference"))
  (locals (newActor :type "Actor Object Reference"))
  (`|ExecutionSequence`
    (:`then_0`
      (bind _returnvalue (`|SpawnActorFromClass` InClass (`SceneComponent.GetSocketTransform` (`self.StaticMesh`) "Placement" "RTS_World") "AlwaysSpawn" "MultiplyWithRoot" null null))
      (bind _output_get (set `local.newActor` _returnvalue))
      (`KismetArrayLibrary.Array_Add` (`self._placedActors`) _output_get)
      (add `self.OnDestroyed` (`local.newActor`) (`|CreateDelegate` :!event `RemovePlacedActor`)))
    (:`then_1`
      (if (not (`/ActorTracker/Blueprints/B_SceneTracker_Base.IsTracking` (`self.B_SceneTracker_InteractableLocator`)))
        (`/Game/Blueprints/Interactables/Locator/B_SceneTracker_InteractableLocator.SetWidgetTrackingEnabled` (`self.B_SceneTracker_InteractableLocator`) null)))
    (:`then_2`
      (return (`local.newActor`)))))

(fn `UserConstructionScript`)