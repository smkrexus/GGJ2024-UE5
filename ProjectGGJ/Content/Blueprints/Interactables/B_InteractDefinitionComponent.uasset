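; Actor component that makes its owner an interactable, supplying definition data and status to the player's interaction display.
; On BeginPlay it constructs a definition object and initializes it through the owner's BPI_Interactable interface.
; On detection it stores the view and runs a detection action, lazily created via a blocking class load and then cached.
; A detection-loaded event follows, and SyncViewData pushes description and status to the B_PlayerView view model.
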(event `self.ReceiveBeginPlay`
  (if (`KismetSystemLibrary.IsValidClass` (`self.InteractDefinitionClass`))
    (`self.AssignDefinition` (`self.InteractDefinitionClass`))
    (add `self.OnDetectionLoaded` (`|CreateDelegate` :!event `SyncViewData`)) ; once finished loading, send updates to view model
  ))

(event `OnDetectComponent`
  (params (view :type "/Game/Blueprints/Player/ViewModel/B_VM_BaseComponent Object Reference"))
  (set `self.view` view)
  (`self.OnDetected` view) ; best to change to controller to return
  (`self.RunDetectionUpdates`))

(event `OnDetectComponentEnd`
  (`self.OnDetectedEnd`))

(event `SyncViewData`
  (bind _data (`self.RetrieveDataFromDefinition`))
  (bind _asviewmodel_player (cast `/Game/Blueprints/Player/B_PlayerView` (`self.view`)))
  (`/Game/Blueprints/Player/B_PlayerView.VM_SetInteractionDescription` _asviewmodel_player _data (make `/Game/Blueprints/HUD/DisplayHandlers/STR_DisplayHandler_Interactable` _data (`self.RetrieveStatus`)) "NewEnumerator0"))

(event `RunDetectionUpdates`
  (`self.detection`
    (:`then`
      _)
    (:`else`
      (bind _returnvalue (`KismetSystemLibrary.LoadClassAsset_Blocking` (`self.DetectionRefreshClass`)))
      (bind _returnvalue_2 (`|GenericCreateObject` _returnvalue))
      (set `self.detection` (cast `/Game/Blueprints/Interactables/Extensions/Actions/B_InteractAction_Base` _returnvalue_2 :!pure true))))
  (`/Game/Blueprints/Interactables/Extensions/Actions/B_InteractAction_Base.OnActivateAction` (`self.detection`) (`self.GetOwner`) (cast `Controller` (`self.GetOwner` (`self.view`)) :!pure true))
  (`self.OnDetectionLoaded`))

(fn `AssignDefinition`
  (params (ID :type "/Game/Blueprints/Interactables/Definitions/B_InteractDefinition_Base Class Reference"))
  (bind _returnvalue (`|GenericCreateObject` ID))
  (set `self.definition` _returnvalue)
  (bind _asbpi_interactable (cast `/Game/Blueprints/Interactables/BPI_Interactable` (`self.GetOwner`)))
  (`/Game/Blueprints/Interactables/Definitions/B_InteractDefinition_Base.InitializeData` (`self.definition`) _asbpi_interactable))

(fn `RetrieveDataFromDefinition`
  (returns (data :type "/Game/Blueprints/Interactables/InteractableInfoData Object Reference"))
  (return (`/Game/Blueprints/Interactables/Definitions/B_InteractDefinition_Base.GetData` (`self.definition`))))

(fn `RetrieveStatus`
  (returns (status :type "/Game/Blueprints/Interactables/Status/STR_InteractStatus Structure"))
  (return (`self.status`)))