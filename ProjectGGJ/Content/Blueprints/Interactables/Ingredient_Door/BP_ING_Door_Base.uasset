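; Base Blueprint for an interactable door that delegates its open/close transition to a separate action actor.
; BeginPlay assigns the interaction area and async-loads the soft transition class, a BP_InteractAction_Base.
; Interacting spawns that action targeting the door, with IsTransition blocking re-triggers until its end callback toggles IsOpen.
; Functions expose the door state and Hinge, while SetOpened sets only the flag.
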(event `self.ReceiveBeginPlay`
  (`/Game/Blueprints/Interactables/B_InteractAreaComponent.AssignArea` (`self.InteractAreaComponent`) (`self.Area_Interaction`))
  (bind _transitionclass (`self.transitionClass`)
    (:`then`
      (bind _class (`|LoadAssetClass` _transitionclass)
        (:`Completed`
          (bind _asbp_interact_action_base (castclass `/Game/Blueprints/Interactables/Extensions/Actions/BP_InteractAction_Base` _class))
          (set `self.transitionClassLoaded` _asbp_interact_action_base))))
    (:`else`)))

(event `self.InteractAreaComponent.OnInteracted`
  (params (controller :type "Controller Object Reference"))
  (if (not (`self.bIsTransition`))
    (bind _returnvalue (`|SpawnActorFromClass` (`self.transitionClassLoaded`) (`self.GetTransform`) "Undefined" "MultiplyWithRoot" null null))
    (add `/Game/Blueprints/Core/Actions/BP_ExtensibleAction_Base.OnActionEnd` _returnvalue (`|CreateDelegate` :!event `OnDoorActionEnded`))
    (set `self.bIsTransition` true)
    (`/Game/Blueprints/Interactables/Extensions/Actions/BP_InteractAction_Base.OnActivateAction` _returnvalue self controller)))

(event `OnDoorActionEnded`
  (set `self.bIsTransition` false)
  (set `self.bIsOpen` (not (`self.bIsOpen`))))

(fn `GetHinge`
  (returns (Hinge :type "SceneComponent Object Reference"))
  (return (`self.Hinge`)))

(fn `IsDoorOpen`
  (returns (IsOpen :type Boolean) (IsTransition :type Boolean))
  (return (`self.bIsOpen`) (`self.bIsTransition`)))

(fn `SetOpened`
  (params (bIsOpen :type Boolean))
  (set `self.bIsOpen` bIsOpen))

(fn `UserConstructionScript`)