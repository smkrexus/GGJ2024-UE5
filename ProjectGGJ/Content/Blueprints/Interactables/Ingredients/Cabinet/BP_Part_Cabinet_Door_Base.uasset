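; Base interactable cabinet door for the ingredients cabinet that swings open and closed by rotating its root.
; Interactions in its area start the transition component once the requirement component approves.
; When a transition ends, it broadcasts Open or Closed to notify-system observers.
; While open, it adds a tray-closed requirement, so the door can only shut once the tray is closed, and removes it on closing.
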(event `self.ReceiveBeginPlay`
  (`/Game/Blueprints/Interactables/B_InteractAreaComponent.AssignArea` (`self.InteractAreaComponent`) (`self.InteractArea`))
  (`/Game/Blueprints/Interactables/B_InteractAreaComponent.AssignRequirement` (`self.InteractAreaComponent`) (`self.InteractRequirementComponent`))
  (`/Game/Blueprints/Core/Notification/B_NotifySystemComponent.AddSubjectState` (`self.NotifySystemComponent`) (select `bool` (`.bIsOpen` (`/Game/Blueprints/Interactables/Extensions/Ingredients/B_InteractTransitionComponent.GetTransitionStates` (`self.InteractTransitionComponent`))) :`false` (struct :`TagName` "Interaction.Ingredients.Cabinet.Door.Closed") :`true` (struct :`TagName` "Interaction.Ingredients.Cabinet.Door.Open") :!type "GameplayTag Structure")))

(event `self.InteractAreaComponent.OnInteracted`
  (params (controller :type "Controller Object Reference"))
  (if (`/Game/Blueprints/Interactables/B_InteractRequirementComponent.IsRequirementMet` (`self.InteractRequirementComponent`) controller self)
    (`/Game/Blueprints/Interactables/Extensions/Ingredients/B_InteractTransitionComponent.StartTransition` (`self.InteractTransitionComponent`) controller)))

(event `/Game/Blueprints/Interactables/Extensions/Interfaces/BPI_Ingredient_Transform.SetTransform`
  (params (transform :type "Transform Structure"))
  (`SceneComponent.K2_SetRelativeRotation` (`self.DefaultSceneRoot`) (.rotation transform) false false))

(event `self.InteractTransitionComponent.OnTransitionEndEvent`
  (bind _interactrequirementcomponent (`self.InteractRequirementComponent`))
  (bind (_bistransition _bisopen) (`/Game/Blueprints/Interactables/Extensions/Ingredients/B_InteractTransitionComponent.GetTransitionStates` (`self.InteractTransitionComponent`)))
  (`/Game/Blueprints/Core/Notification/B_NotifySystemComponent.BroadcastObservers` (`self.NotifySystemComponent`) (make `/Game/Blueprints/Core/Notification/STR_NotifyHandle_Basic` (`/Game/Blueprints/Core/Notification/B_NotifySystemComponent.subjectTag` (`self.NotifySystemComponent`)) (select `bool` _bisopen :`false` (struct :`TagName` "Interaction.Ingredients.Cabinet.Door.Closed") :`true` (struct :`TagName` "Interaction.Ingredients.Cabinet.Door.Open") :!type "GameplayTag Structure") (`KismetStringLibrary.Concat_StrStr` "CABINET_DOOR_" (select `bool` _bisopen :`false` "CLOSED" :`true` "OPEN")) self))
  ;[1 1 1] Add requirement when it opens. Remove it when closed
  (if (`.bIsOpen` (`/Game/Blueprints/Interactables/Extensions/Ingredients/B_InteractTransitionComponent.GetTransitionStates` (`self.InteractTransitionComponent`)))
    (`/Game/Blueprints/Interactables/B_InteractRequirementComponent.Add Requirement` _interactrequirementcomponent "/Game/Blueprints/Interactables/Requirements/B_InteractRequirement_HasSubjectState_Cabinet.B_InteractRequirement_HasSubjectState_Cabinet_C" null (struct :`TagName` "Interaction.Ingredients.Cabinet.Tray.Closed"))
    (else
      (`/Game/Blueprints/Interactables/B_InteractRequirementComponent.RemoveRequirementByTag` _interactrequirementcomponent (struct :`TagName` "Interaction.Ingredients.Cabinet.Tray.Closed")))))

(fn `GetNotifyComponent`
  (returns (NSC :type "/Game/Blueprints/Core/Notification/B_NotifySystemComponent Object Reference"))
  (return (`self.NotifySystemComponent`)))

(fn `GetTransitionSettings`
  (returns (start :type "Transform Structure") (end :type "Transform Structure") (duration :type "Float (double-precision)"))
  (bind (_start _end _duration) (`/Game/Blueprints/Interactables/Extensions/Ingredients/B_InteractTransitionComponent.GetTransitionSettingsByState` (`self.InteractTransitionComponent`)))
  (return _start _end _duration))

(fn `UserConstructionScript`)