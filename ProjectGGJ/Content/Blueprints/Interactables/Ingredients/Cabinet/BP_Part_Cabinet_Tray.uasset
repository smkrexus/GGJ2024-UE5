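; Interactable tray part of an ingredient cabinet, whose static mesh moves through a state-based transition when interacted with.
; InteractAreaComponent is bound to InteractArea on BeginPlay and passes the interacting controller to InteractTransitionComponent to start the transition.
; GetTransitionSettings returns that component's start, end and duration for the current state.
; SetTransform applies only the location to the mesh's relative position, without sweep or teleport.
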(event `self.ReceiveBeginPlay`
  (`/Game/Blueprints/Interactables/B_InteractAreaComponent.AssignArea` (`self.InteractAreaComponent`) (`self.InteractArea`)))

(event `self.InteractAreaComponent.OnInteracted`
  (params (controller :type "Controller Object Reference"))
  (`/Game/Blueprints/Interactables/Extensions/Ingredients/B_InteractTransitionComponent.StartTransition` (`self.InteractTransitionComponent`) controller))

(event `/Game/Blueprints/Interactables/Extensions/Interfaces/BPI_Ingredient_Transform.SetTransform`
  (params (transform :type "Transform Structure"))
  (`SceneComponent.K2_SetRelativeLocation` (`self.StaticMesh`) (.location transform) false false))

(fn `GetTransitionSettings`
  (returns (start :type "Transform Structure") (end :type "Transform Structure") (duration :type "Float (double-precision)"))
  (bind (_start _end _duration) (`/Game/Blueprints/Interactables/Extensions/Ingredients/B_InteractTransitionComponent.GetTransitionSettingsByState` (`self.InteractTransitionComponent`)))
  (return _start _end _duration))

(fn `UserConstructionScript`)