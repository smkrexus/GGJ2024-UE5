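; Base ingredient cabinet that coordinates its attached door and tray interactable parts.
; On BeginPlay it observes each part's notify component, tracking states in per-part maps.
; Doors all open enable tray interaction, mixed doors disable it, and tray states propagate to doors as tags so extended trays can block closing.
; CreateTrays spawns trays at unique random TrayLocations children using a seeded stream.
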(event `self.ReceiveBeginPlay`
  (for _array_element (`self.GetAttachedActors` true)
    (`self.InitializeCabinetParts` _array_element) ; should call each part for actual init instead of each on begin play
  ))

(event `/Game/Blueprints/Core/Notification/BPI_NotifySystemObserver.NotifyUpdate`
  (params (info :type "/Game/Blueprints/Core/Notification/STR_NotifyHandle_Basic Structure"))
  (`|SwitchGameplayTag` (`.category_2_07B5DF2948628D11FE7D1FA9ACAFB0A5` (break `/Game/Blueprints/Core/Notification/STR_NotifyHandle_Basic` info))
    (:`Interaction.Ingredients.Cabinet.Door`
      ;[1 1 1] run events if doors are of same state
      (bind (_outstate _success) (`self.ValidateCabinetState` (`self.doorStates`) info))
      (if _success
        (if (`BlueprintGameplayTagLibrary.IsGameplayTagValid` _outstate)
          (`self.AddStateToDoors` _outstate)
          (`|SwitchGameplayTag` _outstate
            (:`Interaction.Ingredients.Cabinet.Door.Closed`
              (`self.OnStateDoorsClose`))
            (:`Interaction.Ingredients.Cabinet.Door.Open`
              (`self.OnStateDoorsOpen`)))
          (else
            (`self.RemoveStateFromDoors` (struct :`GameplayTags` (struct :`(TagName` "Interaction.Ingredients.Cabinet.Door.Closed") :`(TagName` "Interaction.Ingredients.Cabinet.Door.Open"))))
            (`self.OnStateDoorsMixed`)))))
    (:`Interaction.Ingredients.Cabinet.Tray`
      ;[1 1 1] add states to doors when tray states change, to prevent doors from being closed when trays are extended
      ; doors requirement searches for Cabinet.Tray.Closed
      (bind (_outstate_2 _success_2) (`self.ValidateCabinetState` (`self.trayStates`) info))
      (if _success_2
        (if (`BlueprintGameplayTagLibrary.IsGameplayTagValid` _outstate_2)
          (`self.AddStateToDoors` _outstate_2)
          (else
            (`self.RemoveStateFromDoors` (struct :`GameplayTags` (struct :`(TagName` "Interaction.Ingredients.Cabinet.Tray.Closed") :`(TagName` "Interaction.Ingredients.Cabinet.Tray.Open"))))))))))

(event `OnStateDoorsClose`
  ;[1 1 1] State Events
)

(event `OnStateDoorsOpen`
  ;[1 1 1] State Events
  (bind _keys (`BlueprintMapLibrary.Map_Keys` (`self.trayStates`)))
  (for _array_element _keys
    (`/Game/Blueprints/Interactables/B_InteractAreaComponent.EnableInteraction` (`self.GetComponentByClass` _array_element "/Game/Blueprints/Interactables/B_InteractAreaComponent.B_InteractAreaComponent_C"))))

(event `OnStateDoorsMixed`
  ;[1 1 1] State Events
  (bind _keys (`BlueprintMapLibrary.Map_Keys` (`self.trayStates`)))
  (for _array_element _keys
    (`/Game/Blueprints/Interactables/B_InteractAreaComponent.DisableInteraction` (`self.GetComponentByClass` _array_element "/Game/Blueprints/Interactables/B_InteractAreaComponent.B_InteractAreaComponent_C"))))

(fn `CreateTrays`
  (locals (availableScenes :type "Array of SceneComponent Object Reference") (selectedScenes :type "Array of SceneComponent Object Reference") (selectedIndex :type Integer :default 0))
  (bind _availablescenes (`local.availableScenes`))
  (`self.RemoveTrays`)
  (if (<= (`self.trayCount`) 0)
    (return)
    (else
      (`self.SetSpawnSeed`)
      (set `local.availableScenes` (`SceneComponent.GetChildrenComponents` (`self.TrayLocations`) false))
      (`|ExecutionSequence`
        (:`then_0`
          (for _ (range (`self.trayCount`))
            (bind _output_get (set `local.selectedIndex` (`KismetMathLibrary.RandomIntegerInRangeFromStream` (`self.randomStream`) 0 (`KismetArrayLibrary.Array_LastIndex` (`local.availableScenes`)))))
            (`KismetSystemLibrary.PrintString` (`KismetStringLibrary.Conv_IntToString` _output_get))
            (`KismetArrayLibrary.Array_Add` (`local.selectedScenes`) (`|GetArrayItem` _availablescenes (`local.selectedIndex`)))
            (`KismetArrayLibrary.Array_Remove` _availablescenes (`local.selectedIndex`))))
        (:`then_1`
          (for _array_element (`local.selectedScenes`)
            (bind _returnvalue (`|SpawnActorFromClass` "/Game/Blueprints/Interactables/Ingredients/Cabinet/BP_Part_Cabinet_Tray.BP_Part_Cabinet_Tray_C" (`SceneComponent.K2_GetComponentToWorld` _array_element) "Undefined" "MultiplyWithRoot" null null))
            (`KismetArrayLibrary.Array_Add` (`self.trays`) _returnvalue)
            (`self.K2_AttachToActor` _returnvalue self "None" "KeepWorld" "KeepWorld" "KeepWorld" true)))))))

(fn `GetNotifyComponent`
  (returns (NSC :type "/Game/Blueprints/Core/Notification/B_NotifySystemComponent Object Reference"))
  (return null))

(fn `InitializeCabinetParts`
  (params (actor :type "Actor Object Reference"))
  (`/Engine/EditorBlueprintResources/StandardMacros.IsValid` actor
    (:`Is Valid`
      (`|ExecutionSequence`
        (:`then_0`
          (if (`GameplayStatics.ObjectIsA` (`local.actor`) "/Game/Blueprints/Interactables/Ingredients/Cabinet/BP_Part_Cabinet_Door_Base.BP_Part_Cabinet_Door_Base_C")
            (`/Game/Blueprints/Core/Notification/Utilities/B_Utilities_NotificationMacros.AddObserverToNSC` (`local.actor`) self
              (:`then`
                (`BlueprintMapLibrary.Map_Add` (`self.doorStates`) (`local.actor`) (struct :`TagName` "Interaction.Ingredients.Cabinet.Door.Closed"))
                (bind _nsc (message `/Game/Blueprints/Core/Notification/BPI_NotifySystemInterface.GetNotifyComponent` (`local.actor`)))
                (`/Game/Blueprints/Core/Notification/B_NotifySystemComponent.AddSubjectState` _nsc (struct :`TagName` "Interaction.Ingredients.Cabinet.Tray.Closed"))))))
        (:`then_1`
          (if (`GameplayStatics.ObjectIsA` (`local.actor`) "/Game/Blueprints/Interactables/Ingredients/Cabinet/BP_Part_Cabinet_Tray.BP_Part_Cabinet_Tray_C")
            (`/Game/Blueprints/Core/Notification/Utilities/B_Utilities_NotificationMacros.AddObserverToNSC` (`local.actor`) self
              (:`then`
                (`BlueprintMapLibrary.Map_Add` (`self.trayStates`) (`local.actor`) (struct :`TagName` "Interaction.Ingredients.Cabinet.Tray.Closed"))
                (`/Game/Blueprints/Interactables/B_InteractAreaComponent.DisableInteraction` (`self.GetComponentByClass` (`local.actor`) "/Game/Blueprints/Interactables/B_InteractAreaComponent.B_InteractAreaComponent_C"))))))))
    (:`Is Not Valid`
      (return))))

(fn `RemoveTrays`
  (locals (attachedActors :type "Array of Actor Object Reference"))
  (if (`KismetArrayLibrary.Array_IsEmpty` (`self.trays`))
    (bind _output_get (set `local.attachedActors` (`self.GetAttachedActors` true)))
    (for _array_element _output_get
      (`/Engine/EditorBlueprintResources/StandardMacros.IsValid` _array_element
        (:`Is Valid`
          (if (`GameplayStatics.ObjectIsA` _array_element "/Game/Blueprints/Interactables/Ingredients/Cabinet/BP_Part_Cabinet_Tray.BP_Part_Cabinet_Tray_C")
            (`self.K2_DestroyActor` _array_element)))))
    (else
      (for _array_element_2 (`self.trays`)
        (`/Engine/EditorBlueprintResources/StandardMacros.IsValid` _array_element_2
          (:`Is Valid`
            (`self.K2_DestroyActor` _array_element_2))))
      (`KismetArrayLibrary.Array_Clear` (`self.trays`)))))

(fn `SetSpawnSeed`
  (returns (seed :type Integer))
  (locals (initialSeed :type Integer) (finalSeed :type Integer))
  (set `local.initialSeed` (`self.seed`))
  (if (`self.bUseRandomSeed`)
    (set `local.initialSeed` (`KismetMathLibrary.RandomInteger` 99999)))
  (`KismetMathLibrary.SetRandomStreamSeed` (`self.randomStream`) (`local.initialSeed`))
  (return (`local.initialSeed`)))

(fn `UserConstructionScript`)

(fn `ValidateCabinetState`
  (params (stateMap :type "Map of Actor Object Reference to GameplayTag Structure (by ref)") (notifyHandle :type "/Game/Blueprints/Core/Notification/STR_NotifyHandle_Basic Structure"))
  (returns (OutState :type "GameplayTag Structure") (Success :type Boolean))
  (locals (state :type "GameplayTag Structure"))
  (bind _asactor (cast `Actor` (`.instigator_5_BFFEB6B64822060984F65EB65E5D6305` (break `/Game/Blueprints/Core/Notification/STR_NotifyHandle_Basic` (`local.notifyHandle`))) :!pure true))
  (`|ExecutionSequence`
    (:`then_0`
      (if (`.ReturnValue` (`BlueprintMapLibrary.Map_Find` (`local.stateMap`) _asactor))
        (`BlueprintMapLibrary.Map_Add` (`local.stateMap`) _asactor (`.channel_13_5DCDBF0C42B3BE5076C51295589D0D2E` (break `/Game/Blueprints/Core/Notification/STR_NotifyHandle_Basic` (`local.notifyHandle`))))
        (else
          (return (struct) false))))
    (:`then_1`
      (bind _values (`BlueprintMapLibrary.Map_Values` (`local.stateMap`)))
      (for _array_element _values
        (if (`BlueprintGameplayTagLibrary.IsGameplayTagValid` (`local.state`))
          (if (not (== _array_element (`local.state`)))
            (return (struct) true) ; return none if states do not match
          )
          (else
            (set `local.state` _array_element))))
      (return (`local.state`) true))))