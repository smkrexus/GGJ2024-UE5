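; Base camera interactable that launches a minigame whose result boosts the Scenario SignalStrength stat in reporter game events.
; Interacting with its area creates the minigame for that player, with its level derived from the Latency event level.
; When the minigame stops, the rating maps to a fixed stat increase, larger for better ratings.
; Area inspection is disabled when an event starts and re-enabled when it ends.
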(event `self.ReceiveBeginPlay`
  (`/Game/Blueprints/Interactables/B_InteractAreaComponent.AssignArea` (`self.B_InteractAreaComponent`) (`self.Interact_Area`)))

(event `self.B_Reporter_GameEvents.OnEventStart`
  (params (InTag :type "GameplayTag Structure") (InLevel :type Integer))
  (`/Game/Blueprints/Interactables/B_InteractAreaComponent.SetInspectionEnabled` (`self.B_InteractAreaComponent`) false))

(event `self.B_Reporter_GameEvents.OnEventEnd`
  (params (InTag :type "GameplayTag Structure"))
  (`/Game/Blueprints/Interactables/B_InteractAreaComponent.SetInspectionEnabled` (`self.B_InteractAreaComponent`) true))

(event `self.B_InteractAreaComponent.OnInteracted`
  (params (controller :type "Controller Object Reference"))
  (`/Game/Blueprints/Gameflow/MiniGame/B_MiniGameSimpleStarterComponent.CreateGame` (`self.B_MiniGameSimpleStarterComponent`) (cast `PlayerController` controller :!pure true) (- (`/Game/Blueprints/Gameflow/Components/B_Reporter_GameEvents.GetEventLevel` (`self.B_Reporter_GameEvents`) (struct :`TagName` "Scenario.GameEvents.Latency")) 1)))

(event `self.B_MiniGameSimpleStarterComponent.OnStop`
  (params (InRating :type "/Game/Blueprints/Gameflow/MiniGame/Scoring/E_MiniGame_Rating Enum" :default "NewEnumerator0"))
  (`self.ADD_SIGNAL_STRENGTH` InRating))

(fn `UserConstructionScript`)