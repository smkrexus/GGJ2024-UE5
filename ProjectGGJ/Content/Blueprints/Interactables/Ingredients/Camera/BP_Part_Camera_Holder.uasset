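; BP_Part_Camera_Holder is a camera holder part among the interactable ingredients, inheriting its behavior from its parent class.
; Its only custom logic is GetInteractInvalidText, which supplies the text for an invalid interaction.
; With a valid equipped item in TargetEquipment, the text says that item, by display name, doesn't fit; otherwise it falls back to the InteractAreaComponent's info text.
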(fn `GetInteractInvalidText`
  (returns (OutText :type Text))
  (bind _item (`/Game/Blueprints/Pawn/B_PawnEquipmentComponent.GetEquippedItem` (`self.targetEquipment`)))
  (`/Engine/EditorBlueprintResources/StandardMacros.IsValid` _item
    (:`Is Valid`
      (return (`|FormatText` "{name} doesn't fit at all" (`/Game/Blueprints/Items/ItemInfoData.displayName` (`/Game/Blueprints/Items/Definitions/B_ItemDefinition_Base.GetData` (`/Game/Blueprints/Pawn/Inventory/B_InventoryItem_Base.GetItem` _item))))))
    (:`Is Not Valid`
      (return (`/Game/Blueprints/Interactables/InteractableInfoData.infoText` (`/Game/Blueprints/Interactables/B_InteractAreaComponent.info` (`self.InteractAreaComponent`)))))))

(fn `UserConstructionScript`
  (`parent.UserConstructionScript`))