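; Pickable camera ingredient that doubles as the interaction point for a minigame during reporter game events.
; StateID drives SwapInteractionMode, which enables either the normal interact area or the event one as events start and end, with each area's collision following its interact toggle.
; Event interaction launches the minigame at a level derived from the Latency event.
; Good or Excellent ratings raise the scenario's SignalStrength stat.
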(event `self.ReceiveBeginPlay`
  (`parent.ReceiveBeginPlay`)
  (`self.INIT_INTERACTION_EVENTS`))

(event `self.B_Reporter_GameEvents.OnEventStart`
  (params (InTag :type "GameplayTag Structure") (bIsPaused :type Boolean) (InLevel :type Integer))
  (if (not bIsPaused)
    (`self.INIT_INTERACTION_EVENTS`)
    (set `self._stateID` 1)
    (`self.SwapInteractionMode`)))

(event `self.B_Reporter_GameEvents.OnEventEnd`
  (params (InTag :type "GameplayTag Structure") (bIsPaused :type Boolean))
  (`self.INIT_INTERACTION_EVENTS`)
  (set `self._stateID` 0)
  (`self.SwapInteractionMode`))

(event `self.InteractAreaComponent_Events.OnInteracted`
  (params (controller :type "Controller Object Reference"))
  (`/Game/Blueprints/Gameflow/MiniGame/B_MiniGameSimpleStarterComponent.CreateGame` (`self.B_MiniGameSimpleStarterComponent`) (cast `PlayerController` controller :!pure true) (- (`/Game/Blueprints/Gameflow/Components/B_Reporter_GameEvents.GetEventLevel` (`self.B_Reporter_GameEvents`) (struct :`TagName` "Scenario.GameEvents.Latency")) 1)))

(event `self.InteractAreaComponent.OnInteractToggled`
  (params (CanInteract :type Boolean))
  (bind _interactarea (`self.InteractArea`))
  (if CanInteract
    (`PrimitiveComponent.SetCollisionEnabled` _interactarea "QueryOnly")
    (else
      (`PrimitiveComponent.SetCollisionEnabled` _interactarea "NoCollision"))))

(event `self.InteractAreaComponent_Events.OnInteractToggled`
  (params (CanInteract :type Boolean))
  (bind _interactarea_events (`self.InteractArea_Events`))
  (if CanInteract
    (`PrimitiveComponent.SetCollisionEnabled` _interactarea_events "QueryOnly")
    (else
      (`PrimitiveComponent.SetCollisionEnabled` _interactarea_events "NoCollision"))))

(event `self.B_MiniGameSimpleStarterComponent.OnStop`
  (params (InRating :type "/Game/Blueprints/Gameflow/MiniGame/Scoring/E_MiniGame_Rating Enum" :default "NewEnumerator0"))
  (bind (_outcomponent _outstats) (`/Game/Blueprints/Gameflow/Components/B_Reporter_GameEvents.GetEventsComponent` (`self.B_Reporter_GameEvents`)))
  (switch `/Game/Blueprints/Gameflow/MiniGame/Scoring/E_MiniGame_Rating` InRating
    (:`NewEnumerator1`
      (`/Game/Blueprints/Core/Stats/B_StatComponent.ChangeStatFromTag` _outstats 3.0 (struct :`TagName` "Stats.Event.Scenario.SignalStrength")))
    (:`NewEnumerator2`
      (`/Game/Blueprints/Core/Stats/B_StatComponent.ChangeStatFromTag` _outstats 4.0 (struct :`TagName` "Stats.Event.Scenario.SignalStrength")))))

(event `self.B_MiniGameSimpleStarterComponent.OnClear`)

(fn `SwapInteractionMode`
  (bind _interactareacomponent_events (`self.InteractAreaComponent_Events`))
  (switch `int` (`self._stateID`)
    (:`-1`
      (`/Game/Blueprints/Interactables/B_InteractAreaComponent.AssignArea` _interactareacomponent_events (`self.InteractArea_Events`))
      (`/Game/Blueprints/Interactables/B_InteractAreaComponent.DisableInteraction` _interactareacomponent_events))
    (:`0`
      (`/Game/Blueprints/Interactables/B_InteractAreaComponent.EnableInteraction` (`self.InteractAreaComponent`))
      (`/Game/Blueprints/Interactables/B_InteractAreaComponent.DisableInteraction` (`self.InteractAreaComponent_Events`)))
    (:`1`
      (`/Game/Blueprints/Interactables/B_InteractAreaComponent.EnableInteraction` (`self.InteractAreaComponent_Events`))
      (`/Game/Blueprints/Interactables/B_InteractAreaComponent.DisableInteraction` (`self.InteractAreaComponent`)))))

(fn `UserConstructionScript`
  (`parent.UserConstructionScript`))