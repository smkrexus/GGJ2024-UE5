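; Interactable adjustment table that holds one user at a time and tracks whether it is clean.
; Adding a user disables interaction; removing one re-enables it and spawns dirt spots at the child component locations of a feedback marker, registered to the table.
; Hygiene stat changes toggle the clean state and status text, with clean requiring maximum hygiene.
; A one-second timer after BeginPlay sets up the initial user or dirt state.
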(event `self.ReceiveBeginPlay`
  (bind _interactareacomponent (`self.InteractAreaComponent`))
  (`/Game/Blueprints/Interactables/B_InteractAreaComponent.AssignArea` _interactareacomponent (`self.InteractArea`))
  (message `/Game/Blueprints/Interactables/Requirements/BPI_RequirementObject.AssignRequirement` _interactareacomponent (`self.InteractRequirementComponent`))
  (`KismetSystemLibrary.K2_SetTimerDelegate` (`|CreateDelegate` :!event `DelayedOnBeginPlay`) 1.0))

(event `OnTableUnavailable`
  (`/Game/Blueprints/Interactables/B_InteractAreaComponent.DisableInteraction` (`self.InteractAreaComponent`)))

(event `OnTableAvailable`
  (`/Game/Blueprints/Interactables/B_InteractAreaComponent.EnableInteraction` (`self.InteractAreaComponent`))
  (`self.CONSTRUCT_DIRT_SPOTS`))

(event `DelayedOnBeginPlay`
  (bind __targetuser (`self._targetUser`)
    (:`then`
      (`self.AddUser` __targetuser))
    (:`else`
      (if (`self.IsCleaned`)
        (`self.SetTableCleaned`)
        (else
          (`self.CONSTRUCT_DIRT_SPOTS`))))))

(event `self.EnvironmentAttributes.OnStatChanged`
  (params (statTag :type "GameplayTag Structure"))
  (bind _outstat (`/Game/Blueprints/Core/Stats/B_StatComponent.GetStatFromTag` (`self.EnvironmentAttributes`) (struct :`TagName` "Stats.Environment.Hygiene")))
  (bind _outvalue (`/Game/Blueprints/Core/Stats/B_Stat.GetStatValue` _outstat))
  (bind ((`Max_13_8A895D624DE880DAA7CAD194D3205837` _max)) (break `/Game/Blueprints/Core/Stats/STR_StatDef` (`/Game/Blueprints/Core/Stats/B_Stat.Stat Def` _outstat)))
  (`|SwitchGameplayTag` statTag
    (:`Stats.Environment.Hygiene`
      (`|ExecutionSequence`
        (:`then_0`
          (if (`self.IsCleaned`)
            (if (< _outvalue _max)
              (`self.SetTableDirty`))
            (elif (== _max _outvalue)
              (`self.SetTableCleaned`))))))))

(fn `AddUser`
  (params (InUser :type "Actor Object Reference"))
  (returns (OutSuccess :type Boolean))
  (if (`self.IsAvailable`)
    (set `self.bIsAvailable` false)
    (bind _output_get (set `self._targetUser` (`local.InUser`)))
    (`self.OnUserAdded` _output_get)
    (`self.OnTableUnavailable`)
    (return true)
    (else
      (return false))))

(fn `AddUserDefault`
  (params (InUser :type "Actor Object Reference"))
  (set `self._targetUser` InUser))

(fn `IsAvailable`
  (returns (IsAvailable :type Boolean))
  (return (`self.bIsAvailable`)))

(fn `IsCleaned`
  (returns (IsCleaned :type Boolean))
  (return (`self.bIsCleaned`)))

(fn `RemoveUser`
  (if (not (`self.IsAvailable`))
    (set `self.bIsAvailable` true)
    (`self._targetUser`
      (:`then`
        (set `self._targetUser` null)
        (`self.OnTableAvailable`)
        (`self.OnUserRemoved`))
      (:`else`))))

(fn `SetTableCleaned`
  (set `self.bIsCleaned` true)
  (`/Game/Blueprints/Interactables/B_InteractAreaComponent.SetStatus` (`self.InteractAreaComponent`) (make `/Game/Blueprints/Interactables/Status/STR_InteractStatus` true "Killed 99.99% bacteria, good enough!")))

(fn `SetTableDirty`
  (set `self.bIsCleaned` false)
  (`/Game/Blueprints/Interactables/B_InteractAreaComponent.SetStatus` (`self.InteractAreaComponent`) (make `/Game/Blueprints/Interactables/Status/STR_InteractStatus` true "Doesn't look too clean")))

(fn `UserConstructionScript`)

(fn `ValidateInitialization`
  (returns (OutValidated :type Boolean))
  (return (`/Game/Blueprints/Core/Stats/B_StatComponent.HasInitialized` (`self.EnvironmentAttributes`))))