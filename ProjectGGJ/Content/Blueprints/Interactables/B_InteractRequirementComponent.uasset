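; Actor component that manages the requirements gating an interaction, stored as requirement objects that can be added, removed, checked or refreshed.
; On BeginPlay it adds a view model component to its owner, then recursively async-loads and constructs default requirements one by one.
; List changes and validity refreshes are pushed to the view model.
; The met check skips soft requirements, and a gameplay-tag cheat queried from the GameMode can bypass requirements.
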(event `self.ReceiveBeginPlay`
  (`|ExecutionSequence`
    (:`then_0`
      (bind _returnvalue (`|AddComponentByClass` (`self.GetOwner`) "/Game/Blueprints/Interactables/Requirements/ViewModel/B_VM_InteractRequirementComponent.B_VM_InteractRequirementComponent_C"))
      (bind _output_get (set `self.viewModel` _returnvalue))
      (set `/Game/Blueprints/Interactables/Requirements/ViewModel/B_VM_InteractRequirementComponent.inputComponent` self _output_get))
    (:`then_1`
      (if (`KismetArrayLibrary.Array_IsNotEmpty` (`self.defaultRequirements`))
        (`self.InitializeRequirement` 0)))))

(event `InitializeRequirement`
  (params (requirementID :type Integer))
  (bind _defaultrequirements (`self.defaultRequirements`))
  (bind (_class _tag) (break `/Game/Blueprints/Interactables/Requirements/STR_InteractRequirement_Handle` (`|GetArrayItem` _defaultrequirements requirementID)))
  (if (`KismetArrayLibrary.Array_IsValidIndex` _defaultrequirements requirementID)
    (bind _class_2 (`|LoadAssetClass` _class)
      (:`Completed`
        (`self.Add Requirement` (castclass `/Game/Blueprints/Interactables/Requirements/B_InteractRequirement_Base` _class_2 :!pure true) null _tag)
        (`self.InitializeRequirement` (+ requirementID 1))))))

(event `EventUpdateVM_AllRequirements`
  (bind _viewmodel (`self.viewModel`))
  (`/Game/Blueprints/Interactables/Requirements/ViewModel/B_VM_InteractRequirementComponent.VM_SetAllRequirements` _viewmodel (`self.allRequirements`))
  (`/Game/Blueprints/Interactables/Requirements/ViewModel/B_VM_InteractRequirementComponent.VM_ShouldUpdateRequirements` _viewmodel))

(fn `Add Requirement`
  (params (requirementType :type "/Game/Blueprints/Interactables/Requirements/B_InteractRequirement_Base Class Reference") (options :type "/Game/Blueprints/Interactables/Requirements/Actions/B_RequirementAction_Base Soft Class Reference") (tag :type "GameplayTag Structure"))
  (returns (addedRequirement :type "/Game/Blueprints/Interactables/Requirements/B_InteractRequirement_Base Object Reference"))
  (locals (newRequirement :type "/Game/Blueprints/Interactables/Requirements/B_InteractRequirement_Base Object Reference"))
  (bind _returnvalue (`|GenericCreateObject` requirementType))
  (bind _output_get (set `local.newRequirement` _returnvalue))
  (`KismetArrayLibrary.Array_Add` (`self.allRequirements`) _output_get)
  (`|ExecutionSequence`
    (:`then_0`
      (`/Game/Blueprints/Interactables/Requirements/B_InteractRequirement_Base.InitializeRequirement` (`local.newRequirement`) (`local.options`) (`local.tag`) (`self.GetOwner`)))
    (:`then_1`
      (`self.EventUpdateVM_AllRequirements`))
    (:`then_2`
      (return (`local.newRequirement`)))))

(fn `GetRequirements`
  (returns (allRequirements :type "Array of /Game/Blueprints/Interactables/Requirements/B_InteractRequirement_Base Object Reference"))
  (return (`self.allRequirements`)))

(fn `GetViewModel`
  (returns (viewModel :type "/Game/Blueprints/Interactables/Requirements/ViewModel/B_VM_InteractRequirementComponent Object Reference"))
  (return (`self.viewModel`)))

(fn `HasRequirements`
  (returns (valid :type Boolean))
  (return (`KismetArrayLibrary.Array_IsNotEmpty` (`self.allRequirements`))))

(fn `IsRequirementMet`
  (params (controller :type "Controller Object Reference") (targetActor :type "Actor Object Reference"))
  (returns (valid :type Boolean))
  (`|ExecutionSequence`
    (:`then_0`
      (if (`KismetArrayLibrary.Array_IsEmpty` (`self.allRequirements`))
        (return true)))
    (:`then_1`
      (`self.CHEAT_REQUIREMENT_DISABLED`
        (:`CheatEnabled`
          (return true))))
    (:`then_2`
      (for _array_element (`self.allRequirements`)
        (if (not (`/Game/Blueprints/Interactables/Requirements/B_InteractRequirement_Base.isSoftRequirement` _array_element))
          (bind _valid (`/Game/Blueprints/Interactables/Requirements/B_InteractRequirement_Base.CheckRequirement` _array_element (`local.controller`) (`local.targetActor`)))
          (if (not _valid)
            (return false))))
      (return true))))

(fn `RefreshRequirementValid`
  (params (controller :type "Controller Object Reference") (targetActor :type "Actor Object Reference"))
  (locals (bRequirementPassed :type Boolean :default false))
  (bind _controller (`local.controller`))
  (`|ExecutionSequence`
    (:`then_0`
      (if (`KismetArrayLibrary.Array_IsEmpty` (`self.allRequirements`))
        (return)))
    (:`then_1`
      (for _array_element (`self.allRequirements`)
        (`self.CHEAT_REQUIREMENT_DISABLED`
          (:`CheatEnabled`
            (`/Game/Blueprints/Interactables/Requirements/ViewModel/B_VM_InteractRequirementComponent.VM_SetRequirementValid` (`self.viewModel`) _array_element true) ; Set all to true
            (`self.OnRequirementPassed` (`local.controller`)))
          (:`then`
            (bind _valid (`/Game/Blueprints/Interactables/Requirements/B_InteractRequirement_Base.CheckRequirement` _array_element (`local.controller`) (`local.targetActor`)))
            (bind _output_get (set `local.bRequirementPassed` _valid))
            (`/Game/Blueprints/Interactables/Requirements/ViewModel/B_VM_InteractRequirementComponent.VM_SetRequirementValid` (`self.viewModel`) _array_element _output_get)))))
    (:`then_2`
      (`/Game/Blueprints/Interactables/Requirements/ViewModel/B_VM_InteractRequirementComponent.VM_RefreshRequirementsValidity` (`self.viewModel`)))
    (:`then_3`
      (if (`local.bRequirementPassed`)
        (`self.OnRequirementPassed` _controller)
        (else
          (`self.OnRequirementFailed` _controller))))))

(fn `RemoveRequirement`
  (params (requirementToRemove :type "/Game/Blueprints/Interactables/Requirements/B_InteractRequirement_Base Object Reference") (instigator :type "Controller Object Reference"))
  (bind _requirementtoremove (`local.requirementToRemove`)
    (:`then`
      (bind _returnvalue (`KismetArrayLibrary.Array_RemoveItem` (`self.allRequirements`) _requirementtoremove))
      (if _returnvalue
        (`/Game/Blueprints/Interactables/Requirements/B_InteractRequirement_Base.OnRemove` (`local.requirementToRemove`) (`local.instigator`))
        (`self.EventUpdateVM_AllRequirements`)))
    (:`else`)))

(fn `RemoveRequirementByTag`
  (params (tag :type "GameplayTag Structure"))
  (locals (removeIndex :type Integer :default -1))
  (if (`BlueprintGameplayTagLibrary.IsGameplayTagValid` (`local.tag`))
    (for (_array_element _array_index) (`self.allRequirements`)
      (if (== (`/Game/Blueprints/Interactables/Requirements/B_InteractRequirement_Base.requirementTag` _array_element) (`local.tag`))
        (set `local.removeIndex` _array_index)
        (break)))
    (if (!= (`local.removeIndex`) -1)
      (`KismetArrayLibrary.Array_Remove` (`self.allRequirements`) (`local.removeIndex`))
      (`self.EventUpdateVM_AllRequirements`))))

(fn `ResetRequirements`
  (`KismetArrayLibrary.Array_Clear` (`self.allRequirements`))
  (`self.EventUpdateVM_AllRequirements`))