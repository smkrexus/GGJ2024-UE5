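; Interactable placement spot where the player puts down the equipped item, previewed by a ghost.
; On detection it spawns a fake-item actor with the async-loaded mesh, while the requirement component drives the valid/invalid prompt.
; Interacting drops the whole stack through a placement drop action, and ItemHolder places it at the hidden ghost's transform.
; Placing an item disables the interact area and hides the scene-tracker locator; pickup or release restores both.
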(event `self.ReceiveBeginPlay`
  (bind _interactareacomponent (`self.InteractAreaComponent`))
  (`/Game/Blueprints/Interactables/B_InteractAreaComponent.AssignArea` _interactareacomponent (`self.MainInteractArea`))
  (message `/Game/Blueprints/Interactables/Requirements/BPI_RequirementObject.AssignRequirement` _interactareacomponent (`self.InteractRequirementComponent`)))

(event `self.InteractAreaComponent.OnInteracted`
  (params (controller :type "Controller Object Reference"))
  (bind _asbp_pawn_custom (cast `/Game/Blueprints/Pawn/BP_PawnCustom` (`Controller.K2_GetPawn` controller)))
  (bind _returnvalue (`self.GetComponentByClass` _asbp_pawn_custom "/Game/Blueprints/Pawn/B_PawnEquipmentComponent.B_PawnEquipmentComponent_C"))
  (bind _item (`/Game/Blueprints/Pawn/B_PawnEquipmentComponent.GetEquippedItem` _returnvalue))
  (`/Engine/EditorBlueprintResources/StandardMacros.IsValid` _item
    (:`Is Valid`
      (`/Game/Blueprints/Pawn/B_PawnEquipmentComponent.DropItem` _returnvalue _item (`.stackCount_10_17932609405E05092F7DF690CEF9C84C` (break `/Game/Blueprints/Items/STR_ItemHandle` (`.handle` (`/Game/Blueprints/Pawn/Inventory/B_InventoryItem_Base.GetItem` _item)))) "/Game/Blueprints/Pawn/Equipment/BP_EquipmentAction_Drop_Placement.BP_EquipmentAction_Drop_Placement_C" self))))

(event `self.InteractAreaComponent.OnDetectedEnd`
  ;[1 1 1] Detection Events
  (`self.HideGhost`))

(event `self.InteractAreaComponent.OnDetected`
  (params (controller :type "Controller Object Reference"))
  (bind _returnvalue (`self.GetComponentByClass` (`Controller.K2_GetPawn` controller) "/Game/Blueprints/Pawn/B_PawnEquipmentComponent.B_PawnEquipmentComponent_C"))
  (bind _item (`/Game/Blueprints/Pawn/B_PawnEquipmentComponent.GetEquippedItem` _returnvalue))
  ;[1 1 1] Detection Events
  (bind _output_get (set `self.targetEquipment` _returnvalue))
  (add `/Game/Blueprints/Pawn/B_PawnEquipmentComponent.OnActiveItemDisabled` _output_get (`|CreateDelegate` :!event `RemoveStatus`))
  (`/Engine/EditorBlueprintResources/StandardMacros.IsValid` _item
    (:`Is Valid`
      (`self.ShowGhost` (`/Game/Blueprints/Pawn/Inventory/B_InventoryItem_Base.GetItem` _item) controller)
      (if (not (`/Game/Blueprints/Interactables/B_InteractRequirementComponent.HasRequirements` (`self.InteractRequirementComponent`)))
        (`self.SetStatus` true)))
    (:`Is Not Valid`
      (`self.HideGhost`)
      (if (not (`/Game/Blueprints/Interactables/B_InteractRequirementComponent.HasRequirements` (`self.InteractRequirementComponent`)))
        (`self.RemoveStatus`)))))

(event `self.InteractRequirementComponent.OnRequirementPassed`
  (params (Controller :type "Controller Object Reference"))
  ;[1 1 1] Status feedback (UI) when hovering over item
  (`self.SetStatus` true))

(event `self.InteractRequirementComponent.OnRequirementFailed`
  (params (Controller :type "Controller Object Reference"))
  ;[1 1 1] Status feedback (UI) when hovering over item
  (`self.SetStatus` false))

(event `SetStatus`
  (params (IsAvailable :type Boolean))
  ;[1 1 1] Status feedback (UI) when hovering over item
  (`/Game/Blueprints/Interactables/B_InteractAreaComponent.SetStatus` (`self.InteractAreaComponent`) (make `/Game/Blueprints/Interactables/Status/STR_InteractStatus` true (select `bool` IsAvailable :`false` (`self.GetInteractInvalidText`) :`true` (`self.GetInteractValidText`)))))

(event `RemoveStatus`
  ;[1 1 1] Status feedback (UI) when hovering over item
  (`/Game/Blueprints/Interactables/B_InteractAreaComponent.SetStatus` (`self.InteractAreaComponent`) (make `/Game/Blueprints/Interactables/Status/STR_InteractStatus`)))

(event `self.ItemHolder.OnRequestPlacement`
  (params (itemHandle :type "/Game/Blueprints/Items/STR_ItemHandle Structure") (requestor :type "Controller Object Reference"))
  ;[1 1 1] Placement events
  (`/Game/Blueprints/Interactables/Extensions/Items/B_ItemHolder.PlaceItem` (`self.ItemHolder`) itemHandle (`self.GetPlacementTransform`)))

(event `self.ItemHolder.OnPlaceItem`
  (params (item :type "/Game/Blueprints/Items/BP_Item_Base Object Reference"))
  (bind _viewmodel (`/Game/Blueprints/Interactables/Locator/B_SceneTracker_InteractableLocator.GetViewModel` (`self.SceneTracker_InteractableLocator`)))
  ;[1 1 1] Placement events
  (`PrimitiveComponent.SetCollisionEnabled` (`self.MainInteractArea`) "NoCollision")
  (`/Engine/EditorBlueprintResources/StandardMacros.IsValid` _viewmodel
    (:`Is Valid`
      (`/Game/Blueprints/Interactables/Locator/ViewModel/B_VM_InteractableLocator.VM_SetShouldDisplayLocator` _viewmodel false))))

(event `self.ItemHolder.OnReleaseItem`
  (params (InItem :type "/Game/Blueprints/Items/BP_Item_Base Object Reference"))
  ;[1 1 1] Placement events
  (`PrimitiveComponent.SetCollisionEnabled` (`self.MainInteractArea`) "QueryOnly" :!label _label)
  (`/Game/Blueprints/Interactables/Locator/ViewModel/B_VM_InteractableLocator.VM_SetShouldDisplayLocator` (`/Game/Blueprints/Interactables/Locator/B_SceneTracker_InteractableLocator.GetViewModel` (`self.SceneTracker_InteractableLocator`)) true))

(event `self.ItemHolder.OnPickupItem`
  (params (itemHandle :type "/Game/Blueprints/Items/STR_ItemHandle Structure"))
  ;[1 1 1] Placement events
  (goto _label))

(event `ShowGhost`
  (params (item :type "/Game/Blueprints/Items/Definitions/B_ItemDefinition_Base Object Reference") (InController :type "Controller Object Reference"))
  (bind _returnvalue (`|SpawnActorFromClass` "/Game/Blueprints/Interactables/Extensions/Items/BP_ItemHolder_FakeItem.BP_ItemHolder_FakeItem_C" (`self.Get Ghost Location` item) "AlwaysSpawn" "MultiplyWithRoot" null null))
  (bind _output_get (set `self._ghost` _returnvalue))
  (`self.OnConstructGhost` _output_get InController)
  (bind _object (`|LoadAsset` (`/Game/Blueprints/Items/ItemFirstPersonInfoData.mesh` (`.dataFirstPerson` (`/Game/Blueprints/Items/Definitions/B_ItemDefinition_Base.GetData` item))))
    (:`Completed`
      (bind __ghost (`self._ghost`)
        (:`then`
          (`/Game/Blueprints/Interactables/Extensions/Items/BP_ItemHolder_FakeItem.ShowFakes` __ghost (cast `StaticMesh` _object :!pure true)))
        (:`else`)))))

(event `HideGhost`
  (bind __ghost (`self._ghost`)
    (:`then`
      (`self.K2_DestroyActor` __ghost))
    (:`else`)))

(event `self.SceneTracker_InteractableLocator.OnRangeDetected`
  (params (player :type "Pawn Object Reference"))
  (`/Game/Blueprints/Interactables/Locator/ViewModel/B_VM_InteractableLocator.VM_SetShouldDisplayLocator` (`/Game/Blueprints/Interactables/Locator/B_SceneTracker_InteractableLocator.GetViewModel` (`self.SceneTracker_InteractableLocator`)) (not (`/Game/Blueprints/Interactables/Extensions/Items/B_ItemHolder.HasItem` (`self.ItemHolder`)))))

(event `self.SceneTracker_InteractableLocator.OnRangeExceeded`
  (params (player :type "Pawn Object Reference") (inMaxRange :type Boolean))
  (if (`/Game/Blueprints/Interactables/Extensions/Items/B_ItemHolder.HasItem` (`self.ItemHolder`))
    (`/Game/Blueprints/Interactables/Locator/ViewModel/B_VM_InteractableLocator.VM_SetShouldDisplayLocator` (`/Game/Blueprints/Interactables/Locator/B_SceneTracker_InteractableLocator.GetViewModel` (`self.SceneTracker_InteractableLocator`)) false)
    (else
      (`/Game/Blueprints/Interactables/Locator/ViewModel/B_VM_InteractableLocator.VM_SetShouldDisplayLocator` (`/Game/Blueprints/Interactables/Locator/B_SceneTracker_InteractableLocator.GetViewModel` (`self.SceneTracker_InteractableLocator`)) inMaxRange))))

(fn `Get Ghost Location`
  (params (Item :type "/Game/Blueprints/Items/Definitions/B_ItemDefinition_Base Object Reference"))
  (returns (OutTransform :type "Transform Structure"))
  (bind _item (`local.Item`))
  (return (`KismetMathLibrary.MakeTransform` (`KismetMathLibrary.TransformLocation` (`self.GetTransform`) (`/Game/Blueprints/Items/Definitions/B_ItemDefinition_Base.worldSpawnOffset` _item)) (`self.K2_GetActorRotation`) (`/Game/Blueprints/Items/Definitions/B_ItemDefinition_Base.worldScale` _item))))

(fn `GetInteractInvalidText`
  (returns (OutText :type Text))
  (bind _infotext (`/Game/Blueprints/Interactables/InteractableInfoData.infoText` (`/Game/Blueprints/Interactables/B_InteractAreaComponent.info` (`self.InteractAreaComponent`))))
  (`/Engine/EditorBlueprintResources/StandardMacros.IsValid` (`/Game/Blueprints/Pawn/B_PawnEquipmentComponent.GetEquippedItem` (`self.targetEquipment`))
    (:`Is Valid`
      (return _infotext))
    (:`Is Not Valid`
      (return _infotext))))

(fn `GetInteractValidText`
  (returns (OutText :type Text))
  (`/Engine/EditorBlueprintResources/StandardMacros.IsValid` (`/Game/Blueprints/Pawn/B_PawnEquipmentComponent.GetEquippedItem` (`self.targetEquipment`))
    (:`Is Valid`
      (return (`|FormatText` "Put down {name}" (`/Game/Blueprints/Items/ItemInfoData.displayName` (`/Game/Blueprints/Items/Definitions/B_ItemDefinition_Base.GetData` (`/Game/Blueprints/Pawn/Inventory/B_InventoryItem_Base.GetItem` (`/Game/Blueprints/Pawn/B_PawnEquipmentComponent.GetEquippedItem` (`self.targetEquipment`))))))))
    (:`Is Not Valid`
      (return ""))))

(fn `GetPlacementTransform`
  (returns (OutTransform :type "Transform Structure"))
  (return (`KismetMathLibrary.MakeTransform` (.location (`SceneComponent.K2_GetComponentToWorld` (`self.Visual_Ghost_Hidden`))) (.rotation (`SceneComponent.K2_GetComponentToWorld` (`self.Visual_Ghost_Hidden`))))))

(fn `OnConstructGhost`
  (params (InGhost :type "/Game/Blueprints/Interactables/Extensions/Items/BP_ItemHolder_FakeItem Object Reference") (InController :type "Controller Object Reference")))

(fn `UserConstructionScript`)