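; Interactable joint point that tracks a patient's bone while it needs attention and hosts the chiropractic adjustment mini-game on it.
; Interacting swaps input mappings, hides the marker and shows a shared bone-twister HUD flagging any known joint issue.
; Mouse input rotates the bone; ExternalInteract ends the game with effects, restores navigation, cracks the bone and reports to game state and mode.
; DisableAttention also runs on BeginPlay, lazily caching the game state.
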(event `self.ReceiveBeginPlay`
  (`self.DisableAttention`))

(event `self.ReceiveTick`
  (params (DeltaSeconds :type "Float (single-precision)"))
  (if (`self.IsRequiringAttention`)
    (`self.UpdateAttentionLocation`)))

(event `/Game/Blueprints/Interactables/BPI_Interactable.Interact`
  (`self.OnActivateOptionalInteract`)
  (bind _foundwidgets (`WidgetBlueprintLibrary.GetAllWidgetsOfClass` "/Game/Blueprints/HUD/BP_Widget_HUDBoneTwister.BP_Widget_HUDBoneTwister_C"))
  (if (`KismetArrayLibrary.Array_IsNotEmpty` _foundwidgets)
    (bind _output (`|GetArrayItem` _foundwidgets))
    (`Widget.SetVisibility` _output "Visible")
    (`/Game/Blueprints/HUD/BP_Widget_HUDBoneTwister.RemindHealthIssue` _output (`self.hasJointIssue`)) ; should bind instead
    (else
      (bind _returnvalue (`|GenericCreateObject` "/Game/Blueprints/HUD/BP_Widget_HUDBoneTwister.BP_Widget_HUDBoneTwister_C"))
      (`UserWidget.AddToViewport` _returnvalue 0)
      (`/Game/Blueprints/HUD/BP_Widget_HUDBoneTwister.RemindHealthIssue` _returnvalue (`self.hasJointIssue`)))))

(event `OnDisableAttention`
  (`self.gameState`
    (:`then`
      (`/Game/Blueprints/BP_Patient.Crack` (`/Game/Blueprints/Gameflow/BP_GameStateCustom.currentPatient` (`self.gameState`)) (`self.boneName`)))
    (:`else`
      (bind _asbp_game_state_custom (cast `/Game/Blueprints/Gameflow/BP_GameStateCustom` (`GameplayStatics.GetGameState`)))
      (bind _output_get (set `self.gameState` _asbp_game_state_custom))))
  (`/Game/Blueprints/Gameflow/BP_GameStateCustom.RemoveActivatedPoint` _output_get self))

(event `OnActivateOptionalInteract`
  (bind _game_mode (`/Game/Blueprints/Gameflow/BP_Utils.Game Mode`))
  ;[1 1 1] Mini game starts with this event
  (`GameplayStatics.PlaySoundAtLocation` "/Game/Assets/Audio/Sound_GroanStart.Sound_GroanStart" (`self.K2_GetActorLocation`) (struct) 1.0 1.0 0.0 null null null null)
  (`/Game/Blueprints/Gameflow/GM_GGJ2024_Base.SetInteractFocusMode` _game_mode true "/Game/Inputs/IM_BoneInteractionInputMap.IM_BoneInteractionInputMap" "/Game/Inputs/IM_CustomInputMap.IM_CustomInputMap") ; set to mini-game mode
  (`self.DisableVisuals`) ; prevent cluttering of screen
  (`/Game/Blueprints/Gameflow/GM_GGJ2024_Base.Event Begin Action` _game_mode))

(event `/Game/Blueprints/Interactables/BPI_Interactable.ExternalInteract`
  (bind _returnvalue (`self.K2_GetActorLocation`))
  ;[1 1 1] Mini game ends with this event
  (`GameplayStatics.PlaySoundAtLocation` "/Game/Assets/Audio/Sound_Groan.Sound_Groan" _returnvalue (struct) 1.0 1.0 0.0 null null null null)
  (`NiagaraFunctionLibrary.SpawnSystemAtLocation` "/Game/Assets/VFX/NS_JointCrack.NS_JointCrack" _returnvalue)
  (`/Game/Blueprints/Gameflow/GM_GGJ2024_Base.SetInteractFocusMode` (`/Game/Blueprints/Gameflow/BP_Utils.Game Mode`) false "/Game/Inputs/IM_CustomInputMap.IM_CustomInputMap" "/Game/Inputs/IM_BoneInteractionInputMap.IM_BoneInteractionInputMap") ; set to player navigation mode
  (`|ExecutionSequence`
    (:`then_0`
      (bind _foundwidgets (`WidgetBlueprintLibrary.GetAllWidgetsOfClass` "/Game/Blueprints/HUD/BP_Widget_HUDBoneTwister.BP_Widget_HUDBoneTwister_C"))
      (if (`KismetArrayLibrary.Array_IsNotEmpty` _foundwidgets)
        (`Widget.SetVisibility` (`|GetArrayItem` _foundwidgets) "Hidden") ; only hides it
      ))
    (:`then_1`
      (`self.DisableAttention`))
    (:`then_2`
      (bind _asbp_game_state_custom (cast `/Game/Blueprints/Gameflow/BP_GameStateCustom` (`GameplayStatics.GetGameState`)))
      (`/Game/Blueprints/Gameflow/BP_Stats.CountAdjustment` (`/Game/Blueprints/Gameflow/BP_GameStateCustom.stats` _asbp_game_state_custom))
      (`/Game/Blueprints/Gameflow/GM_GGJ2024_Base.Event Complete Action` (`/Game/Blueprints/Gameflow/BP_Utils.Game Mode`) (`self.boneName`)))))

(event `OnCreateAttention`
  ;[0.1562 0.04883 0.04883] Hide /unhide main HUD, deprecated as need to see elements
)

(event `/Game/Blueprints/Interactables/BPI_Interactable.ExternalInteractMouse`
  (params (mouseAxis :type "Vector2D Structure"))
  (`self.MoveJoint` mouseAxis))

(fn `CreateAttention`
  (`self.UpdateAttentionLocation`)
  (set `self.isNeedAttention` true)
  (`PrimitiveComponent.SetCollisionEnabled` (`self.Debug`) "QueryOnly")
  (`SceneComponent.SetVisibility` (`self.Debug`) true false)
  (`ActorComponent.Activate` (`self.Niagara`) true)
  (`self.OnCreateAttention`))

(fn `DisableAttention`
  (set `self.isNeedAttention` false)
  (`self.DisableVisuals`)
  (`self.OnDisableAttention`))

(fn `DisableVisuals`
  (`PrimitiveComponent.SetCollisionEnabled` (`self.Debug`) "NoCollision")
  (`SceneComponent.SetVisibility` (`self.Debug`) false false)
  (`ActorComponent.Deactivate` (`self.Niagara`))
  (set `self.isNeedAttention` false))

(fn `GetInteractName`
  (returns (name :type String))
  (return "Interact"))

(fn `GetInteractSound`
  (returns (sound :type "SoundCue Object Reference"))
  (return "/Game/Assets/Audio/Sound_JointInteract.Sound_JointInteract"))

(fn `GetItemInfo`
  (returns (itemInfo :type Text))
  (return (select `bool` (`self.hasJointIssue`) :`false` "Healthy" :`true` "Known Injury" :!type "Text")))

(fn `GetItemName`
  (returns (itemName :type Text))
  (return (`KismetTextLibrary.Conv_NameToText` (`self.boneName`))))

(fn `IsRequiringAttention`
  (returns (isRequireAttention :type Boolean))
  (return (`self.isNeedAttention`)))

(fn `MoveJoint`
  (params (moveDirection :type "Vector2D Structure"))
  (`/Game/Blueprints/BP_Patient.RotateBone` (`/Game/Blueprints/Gameflow/BP_GameStateCustom.currentPatient` (`self.gameState`)) moveDirection (`self.boneName`)))

(fn `RegisterJointIssue`
  (params (hasIssue :type Boolean))
  (set `self.hasJointIssue` hasIssue))

(fn `UpdateAttentionLocation`
  (`self.K2_SetActorLocation` (`/Game/Blueprints/BP_Patient.GetBonePosition` (`/Game/Blueprints/Gameflow/BP_GameStateCustom.currentPatient` (`self.gameState`)) (`self.boneName`)) false true))

(fn `UserConstructionScript`)