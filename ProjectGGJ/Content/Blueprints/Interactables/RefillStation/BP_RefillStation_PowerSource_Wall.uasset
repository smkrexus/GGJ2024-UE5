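; Wall variant of the refill station power source, with a wire whose free end sets where the interaction takes place.
; The construction script shapes the wire spline mesh from the start and end of an editor-placed DEV spline.
; It also moves the tracker locator, hidden ghost visual and interact area to the spline's end, raising the area by half its Z extent.
; GetGhostLocation returns that end in world space, applying the item's spawn offset and scale.
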(fn `Get Ghost Location`
  (params (Item :type "/Game/Blueprints/Items/Definitions/B_ItemDefinition_Base Object Reference"))
  (returns (OutTransform :type "Transform Structure"))
  (bind _item (`local.Item`))
  (return (`KismetMathLibrary.MakeTransform` (+ (.location (`SplineComponent.GetTransformAtTime` (`self.DEV_WireSpline`) 1.0 "World" false false)) (`/Game/Blueprints/Items/Definitions/B_ItemDefinition_Base.worldSpawnOffset` _item)) (.rotation (`SplineComponent.GetTransformAtTime` (`self.DEV_WireSpline`) 1.0 "World" false false)) (`/Game/Blueprints/Items/Definitions/B_ItemDefinition_Base.worldScale` _item))))

(fn `UserConstructionScript`
  (bind _dev_wirespline (`self.DEV_WireSpline`))
  (bind _dev_wirespline_2 (`self.DEV_WireSpline`))
  (bind (_boxextent_x _boxextent_y _boxextent_z) (`KismetMathLibrary.BreakVector` (`BoxComponent.BoxExtent` (`self.MainInteractArea`))))
  (bind _location (.location (`SplineComponent.GetTransformAtTime` _dev_wirespline_2 1.0 "Local" false false)))
  (`SplineMeshComponent.SetStartAndEnd` (`self.Wire_SplineMesh`) (.location (`SplineComponent.GetTransformAtTime` _dev_wirespline_2 0.0 "Local" false false)) (`SplineComponent.GetTangentAtTime` _dev_wirespline 0.0 "Local" false) _location (`SplineComponent.GetTangentAtTime` _dev_wirespline 1.0 "Local" false) true)
  (`SceneComponent.K2_SetRelativeLocationAndRotation` (`self.SceneTracker_InteractableLocator`) _location (.rotation (`SplineComponent.GetTransformAtTime` _dev_wirespline_2 1.0 "Local" false false)) false false)
  (`SceneComponent.K2_SetRelativeLocationAndRotation` (`self.Visual_Ghost_Hidden`) _location (.rotation (`SplineComponent.GetTransformAtTime` _dev_wirespline_2 1.0 "Local" false false)) false false)
  (`SceneComponent.K2_SetRelativeLocationAndRotation` :`self` (`self.MainInteractArea`) :`NewLocation` (+ _location (`KismetMathLibrary.MakeVector` 0.0 0.0 (* _boxextent_z 0.5)))))