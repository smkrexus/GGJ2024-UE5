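; Item-ghost interactable refill station where players place an equipped item and toggle refilling with a switch.
; The item holder sets the refill component's target, and the refill requirement is linked to the switch's requirement component to drive status text and inspection.
; Refill events update switch status and tint an optional poster's emissive color through a dynamic material.
; The placement ghost shows an unsupported material when refill is invalid.
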(event `self.ReceiveBeginPlay`
  (bind _interactareacomponent_switch (`self.InteractAreaComponent_Switch`))
  (`parent.ReceiveBeginPlay`)
  (`|ExecutionSequence`
    (:`then_0`
      (`/Game/Blueprints/Interactables/B_InteractAreaComponent.AssignArea` _interactareacomponent_switch (`self.Switch`))
      (message `/Game/Blueprints/Interactables/Requirements/BPI_RequirementObject.AssignRequirement` _interactareacomponent_switch (`self.InteractRequirementComponent_Switch`)))
    (:`then_1`
      (if (`self.bDisplayPoster`)
        (`self.DisplayPoster`)
        (bind _returnvalue (`KismetMaterialLibrary.CreateDynamicMaterialInstance` (`self._posterMaterial`)))
        (bind _output_get (set `self._posterDMI` _returnvalue))
        (`PrimitiveComponent.SetMaterial` (`self._posterComponent`) 0 _output_get)
        (`self.DISPLAY_STATION_COLOR` (`self.GetStationColors`))))))

(event `self.InteractRequirementComponent.OnRequirementAdded`
  (params (addedRequirement :type "/Game/Blueprints/Interactables/Requirements/B_InteractRequirement_Base Object Reference"))
  ; Shares the requirement for refill to other components that require them
  (if (== (`/Game/Blueprints/Interactables/Requirements/B_InteractRequirement_Base.requirementTag` addedRequirement) (`/Game/Blueprints/Interactables/Extensions/Ingredients/B_RefillComponent.RequirementTag` (`self.RefillComponent`)))
    (`/Game/Blueprints/Interactables/Extensions/Ingredients/B_RefillComponent.AssignRequirementCondition` (`self.RefillComponent`) addedRequirement)
    (`/Game/Blueprints/Interactables/B_InteractRequirementComponent.LinkRequirement` (`self.InteractRequirementComponent_Switch`) addedRequirement)))

(event `self.RefillComponent.OnRefillStart`
  (`/Game/Blueprints/Interactables/B_InteractAreaComponent.SetStatus` (`self.InteractAreaComponent_Switch`) (make `/Game/Blueprints/Interactables/Status/STR_InteractStatus` true "Filling in Progress"))
  (`self.DISPLAY_STATION_COLOR` (`.Valid` (`self.GetStationColors`))))

(event `self.RefillComponent.OnRefillStop`
  (params (isFull :type Boolean))
  (if isFull
    (`/Game/Blueprints/Interactables/B_InteractAreaComponent.SetStatus` (`self.InteractAreaComponent_Switch`) (make `/Game/Blueprints/Interactables/Status/STR_InteractStatus` true "Please remove item")) ; bugs on these set status
    (`self.DISPLAY_STATION_COLOR` (`.Completed` (`self.GetStationColors`)))
    (else
      (`/Game/Blueprints/Interactables/B_InteractAreaComponent.SetStatus` (`self.InteractAreaComponent_Switch`) (make `/Game/Blueprints/Interactables/Status/STR_InteractStatus`))
      (`self.DISPLAY_STATION_COLOR` (`self.GetStationColors`)))))

(event `self.RefillComponent.OnRefillFailed`
  (`self.DISPLAY_STATION_COLOR` (`.Invalid` (`self.GetStationColors`))))

(event `self.ItemHolder.OnPlaceItem`
  (params (item :type "/Game/Blueprints/Items/BP_Item_Base Object Reference"))
  (`/Game/Blueprints/Interactables/Extensions/Ingredients/B_RefillComponent.AssignRefillTarget` (`self.RefillComponent`) item))

(event `self.ItemHolder.OnPickupItem`
  (params (itemHandle :type "/Game/Blueprints/Items/STR_ItemHandle Structure"))
  (bind _visual_ghost_hidden (`self.Visual_Ghost_Hidden`))
  (`PrimitiveComponent.SetCollisionEnabled` _visual_ghost_hidden "QueryAndPhysics")
  (`SceneComponent.SetVisibility` _visual_ghost_hidden true true)
  (`/Game/Blueprints/Interactables/Extensions/Ingredients/B_RefillComponent.ClearRefillTarget` (`self.RefillComponent`)))

(event `self.InteractAreaComponent_Switch.OnInteracted`
  (params (controller :type "Controller Object Reference"))
  (if (`Controller.IsLocalPlayerController` controller)
    (if (`/Game/Blueprints/Interactables/Extensions/Ingredients/B_RefillComponent.IsRefillValid` (`self.RefillComponent`) controller)
      (if (`.bIsRefilling` (`/Game/Blueprints/Interactables/Extensions/Ingredients/B_RefillComponent.GetRefillState` (`self.RefillComponent`)))
        (`/Game/Blueprints/Interactables/Extensions/Ingredients/B_RefillComponent.StopRefill` (`self.RefillComponent`))
        (else
          (`/Game/Blueprints/Interactables/Extensions/Ingredients/B_RefillComponent.StartRefill` (`self.RefillComponent`)))))))

(event `self.InteractAreaComponent_Switch.OnDetected`
  (params (controller :type "Controller Object Reference"))
  ;[0.02083 0.01519 0.001783] Update detected status for VM sync variables
  (`self.targetEquipment`
    (:`then`)
    (:`else`
      (set `self.targetEquipment` (`self.GetComponentByClass` (`Controller.K2_GetPawn` controller) "/Game/Blueprints/Pawn/B_PawnEquipmentComponent.B_PawnEquipmentComponent_C")))))

(event `self.InteractRequirementComponent_Switch.OnRequirementPassed`
  (params (Controller :type "Controller Object Reference"))
  ;[0.02083 0.01519 0.001783] Update detected status for VM sync variables
  (`/Game/Blueprints/Interactables/B_InteractAreaComponent.SetInspectionEnabled` (`self.InteractAreaComponent_Switch`) (not (`/Game/Blueprints/Interactables/Extensions/Items/B_ItemHolder.HasItem` (`self.ItemHolder`))))
  (`|ExecutionSequence`
    (:`then_0`
      (if (`/Game/Blueprints/Interactables/Extensions/Items/B_ItemHolder.HasItem` (`self.ItemHolder`))
        (`/Game/Blueprints/Interactables/B_InteractAreaComponent.SetStatus` (`self.InteractAreaComponent_Switch`) (make `/Game/Blueprints/Interactables/Status/STR_InteractStatus` true (select `int` (`/Game/Blueprints/Interactables/Extensions/Ingredients/B_RefillComponent.GetRefillState` (`self.RefillComponent`)) :`0` "Start Refill" :`1` "Filling in Progress" :`2` "Please remove item" :!type "Text")))
        (else
          (`/Game/Blueprints/Interactables/B_InteractAreaComponent.SetStatus` (`self.InteractAreaComponent_Switch`) (make `/Game/Blueprints/Interactables/Status/STR_InteractStatus` true (`|FormatText` "Place {item} to charge" (`/Game/Blueprints/Items/ItemInfoData.displayName` (`/Game/Blueprints/Items/Definitions/B_ItemDefinition_Base.GetData` (`/Game/Blueprints/Pawn/Inventory/B_InventoryItem_Base.GetItem` (`/Game/Blueprints/Pawn/B_PawnEquipmentComponent.GetEquippedItem` (`self.targetEquipment`)))))))))))))

(event `self.InteractRequirementComponent_Switch.OnRequirementFailed`
  (params (Controller :type "Controller Object Reference"))
  ;[0.02083 0.01519 0.001783] Update detected status for VM sync variables
  (`/Game/Blueprints/Interactables/B_InteractAreaComponent.SetInspectionEnabled` (`self.InteractAreaComponent_Switch`) true)
  (`|ExecutionSequence`
    (:`then_0`
      (if (`/Game/Blueprints/Interactables/Extensions/Items/B_ItemHolder.HasItem` (`self.ItemHolder`))
        (`/Game/Blueprints/Interactables/B_InteractAreaComponent.SetStatus` (`self.InteractAreaComponent_Switch`) (make `/Game/Blueprints/Interactables/Status/STR_InteractStatus` true (`|FormatText` "{item} is incompatible, unable to charge" (`/Game/Blueprints/Items/ItemInfoData.displayName` (`/Game/Blueprints/Items/B_ItemDefinitionComponent.RetrieveData` (`/Game/Blueprints/Items/BP_Item_Base.ItemDefinitionComponent` (`/Game/Blueprints/Interactables/Extensions/Items/B_ItemHolder.GetItem` (`self.ItemHolder`))))))))
        (else
          (`/Game/Blueprints/Interactables/B_InteractAreaComponent.SetStatus` (`self.InteractAreaComponent_Switch`) (make `/Game/Blueprints/Interactables/Status/STR_InteractStatus` true "Waiting for item")))))))

(fn `DisplayPoster`
  (if (`self.bDisplayPoster`)
    (`self._posterComponent`
      (:`then`)
      (:`else`
        (bind _returnvalue (`AddComponent|NODE_AddStaticMeshComponent-0` :`RelativeTransform` (`self._posterTransform`)))
        (bind _output_get (set `self._posterComponent` _returnvalue))
        (`PrimitiveComponent.SetMaterial` _output_get 0 (`self._posterMaterial`))))))

(fn `GetInteractValidText`
  (returns (OutText :type Text))
  (`/Engine/EditorBlueprintResources/StandardMacros.IsValid` (`/Game/Blueprints/Pawn/B_PawnEquipmentComponent.GetEquippedItem` (`self.targetEquipment`))
    (:`Is Valid`
      (return (`|FormatText` "Refill {name}" (`/Game/Blueprints/Items/ItemInfoData.displayName` (`/Game/Blueprints/Items/Definitions/B_ItemDefinition_Base.GetData` (`/Game/Blueprints/Pawn/Inventory/B_InventoryItem_Base.GetItem` (`/Game/Blueprints/Pawn/B_PawnEquipmentComponent.GetEquippedItem` (`self.targetEquipment`))))))))
    (:`Is Not Valid`
      (return ""))))

(fn `GetStationColors`
  (returns (Base :type "LinearColor Structure") (Completed :type "LinearColor Structure") (Valid :type "LinearColor Structure") (Invalid :type "LinearColor Structure"))
  (return (struct :`R` 1.0 :`G` 0.713726 :`A` 1.0) (struct :`R` 0.554766 :`G` 1.0 :`B` 0.47574 :`A` 1.0) (struct :`R` 4.0 :`G` 2.0 :`A` 1.0) (struct :`R` 3.0 :`A` 1.0)))

(fn `OnConstructGhost`
  (params (InGhost :type "/Game/Blueprints/Interactables/Extensions/Items/BP_ItemHolder_FakeItem Object Reference") (InController :type "Controller Object Reference"))
  (if (not (`/Game/Blueprints/Interactables/Extensions/Ingredients/B_RefillComponent.IsRefillValid` (`self.RefillComponent`) (`local.InController`)))
    (`/Game/Blueprints/Interactables/Extensions/Items/BP_ItemHolder_FakeItem.SetCustomMaterial` (`local.InGhost`) "/Game/Assets/Materials/MI_BasicTranslucent_Interact_Unsupported.MI_BasicTranslucent_Interact_Unsupported")))

(fn `UserConstructionScript`
  (`parent.UserConstructionScript`)
  (`self.DisplayPoster`))