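; BP_TagManager manages taggable items for the local player, highlighting the one closest to the camera's view and offering tag input for it.
; On BeginPlay it waits for controller initialization, then creates its view model and caches the pawn camera.
; Its item container drives it through events that toggle ticking, focus and tag inputs as items come and go.
; It also tracks the items' highest tag priority for validation checks.
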(event `self.ReceiveBeginPlay`
  (if (`Controller.IsLocalController` (`GameplayStatics.GetPlayerController` 0))
    (`self.ValidateController`)))

(event `ValidateController`
  (bind _outvalidated (message `/Game/Blueprints/Gameflow/Components/BPI_Gameflow_Validator.ValidateInitialization` (`GameplayStatics.GetPlayerController` 0)))
  (if _outvalidated
    (`self.ValidateControllerSuccess`)
    (else
      (`KismetSystemLibrary.K2_SetTimerDelegate` (`|CreateDelegate` :!event `ValidateController`) 0.5))))

(event `ValidateControllerSuccess`
  (bind _returnvalue (`|AddComponentByClass` "/Game/Blueprints/Interactables/Extensions/Tag/ViewModel/B_VM_TagManager.B_VM_TagManager_C"))
  (set `self.vm_patientManager` _returnvalue)
  (`self.Initialize`))

(event `self.ReceiveTick`
  (params (DeltaSeconds :type "Float (single-precision)"))
  (bind _camera (`self.camera`))
  (`/Engine/EditorBlueprintResources/StandardMacros.IsValid` (`self.camera`)
    (:`Is Valid`
      (`/Game/Blueprints/Interactables/Extensions/Tag/B_TagItemContainer.FindClosestItem` (`self.B_TagItemContainer`) (`SceneComponent.K2_GetComponentLocation` _camera) (`SceneComponent.GetForwardVector` _camera)))
    (:`Is Not Valid`
      (`self.SetActorTickEnabled` false)
      (`self.Initialize`) ; try find camera again
    )))

(event `self.B_TagItemContainer.OnItemAdded`
  (params (itemCount :type Integer))
  (`self.FindHighestPriority`)
  (if (== itemCount 1)
    (`self.SetActorTickEnabled` true)
    (bind _outinputcontroller (`/Game/Blueprints/Core/Utilities/BP_Utils.AddInputController` (`GameplayStatics.GetPlayerController` 0) "/Game/Blueprints/Interactables/Extensions/Tag/Input/B_InputController_TagList.B_InputController_TagList_C" self))
    (set `self.inputs` _outinputcontroller)))

(event `self.B_TagItemContainer.OnItemRemoved`
  (params (itemCount :type Integer))
  (`self.FindHighestPriority`)
  (if (== itemCount 0)
    (`self.SetActorTickEnabled` false)
    (if (not (`/Game/Blueprints/Interactables/Extensions/Tag/B_TagItemContainer.HasTaggedItem` (`self.B_TagItemContainer`)))
      (`/Game/Blueprints/Core/Inputs/B_InputController_Base.RemoveInputs` (`self.inputs`) true))))

(event `self.B_TagItemContainer.OnTagRemove`
  (params (tagCount :type Integer))
  (if (== tagCount 0)
    (if (not (`/Game/Blueprints/Interactables/Extensions/Tag/B_TagItemContainer.HasTagOpportunities` (`self.B_TagItemContainer`)))
      (`/Game/Blueprints/Core/Inputs/B_InputController_Base.RemoveInputs` (`self.inputs`) true))))

(event `self.B_TagItemContainer.OnClosestItemFound`
  (params (Item :type "/Game/Blueprints/Interactables/Extensions/Tag/BP_TagItem_Base Object Reference"))
  (`/Game/Blueprints/Core/Inputs/B_InputController_Base.ActivateSecondaryInput` (`self.inputs`) "tag.available")
  (`/Game/Blueprints/Interactables/Extensions/Tag/BP_TagItem_Base.EnableFocus` Item))

(event `self.B_TagItemContainer.OnClosestItemLost`
  (params (OutItem :type "/Game/Blueprints/Interactables/Extensions/Tag/BP_TagItem_Base Object Reference"))
  (`/Game/Blueprints/Core/Inputs/B_InputController_Base.RemoveSecondaryInput` (`self.inputs`) "tag.available")
  (`/Game/Blueprints/Interactables/Extensions/Tag/BP_TagItem_Base.DisableFocus` OutItem))

(event `self.B_TagItemContainer.OnClosestItemChanged`
  (params (Item :type "/Game/Blueprints/Interactables/Extensions/Tag/BP_TagItem_Base Object Reference") (PreviousItem :type "/Game/Blueprints/Interactables/Extensions/Tag/BP_TagItem_Base Object Reference")))

(fn `FindHighestPriority`
  (if (`BlueprintSetLibrary.Set_IsEmpty` (`/Game/Blueprints/Interactables/Extensions/Tag/B_TagItemContainer.GetItems` (`self.B_TagItemContainer`)))
    (`self.ResetPriority`)
    (return)
    (else
      (set `self._tagPriority` (`self._minPriority`))
      (bind _valuepin (`|SetForEach` (`/Game/Blueprints/Interactables/Extensions/Tag/B_TagItemContainer.GetItems` (`self.B_TagItemContainer`)))
        (:`then`
          (bind ((`Value_5_55073F624202929313316F8B4DEC377F` _value)) (break `/Game/Blueprints/Interactables/Extensions/Tag/Priority/STR_TagPriorityHandle` (`/Game/Blueprints/Interactables/Extensions/Tag/ViewModel/B_VM_TagTarget.VM_GetTagPriority` (`/Game/Blueprints/Interactables/Extensions/Tag/BP_TagItem_Base.ViewModel_TagTarget` _valuepin))))
          (if (> _value (`self._tagPriority`))
            (set `self._tagPriority` _value)))))))

(fn `GetViewModel`
  (returns (OutViewModel :type "/Game/Blueprints/Interactables/Extensions/Tag/ViewModel/B_VM_TagManager Object Reference"))
  (return (`self.vm_patientManager`)))

(fn `Initialize`
  (set `self.camera` (`self.GetComponentByClass` (`GameplayStatics.GetPlayerPawn` 0) "/Script/Engine.CameraComponent"))
  (set `self.bHasInitialized` true))

(fn `ResetPriority`
  (set `self._tagPriority` -1))

(fn `UserConstructionScript`)

(fn `ValidateInitialization`
  (returns (OutValidated :type Boolean))
  (return (`self.bHasInitialized`)))

(fn `ValidatePriority`
  (params (InPriority :type Integer))
  (returns (OutValid :type Boolean))
  (`|ExecutionSequence`
    (:`then_0`
      (if (< (`self._tagPriority`) 0)
        (return true)))
    (:`then_1`
      (return (>= (`local.InPriority`) (`self._tagPriority`))))))