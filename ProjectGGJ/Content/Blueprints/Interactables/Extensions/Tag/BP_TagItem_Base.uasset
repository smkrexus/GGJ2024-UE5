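; BP_TagItem_Base is the base actor for a taggable interactable that players can tag to show its info.
; When a locally controlled pawn enters TrackRadius, it registers with the pawn's tag container, enables the scene-tracker locator and prompts if untagged.
; SetTagged sends the item's message to BP_TagManager's view model or clears it, updating the tag view model.
; Focus toggles the locator's in-range state; Clear cleans up and destroys the actor.
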(event `self.ReceiveBeginPlay`
  (bind _returnvalue (`GameplayStatics.GetActorOfClass` "/Game/Blueprints/Interactables/Extensions/Tag/BP_TagManager.BP_TagManager_C"))
  (set `self._tagManager` _returnvalue))

(event `self.TrackRadius.OnComponentBeginOverlap`
  (params (OverlappedComponent :type "PrimitiveComponent Object Reference") (OtherActor :type "Actor Object Reference") (OtherComp :type "PrimitiveComponent Object Reference") (OtherBodyIndex :type Integer) (bFromSweep :type Boolean) (SweepResult :type "HitResult Structure (by ref)"))
  (bind _b_prompttarget (`self.B_PromptTarget`))
  (bind _aspawn (cast `Pawn` OtherActor))
  (if (`Pawn.IsLocallyControlled` _aspawn)
    (bind _output_get (set `self.tagContainer` (`self.GetComponentByClass` _aspawn "/Game/Blueprints/Interactables/Extensions/Tag/B_TagItemContainer.B_TagItemContainer_C")))
    (`/Game/Blueprints/Interactables/Extensions/Tag/B_TagItemContainer.AddItem` _output_get self)
    (`/Game/Blueprints/Interactables/Locator/B_SceneTracker_InteractableLocator.SetWidgetTrackingEnabled` (`self.B_SceneTracker_InteractableLocator`) null) ; using defaults
    (if (not (`self.IsTagged`))
      (`/Game/Blueprints/Core/Notification/Prompt/B_PromptTarget.SetInputTarget` _b_prompttarget self)
      (`/Game/Blueprints/Core/Notification/Prompt/B_PromptTarget.AddPrompt` _b_prompttarget)
      (`/Game/Blueprints/Core/Notification/Prompt/B_VM_PromptHandler_Base.VM_SetDisplayName` (`/Game/Blueprints/Core/Notification/Prompt/B_PromptTarget.GetViewModel` (`self.B_PromptTarget`)) (`self._prompt`)))))

(event `self.TrackRadius.OnComponentEndOverlap`
  (params (OverlappedComponent :type "PrimitiveComponent Object Reference") (OtherActor :type "Actor Object Reference") (OtherComp :type "PrimitiveComponent Object Reference") (OtherBodyIndex :type Integer))
  (bind _returnvalue (`self.GetComponentByClass` OtherActor "/Game/Blueprints/Interactables/Extensions/Tag/B_TagItemContainer.B_TagItemContainer_C"))
  (`/Engine/EditorBlueprintResources/StandardMacros.IsValid` _returnvalue
    (:`Is Valid`
      (`/Game/Blueprints/Interactables/Extensions/Tag/B_TagItemContainer.RemoveItem` _returnvalue self)
      (`/Game/Blueprints/Core/Notification/Prompt/B_PromptTarget.ClearPrompt` (`self.B_PromptTarget`))
      (`/ActorTracker/Blueprints/B_SceneTracker_Base.SetTrackingEnabled` (`self.B_SceneTracker_InteractableLocator`) false))))

(event `self.B_SceneTracker_InteractableLocator.OnTrackingEnabled`
  (`/Game/Blueprints/Interactables/Locator/ViewModel/B_VM_InteractableLocator.VM_SetShouldDisplayLocator` (`/Game/Blueprints/Interactables/Locator/B_SceneTracker_InteractableLocator.GetViewModel` (`self.B_SceneTracker_InteractableLocator`)) true)
  (`/Game/Blueprints/Interactables/Locator/ViewModel/B_VM_InteractableLocator.VM_SetExtensionViewModel` (`/Game/Blueprints/Interactables/Locator/B_SceneTracker_InteractableLocator.GetViewModel` (`self.B_SceneTracker_InteractableLocator`)) (`self.ViewModel_TagTarget`)))

(event `self.B_SceneTracker_InteractableLocator.OnTrackingDisabled`
  (bind _viewmodel (`/Game/Blueprints/Interactables/Locator/B_SceneTracker_InteractableLocator.GetViewModel` (`self.B_SceneTracker_InteractableLocator`)))
  (`/Engine/EditorBlueprintResources/StandardMacros.IsValid` _viewmodel
    (:`Is Valid`
      (`/Game/Blueprints/Interactables/Locator/ViewModel/B_VM_InteractableLocator.VM_SetShouldDisplayLocator` _viewmodel false))))

(fn `Clear`
  (`/ActorTracker/Blueprints/B_SceneTracker_Base.SetTrackingEnabled` (`self.B_SceneTracker_InteractableLocator`) false)
  (`/Game/Blueprints/Core/Notification/Prompt/B_PromptTarget.ClearPrompt` (`self.B_PromptTarget`))
  (`/Game/Blueprints/Interactables/Extensions/Tag/B_TagItemContainer.DisableTag` (`self.tagContainer`) self)
  (set `self.tagContainer` null)
  (`self.K2_DestroyActor`))

(fn `DisableFocus`
  (`/Game/Blueprints/Interactables/Locator/ViewModel/B_VM_InteractableLocator.VM_SetInRange` (`/Game/Blueprints/Interactables/Locator/B_SceneTracker_InteractableLocator.GetViewModel` (`self.B_SceneTracker_InteractableLocator`)) false))

(fn `EnableFocus`
  (`/Game/Blueprints/Interactables/Locator/ViewModel/B_VM_InteractableLocator.VM_SetInRange` (`/Game/Blueprints/Interactables/Locator/B_SceneTracker_InteractableLocator.GetViewModel` (`self.B_SceneTracker_InteractableLocator`)) true))

(fn `GetItem`
  (returns (OutItem :type "Actor Object Reference"))
  (return (`self._tagItem`)))

(fn `IsTagged`
  (returns (OutValid :type Boolean))
  (return (`self.bIsTagged`)))

(fn `SetTagged`
  (params (InTagged :type Boolean))
  (if (!= InTagged (`self.bIsTagged`))
    (bind _output_get (set `self.bIsTagged` (`local.InTagged`)))
    (if _output_get
      (bind _outinfo (message `/Game/Blueprints/Interactables/Extensions/Tag/BPI_TagItem.TagItem` (`self.GetItem`)))
      (bind _returnvalue (`|GenericCreateObject` "/Game/Blueprints/Interactables/Extensions/Tag/B_TagInfo_ListItem.B_TagInfo_ListItem_C" _outinfo (`self.ViewModel_TagTarget`)))
      (`/Game/Blueprints/Interactables/Extensions/Tag/B_VM_TagManager.VM_SetDisplayInfo` (`/Game/Blueprints/Interactables/Extensions/Tag/BP_TagManager.GetViewModel` (`self._tagManager`)) _returnvalue)
      (`/Game/Blueprints/Core/Notification/Prompt/B_PromptTarget.ClearPrompt` (`self.B_PromptTarget`))
      (`/Game/Blueprints/Interactables/Extensions/Tag/B_VM_TagTarget.VM_SetTagged` (`self.ViewModel_TagTarget`) true)
      (else
        (message `/Game/Blueprints/Interactables/Extensions/Tag/BPI_TagItem.TagClear` (`self.GetItem`))
        (`/Game/Blueprints/Interactables/Extensions/Tag/B_VM_TagManager.VM_ClearDisplayInfo` (`/Game/Blueprints/Interactables/Extensions/Tag/BP_TagManager.GetViewModel` (`self._tagManager`)) 1.0 false)
        (`/Game/Blueprints/Interactables/Extensions/Tag/B_VM_TagTarget.VM_SetTagged` (`self.ViewModel_TagTarget`) false)))))

(fn `UserConstructionScript`
  (`/Game/Blueprints/Interactables/Extensions/Tag/B_VM_TagTarget.VM_SetTagInfo` (`self.ViewModel_TagTarget`) (`self._prompt`)))