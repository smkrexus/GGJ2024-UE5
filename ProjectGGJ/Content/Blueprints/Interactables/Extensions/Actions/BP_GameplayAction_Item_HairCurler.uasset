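; Gameplay action for the hair curler item that applies effects to whatever interactable the player's pawn detects while the action is active.
; On activation it binds to the target BP_PawnInteractionComponent's detection events and immediately handles any interactable already detected.
; Detection applies effects to the interactable's owning actor and detection end removes them, while the empty-interactable handler does nothing.
; Ending the action unbinds all three events.
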(fn `Detect`
  (params (interactable :type "/Game/Blueprints/Interactables/BPI_Interactable Interface"))
  (`self.ApplyEffects` (`ActorComponent.GetOwner` (cast `ActorComponent` (`KismetSystemLibrary.Conv_InterfaceToObject` interactable) :!pure true))))

(fn `DetectEnd`
  (params (interactable :type "/Game/Blueprints/Interactables/BPI_Interactable Interface"))
  (`self.RemoveEffects` (`ActorComponent.GetOwner` (cast `ActorComponent` (`KismetSystemLibrary.Conv_InterfaceToObject` interactable) :!pure true))))

(fn `Empty`)

(fn `EndAction`
  (bind __interactioncomponent (`self._interactionComponent`))
  (remove `/Game/Blueprints/Pawn/BP_PawnInteractionComponent.OnDetectInteractable` __interactioncomponent (`|CreateDelegate` :!event `Detect`))
  (remove `/Game/Blueprints/Pawn/BP_PawnInteractionComponent.OnDetectInteractableEnd` __interactioncomponent (`|CreateDelegate` :!event `DetectEnd`))
  (remove `/Game/Blueprints/Pawn/BP_PawnInteractionComponent.OnEmptyInteractable` __interactioncomponent (`|CreateDelegate` :!event `Empty`))
  (`parent.EndAction`))

(fn `OnActivateAction`
  (params (InHandle :type "/Game/Blueprints/Core/GameplayEffect/STR_GameplayActionHandle Structure"))
  (`parent.OnActivateAction` InHandle)
  (bind _asbp_pawn_interaction_component (cast `/Game/Blueprints/Pawn/BP_PawnInteractionComponent` (`.target_15_219133CC4B21F50C899FB9A5DDC3A199` (break `/Game/Blueprints/Core/GameplayEffect/STR_GameplayActionHandle` InHandle))))
  (add `/Game/Blueprints/Pawn/BP_PawnInteractionComponent.OnDetectInteractable` _asbp_pawn_interaction_component (`|CreateDelegate` :!event `Detect`))
  (add `/Game/Blueprints/Pawn/BP_PawnInteractionComponent.OnDetectInteractableEnd` _asbp_pawn_interaction_component (`|CreateDelegate` :!event `DetectEnd`))
  (add `/Game/Blueprints/Pawn/BP_PawnInteractionComponent.OnEmptyInteractable` _asbp_pawn_interaction_component (`|CreateDelegate` :!event `Empty`))
  (bind _output_get (set `self._interactionComponent` _asbp_pawn_interaction_component))
  (if (`/Game/Blueprints/Pawn/BP_PawnInteractionComponent.HasInteractable` _output_get)
    (`self.Detect` (`/Game/Blueprints/Pawn/BP_PawnInteractionComponent.GetInteractable` _output_get))))

(fn `UserConstructionScript`
  (`parent.UserConstructionScript`))