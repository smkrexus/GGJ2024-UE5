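; Interact action that swings a BP_ING_Door_Base door open or closed by rotating its hinge.
; On activation it picks start and end rotations from the door's open state and starts a one-shot timer lasting the swing duration.
; Tick uses that timer's progress as the lerp alpha for the hinge rotation.
; Ending the action clears the timer and snaps the hinge to its end rotation.
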(event `self.ReceiveTick`
  (params (DeltaSeconds :type "Float (single-precision)"))
  (bind (_percent _elapsed _total _validtimer) (`/Game/Blueprints/Core/Utilities/BP_Utils.GetTimerInfo` (`self.swingTimer`)))
  (if _validtimer
    (`SceneComponent.K2_SetRelativeRotation` (`/Game/Blueprints/Interactables/Ingredient_Door/BP_ING_Door_Base.GetHinge` (`self.door`)) (`KismetMathLibrary.RLerp` (`self.startRotation`) (`self.endRotation`) _percent) false false)))

(fn `EndAction`
  (`KismetSystemLibrary.K2_ClearAndInvalidateTimerHandle` (`self.swingTimer`))
  (`SceneComponent.K2_SetRelativeRotation` (`/Game/Blueprints/Interactables/Ingredient_Door/BP_ING_Door_Base.GetHinge` (`self.door`)) (`self.endRotation`) false false) ; ensure end action values
  (`parent.EndAction`))

(fn `OnActivateAction`
  (params (targetActor :type "Actor Object Reference") (instigator :type "Controller Object Reference"))
  (bind _doorangle (`self.doorAngle`))
  (bind _isopen (`/Game/Blueprints/Interactables/Ingredient_Door/BP_ING_Door_Base.IsDoorOpen` (`self.door`)))
  (bind _asbp_ing_door_base (cast `/Game/Blueprints/Interactables/Ingredient_Door/BP_ING_Door_Base` targetActor))
  (set `self.door` _asbp_ing_door_base)
  (set `self.startRotation` (select `bool` _isopen :`false` (struct) :`true` _doorangle))
  (set `self.endRotation` (select `bool` _isopen :`false` _doorangle))
  (bind _returnvalue (`KismetSystemLibrary.K2_SetTimerDelegate` (`|CreateDelegate` :!event `EndAction`) (`self.swingDuration`)))
  (set `self.swingTimer` _returnvalue))

(fn `UserConstructionScript`
  (`parent.UserConstructionScript`))