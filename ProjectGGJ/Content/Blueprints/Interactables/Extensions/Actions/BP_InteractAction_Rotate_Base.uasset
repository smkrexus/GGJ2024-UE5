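; Base interact action that rotates a target actor between a start and end rotation over a set duration.
; On activation it reads the rotations and duration from the target's transition settings message and starts a swing timer.
; Tick lerps rotation by timer progress and sends it through SetTransformMessage, with location fixed at zero and scale at one.
; Ending the action clears the timer.
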(event `self.ReceiveTick`
  (params (DeltaSeconds :type "Float (single-precision)"))
  (bind (_percent _elapsed _total _validtimer) (`/Game/Blueprints/Core/Utilities/BP_Utils.GetTimerInfo` (`self.swingTimer`)))
  (if _validtimer
    (message `/Game/Blueprints/Interactables/Extensions/Interfaces/BPI_Ingredient_Transform.SetTransform` (`self.target`) (`KismetMathLibrary.MakeTransform` (0.0 0.0 0.0) (`KismetMathLibrary.RLerp` (`self.startRotation`) (`self.endRotation`) _percent)))))

(fn `EndAction`
  (`KismetSystemLibrary.K2_ClearAndInvalidateTimerHandle` (`self.swingTimer`))
  (`parent.EndAction`))

(fn `OnActivateAction`
  (params (targetActor :type "Actor Object Reference") (instigator :type "Controller Object Reference"))
  (bind _output_get (set `self.target` targetActor))
  (bind (_start _end _duration) (message `/Game/Blueprints/Interactables/Extensions/Interfaces/BPI_Ingredient_Transform.GetTransitionSettings` _output_get))
  (set `self.startRotation` (.rotation _start))
  (set `self.endRotation` (.rotation _end))
  (bind _returnvalue (`KismetSystemLibrary.K2_SetTimerDelegate` (`|CreateDelegate` :!event `EndAction`) _duration))
  (set `self.swingTimer` _returnvalue))

(fn `UserConstructionScript`
  (`parent.UserConstructionScript`))