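; Interact action that slides a BP_ING_Door_Base door between its default location and an offset one.
; On activation it picks start and end from the door's open state, adding DefaultLocation to SlideLocation each time, and starts a one-shot timer.
; Tick uses the timer's percent to lerp the door hinge's relative location.
; EndAction clears the timer and snaps the hinge to the end location.
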(event `self.ReceiveTick`
  (params (DeltaSeconds :type "Float (single-precision)"))
  (bind (_percent _elapsed _total _validtimer) (`/Game/Blueprints/Core/Utilities/BP_Utils.GetTimerInfo` (`self.slideTimer`)))
  (if _validtimer
    (`SceneComponent.K2_SetRelativeLocation` (`/Game/Blueprints/Interactables/Ingredient_Door/BP_ING_Door_Base.GetHinge` (`self.door`)) (`KismetMathLibrary.VLerp` (`self.startLocation`) (`self.endLocation`) _percent) false false)))

(fn `EndAction`
  (`KismetSystemLibrary.K2_ClearAndInvalidateTimerHandle` (`self.slideTimer`))
  (`SceneComponent.K2_SetRelativeLocation` (`/Game/Blueprints/Interactables/Ingredient_Door/BP_ING_Door_Base.GetHinge` (`self.door`)) (`self.endLocation`) false false)
  (`parent.EndAction`))

(fn `OnActivateAction`
  (params (targetActor :type "Actor Object Reference") (instigator :type "Controller Object Reference"))
  (bind _slidelocation (`self.slideLocation`))
  (bind _isopen (`/Game/Blueprints/Interactables/Ingredient_Door/BP_ING_Door_Base.IsDoorOpen` (`self.door`)))
  (bind _asbp_ing_door_base (cast `/Game/Blueprints/Interactables/Ingredient_Door/BP_ING_Door_Base` targetActor))
  (set `self.door` _asbp_ing_door_base)
  (set `self.slideLocation` (+ (`self.slideLocation`) (`self.defaultLocation`)))
  (set `self.startLocation` (select `bool` _isopen :`false` (`self.defaultLocation`) :`true` _slidelocation))
  (set `self.endLocation` (select `bool` _isopen :`false` _slidelocation :`true` (`self.defaultLocation`)))
  (bind _returnvalue (`KismetSystemLibrary.K2_SetTimerDelegate` (`|CreateDelegate` :!event `EndAction`) (`self.slideDuration`)))
  (set `self.slideTimer` _returnvalue))

(fn `UserConstructionScript`
  (`parent.UserConstructionScript`))