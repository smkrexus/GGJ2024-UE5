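; Base Blueprint for a ring light ingredient interactable that the player can grab and release.
; On BeginPlay it assigns its main interact area to the interact area component.
; An interaction forwards the controller as a grab request to the grab definition component.
; Grab and release events print debug text and toggle the stand's collision off while held and back on when released.
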(event `self.ReceiveBeginPlay`
  (`/Game/Blueprints/Interactables/B_InteractAreaComponent.AssignArea` (`self.B_InteractAreaComponent`) (`self.InteractArea_Main`)))

(event `self.B_InteractAreaComponent.OnInteracted`
  (params (controller :type "Controller Object Reference"))
  (`/Game/Blueprints/Pawn/Interaction/B_GrabDefinitionComponent.SendGrabRequest` (`self.B_GrabDefinitionComponent`) controller))

(event `self.B_GrabDefinitionComponent.OnGrab`
  (`KismetSystemLibrary.PrintText` "Grab!")
  (`PrimitiveComponent.SetCollisionEnabled` (`self.Stand`) "NoCollision"))

(event `self.B_GrabDefinitionComponent.OnRelease`
  (`KismetSystemLibrary.PrintText` "Release!")
  (`PrimitiveComponent.SetCollisionEnabled` (`self.Stand`) "QueryAndPhysics"))

(fn `UserConstructionScript`)