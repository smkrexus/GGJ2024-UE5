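; Interactable patient health chart that opens a patient history screen, supplying "Patient History" as its interact name along with an interact sound.
; Interact swaps the player controller to the interaction-lock input mapping, hides the HUD and shows the history widget, creating it only if none exists.
; ExternalInteract reverses this by restoring normal input and the HUD and hiding, rather than removing, the history widget for reuse.
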(event `/Game/Blueprints/Interactables/BPI_Interactable.Interact`
  (bind _asbp_pawn_controller_custom (cast `/Game/Blueprints/BP_PawnControllerCustom` (`GameplayStatics.GetPlayerController` 0)))
  (`/Game/Blueprints/BP_PawnControllerCustom.DisableMappingContext` _asbp_pawn_controller_custom "/Game/Inputs/IM_CustomInputMap.IM_CustomInputMap")
  (`/Game/Blueprints/BP_PawnControllerCustom.SetMappingContext` _asbp_pawn_controller_custom "/Game/Inputs/IM_LockInteractionMap.IM_LockInteractionMap") ; set to interact lock
  (`|ExecutionSequence`
    (:`then_0`
      (bind _foundwidgets (`WidgetBlueprintLibrary.GetAllWidgetsOfClass` "/Game/Blueprints/HUD/BP_Widget_HUDCustom.BP_Widget_HUDCustom_C"))
      (if (`KismetArrayLibrary.Array_IsNotEmpty` _foundwidgets)
        (`Widget.SetVisibility` (`|GetArrayItem` _foundwidgets) "Hidden") ; only hides it
      ))
    (:`then_1`
      (bind _foundwidgets_2 (`WidgetBlueprintLibrary.GetAllWidgetsOfClass` "/Game/Blueprints/HUD/BP_Widget_PatientHistory.BP_Widget_PatientHistory_C"))
      (if (`KismetArrayLibrary.Array_IsNotEmpty` _foundwidgets_2)
        (`Widget.SetVisibility` (`|GetArrayItem` _foundwidgets_2) "Visible")
        (else
          (bind _returnvalue (`|GenericCreateObject` "/Game/Blueprints/HUD/BP_Widget_PatientHistory.BP_Widget_PatientHistory_C"))
          (`UserWidget.AddToViewport` _returnvalue 0))))))

(event `/Game/Blueprints/Interactables/BPI_Interactable.ExternalInteract`
  (bind _asbp_pawn_controller_custom (cast `/Game/Blueprints/BP_PawnControllerCustom` (`GameplayStatics.GetPlayerController` 0)))
  (`/Game/Blueprints/BP_PawnControllerCustom.DisableMappingContext` _asbp_pawn_controller_custom "/Game/Inputs/IM_LockInteractionMap.IM_LockInteractionMap")
  (`/Game/Blueprints/BP_PawnControllerCustom.SetMappingContext` _asbp_pawn_controller_custom "/Game/Inputs/IM_CustomInputMap.IM_CustomInputMap") ; set to normal
  (`|ExecutionSequence`
    (:`then_0`
      (bind _foundwidgets (`WidgetBlueprintLibrary.GetAllWidgetsOfClass` "/Game/Blueprints/HUD/BP_Widget_HUDCustom.BP_Widget_HUDCustom_C"))
      (if (`KismetArrayLibrary.Array_IsNotEmpty` _foundwidgets)
        (`Widget.SetVisibility` (`|GetArrayItem` _foundwidgets) "Visible") ; only hides it
      ))
    (:`then_1`
      (bind _foundwidgets_2 (`WidgetBlueprintLibrary.GetAllWidgetsOfClass` "/Game/Blueprints/HUD/BP_Widget_PatientHistory.BP_Widget_PatientHistory_C"))
      (if (`KismetArrayLibrary.Array_IsNotEmpty` _foundwidgets_2)
        (`Widget.SetVisibility` (`|GetArrayItem` _foundwidgets_2) "Hidden")))))

(fn `GetInteractName`
  (returns (name :type String))
  (return "Patient History"))

(fn `GetInteractSound`
  (returns (sound :type "SoundCue Object Reference"))
  (return "/Game/Assets/Audio/Sound_JointInteract.Sound_JointInteract"))

(fn `UserConstructionScript`)