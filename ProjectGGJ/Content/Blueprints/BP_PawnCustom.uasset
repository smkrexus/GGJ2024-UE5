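; Custom player pawn with hand-built movement, jumping, look controls, an interaction raycast and a debug damage key that lowers health in the player state.
; Movement input either offsets actor location or adds impulses to a physics sphere, with optional boost.
; Each tick a downward sphere trace drives ground state and manual gravity on vertical air speed, avoiding wall sticking, and zeroes Z velocity on flat ground to stop bouncing.
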(event Custom|InteractionRaycast
  (bind _camera (Variables|Default|GetCamera))
  ;[1 1 1] Interaction for chiropractic point
  (Default|RaycastInteraction (Variables|Default|GetBP_PawnInteractionComponent) (Transformation|GetWorldLocation _camera) (Math|Vector|GetForwardVector _camera)))

(event Custom|OnGroundExit
  ;[1 1 1] Ground check events
  (Variables|ShouldBeLocal|SetonGround false)
  (Development|PrintString "Left off ground"))

(event Custom|OnGroundLanded
  (params (ImpactLocation :type Vector))
  (bind _returnvalue (Transformation|GetActorLocation))
  ;[1 1 1] Ground check events
  (Development|PrintString "OnGroundFlat")
  (Transformation|SetActorLocation (Math|Vector|MakeVector (.x _returnvalue) (.y _returnvalue) (+ (.Z (Math|Vector|BreakVector ImpactLocation)) 5e+01)) false false) ; ensure actor not in ground
  (Variables|ShouldBeLocal|SetonGround true)
  (Variables|ShouldBeLocal|SetAirSpeed 0.0)
  (Variables|ShouldBeLocal|SetAirDuration 0.0))

(event EventBeginPlay)

(event Collision|EventActorBeginOverlap
  (params (OtherActor :type Actor%20Object%20Reference)))

(event EventTick
  (params (DeltaSeconds :type Float%20%28single-precision%29))
  (bind _returnvalue (Transformation|GetActorLocation))
  (bind _returnvalue_2 (Transformation|GetActorLocation))
  (Utilities|FlowControl|Sequence
    (:then_0
      ;[1 1 1] Update move input
      (if (Utilities|HasDirectionalInput (Variables|InputValues|GetmoveDirection))
        (CallFunction|ActionMove DeltaSeconds)))
    (:then_1
      ;[1 1 1] Simulate gravity for falling/jumping, manual gravity as enabling gravity on sphere will cause it to stuck on wall, should put as gravity component...
      (bind (_outhit _returnvalue_3) (Collision|SphereTraceByChannel _returnvalue_2 (- _returnvalue_2 "0.000000,0.000000,35.000000") 2e+01 "TraceTypeQuery1" false 0 "ForDuration" true "(R=1.000000,G=0.000000,B=0.000000,A=1.000000)" "(R=0.000000,G=1.000000,B=0.000000,A=1.000000)" 0.1))
      (if _returnvalue_3
        (Utilities|IsGrounded
          (:True
            (Utilities|IsGroundFlat (.impactnormal _outhit)
              (:true
                (|EnableBounceDampening))
              (:false
                _)))
          (:False
            (CallFunction|OnGroundLanded (.impactpoint _outhit))))
        (Utilities|HasAirSpeed
          (:true
            (Transformation|SetActorLocation (Math|Vector|MakeVector (.x _returnvalue) (.y _returnvalue) (+ (.z _returnvalue) (Variables|ShouldBeLocal|GetAirSpeed))) false true :!label _label)))
        (else
          (Utilities|FlowControl|Sequence
            (:then_0
              (Utilities|IsGrounded
                (:True
                  (CallFunction|OnGroundExit))))
            (:then_1
              (Utilities|SetVelocitybyGravity DeltaSeconds)
              (goto _label))))))
    (:then_2
      (CallFunction|InteractionRaycast))))

(event Input|KeyboardEvents|DebugKeyF
  (params (Key :type Key%20Structure :default "None") (ActionValue :type Input%20Action%20Value%20Structure))
  ;[1 0.005208 0.005208] Debug to show HUD feedback
  (:Pressed
    (Development|PrintString "Debug Key pressed... damaging")
    (CallFunction|Damage 1e+01)))

(event EventAddInputMovement
  (params (direction :type Vector%202D%20Structure))
  (Variables|InputValues|SetmoveDirection direction))

(event EventAddInputMovementBoost
  (params (enabled :type Boolean))
  (Variables|InputValues|SetisAddBoost enabled))

(event EventActionMove
  (params (tickTime :type Float%20%28double-precision%29))
  (|UpdatePawnMovement tickTime))

(event EventAddInputJump
  (Utilities|IsGrounded
    (:True
      (CallFunction|ActionJump))))

(event EventActionJump
  (|SetJumpSettings))

(event EventAddInputLook
  (params (lookDirection :type Vector%202D%20Structure))
  (if (Utilities|HasDirectionalInput lookDirection)
    (CallFunction|ActionLook lookDirection)))

(event EventActionLook
  (params (lookDirection :type Vector%202D%20Structure))
  (|UpdateAllRotations lookDirection))

(fn ConstructionScript)

(fn GetPlayerInfo
  (Variables|Default|GetplayerInfo
    (:then
      _)
    (:else
      (bind _asbp_player_state_custom (Utilities|Casting|CastToBP_PlayerStateCustom (Game|GetPlayerState 0)))
      (Variables|Default|SetplayerInfo _asbp_player_state_custom)))
  (return (Variables|Default|GetplayerInfo)))

(fn Damage
  (params (damage :type Float%20%28double-precision%29))
  (bind _info (CallFunction|GetPlayerInfo))
  (Default|SetHealth _info (- (.health (Default|GetHealth _info)) damage)))