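; Room manager that detects rooms in front of the player camera and notifies listeners when they are found or lost.
; After gameflow validation, it initializes every BP_Room_Base and starts a looping search timer.
; Searches fan sphere traces across a cone for "room_main" components, ignoring entered rooms, then diff results against the previous set.
; Indicator display assets async-load when detections increase and unload when none remain.
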(event `self.ReceiveBeginPlay`
  (`/Game/Blueprints/Gameflow/Validators/B_ValidateGameflowComponent.RunValidation` (`self.ValidatorGameflow`)))

(event `self.ValidatorGameflow.OnValidationCompleted`
  ;[0.7396 0 0.0035] BUG ALERT
  (set `self._camera` (`self.GetComponentByClass` (`GameplayStatics.GetPlayerPawn` 0) "/Script/Engine.CameraComponent")) ; This can be null once player dies, fix later
  (bind _outactors (`GameplayStatics.GetAllActorsOfClass` "/Game/Blueprints/Room/BP_Room_Base.BP_Room_Base_C"))
  (for _array_element _outactors
    (`/Game/Blueprints/Room/BP_Room_Base.Initialize` _array_element self))
  ;[0.3913 0 0 0.5] BUG ALERT Will need to account for pause / cinematic states eventually
  (bind _returnvalue (`KismetSystemLibrary.K2_SetTimerDelegate` (`|CreateDelegate` :!event `SearchRooms`) 1.0 true true))
  (set `self._searchRoomTimer` _returnvalue))

(event `MarkEntered`
  (params (InRoom :type "/Game/Blueprints/Room/BP_Room_Base Object Reference"))
  (`KismetArrayLibrary.Array_AddUnique` (`self._enteredRooms`) InRoom))

(event `ClearEntered`
  (params (InRoom :type "/Game/Blueprints/Room/BP_Room_Base Object Reference"))
  (`KismetArrayLibrary.Array_RemoveItem` (`self._enteredRooms`) InRoom))

(event `ValidateFoundRooms`
  (params (FoundRooms :type "Set of Actor Object Reference"))
  ;[0.07292 0.05984 0 1 32] ROOM DETECTION BY TRACE
  (if (> (`BlueprintSetLibrary.Set_Length` FoundRooms) (`BlueprintSetLibrary.Set_Length` (`self._detectedRooms`)))
    (`self.OnRoomsFound` FoundRooms)
    ;;[0.4844 0.4844 0.4844 0.5] If asset are unloaded, this will load them
    ;; Instantly sends OnAssetReady if already loaded
    (`self.RequestAssetLoad`)))

(event `LoadAssetList`
  (params (ID :type "Array of PrimaryAssetId Structure"))
  ;[0.07292 0.05984 0 1 32] ROOM DETECTION BY TRACE
  ;;[0.4844 0.4844 0.4844 0.5] If asset are unloaded, this will load them
  ;; Instantly sends OnAssetReady if already loaded
  (`AsyncActionLoadPrimaryAssetList.AsyncLoadPrimaryAssetList` ID
    (:`Completed`
      (`self.OnAssetLoaded`))))

(event `ValidateLostRooms`
  (params (FoundRooms :type "Set of Actor Object Reference"))
  ;[0.07292 0.05984 0 1 32] ROOM DETECTION BY TRACE
  (`|ExecutionSequence`
    (:`then_0`
      (bind _result (`BlueprintSetLibrary.Set_Difference` (`self._detectedRooms`) FoundRooms)) ; find items in last detected rooms that does not exist in found rooms = lost rooms\nif there are lost rooms, push lost rooms event\n\nwhen last detected rooms has not been assigned, there will be no lost rooms\nwhen all items in found room exist in  last detected room, then difference is 0 = no lost rooms\nwhen no items in found room, then difference is all items in last detected rooms = all lost rooms
      (if (`BlueprintSetLibrary.Set_IsNotEmpty` _result)
        (`self.OnRoomsLost` _result)))
    (:`then_1`
      (if (and (`BlueprintSetLibrary.Set_IsEmpty` FoundRooms) (`BlueprintSetLibrary.Set_IsNotEmpty` (`self._detectedRooms`)))
        ;;[0.02732 0.06771 0.01199] If no rooms detected, safe to unload
        (bind _outprimaryassetidlist (`KismetSystemLibrary.GetPrimaryAssetIdList` "PDA_RoomIndicatorDisplayInfo_C"))
        (`KismetSystemLibrary.UnloadPrimaryAssetList` _outprimaryassetidlist)))))

(fn `GetDetectorCamera`
  (returns (OutCamera :type "CameraComponent Object Reference"))
  (return (`self._camera`)))

(fn `GetIndicatorDisplayInfo`
  (params (InType :type "/Game/Blueprints/Room/Episode/E_RoomEpisodeTypes Enum (by ref)"))
  (returns (OutInfo :type "/Game/Blueprints/Room/Indicator/PDA_RoomIndicatorDisplayInfo Object Reference"))
  (locals (asset :type "Object Object Reference"))
  (bind _output_get (set `local.asset` (`KismetSystemLibrary.GetObjectFromPrimaryAssetId` (`KismetSystemLibrary.GetPrimaryAssetIdFromSoftObjectReference` (`BlueprintMapLibrary.Map_Find` (defaults `Object` (`self._indicatorSettingClass`)) (`local.InType`))))))
  (`/Engine/EditorBlueprintResources/StandardMacros.IsValid` _output_get
    (:`Is Valid`
      (bind _aspda_room_indicator_display_info (cast `/Game/Blueprints/Room/Indicator/PDA_RoomIndicatorDisplayInfo` _output_get))
      (return _aspda_room_indicator_display_info))
    (:`Is Not Valid`
      (return null))))

(fn `IsAssetReady`
  (returns (OutValid :type Boolean))
  (bind _outprimaryassetidlist (`KismetSystemLibrary.GetPrimaryAssetIdList` "PDA_RoomIndicatorDisplayInfo_C"))
  (for _array_element _outprimaryassetidlist
    (if (not (`KismetSystemLibrary.IsValid` (`KismetSystemLibrary.GetObjectFromPrimaryAssetId` _array_element)))
      (return false)))
  (return true))

(fn `RequestAssetLoad`
  (if (`self.IsAssetReady`)
    (`self.OnAssetLoaded`)
    (else
      (bind _outprimaryassetidlist (`KismetSystemLibrary.GetPrimaryAssetIdList` "PDA_RoomIndicatorDisplayInfo_C"))
      (`self.LoadAssetList` _outprimaryassetidlist))))

(fn `SearchRooms`
  (locals (rooms :type "Set of Actor Object Reference"))
  (bind _rooms (`local.rooms`))
  (bind _outrooms (`self.TraceCone` 5 60.0 2000.0))
  (set `local.rooms` _outrooms)
  (`self.ValidateLostRooms` _rooms)
  (`self.ValidateFoundRooms` _rooms)
  (bind _output_get (set `self._detectedRooms` (`local.rooms`)))
  (bind _valuepin (`|SetForEach` _output_get)
    (:`then`
      (`KismetSystemLibrary.DrawDebugString` (`self.K2_GetActorLocation` _valuepin) "FOUND!" null (struct :`R` 0.085672 :`G` 1.0 :`B` 0.213759 :`A` 1.0) 1.0))))

(fn `TraceCone`
  (params (InSegments :type Integer) (InAngle :type "Float (double-precision)") (InTraceDistance :type "Float (double-precision)"))
  (returns (OutRooms :type "Set of Actor Object Reference"))
  (locals (traceCount :type Integer :default 0) (anglePerSegment :type "Float (double-precision)") (traceDistance :type "Float (double-precision)" :default 0.0) (traceAngle :type "Float (double-precision)") (foundRooms :type "Set of Actor Object Reference"))
  (bind _traceangle (`local.traceAngle`))
  (bind _returnvalue (`SceneComponent.K2_GetComponentLocation` (`self._camera`)))
  (bind _x (.x (`SceneComponent.GetForwardVector` (`self._camera`))))
  (bind _y (.y (`SceneComponent.GetForwardVector` (`self._camera`))))
  (set `local.traceCount` (+ (`KismetMathLibrary.Clamp` InSegments 1 10) 1))
  (set `local.anglePerSegment` (/ (`KismetMathLibrary.FClamp` (`KismetMathLibrary.Abs` (`local.InAngle`)) 0.0 360.0) (`local.InSegments`)))
  (set `local.traceDistance` (`KismetMathLibrary.FClamp` (`KismetMathLibrary.Abs` (`local.InTraceDistance`)) 1.0 9999.0))
  (set `local.traceAngle` (* (`KismetMathLibrary.FClamp` (`KismetMathLibrary.Abs` (`local.InAngle`)) 0.0 360.0) 0.5 -1.0)) ; starting angle
  (for _index (range (`local.traceCount`))
    (set `local.traceAngle` (+ (* (`local.anglePerSegment`) (`KismetMathLibrary.SignOfInteger` _index)) (`local.traceAngle`)))
    (bind (_outhits _returnvalue_2) (`KismetSystemLibrary.SphereTraceMulti` _returnvalue (+ _returnvalue (* (`KismetMathLibrary.MakeVector` (- (* _x (`KismetMathLibrary.DegCos` _traceangle)) (* _y (`KismetMathLibrary.DegSin` _traceangle))) (+ (* _x (`KismetMathLibrary.DegSin` _traceangle)) (* _y (`KismetMathLibrary.DegCos` _traceangle))) (.z (`SceneComponent.GetForwardVector` (`self._camera`)))) (`local.traceDistance`))) 100.0 "TraceTypeQuery4" false (`self._enteredRooms`) "None" true (struct :`R` 1.0 :`A` 1.0) (struct :`G` 1.0 :`A` 1.0) 0.1))
    (if _returnvalue_2
      (for _array_element _outhits
        (bind (_bblockinghit _binitialoverlap _time _distance _location _impactpoint _normal _impactnormal _physmat _hitactor _hitcomponent) (`GameplayStatics.BreakHitResult` _array_element))
        (if (`KismetArrayLibrary.Array_Contains` (`ActorComponent.ComponentTags` _hitcomponent) "room_main")
          (`BlueprintSetLibrary.Set_Add` (`local.foundRooms`) _hitactor)))))
  (return (`local.foundRooms`)))

(fn `UserConstructionScript`)