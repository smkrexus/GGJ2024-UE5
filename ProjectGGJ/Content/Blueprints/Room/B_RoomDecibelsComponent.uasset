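; Room component that registers noise (decibels) and tracks the room's immunity to it.
; Actors add or remove thresholds in a map; the active threshold rises to the highest, broadcasts changes, and resets to -1 only when the map empties.
; Positive amounts are forwarded to the GameState's GameDecibels, even when impact falls within immunity, which only marks the returned result as failed.
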(fn `AddImmunityThreshold`
  (params (InActor :type "Actor Object Reference") (InThreshold :type Integer))
  (`BlueprintMapLibrary.Map_Add` (`self._immunityMap`) InActor InThreshold)
  (`self.FindMaxThreshold`))

(fn `FindMaxThreshold`
  (if (`BlueprintMapLibrary.Map_IsEmpty` (`self._immunityMap`))
    (bind _output_get (set `self._immunityThreshold` -1))
    (`self.OnImmunityThresholdChanged` _output_get)
    (else
      (bind _values (`BlueprintMapLibrary.Map_Values` (`self._immunityMap`)))
      (for _array_element _values
        (if (> _array_element (`self._immunityThreshold`))
          (bind _output_get_2 (set `self._immunityThreshold` _array_element))
          (`self.OnImmunityThresholdChanged` _output_get_2))))))

(fn `GetImmunityThreshold`
  (returns (OutThreshold :type Integer))
  (return (`self._immunityThreshold`)))

(fn `RegisterDecibels`
  (params (InAmount :type Integer) (InImpact :type Integer))
  (returns (bSuccess :type Boolean))
  (locals (bRegisterSuccess :type Boolean :default true))
  (`|ExecutionSequence`
    (:`then_0`
      (if (<= (`local.InAmount`) 0)
        (return false)))
    (:`then_1`
      (if (and (>= (`KismetMathLibrary.SignOfInteger` (`self._immunityThreshold`)) 0) (<= (`local.InImpact`) (`self._immunityThreshold`)))
        (set `local.bRegisterSuccess` false)))
    (:`then_2`
      (`/Game/Blueprints/Gameflow/Components/B_GameDecibels.AddDecibels` (`/Game/Blueprints/Gameflow/GS_GameStateCustom.GameDecibels` (`/Game/Blueprints/Core/Utilities/BP_Utils.Game State`)) (`local.InAmount`) (`local.InImpact`))
      (return (`local.bRegisterSuccess`)))))

(fn `RemoveImmunityThreshold`
  (params (InActor :type "Actor Object Reference (by ref)"))
  (`BlueprintMapLibrary.Map_Remove` (`self._immunityMap`) InActor)
  (`self.FindMaxThreshold`))