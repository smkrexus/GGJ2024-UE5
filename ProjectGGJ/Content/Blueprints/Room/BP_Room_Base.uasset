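; Base room actor that tracks actors inside it, raises player enter/exit events and drives the room's dynamic indicators.
; Indicator definitions compete by priority, with a random pick among the highest becoming the displayed handle.
; While the manager reports the room detected, a timer loop finds indicators inside the detector camera's view cone and facing it, using dot products.
; A cooldown timer throttles display updates, which show a shuffled, capped subset and hide the rest.
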(event `EnterRoom`
  ; Player Enter / Exit events
  (`self.OnEnter` self))

(event `ExitRoom`
  ; Player Enter / Exit events
  (`self.OnExit` self))

(event `self.ReceiveActorBeginOverlap`
  (params (OtherActor :type "Actor Object Reference"))
  (bind _bsuccess (`self.AddRoomItem` OtherActor))
  (if _bsuccess
    (bind _ascharacter (cast `Character` OtherActor))
    (if (`Pawn.IsPlayerControlled` _ascharacter)
      (`self.EnterRoom`)
      (add `Pawn.ReceiveControllerChangedDelegate` _ascharacter (`|CreateDelegate` :!event `PawnControllerChanged`)))))

(event `self.ReceiveActorEndOverlap`
  (params (OtherActor :type "Actor Object Reference"))
  (bind _bremoved (`self.RemoveRoomItem` OtherActor))
  (if _bremoved
    (bind _ascharacter (cast `Character` OtherActor))
    (if (`Pawn.IsPlayerControlled` _ascharacter)
      (`self.ExitRoom`)
      (remove `Pawn.ReceiveControllerChangedDelegate` _ascharacter (`|CreateDelegate` :!event `PawnControllerChanged`)))))

(event `OnRequestDisplayIndicatorAvailable`
  (`KismetSystemLibrary.K2_ClearAndInvalidateTimerHandle` (`self._indicatorRequestTimer`)))

(event `ResetIndicators`
  (bind _valuepin (`|SetForEach` (`self._indicators`))
    (:`then`
      (`/Game/Blueprints/Room/Indicator/BP_Room_DynamicIndicator_Base.Hide` _valuepin))))

(event `PawnControllerChanged`
  (params (Pawn :type "Pawn Object Reference") (OldController :type "Controller Object Reference") (NewController :type "Controller Object Reference"))
  (remove `Pawn.ReceiveControllerChangedDelegate` Pawn (`|CreateDelegate` :!event `PawnControllerChanged`))
  (`self.ExitRoom`))

(event `RequestNewIndicatorDisplay`
  (params (InDefinition :type "/Game/Blueprints/Room/Indicator/B_RoomIndicatorItem Object Reference"))
  (bind _outvalid (`/Game/Blueprints/Room/Indicator/B_RoomIndicatorItem.IsEqual` InDefinition (`self._indicatorDisplayHandle`)))
  (if (not _outvalid)
    (set `self._indicatorDisplayHandle` (`/Game/Blueprints/Room/Indicator/B_RoomIndicatorItem.GetHandle` InDefinition))
    (`self.OnIndicatorDefinitionChanged` (`self._indicatorDisplayHandle`))))

(event `RequestEmptyIndicatorDisplay`
  (set `self._indicatorDisplayHandle` (make `/Game/Blueprints/Room/Indicator/STR_RoomIndicatorHandle` "NewEnumerator0"))
  (`self.ResetIndicators`)
  (`KismetSystemLibrary.K2_ClearAndInvalidateTimerHandle` (`self._indicatorRequestTimer`))
  (`self.OnIndicatorDefinitionRemoved`))

(event `ValidateDetectionStart`
  (params (DetectedRooms :type "Set of Actor Object Reference"))
  (`self.SHOULD_APPLY_TO_SELF` DetectedRooms)
  (set `self._detectorView` (`/Game/Blueprints/Room/BP_RoomManager.GetDetectorCamera` (`self.GetManager`))) ; camera can change without changing detection
  (if (not (`self.bIsDetected`))
    (set `self.bIsDetected` true)
    (`self.TickIndicator`)
    (add `/Game/Blueprints/Room/BP_RoomManager.OnAssetLoaded` (`self.GetManager`) (`|CreateDelegate` :!event `BroadcastAssetLoaded`))))

(event `ValidateDetectionEnd`
  (params (InActor :type "Set of Actor Object Reference"))
  (`self.SHOULD_APPLY_TO_SELF` InActor)
  (set `self.bIsDetected` false)
  (`self.ResetIndicators`)
  (bind _valuepin (`|SetForEach` (`self._indicators`))
    (:`then`
      (`/Game/Blueprints/Room/Indicator/BP_Room_DynamicIndicator_Base.ClearReadyState` _valuepin))
    (:`CompletedPin`
      (`KismetSystemLibrary.DrawDebugString` (`self.K2_GetActorLocation`) "LOST!" null (struct :`R` 1.0 :`G` 0.025159 :`B` 0.089669 :`A` 1.0) 1.0))))

(event `BroadcastAssetLoaded`
  (remove `/Game/Blueprints/Room/BP_RoomManager.OnAssetLoaded` (`self._manager`) (`|CreateDelegate` :!event `BroadcastAssetLoaded`))
  (`self.OnIndicatorAssetReady`))

(event `TickIndicator`
  (bind __detectorview (`self._detectorView`))
  (`/Engine/EditorBlueprintResources/StandardMacros.IsValid` (`self._detectorView`)
    (:`Is Valid`
      (if (`self.bIsDetected`)
        (bind _outindicators (`self.FindValidIndicators` (`SceneComponent.K2_GetComponentLocation` __detectorview) (`SceneComponent.GetForwardVector` __detectorview)))
        ; Valid after every 2s
        (`self.RequestDisplayIndicators` _outindicators)
        ; Process next tick after 1s, invalidated if detection is false
        (`KismetSystemLibrary.K2_SetTimerDelegate` (`|CreateDelegate` :!event `TickIndicator`) 1.0 false true)))
    (:`Is Not Valid`
      (`KismetSystemLibrary.PrintText` "DetectorView Invalid: Skip Display Indicator" true true (struct :`R` 1.0 :`B` 0.052689 :`A` 1.0)))))

(fn `AddIndicatorDefinition`
  (params (InItem :type "/Game/Blueprints/Room/Indicator/B_RoomIndicatorItem Object Reference (by ref)"))
  (`KismetArrayLibrary.Array_Add` (`self._indicatorDefinitions`) InItem)
  (`|ExecutionSequence`
    (:`then_0`
      (if (< (`.priority_5_7F1972D845DFBC8CC87C159501229E95` (break `/Game/Blueprints/Room/Indicator/STR_RoomIndicatorHandle` (`/Game/Blueprints/Room/Indicator/B_RoomIndicatorItem.GetHandle` (`local.InItem`)))) (`.priority_5_7F1972D845DFBC8CC87C159501229E95` (break `/Game/Blueprints/Room/Indicator/STR_RoomIndicatorHandle` (`self._indicatorDisplayHandle`))))
        (return)))
    (:`then_1`
      (if (> (`.priority_5_7F1972D845DFBC8CC87C159501229E95` (break `/Game/Blueprints/Room/Indicator/STR_RoomIndicatorHandle` (`/Game/Blueprints/Room/Indicator/B_RoomIndicatorItem.GetHandle` (`local.InItem`)))) (`.priority_5_7F1972D845DFBC8CC87C159501229E95` (break `/Game/Blueprints/Room/Indicator/STR_RoomIndicatorHandle` (`self._indicatorDisplayHandle`))))
        (set `self.bShouldDisplayIndicators` true)
        (`self.RequestNewIndicatorDisplay` (`local.InItem`))
        (return)))
    (:`then_2`
      (bind (_outdefintion _outsuccess) (`self.FindValidIndicatorDisplay`))
      (bind _output_get (set `self.bShouldDisplayIndicators` _outsuccess))
      (if _output_get
        (`self.RequestNewIndicatorDisplay` _outdefintion)))))

(fn `AddRoomItem`
  (params (InActor :type "Actor Object Reference") (Identifier :type Name))
  (returns (bSuccess :type Boolean))
  (`|ExecutionSequence`
    (:`then_0`
      (if (`BlueprintSetLibrary.Set_Contains` (`self._allActors`) (`local.InActor`))
        (return false)))
    (:`then_1`
      (`BlueprintSetLibrary.Set_Add` (`self._allActors`) (`local.InActor`))
      (message `/Game/Blueprints/Room/BPI_RoomItemSystem.AddRoom` (`local.InActor`) self))
    (:`then_2`
      ; Convert this to map later on once have more identifiers
      ; Each identifier will be mapped to a list / set of actors to be easily retrieved
      (if (== (`local.Identifier`) "Indicator")
        (`BlueprintSetLibrary.Set_Add` (`self._indicators`) (cast `/Game/Blueprints/Room/Indicator/BP_Room_DynamicIndicator_Base` (`local.InActor`) :!pure true))))
    (:`then_3`
      (return true))))

(fn `FindValidIndicatorDisplay`
  (returns (OutDefintion :type "/Game/Blueprints/Room/Indicator/B_RoomIndicatorItem Object Reference") (OutSuccess :type Boolean))
  (locals (highestPriority :type Integer :default -1) (validDefinitions :type "Array of /Game/Blueprints/Room/Indicator/B_RoomIndicatorItem Object Reference"))
  (`|ExecutionSequence`
    (:`then_0`
      (if (not (`self.HasIndicatorsToDisplay`))
        (return null false)))
    (:`then_1`
      (for _array_element (`self._indicatorDefinitions`)
        (bind ((`priority_5_7F1972D845DFBC8CC87C159501229E95` _priority)) (break `/Game/Blueprints/Room/Indicator/STR_RoomIndicatorHandle` (`/Game/Blueprints/Room/Indicator/B_RoomIndicatorItem.GetHandle` _array_element)))
        (if (< (`local.highestPriority`) _priority)
          (set `local.highestPriority` _priority))))
    (:`then_2`
      (for _array_element_2 (`self._indicatorDefinitions`)
        (bind _outvalid (`/Game/Blueprints/Room/Indicator/B_RoomIndicatorItem.ValidatePriority` _array_element_2 (`local.highestPriority`)))
        (if _outvalid
          (`KismetArrayLibrary.Array_Add` (`local.validDefinitions`) _array_element_2))))
    (:`then_3`
      (if (`KismetArrayLibrary.Array_IsEmpty` (`local.validDefinitions`))
        (return null false)
        (else
          (return (`KismetArrayLibrary.Array_Random` (`local.validDefinitions`)) true))))))

(fn `FindValidIndicators`
  (params (InOrigin :type "Vector Structure") (InForward :type "Vector Structure"))
  (returns (OutIndicators :type "Set of /Game/Blueprints/Room/Indicator/BP_Room_DynamicIndicator_Base Object Reference") (OutInvalid :type "Set of /Game/Blueprints/Room/Indicator/BP_Room_DynamicIndicator_Base Object Reference"))
  (locals (validIndicators :type "Set of /Game/Blueprints/Room/Indicator/BP_Room_DynamicIndicator_Base Object Reference") (invalidIndicators :type "Set of /Game/Blueprints/Room/Indicator/BP_Room_DynamicIndicator_Base Object Reference") (current :type "/Game/Blueprints/Room/Indicator/BP_Room_DynamicIndicator_Base Object Reference") (referenceDirection :type "Vector Structure"))
  (`|ExecutionSequence`
    (:`then_0`
      (if (`BlueprintSetLibrary.Set_IsEmpty` (`self._indicators`))
        (return)))
    (:`then_1`
      (if (not (`self.bShouldDisplayIndicators`))
        (return _ (`self._indicators`))))
    (:`then_2`
      (bind _valuepin (`|SetForEach` (`self._indicators`))
        (:`then`
          (set `local.current` _valuepin)
          (set `local.referenceDirection` (`KismetMathLibrary.Normal` (- (`/Game/Blueprints/Room/Indicator/BP_Room_DynamicIndicator_Base.GetReferenceLocation` (`local.current`)) (`local.InOrigin`))))
          (if (and (> (`KismetMathLibrary.Dot_VectorVector` (`local.referenceDirection`) (`KismetMathLibrary.Normal` (`local.InForward`))) 0.85) (>= (`KismetMathLibrary.Dot_VectorVector` (`self.GetActorForwardVector` (`local.current`)) (* (`local.referenceDirection`) -1)) -0.05))
            (`BlueprintSetLibrary.Set_Add` (`local.validIndicators`) (`local.current`))
            (else
              (`BlueprintSetLibrary.Set_Add` (`local.invalidIndicators`) (`local.current`)))))
        (:`CompletedPin`
          (return (`local.validIndicators`) (`local.invalidIndicators`)))))))

(fn `GetIndicatorDisplay`
  (returns (OutHandle :type "/Game/Blueprints/Room/Indicator/STR_RoomIndicatorHandle Structure"))
  (return (`self._indicatorDisplayHandle`)))

(fn `GetManager`
  (returns (_manager :type "/Game/Blueprints/Room/BP_RoomManager Object Reference"))
  (return (`self._manager`)))

(fn `HasIndicatorsToDisplay`
  (returns (OutValid :type Boolean))
  (`|ExecutionSequence`
    (:`then_0`
      (if (`KismetArrayLibrary.Array_IsEmpty` (`self._indicatorDefinitions`))
        (return false)))
    (:`then_1`
      (for _array_element (`self._indicatorDefinitions`)
        (bind _outvalid (`/Game/Blueprints/Room/Indicator/B_RoomIndicatorItem.ValidatePriority` _array_element 0)) ; at least one 0 or more to be considered valid
        (if _outvalid
          (return true))))
    (:`then_2`
      (return false))))

(fn `Initialize`
  (params (InManager :type "/Game/Blueprints/Room/BP_RoomManager Object Reference"))
  (bind __manager (`self.GetManager`))
  (set `self._manager` InManager)
  (add `self.OnEnter` (`|CreateDelegate` (`self.GetManager`) :!event `MarkEntered`))
  (add `self.OnExit` (`|CreateDelegate` (`self.GetManager`) :!event `ClearEntered`))
  (add `/Game/Blueprints/Room/BP_RoomManager.OnRoomsLost` __manager (`|CreateDelegate` :!event `ValidateDetectionEnd`))
  (add `/Game/Blueprints/Room/BP_RoomManager.OnRoomsFound` __manager (`|CreateDelegate` :!event `ValidateDetectionStart`))
  (set `self.bInitialized` true))

(fn `RemoveIndicatorDefinition`
  (params (InType :type "/Game/Blueprints/Room/Indicator/B_RoomIndicatorItem Object Reference (by ref)"))
  (bind _returnvalue (`KismetArrayLibrary.Array_RemoveItem` (`self._indicatorDefinitions`) InType))
  (if _returnvalue
    (bind (_outdefintion _outsuccess) (`self.FindValidIndicatorDisplay`))
    (bind _output_get (set `self.bShouldDisplayIndicators` _outsuccess))
    (if _output_get
      (`self.RequestNewIndicatorDisplay` _outdefintion)
      (else
        (`self.RequestEmptyIndicatorDisplay`)))))

(fn `RemoveIndicatorDefinitionBatch`
  (params (InTypes :type "Array of /Game/Blueprints/Room/Indicator/B_RoomIndicatorItem Object Reference (by ref)"))
  (`|ExecutionSequence`
    (:`then_0`
      (if (`KismetArrayLibrary.Array_IsEmpty` (`local.InTypes`))
        (return)))
    (:`then_1`
      (for _array_element (`local.InTypes`)
        (bind _returnvalue (`KismetArrayLibrary.Array_RemoveItem` (`self._indicatorDefinitions`) _array_element))
        (if _returnvalue
          _)))
    (:`then_2`
      (bind (_outdefintion _outsuccess) (`self.FindValidIndicatorDisplay`))
      (bind _output_get (set `self.bShouldDisplayIndicators` _outsuccess))
      (if _output_get
        (`self.RequestNewIndicatorDisplay` _outdefintion)
        (else
          (`self.RequestEmptyIndicatorDisplay`))))))

(fn `RemoveRoomItem`
  (params (removeActor :type "Actor Object Reference (by ref)"))
  (returns (bRemoved :type Boolean))
  (bind _returnvalue (`BlueprintSetLibrary.Set_Remove` (`self._allActors`) (`local.removeActor`)))
  (if _returnvalue
    (message `/Game/Blueprints/Room/BPI_RoomItemSystem.RemoveRoom` (`local.removeActor`) self)
    (return true)
    (else
      (return false))))

(fn `RequestDisplayIndicators`
  (params (InRequests :type "Set of /Game/Blueprints/Room/Indicator/BP_Room_DynamicIndicator_Base Object Reference (by ref)"))
  (returns (OutSuccess :type Boolean))
  (`|ExecutionSequence`
    (:`then_0`
      (if (`BlueprintSetLibrary.Set_IsEmpty` (`local.InRequests`))
        (return false)))
    (:`then_1`
      (if (`KismetSystemLibrary.K2_IsValidTimerHandle` (`self._indicatorRequestTimer`))
        (return false)))
    (:`then_2`
      (bind _returnvalue (`KismetSystemLibrary.K2_SetTimerDelegate` (`|CreateDelegate` :!event `OnRequestDisplayIndicatorAvailable`) 2.0))
      (set `self._indicatorRequestTimer` _returnvalue)
      (`self.UpdateIndicatorDisplays` (`local.InRequests`))
      (return true))))

(fn `UpdateIndicatorDisplays`
  (params (InRequests :type "Set of /Game/Blueprints/Room/Indicator/BP_Room_DynamicIndicator_Base Object Reference (by ref)"))
  (locals (selected :type "Array of /Game/Blueprints/Room/Indicator/BP_Room_DynamicIndicator_Base Object Reference") (numRemove :type Integer) (selectedRequests :type "Set of /Game/Blueprints/Room/Indicator/BP_Room_DynamicIndicator_Base Object Reference"))
  (bind _kmaxindicators (`self.kMaxIndicators`))
  (bind _returnvalue (`BlueprintSetLibrary.Set_Length` (`local.InRequests`)))
  (bind _result (`BlueprintSetLibrary.Set_ToArray` InRequests))
  (bind _output_get (set `local.selected` _result))
  (`KismetArrayLibrary.Array_Shuffle` _output_get)
  (`|ExecutionSequence`
    (:`then_0`
      ; Check if exceed indicator count, if so, remove excess
      (if (> _returnvalue _kmaxindicators)
        (bind _output_get_2 (set `local.numRemove` (- _returnvalue _kmaxindicators)))
        (for _ (range _output_get_2)
          (`KismetArrayLibrary.Array_Remove` (`local.selected`)))))
    (:`then_1`
      (`BlueprintSetLibrary.Set_AddItems` (`local.selectedRequests`) (`local.selected`))
      ; Disable then show new ones
      (bind _result_2 (`BlueprintSetLibrary.Set_Difference` (`self._indicators`) (`local.selectedRequests`)))
      (bind _valuepin (`|SetForEach` _result_2)
        (:`then`
          (if (`/Game/Blueprints/Room/Indicator/BP_Room_DynamicIndicator_Base.IsDisplayEnabled` _valuepin)
            (`/Game/Blueprints/Room/Indicator/BP_Room_DynamicIndicator_Base.Hide` _valuepin)))))
    (:`then_2`
      (bind _valuepin_2 (`|SetForEach` (`local.selectedRequests`))
        (:`then`
          (if (not (`/Game/Blueprints/Room/Indicator/BP_Room_DynamicIndicator_Base.IsDisplayEnabled` _valuepin_2))
            (`/Game/Blueprints/Room/Indicator/BP_Room_DynamicIndicator_Base.Display` _valuepin_2)))))))

(fn `UserConstructionScript`)

(fn `ValidateInitialization`
  (returns (OutValidated :type Boolean))
  (return (`self.bInitialized`)))