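; Base actor for a dynamic indicator placed in a room, marking a reference point that can be shown or hidden.
; Its room item component registers the indicator with the room when that room registers.
; The world location comes from a local reference point rotated by the actor's yaw and added to its location.
; Display and Hide toggle ticking, which draws a debug sphere at that location each frame.
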(event `self.ReceiveTick`
  (params (DeltaSeconds :type "Float (single-precision)"))
  (if (`self.bIsDisplayEnabled`)
    (`KismetSystemLibrary.DrawDebugSphere` (`self.GetReferenceLocation`) 25.0 12 (struct :`G` 0.94225 :`B` 1.0 :`A` 1.0) 0.1)))

(event `self.B_RoomItemComponent.OnRegisterRoom`
  (params (RegisteredRoom :type "/Game/Blueprints/Room/BP_Room_Base Object Reference"))
  (`/Game/Blueprints/Room/BP_Room_Base.RegisterIndicator` RegisteredRoom self))

(event `self.B_RoomItemComponent.OnUnregisterRoom`
  (params (UnregisteredRoom :type "/Game/Blueprints/Room/BP_Room_Base Object Reference")))

(fn `Display`
  (set `self.bIsDisplayEnabled` true)
  (`self.SetActorTickEnabled` true))

(fn `GetReferenceLocation`
  (returns (OutLocation :type "Vector Structure"))
  (return (+ (`self.K2_GetActorLocation`) (`KismetMathLibrary.RotateAngleAxis` (`self._referencePoint`) (.yaw (`self.K2_GetActorRotation`)) (`self.GetActorUpVector`)))))

(fn `GetReferencePoint`
  (returns (OutPoint :type "Vector Structure"))
  (return (`self._referencePoint`)))

(fn `GetRoom`
  (returns (OutRoom :type "/Game/Blueprints/Room/BP_Room_Base Object Reference"))
  (return (`/Game/Blueprints/Room/B_RoomItemComponent.GetRoom` (`self.B_RoomItemComponent`))))

(fn `Hide`
  (set `self.bIsDisplayEnabled` false)
  (`self.SetActorTickEnabled` false))

(fn `IsDisplayEnabled`
  (returns (OutValid :type Boolean))
  (return (`self.bIsDisplayEnabled`)))

(fn `UserConstructionScript`)