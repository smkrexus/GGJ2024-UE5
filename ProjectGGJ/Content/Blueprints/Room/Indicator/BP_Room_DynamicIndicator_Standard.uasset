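; Standard room indicator actor that shows or hides a tracked interactable-locator widget and registers rooms with its room item component.
; The construction script centres a box toward the reference point's XY midpoint, sizes its X extent from that half-distance, and places the locator at the point plus an offset.
; Display and Hide overrides toggle locator tracking, whose enabled and disabled events drive the view model's visibility flag.
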(event `/Game/Blueprints/Room/BPI_RoomItemSystem.AddRoom`
  (params (InRoom :type "/Game/Blueprints/Room/BP_Room_Base Object Reference"))
  (`/Game/Blueprints/Room/B_RoomItemComponent.RegisterRoom` (`self.B_RoomItemComponent`) InRoom))

(event `self.B_SceneTracker_InteractableLocator.OnTrackingEnabled`
  (bind _viewmodel (`/Game/Blueprints/Interactables/Locator/B_SceneTracker_InteractableLocator.GetViewModel` (`self.B_SceneTracker_InteractableLocator`)))
  (`/Engine/EditorBlueprintResources/StandardMacros.IsValid` _viewmodel
    (:`Is Valid`
      (`/Game/Blueprints/Interactables/Locator/ViewModel/B_VM_InteractableLocator.VM_SetShouldDisplayLocator` _viewmodel true))))

(event `self.B_SceneTracker_InteractableLocator.OnTrackingDisabled`
  (bind _viewmodel (`/Game/Blueprints/Interactables/Locator/B_SceneTracker_InteractableLocator.GetViewModel` (`self.B_SceneTracker_InteractableLocator`)))
  (`/Engine/EditorBlueprintResources/StandardMacros.IsValid` _viewmodel
    (:`Is Valid`
      (`/Game/Blueprints/Interactables/Locator/ViewModel/B_VM_InteractableLocator.VM_SetShouldDisplayLocator` _viewmodel false))))

(fn `Display`
  (`parent.Display`)
  (`/Game/Blueprints/Interactables/Locator/B_SceneTracker_InteractableLocator.SetWidgetTrackingEnabled` (`self.B_SceneTracker_InteractableLocator`) null))

(fn `Hide`
  (`parent.Hide`)
  (`/ActorTracker/Blueprints/B_SceneTracker_Base.SetTrackingEnabled` (`self.B_SceneTracker_InteractableLocator`) false))

(fn `UserConstructionScript`
  (bind _box (`self.Box`))
  (bind _returnvalue (* (`self.GetReferencePoint`) 0.5))
  (`parent.UserConstructionScript`)
  (`SceneComponent.K2_SetRelativeLocation` _box (`KismetMathLibrary.MakeVector` (.x _returnvalue) (.y _returnvalue)) false false)
  (`BoxComponent.SetBoxExtent` _box (`KismetMathLibrary.MakeVector` (+ (`KismetMathLibrary.VSizeXY` _returnvalue) (`self._extentModification`)) (.y (`BoxComponent.BoxExtent` (`self.Box`))) (.z (`BoxComponent.BoxExtent` (`self.Box`)))) true)
  (set `self._indicatorLocation` (+ (`self.GetReferencePoint`) (`self._indicatorOffset`)))
  (`SceneComponent.K2_SetRelativeLocation` (`self.B_SceneTracker_InteractableLocator`) (`self._indicatorLocation`) false false))