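; Actor component that tracks which room its owning item is in.
; One tick after BeginPlay it hands the owner to the first overlapping BP_Room_Base via AddRoomItem.
; RegisterRoom stores the room or switches through ChangeRoom, which clears the previous one before registering the new one.
; Register and unregister each fire a notification call, with optional debug prints.
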(event `self.ReceiveBeginPlay`
  (bind _overlappingactors (`Actor.GetOverlappingActors` (`self.GetOwner`) "/Game/Blueprints/Room/BP_Room_Base.BP_Room_Base_C"))
  (`KismetSystemLibrary.DelayUntilNextTick`)
  (if (`KismetArrayLibrary.Array_IsNotEmpty` _overlappingactors)
    (`/Game/Blueprints/Room/BP_Room_Base.AddRoomItem` (`|GetArrayItem` _overlappingactors) (`self.GetOwner`))))

(fn `ChangeRoom`
  (params (InPreviousRoom :type "/Game/Blueprints/Room/BP_Room_Base Object Reference") (InNewRoom :type "/Game/Blueprints/Room/BP_Room_Base Object Reference"))
  (returns (OutSuccess :type Boolean))
  (`|ExecutionSequence`
    (:`then_0`
      (if (not (and (`KismetSystemLibrary.IsValid` (`local.InPreviousRoom`)) (`KismetSystemLibrary.IsValid` (`local.InNewRoom`))))
        (return false)))
    (:`then_1`
      (if (== (`local.InPreviousRoom`) (`local.InNewRoom`))
        (return false)))
    (:`then_2`
      (`self.ClearRoom` (`local.InPreviousRoom`))
      (`self.RegisterRoom` (`local.InNewRoom`)))
    (:`then_3`
      (return true))))

(fn `ClearRoom`
  (params (InRoom :type "/Game/Blueprints/Room/BP_Room_Base Object Reference"))
  (`/Engine/EditorBlueprintResources/StandardMacros.IsValid` (`self._room`)
    (:`Is Valid`
      (if (== (`local.InRoom`) (`self._room`))
        (`self.DEBUG_UNREGISTER`)
        (set `self._room` null)
        (`self.OnUnregisterRoom` (`local.InRoom`))))))

(fn `GetRoom`
  (returns (OutRoom :type "/Game/Blueprints/Room/BP_Room_Base Object Reference"))
  (return (`self._room`)))

(fn `RegisterRoom`
  (params (InRoom :type "/Game/Blueprints/Room/BP_Room_Base Object Reference"))
  (`/Engine/EditorBlueprintResources/StandardMacros.IsValid` (`self.GetRoom`)
    (:`Is Valid`
      (`self.ChangeRoom` (`self.GetRoom`) (`local.InRoom`)))
    (:`Is Not Valid`
      ; New room detected
      (bind _output_get (set `self._room` (`local.InRoom`)))
      (`self.OnRegisterRoom` _output_get)
      (`self.DEBUG_REGISTER`))))