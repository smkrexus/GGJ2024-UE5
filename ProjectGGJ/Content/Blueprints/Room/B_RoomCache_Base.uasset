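; Base room cache Blueprint that stores a list of objects for an owning room, set through Initialize.
; Add and Remove edit the list and call the OnCacheModified hook, which is empty here along with Refresh.
; Search and SearchInternal return a shuffled copy trimmed to a requested count, with a negative count returning everything, working on the cache or a supplied array respectively.
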(fn `Add`
  (params (InItems :type "Array of Object Object Reference"))
  (if (`KismetArrayLibrary.Array_IsEmpty` InItems)
    (return)
    (else
      (`KismetArrayLibrary.Array_Append` (`self._objects`) (`local.InItems`))
      (`self.OnCacheModified` (`self._objects`)))))

(fn `GetRoom`
  (returns (OutRoom :type "/Game/Blueprints/Room/BP_Room_Base Object Reference"))
  (return (`self._room`)))

(fn `Initialize`
  (params (InRoom :type "/Game/Blueprints/Room/BP_Room_Base Object Reference"))
  (set `self._room` InRoom))

(fn `IsValidCache`
  (returns (OutValid :type Boolean))
  (if (`KismetArrayLibrary.Array_IsEmpty` (`self._objects`))
    (return false)
    (else
      (return true))))

(fn `OnCacheModified`
  (params (InCache :type "Array of Object Object Reference")))

(fn `Refresh`)

(fn `Remove`
  (params (InItems :type "Array of Object Object Reference"))
  (if (`KismetArrayLibrary.Array_IsEmpty` InItems)
    (return)
    (else
      (for _array_element (`local.InItems`)
        (`KismetArrayLibrary.Array_RemoveItem` (`self._objects`) _array_element))
      (`self.OnCacheModified` (`self._objects`)))))

(fn `Search`
  (params (InMax :type Integer))
  (returns (OutItems :type "Array of Object Object Reference"))
  (locals (searchMax :type Integer) (output :type "Array of Object Object Reference") (cache :type "Array of Object Object Reference") (numToRemove :type Integer))
  (bind _inmax (`local.InMax`))
  (`|ExecutionSequence`
    (:`then_0`
      (if (or (`KismetArrayLibrary.Array_IsEmpty` (`self._objects`)) (== _inmax 0))
        (return)
        (else
          (bind _output_get (set `local.output` (`self._objects`)))
          (`KismetArrayLibrary.Array_Shuffle` _output_get))))
    (:`then_1`
      (if (< _inmax 0)
        (return (`local.output`))))
    (:`then_2`
      (bind _output_get_2 (set `local.searchMax` (`KismetMathLibrary.Clamp` (`local.InMax`) 1 (`KismetArrayLibrary.Array_Length` (`self._objects`)))))
      (if (== _output_get_2 (`KismetArrayLibrary.Array_Length` (`self._objects`)))
        (return (`local.output`))))
    (:`then_3`
      (bind _output_get_3 (set `local.numToRemove` (- (`KismetArrayLibrary.Array_Length` (`local.output`)) (`local.searchMax`))))
      (for _ (range _output_get_3)
        (`KismetArrayLibrary.Array_Remove` (`local.output`)))
      (return (`local.output`)))))

(fn `SearchInternal`
  (params (InMax :type Integer) (InItems :type "Array of Object Object Reference"))
  (returns (OutItems :type "Array of Object Object Reference"))
  (locals (searchMax :type Integer :default 0) (cache :type "Array of Object Object Reference") (numToRemove :type Integer))
  (bind _inmax (`local.InMax`))
  (`|ExecutionSequence`
    (:`then_0`
      (if (or (`KismetArrayLibrary.Array_IsEmpty` (`local.InItems`)) (== _inmax 0))
        (return)
        (else
          (bind _output_get (set `local.cache` (`local.InItems`)))
          (`KismetArrayLibrary.Array_Shuffle` _output_get))))
    (:`then_1`
      (if (< _inmax 0)
        (return (`local.cache`))))
    (:`then_2`
      (bind _output_get_2 (set `local.searchMax` (`KismetMathLibrary.Clamp` (`local.InMax`) 1 (`KismetArrayLibrary.Array_Length` (`local.cache`)))))
      (if (== _output_get_2 (`KismetArrayLibrary.Array_Length` (`local.cache`)))
        (return (`local.cache`))))
    (:`then_3`
      (set `local.numToRemove` (- (`KismetArrayLibrary.Array_Length` (`local.cache`)) (`local.searchMax`)))
      (for _ (range (`local.numToRemove`))
        (`KismetArrayLibrary.Array_Remove` (`local.cache`)))
      (return (`local.cache`)))))