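; Patient actor for a chiropractic game, with poseable, manipulable joints, a random health profile, and pain and complaint stats.
; Initialization adds pose options shown when a player is near, spawns data-table-driven joint points on controllable bones, and assigns their profile issues.
; Crack and RotateBone match bone-name substrings to set anim-instance rotators, randomly or from input.
; Anger fills a complaint meter that triggers timed, counted complaints; a view model mirrors these stats.
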(event `self.PatientPoseManager.OnPoseChanged`
  (params (oldPose :type "/Game/Blueprints/Patient/Poses/STR_PatientPoseHandle Structure") (newPose :type "/Game/Blueprints/Patient/Poses/STR_PatientPoseHandle Structure"))
  ;[0.000172 0 0.01042] POSE TESTS
  (`/Game/Skeletal/BPA_Patient.SetPose` (`self.patientAnim`) newPose))

(event `self.SceneTracker_PatientLocator.OnRangeDetected`
  (params (player :type "Pawn Object Reference"))
  (bind _patient_contextcomponent (`self.Patient_ContextComponent`))
  ;[0.000172 0 0.01042] POSE TESTS
  (if (not (`/Game/Blueprints/Core/Contexts/B_ContextComponent.IsContextActive` (`self.Patient_ContextComponent`)))
    (`/Game/Blueprints/Core/Contexts/B_ContextComponent.AddToScreen` _patient_contextcomponent (`Pawn.GetController` player) "contextOptions")
    (`/Game/Blueprints/Core/Contexts/B_ContextComponent.SetContextActive` _patient_contextcomponent true)))

(event `self.SceneTracker_PatientLocator.OnRangeExceeded`
  (params (player :type "Pawn Object Reference") (inMaxRange :type Boolean))
  ;[0.000172 0 0.01042] POSE TESTS
  (if (`/Game/Blueprints/Core/Contexts/B_ContextComponent.IsContextActive` (`self.Patient_ContextComponent`))
    (`/Game/Blueprints/Core/Contexts/B_ContextComponent.SetContextActive` (`self.Patient_ContextComponent`) false)))

(event `self.ReceiveBeginPlay`)

(event `Initialize`
  (`|ExecutionSequence`
    (:`then_0`
      (`|ExecutionSequence`
        (:`then_0`
          (bind _created_stat (`/Game/Blueprints/Gameflow/BP_Utils.Create Stat` "NewEnumerator7" self))
          (bind _output_get (set `self.ComplaintMeter` _created_stat))
          (add `/Game/Blueprints/Gameflow/BP_Stat.OnStatChanged` _output_get (`|CreateDelegate` :!event `VM_UpdateStat_Complaint`)))
        (:`then_1`
          (bind _created_stat_2 (`/Game/Blueprints/Gameflow/BP_Utils.Create Stat` "NewEnumerator6" self))
          (bind _output_get_2 (set `self.Pain` _created_stat_2))
          (add `/Game/Blueprints/Gameflow/BP_Stat.OnStatChanged` _output_get_2 (`|CreateDelegate` :!event `VM_UpdateStat_Pain`)))
        (:`then_2`
          (bind _asbpa_patient (cast `/Game/Skeletal/BPA_Patient` (`SkeletalMeshComponent.GetAnimInstance` (`self.SkeletalMesh`))))
          (set `self.patientAnim` _asbpa_patient)
          ;[0.000172 0 0.01042] POSE TESTS
          (bind _returnvalue (`|GenericCreateObject` "/Game/Blueprints/Patient/Poses/B_ContextItem_PatientPose.B_ContextItem_PatientPose_C"))
          (`/Game/Blueprints/Patient/Poses/B_ContextItem_PatientPose.SetPoseInfo` _returnvalue (`/Game/Blueprints/Patient/Poses/B_PatientPoseManager.GetPoseHandle` (`self.PatientPoseManager`) 0))
          (`/Game/Blueprints/Core/Contexts/B_ContextComponent.AddContext` (`self.Patient_ContextComponent`) "/Game/Blueprints/Patient/Poses/BP_ContextEntry_PatientPose.BP_ContextEntry_PatientPose_C" _returnvalue (`self.PatientPoseManager`))
          (bind _returnvalue_2 (`|GenericCreateObject` "/Game/Blueprints/Patient/Poses/B_ContextItem_PatientPose.B_ContextItem_PatientPose_C"))
          (`/Game/Blueprints/Patient/Poses/B_ContextItem_PatientPose.SetPoseInfo` _returnvalue_2 (`/Game/Blueprints/Patient/Poses/B_PatientPoseManager.GetPoseHandle` (`self.PatientPoseManager`) 1))
          (`/Game/Blueprints/Core/Contexts/B_ContextComponent.AddContext` (`self.Patient_ContextComponent`) "/Game/Blueprints/Patient/Poses/BP_ContextEntry_PatientPose.BP_ContextEntry_PatientPose_C" _returnvalue_2 (`self.PatientPoseManager`)))))
    (:`then_1`
      (for _index (range (`SkinnedMeshComponent.GetNumBones` (`self.SkeletalMesh`)))
        (bind _returnvalue_3 (`SkinnedMeshComponent.GetBoneName` (`self.SkeletalMesh`) _index))
        (if (`/Game/Skeletal/BPA_Patient.HasBoneControl` (`self.patientAnim`) _returnvalue_3)
          (`self.SpawnJointsByName` _returnvalue_3) ; different joint BPs can be spawned this way, child BPs can have their own settings / look\ncan remove the need to set through initialization
        )))
    (:`then_2`
      (bind _returnvalue_4 (`|GenericCreateObject` "/Game/Blueprints/Patient/BP_PatientProfile.BP_PatientProfile_C"))
      (set `self.patientProfile` _returnvalue_4)
      (`|ExecutionSequence`
        (:`then_0`
          (bind _keys (`BlueprintMapLibrary.Map_Keys` (`self.boneDictionary`))))
        (:`then_1`
          (`/Game/Blueprints/Patient/BP_PatientProfile.CreateRandomProfile` (`self.patientProfile`) _keys))
        (:`then_2`
          (for _array_element _keys
            (`|ExecutionSequence`
              (:`then_0`
                (bind _value (`BlueprintMapLibrary.Map_Find` (`self.boneDictionary`) _array_element))
                (`/Game/Blueprints/Interactables/BP_ChiropractorPoint.RegisterJointIssue` _value (`/Game/Blueprints/Patient/BP_PatientProfile.HasJointIssue` (`self.patientProfile`) _array_element "NewEnumerator0")))
              (:`then_1`
                (`/Game/Blueprints/Patient/B_PatientJointManager.AddJoint` (`self.GetManager`) _value)))))
        (:`then_3`
          (bind _healthchart (`self.healthChart`)
            (:`then`
              (`/Game/Blueprints/Interactables/BP_PatientHealthChart.Initialize` _healthchart self))
            (:`else`)))))
    (:`then_3`
      (bind _returnvalue_5 (`|AddComponentByClass` "/Game/Blueprints/Patient/ViewModel/B_VM_Patient.B_VM_Patient_C"))
      (set `self.vm_patient` _returnvalue_5)
      (`self.VM_UpdateStat_Pain`)
      (`self.VM_UpdateStat_Complaint`))))

(event `OnComplaintTimerEnd`
  (`KismetSystemLibrary.K2_ClearAndInvalidateTimerHandle` (`self.complaintTimer`))
  (`/Game/Blueprints/Gameflow/BP_Stat.Reset` (`self.ComplaintMeter`))
  (`self.VM_ClearComplaintTimer`))

(event `self.ReceiveTick`
  (params (DeltaSeconds :type "Float (single-precision)"))
  (if (`KismetSystemLibrary.K2_IsValidTimerHandle` (`self.complaintTimer`))
    (`self.VM_UpdateComplaintTimer`)))

(event `VM_UpdateStat_Pain`
  (`/Game/Blueprints/Patient/ViewModel/B_VM_Patient.VM_SetPain` (`self.vm_patient`) (`self.Pain`)))

(event `VM_UpdateStat_Complaint`
  (`/Game/Blueprints/Patient/ViewModel/B_VM_Patient.VM_SetComplaint` (`self.vm_patient`) (`self.ComplaintMeter`)))

(event `VM_UpdateComplaintMode`
  (`/Game/Blueprints/Patient/ViewModel/B_VM_Patient.VM_SetComplaintMode` (`self.vm_patient`) (`KismetSystemLibrary.K2_IsValidTimerHandle` (`self.complaintTimer`))))

(event `VM_UpdateComplaintCount`
  (`/Game/Blueprints/Patient/ViewModel/B_VM_Patient.VM_SetComplaintCount` (`self.vm_patient`) (`self.complaints`)))

(event `VM_UpdateComplaintTimer`
  (`/Game/Blueprints/Patient/ViewModel/B_VM_Patient.VM_SetComplaintTimer` (`self.vm_patient`) (`KismetSystemLibrary.K2_GetTimerElapsedTimeHandle` (`self.complaintTimer`)) (`self.max`)))

(event `VM_ClearComplaintTimer`
  (`/Game/Blueprints/Patient/ViewModel/B_VM_Patient.VM_SetComplaintTimer` (`self.vm_patient`) 0.0 (`self.max`))
  (`self.VM_UpdateComplaintMode`))

(fn `Crack`
  (params (bone :type Name))
  (returns (rotation :type "Rotator Structure"))
  (bind _returnvalue (`KismetMathLibrary.RandomFloatInRange` -10.0 10.0))
  (bind _returnvalue_2 (`KismetMathLibrary.RandomFloatInRange` -20.0 20.0))
  (bind _returnvalue_3 (`KismetMathLibrary.RandomFloatInRange` -5.0 5.0))
  (bind _patientanim (`self.patientAnim`))
  (bind _patientanim_2 (`self.patientAnim`))
  (bind _patientanim_3 (`self.patientAnim`))
  (bind _patientanim_4 (`self.patientAnim`))
  (bind _patientanim_5 (`self.patientAnim`))
  (bind _patientanim_6 (`self.patientAnim`))
  (bind _returnvalue_4 (`KismetMathLibrary.MakeRotator` _returnvalue _returnvalue _returnvalue))
  (`|ExecutionSequence`
    (:`then_0`
      (if (`KismetStringLibrary.Contains` (`KismetStringLibrary.Conv_NameToString` (`local.bone`)) "spine")
        (bind _output_get (set `/Game/Skeletal/BPA_Patient.spine` (`KismetMathLibrary.MakeRotator` _returnvalue_3 _returnvalue_3) (`self.patientAnim`)))
        (return _output_get)))
    (:`then_1`
      (if (`KismetStringLibrary.Contains` (`KismetStringLibrary.Conv_NameToString` (`local.bone`)) "upperarm")
        (if (`KismetStringLibrary.Contains` (`KismetStringLibrary.Conv_NameToString` (`local.bone`)) "_l")
          (bind _output_get_2 (set `/Game/Skeletal/BPA_Patient.arm_l` _returnvalue_4 _patientanim_2))
          (return _output_get_2)
          (else
            (bind _output_get_3 (set `/Game/Skeletal/BPA_Patient.arm_r` _returnvalue_4 _patientanim_2))
            (return _output_get_3)))))
    (:`then_2`
      (if (`KismetStringLibrary.Contains` (`KismetStringLibrary.Conv_NameToString` (`local.bone`)) "hand")
        (if (`KismetStringLibrary.Contains` (`KismetStringLibrary.Conv_NameToString` (`local.bone`)) "_l")
          (bind _output_get_4 (set `/Game/Skeletal/BPA_Patient.wrist_l` _returnvalue_4 _patientanim_3))
          (return _output_get_4)
          (else
            (bind _output_get_5 (set `/Game/Skeletal/BPA_Patient.wrist_r` _returnvalue_4 _patientanim_3))
            (return _output_get_5)))))
    (:`then_3`
      (if (`KismetStringLibrary.Contains` (`KismetStringLibrary.Conv_NameToString` (`local.bone`)) "thigh")
        (if (`KismetStringLibrary.Contains` (`KismetStringLibrary.Conv_NameToString` (`local.bone`)) "_l")
          (bind _output_get_6 (set `/Game/Skeletal/BPA_Patient.leg_l` _returnvalue_4 _patientanim_4))
          (return _output_get_6)
          (else
            (bind _output_get_7 (set `/Game/Skeletal/BPA_Patient.leg_r` _returnvalue_4 _patientanim_4))
            (return _output_get_7)))))
    (:`then_4`
      (if (`KismetStringLibrary.Contains` (`KismetStringLibrary.Conv_NameToString` (`local.bone`)) "calf")
        (if (`KismetStringLibrary.Contains` (`KismetStringLibrary.Conv_NameToString` (`local.bone`)) "_l")
          (bind _output_get_8 (set `/Game/Skeletal/BPA_Patient.knee_l` _returnvalue_4 _patientanim_5))
          (return _output_get_8)
          (else
            (bind _output_get_9 (set `/Game/Skeletal/BPA_Patient.knee_r` _returnvalue_4 _patientanim_5))
            (return _output_get_9)))))
    (:`then_5`
      (if (`KismetStringLibrary.Contains` (`KismetStringLibrary.Conv_NameToString` (`local.bone`)) "foot")
        (if (`KismetStringLibrary.Contains` (`KismetStringLibrary.Conv_NameToString` (`local.bone`)) "_l")
          (bind _output_get_10 (set `/Game/Skeletal/BPA_Patient.foot_l` _returnvalue_4 _patientanim_6))
          (return _output_get_10)
          (else
            (bind _output_get_11 (set `/Game/Skeletal/BPA_Patient.foot_r` _returnvalue_4 _patientanim_6))
            (return _output_get_11)))))
    (:`then_6`
      (if (`KismetStringLibrary.Contains` (`KismetStringLibrary.Conv_NameToString` (`local.bone`)) "lowerarm")
        (if (`KismetStringLibrary.Contains` (`KismetStringLibrary.Conv_NameToString` (`local.bone`)) "_l")
          (bind _output_get_12 (set `/Game/Skeletal/BPA_Patient.elbow_l` _returnvalue_4 _patientanim))
          (return _output_get_12)
          (else
            (bind _output_get_13 (set `/Game/Skeletal/BPA_Patient.elbow_r` _returnvalue_4 _patientanim))
            (return _output_get_13)))))
    (:`then_7`
      (if (`KismetStringLibrary.Contains` (`KismetStringLibrary.Conv_NameToString` (`local.bone`)) "head")
        (bind _output_get_14 (set `/Game/Skeletal/BPA_Patient.head` (`KismetMathLibrary.MakeRotator` _returnvalue_2 _returnvalue_2) (`self.patientAnim`)))
        (return _output_get_14)))))

(fn `GetBonePosition`
  (params (boneName :type Name))
  (returns (position :type "Vector Structure"))
  (bind _returnvalue_location (`KismetMathLibrary.BreakTransform` (`SkinnedMeshComponent.GetBoneTransform` (`self.SkeletalMesh`) boneName "RTS_World")))
  (return _returnvalue_location))

(fn `GetJointLimit`
  (params (boneName :type Name))
  (returns (limits :type "/Game/Blueprints/Patient/STR_RotateBoneLimits Structure"))
  (return (make `/Game/Blueprints/Patient/STR_RotateBoneLimits` boneName (-30.0 30.0) (-30.0 30.0))))

(fn `GetManager`
  (returns (manager :type "/Game/Blueprints/Patient/B_PatientJointManager Object Reference"))
  (return (`self.PatientJointManager`)))

(fn `GetPatientProfile`
  (returns (patientProfile :type "/Game/Blueprints/Patient/BP_PatientProfile Object Reference"))
  (return (`self.patientProfile`)))

(fn `IncreaseAnger`
  (if (`KismetSystemLibrary.K2_IsValidTimerHandle` (`self.complaintTimer`))
    (`|ExecutionSequence` :!label _label
      (:`then_0`
        (bind _returnvalue (`KismetSystemLibrary.K2_SetTimerDelegate` (`|CreateDelegate` :!event `OnComplaintTimerEnd`) (`self.max`)))
        (set `self.complaintTimer` _returnvalue)
        (set `self.complaints` (+ (`self.complaints`) 1)))
      (:`then_1`
        (`self.VM_UpdateComplaintMode`)
        (`self.VM_UpdateComplaintCount`)))
    (else
      (bind _new_value (`/Game/Blueprints/Gameflow/BP_Stat.Change` (`self.ComplaintMeter`) 1.0))
      (bind _returnvalue_2 (`|GetDataTableRow` "/Game/Blueprints/Gameflow/DT_StatDefs.DT_StatDefs" "ComplaintThreshold")
        (:`then`
          (if (== (`.Max_13_8A895D624DE880DAA7CAD194D3205837` (break `/Game/Blueprints/Gameflow/BP_StatDef` _returnvalue_2)) _new_value)
            (goto _label)))))))

(fn `RotateBone`
  (params (input :type "Vector2D Structure") (boneName :type Name))
  (returns (rotation :type "Rotator Structure"))
  (bind _patientanim (`self.patientAnim`))
  (bind _patientanim_2 (`self.patientAnim`))
  (bind _patientanim_3 (`self.patientAnim`))
  (bind _patientanim_4 (`self.patientAnim`))
  (bind _patientanim_5 (`self.patientAnim`))
  (bind _patientanim_6 (`self.patientAnim`))
  (bind _spine (`/Game/Skeletal/BPA_Patient.spine` (`self.patientAnim`)))
  (bind _head (`/Game/Skeletal/BPA_Patient.head` (`self.patientAnim`)))
  (bind _arm_l (`/Game/Skeletal/BPA_Patient.arm_l` _patientanim))
  (bind _arm_r (`/Game/Skeletal/BPA_Patient.arm_r` _patientanim))
  (bind _elbow_r (`/Game/Skeletal/BPA_Patient.elbow_r` _patientanim_6))
  (bind _elbow_l (`/Game/Skeletal/BPA_Patient.elbow_l` _patientanim_6))
  (bind _wrist_l (`/Game/Skeletal/BPA_Patient.wrist_l` _patientanim_2))
  (bind _wrist_r (`/Game/Skeletal/BPA_Patient.wrist_r` _patientanim_2))
  (bind _leg_l (`/Game/Skeletal/BPA_Patient.leg_l` _patientanim_3))
  (bind _leg_r (`/Game/Skeletal/BPA_Patient.leg_r` _patientanim_3))
  (bind _knee_l (`/Game/Skeletal/BPA_Patient.knee_l` _patientanim_4))
  (bind _knee_r (`/Game/Skeletal/BPA_Patient.knee_r` _patientanim_4))
  (bind _foot_l (`/Game/Skeletal/BPA_Patient.foot_l` _patientanim_5))
  (bind _foot_r (`/Game/Skeletal/BPA_Patient.foot_r` _patientanim_5))
  (`|ExecutionSequence`
    (:`then_0`
      (`self.FindBone` (`local.boneName`) "head")
      (`self.SetBoneRotation` (`local.input`) _head)
      (return _head))
    (:`then_1`
      (`self.FindBone` (`local.boneName`) "spine")
      (`self.SetBoneRotation` (`local.input`) _spine)
      (return _spine))
    (:`then_2`
      (`self.FindBonePerSide` (`local.boneName`) "upperarm"
        (:`left`
          (`self.SetBoneRotationPerSide` (`local.input`) _arm_l _arm_r :!label _label
            (:`OutLeft`
              (return _arm_l))
            (:`OutRIght`
              (return _arm_r))))
        (:`right`
          (goto _label :!via `Right`))))
    (:`then_3`
      (`self.FindBonePerSide` (`local.boneName`) "hand"
        (:`left`
          (`self.SetBoneRotationPerSide` (`local.input`) _wrist_l _wrist_r :!label _label_2
            (:`OutLeft`
              (return _wrist_l))
            (:`OutRIght`
              (return _wrist_r))))
        (:`right`
          (goto _label_2 :!via `Right`))))
    (:`then_4`
      (`self.FindBonePerSide` (`local.boneName`) "thigh"
        (:`left`
          (`self.SetBoneRotationPerSide` (`local.input`) _leg_l _leg_r :!label _label_3
            (:`OutLeft`
              (return _leg_l))
            (:`OutRIght`
              (return _leg_r))))
        (:`right`
          (goto _label_3 :!via `Right`))))
    (:`then_5`
      (`self.FindBonePerSide` (`local.boneName`) "calf"
        (:`left`
          (`self.SetBoneRotationPerSide` (`local.input`) _knee_l _knee_r :!label _label_4
            (:`OutLeft`
              (return _knee_l))
            (:`OutRIght`
              (return _knee_r))))
        (:`right`
          (goto _label_4 :!via `Right`))))
    (:`then_6`
      (`self.FindBonePerSide` (`local.boneName`) "foot"
        (:`left`
          (`self.SetBoneRotationPerSide` (`local.input`) _foot_l _foot_r :!label _label_5
            (:`OutLeft`
              (return _foot_l))
            (:`OutRIght`
              (return _foot_r))))
        (:`right`
          (goto _label_5 :!via `Right`))))
    (:`then_7`
      (`self.FindBonePerSide` (`local.boneName`) "lowerarm"
        (:`left`
          (`self.SetBoneRotationPerSide` (`local.input`) _elbow_l _elbow_r :!label _label_6
            (:`OutLeft`
              (return _elbow_l))
            (:`OutRIght`
              (return _elbow_r))))
        (:`right`
          (goto _label_6 :!via `Right`))))))

(fn `SpawnJointsByName`
  (params (jointName :type Name))
  (locals (spawnedJoint :type "/Game/Blueprints/Interactables/BP_ChiropractorPoint Object Reference"))
  (bind _jointname (`local.jointName`))
  (bind _jointspawndata (`self.jointSpawnData`))
  (bind _outrownames (`DataTableFunctionLibrary.GetDataTableRowNames` _jointspawndata))
  (for _array_element _outrownames
    (bind _returnvalue (`|GetDataTableRow` _jointspawndata _array_element)
      (:`then`
        (bind (_bonename _spawnclass) (break `/Game/Blueprints/Patient/Data/STR_PatientJointSetting` _returnvalue))
        (if (== _bonename (`local.jointName`))
          (bind _returnvalue_2 (`KismetSystemLibrary.LoadClassAsset_Blocking` _spawnclass))
          (bind _returnvalue_3 (`|SpawnActorFromClass` (castclass `/Game/Blueprints/Interactables/BP_ChiropractorPoint` _returnvalue_2 :!pure true) (`SkinnedMeshComponent.GetBoneTransform` (`self.SkeletalMesh`) (`local.jointName`) "RTS_World") "Undefined" "MultiplyWithRoot" null null))
          (bind _output_get (set `local.spawnedJoint` _returnvalue_3))
          (`/Game/Blueprints/Interactables/BP_ChiropractorPoint.SetOwningPatient` _output_get self)
          (break)))))
  (`local.spawnedJoint`
    (:`then`
      (`/Game/Blueprints/Interactables/BP_ChiropractorPoint.DefineJointProperties` (`local.spawnedJoint`) _jointname (`self.GetJointLimit` _jointname))
      (`BlueprintMapLibrary.Map_Add` (`self.boneDictionary`) (`local.jointName`) (`local.spawnedJoint`)))
    (:`else`)))

(fn `UserConstructionScript`)