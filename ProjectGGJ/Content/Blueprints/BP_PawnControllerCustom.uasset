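; BP_PawnControllerCustom is a player controller that relays Enhanced Input to the player's custom pawn.
; BeginPlay sets game-only input, caches the pawn and its BPI_PawnInputHandler interface, and adds the IM_CustomInputMap mapping context.
; Jump, move, look, boost and interact actions forward through that interface, with move and boost also forwarding on completion.
; DisableMappingContext removes the mapping, while a Possess call sits unconnected.
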(event `self.ReceiveBeginPlay`
  (bind _returnvalue (`GameplayStatics.GetPlayerPawn` 0))
  (`WidgetBlueprintLibrary.SetInputMode_GameOnly` self)
  (`|ExecutionSequence`
    (:`then_0`
      (bind _asbp_pawn_custom (cast `/Game/Blueprints/BP_PawnCustom` _returnvalue))
      (bind _output_get (set `self.PlayerPawn` _asbp_pawn_custom)))
    (:`then_1`
      (bind _asbpi_pawn_input_handler (cast `/Game/Blueprints/Pawn/BPI_PawnInputHandler` _returnvalue))
      (set `self.PawnInputHandler` _asbpi_pawn_input_handler))
    (:`then_2`
      (`EnhancedInputSubsystemInterface.AddMappingContext` (subsystem `EnhancedInputLocalPlayerSubsystem`) "/Game/Inputs/IM_CustomInputMap.IM_CustomInputMap" 0 (struct)) ; required setup to use enhanced input
    )))

(event `EnhancedInput|/Game/Inputs/IA_CustomActionJump`
  (params (ActionValue :type Boolean) (ElapsedSeconds :type "Float (double-precision)") (TriggeredSeconds :type "Float (double-precision)") (InputAction :type "InputAction Object Reference" :default "/Game/Inputs/IA_CustomActionJump.IA_CustomActionJump"))
  ;[1 1 1] Input Events - Enhanced input
  (:`Triggered`
    (`/Game/Blueprints/Pawn/BPI_PawnInputHandler.AddInputJump` (`self.PawnInputHandler`))))

(event `EnhancedInput|/Game/Inputs/IA_CustomActionMove`
  (params (ActionValue :type "Vector2D Structure") (ElapsedSeconds :type "Float (double-precision)") (TriggeredSeconds :type "Float (double-precision)") (InputAction :type "InputAction Object Reference" :default "/Game/Inputs/IA_CustomActionMove.IA_CustomActionMove"))
  ;[1 1 1] Input Events - Enhanced input
  (:`Triggered`
    (`/Game/Blueprints/Pawn/BPI_PawnInputHandler.AddInputMovement` (`self.PawnInputHandler`) ActionValue :!label _label))
  (:`Completed`
    (goto _label)))

(event `EnhancedInput|/Game/Inputs/IA_CustomLook`
  (params (ActionValue :type "Vector2D Structure") (ElapsedSeconds :type "Float (double-precision)") (TriggeredSeconds :type "Float (double-precision)") (InputAction :type "InputAction Object Reference" :default "/Game/Inputs/IA_CustomLook.IA_CustomLook"))
  ;[1 1 1] Input Events - Enhanced input
  (:`Triggered`
    (`/Game/Blueprints/Pawn/BPI_PawnInputHandler.AddInputLook` (`self.PawnInputHandler`) ActionValue)))

(event `EnhancedInput|/Game/Inputs/IA_CustomBoost`
  (params (ActionValue :type Boolean) (ElapsedSeconds :type "Float (double-precision)") (TriggeredSeconds :type "Float (double-precision)") (InputAction :type "InputAction Object Reference" :default "/Game/Inputs/IA_CustomBoost.IA_CustomBoost"))
  ;[1 1 1] Input Events - Enhanced input
  (:`Started`
    (`/Game/Blueprints/Pawn/BPI_PawnInputHandler.AddInputMovementBoost` (`self.PawnInputHandler`) ActionValue :!label _label_2))
  (:`Completed`
    (goto _label_2)))

(event `EnhancedInput|/Game/Inputs/IA_CustomInteract`
  (params (ActionValue :type Boolean) (ElapsedSeconds :type "Float (double-precision)") (TriggeredSeconds :type "Float (double-precision)") (InputAction :type "InputAction Object Reference" :default "/Game/Inputs/IA_CustomInteract.IA_CustomInteract"))
  (:`Started`
    (`/Game/Blueprints/Pawn/BPI_PawnInputHandler.AddInputInteract` (`self.PawnInputHandler`))))

(fn `DisableMappingContext`
  (`EnhancedInputSubsystemInterface.RemoveMappingContext` (subsystem `EnhancedInputLocalPlayerSubsystem`) "/Game/Inputs/IM_CustomInputMap.IM_CustomInputMap" (struct)))

(fn `UserConstructionScript`)