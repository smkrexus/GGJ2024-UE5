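; Radio amenity that the player can switch on and off to mask noise in the room it occupies.
; Interacting with the button area flips IsActive, which starts or stops the music audio and FX.
; While on, its decibel emitter gives the room a minimum noise immunity threshold, removed when switched off.
; The immunity state is reapplied when the room item component registers its room, avoiding a manual initialization timer.
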(event `self.ReceiveBeginPlay`
  (`/Game/Blueprints/Interactables/B_InteractAreaComponent.AssignArea` (`self.InteractAreaComponent_Radio`) (`self.RadioButton`))
  (`self.UpdateRadioState` (`self.bIsActive`)))

(event `self.InteractAreaComponent_Radio.OnInteracted`
  (params (controller :type "Controller Object Reference"))
  (bind _output_get (set `self.bIsActive` (not (`self.bIsActive`))))
  (`self.UpdateRadioState` _output_get))

(event `AddRoomDecibelImmunity`
  (bind _outroom (`/Game/Blueprints/Room/B_RoomItemComponent.GetRoom` (`self.B_RoomItemComponent`)))
  ;[1 1 1] When switch on, room has this level of immunity at minimum
  (`/Engine/EditorBlueprintResources/StandardMacros.IsValid` _outroom
    (:`Is Valid`
      (`/Game/Blueprints/Environment/Decibels/B_DecibelEmitterComponent.MaskSound` (`self.DecibelEmitterComponent`) _outroom))))

(event `RemoveRoomDecibelImmunity`
  (bind _outroom (`/Game/Blueprints/Room/B_RoomItemComponent.GetRoom` (`self.B_RoomItemComponent`)))
  ;[1 1 1] When switch on, room has this level of immunity at minimum
  (`/Engine/EditorBlueprintResources/StandardMacros.IsValid` _outroom
    (:`Is Valid`
      (`/Game/Blueprints/Room/B_RoomDecibelsComponent.RemoveImmunityThreshold` (`/Game/Blueprints/Room/BP_Room_Base.RoomDecibelsComponent` _outroom) self))))

(event `self.B_RoomItemComponent.OnRegisterRoom`
  (params (RegisteredRoom :type "/Game/Blueprints/Room/BP_Room_Base Object Reference"))
  ; Handles initialisation events rather than manual timer
  (if (`self.bIsActive`)
    (`self.AddRoomDecibelImmunity`)
    (else
      (`self.RemoveRoomDecibelImmunity`))))

(fn `TurnOff`
  (`ActorComponent.Deactivate` (`self.FX_MusicFeedback`))
  (`AudioComponent.Stop` (`self.Audio_MusicFeedack`))
  (`self.RemoveRoomDecibelImmunity`))

(fn `TurnOn`
  (`ActorComponent.Activate` (`self.FX_MusicFeedback`) true)
  (`AudioComponent.Play` (`self.Audio_MusicFeedack`) 0.0)
  (`self.AddRoomDecibelImmunity`))

(fn `UpdateRadioState`
  (params (newState :type Boolean))
  (if (`local.newState`)
    (`self.TurnOn`)
    (else
      (`self.TurnOff`))))

(fn `UserConstructionScript`
  (`parent.UserConstructionScript`))