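; BP_NotifySubject_Example is an example subject for the notification system, broadcasting test notifications through its BNotifySystemComponent.
; When Notify is set, BeginPlay starts a looping five-second timer, apparently driving TestNotifyLoop.
; That event broadcasts a basic notify handle to observers with a random boolean state, a generic subject key and itself as instigator.
; GetNotifyComponent exposes the component.
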(event `self.ReceiveBeginPlay`
  (if (`self.notify`)
    (`KismetSystemLibrary.K2_SetTimerDelegate` (`|CreateDelegate` :!event `TestNotifyLoop`) 5.0 true)))

(event `TestNotifyLoop`
  (`/Game/Blueprints/Core/Notification/B_NotifySystemComponent.BroadcastObservers` (`self.B_NotifySystemComponent`) (make `/Game/Blueprints/Core/Notification/STR_NotifyHandle_Basic` (struct) (struct) (`KismetMathLibrary.RandomBool`) "KEY_NOTIFY_GENERICSUBJECT" self)))

(fn `GetNotifyComponent`
  (returns (NSC :type "/Game/Blueprints/Core/Notification/B_NotifySystemComponent Object Reference"))
  (return (`self.B_NotifySystemComponent`)))

(fn `UserConstructionScript`)