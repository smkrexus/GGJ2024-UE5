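; Base gameplay effect Blueprint that applies an effect described by a handle, either immediately or periodically.
; ApplyGameplayEffect stores the handle, then either starts a looping timer when its interval is positive or fires the applied event at once.
; ApplyGameplayEffectTick re-fires that event with the stored handle.
; CompleteGameplayEffect clears the timer and fires the end event, while EndAction clears it and defers to the parent.
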(fn `ApplyGameplayEffect`
  (params (InHandle :type "/Game/Blueprints/Core/GameplayEffect/STR_GameplayEffectHandle Structure"))
  (bind _output_get (set `self._gameplayEffectHandle` InHandle))
  (bind (_attributetag _value _interval) (break `/Game/Blueprints/Core/GameplayEffect/STR_GameplayEffectHandle` _output_get))
  (if (> _interval 0.0)
    (bind _returnvalue (`KismetSystemLibrary.K2_SetTimerDelegate` (`|CreateDelegate` :!event `ApplyGameplayEffectTick`) _interval true))
    (set `self._tickHandle` _returnvalue)
    (else
      (`self.OnGameplayEffectApplied` (`self.GetHandle`)) ; immediate effect
    )))

(fn `ApplyGameplayEffectTick`
  (`self.OnGameplayEffectApplied` (`self.GetHandle`)))

(fn `CompleteGameplayEffect`
  (`KismetSystemLibrary.K2_ClearAndInvalidateTimerHandle` (`self._tickHandle`))
  (`self.OnGameplayEffectEnd` (`self.GetHandle`)))

(fn `EndAction`
  (`KismetSystemLibrary.K2_ClearAndInvalidateTimerHandle` (`self._tickHandle`))
  (`parent.EndAction`))

(fn `GetHandle`
  (returns (OutHandle :type "/Game/Blueprints/Core/GameplayEffect/STR_GameplayEffectHandle Structure"))
  (return (`self._gameplayEffectHandle`)))

(fn `UserConstructionScript`
  (`parent.UserConstructionScript`))