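; Gameplay effect feedback actor that plays a one-shot particle system when its effect's feedback is displayed.
; DisplayFeedback runs the parent logic, then, if the FX asset is valid, spawns it at GetSpawnLocation and starts a one-second timer.
; GetSpawnLocation is a separate function that returns the actor's own location.
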(fn `DisplayFeedback`
  (params (InHandle :type "/Game/Blueprints/Core/GameplayEffect/STR_GameplayActionHandle Structure"))
  (`parent.DisplayFeedback` InHandle)
  (bind _fx (`self.FX`)
    (:`then`
      (`NiagaraFunctionLibrary.SpawnSystemAtLocation` _fx (`self.GetSpawnLocation`))
      (`KismetSystemLibrary.K2_SetTimerDelegate` (`|CreateDelegate` :!event `K2_DestroyActor`) 1.0))
    (:`else`)))

(fn `GetSpawnLocation`
  (returns (ReturnValue :type "Vector Structure"))
  (return (`self.K2_GetActorLocation`)))

(fn `UserConstructionScript`
  (`parent.UserConstructionScript`))