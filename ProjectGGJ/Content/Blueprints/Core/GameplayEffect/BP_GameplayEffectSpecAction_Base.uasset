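; Base gameplay action that applies a list of gameplay effects to its target actor and removes them when the action ends.
; On activation it stores the action handle, finds the target's gameplay attribute component, adds each effect and caches that component.
; Ending the action removes the effects through the cached component before calling the parent.
; A separate RemoveEffects function strips them from any given actor and clears the cache.
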(fn `ApplyEffects`
  (params (InObject :type "Object Object Reference"))
  (locals (GAComponent :type "/Game/Blueprints/Core/GameplayEffect/B_GameplayAttributeComponent_Base Object Reference"))
  (bind _asactor (cast `Actor` InObject))
  (bind _returnvalue (`self.GetComponentByClass` _asactor "/Game/Blueprints/Core/GameplayEffect/B_GameplayAttributeComponent_Base.B_GameplayAttributeComponent_Base_C"))
  (`/Engine/EditorBlueprintResources/StandardMacros.IsValid` _returnvalue
    (:`Is Valid`
      (set `self._gameplayEffectComponent` _returnvalue)
      (for _array_element (`self.effects`)
        (`/Game/Blueprints/Core/GameplayEffect/B_GameplayAttributeComponent_Base.AddGameplayEffect` (`self._gameplayEffectComponent`) _array_element)))
    (:`Is Not Valid`
      (return))))

(fn `EndAction`
  (`|ExecutionSequence`
    (:`then_0`
      (`self.VerifyRemoveEffects`))
    (:`then_1`
      (`parent.EndAction`))))

(fn `GetActionHandle`
  (returns (OutHandle :type "/Game/Blueprints/Core/GameplayEffect/STR_GameplayActionHandle Structure"))
  (return (`self._gameplayAction`)))

(fn `OnActivateAction`
  (params (InHandle :type "/Game/Blueprints/Core/GameplayEffect/STR_GameplayActionHandle Structure"))
  (locals (gameplayEffectComponent :type "/Game/Blueprints/Core/GameplayEffect/B_GameplayAttributeComponent_Base Object Reference"))
  (bind _target (break `/Game/Blueprints/Core/GameplayEffect/STR_GameplayActionHandle` InHandle))
  (set `self._gameplayAction` InHandle)
  (`/Engine/EditorBlueprintResources/StandardMacros.IsValid` _target
    (:`Is Valid`
      (`self.ApplyEffects` _target))
    (:`Is Not Valid`
      (`KismetSystemLibrary.PrintString` "Invalid target"))))

(fn `RemoveEffects`
  (params (InObject :type "Object Object Reference"))
  (locals (GAComponent :type "/Game/Blueprints/Core/GameplayEffect/B_GameplayAttributeComponent_Base Object Reference"))
  (bind _asactor (cast `Actor` InObject))
  (bind _returnvalue (`self.GetComponentByClass` _asactor "/Game/Blueprints/Core/GameplayEffect/B_GameplayAttributeComponent_Base.B_GameplayAttributeComponent_Base_C"))
  (`/Engine/EditorBlueprintResources/StandardMacros.IsValid` _returnvalue
    (:`Is Valid`
      (set `local.GAComponent` _returnvalue)
      (for _array_element (`self.effects`)
        (`/Game/Blueprints/Core/GameplayEffect/B_GameplayAttributeComponent_Base.RemoveGameplayEffect` (`local.GAComponent`) _array_element))
      (set `self._gameplayEffectComponent` null))))

(fn `UserConstructionScript`
  (`parent.UserConstructionScript`))

(fn `VerifyRemoveEffects`
  (bind __gameplayeffectcomponent (`self._gameplayEffectComponent`)
    (:`then`
      (for _array_element (`self.effects`)
        (`/Game/Blueprints/Core/GameplayEffect/B_GameplayAttributeComponent_Base.RemoveGameplayEffect` __gameplayeffectcomponent _array_element)))
    (:`else`)))