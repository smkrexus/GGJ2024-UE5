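; Test actor that exercises objective contexts through a proximity trigger and interactable locator.
; A locally controlled pawn entering or leaving the sphere toggles tracking, while range events update the locator's view model.
; Tracking pushes or clears an objective context on BP_SocialMediaManager's objective component, adding the objective by tag with self as scope.
; A looping timer, apparently driving the manager's counter, runs until completion, clearing or tracking loss, with debug prints throughout.
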(event `self.B_SceneTracker_InteractableLocator.OnRangeDetected`
  (params (player :type "Pawn Object Reference"))
  (bind _viewmodel (`/Game/Blueprints/Interactables/Locator/B_SceneTracker_InteractableLocator.GetViewModel` (`self.B_SceneTracker_InteractableLocator`)))
  (`/Game/Blueprints/Interactables/Locator/ViewModel/B_VM_InteractableLocator.VM_SetShouldDisplayLocator` _viewmodel true)
  (`/Game/Blueprints/Interactables/Locator/ViewModel/B_VM_InteractableLocator.VM_SetInRange` _viewmodel true))

(event `self.B_SceneTracker_InteractableLocator.OnRangeExceeded`
  (params (player :type "Pawn Object Reference") (inMaxRange :type Boolean))
  (bind _viewmodel (`/Game/Blueprints/Interactables/Locator/B_SceneTracker_InteractableLocator.GetViewModel` (`self.B_SceneTracker_InteractableLocator`)))
  (if inMaxRange
    (`/Game/Blueprints/Interactables/Locator/ViewModel/B_VM_InteractableLocator.VM_SetShouldDisplayLocator` _viewmodel true)
    (`/Game/Blueprints/Interactables/Locator/ViewModel/B_VM_InteractableLocator.VM_SetInRange` _viewmodel false)
    (else
      (`/Game/Blueprints/Interactables/Locator/ViewModel/B_VM_InteractableLocator.VM_SetShouldDisplayLocator` _viewmodel false))))

(event `self.Sphere.OnComponentBeginOverlap`
  (params (OverlappedComponent :type "PrimitiveComponent Object Reference") (OtherActor :type "Actor Object Reference") (OtherComp :type "PrimitiveComponent Object Reference") (OtherBodyIndex :type Integer) (bFromSweep :type Boolean) (SweepResult :type "HitResult Structure (by ref)"))
  (bind _aspawn (cast `Pawn` OtherActor))
  (if (`Pawn.IsLocallyControlled` _aspawn)
    (`/ActorTracker/Blueprints/B_SceneTracker_Base.SetTrackingEnabled` (`self.B_SceneTracker_InteractableLocator`) true)))

(event `self.Sphere.OnComponentEndOverlap`
  (params (OverlappedComponent :type "PrimitiveComponent Object Reference") (OtherActor :type "Actor Object Reference") (OtherComp :type "PrimitiveComponent Object Reference") (OtherBodyIndex :type Integer))
  (bind _aspawn (cast `Pawn` OtherActor))
  (if (`Pawn.IsLocallyControlled` _aspawn)
    (`/ActorTracker/Blueprints/B_SceneTracker_Base.SetTrackingEnabled` (`self.B_SceneTracker_InteractableLocator`) false)))

(event `self.B_SceneTracker_InteractableLocator.OnTrackingEnabled`
  (bind _in_objective (`self.In Objective`))
  (bind _objectivetag (defaults `Object` _in_objective))
  (bind _returnvalue (`GameplayStatics.GetActorOfClass` "/Game/Blueprints/SocialMedia/BP_SocialMediaManager.BP_SocialMediaManager_C"))
  (bind _returnvalue_2 (`self.GetComponentByClass` _returnvalue "/Game/Blueprints/Core/Objective/Component/B_ObjectiveDynamicComponent_Base.B_ObjectiveDynamicComponent_Base_C"))
  (add `/Game/Blueprints/Core/Objective/Component/B_ObjectiveDynamicComponent_Base.OnObjectiveContextCleared` _returnvalue_2 (`|CreateDelegate` :!event `Clear`))
  (add `/Game/Blueprints/Core/Objective/Component/B_ObjectiveDynamicComponent_Base.OnObjectiveContextCompleted` _returnvalue_2 (`|CreateDelegate` :!event `Complete`))
  (`/Game/Blueprints/Core/Objective/Component/B_ObjectiveDynamicComponent_Base.PushContext` _returnvalue_2 _in_objective)
  (bind _outsuccess (`/Game/Blueprints/Core/Objective/Component/B_ObjectiveDynamicComponent_Base.AddObjectiveByTag` _returnvalue_2 _objectivetag self))
  (`KismetSystemLibrary.PrintText` (`|FormatText` "Objective Context {a}: Started {b}" (`BlueprintGameplayTagLibrary.GetTagName` _objectivetag) _outsuccess))
  (bind _returnvalue_3 (`KismetSystemLibrary.K2_SetTimerDelegate` (`|CreateDelegate` :!event `Test`) 1.0 true))
  (set `self.testTimer` _returnvalue_3))

(event `self.B_SceneTracker_InteractableLocator.OnTrackingDisabled`
  (bind _returnvalue (`GameplayStatics.GetActorOfClass` "/Game/Blueprints/SocialMedia/BP_SocialMediaManager.BP_SocialMediaManager_C"))
  (bind _returnvalue_2 (`self.GetComponentByClass` _returnvalue "/Game/Blueprints/Core/Objective/Component/B_ObjectiveDynamicComponent_Base.B_ObjectiveDynamicComponent_Base_C"))
  (`/Game/Blueprints/Core/Objective/Component/B_ObjectiveDynamicComponent_Base.ClearContext` _returnvalue_2 (`self.In Objective`) self)
  (remove `/Game/Blueprints/Core/Objective/Component/B_ObjectiveDynamicComponent_Base.OnObjectiveContextCleared` _returnvalue_2 (`|CreateDelegate` :!event `Clear`))
  (`KismetSystemLibrary.PrintText` (`|FormatText` "Remove Context {a}" (`BlueprintGameplayTagLibrary.GetTagName` (defaults `Object` (`self.In Objective`)))))
  (`KismetSystemLibrary.K2_ClearAndInvalidateTimerHandle` (`self.testTimer`)))

(event `Complete`
  (params (InTag :type "GameplayTag Structure") (bSuccess :type Boolean))
  (`KismetSystemLibrary.K2_ClearAndInvalidateTimerHandle` (`self.testTimer`))
  (`KismetSystemLibrary.PrintText` (`|FormatText` "Completed {a}: {b}" (`BlueprintGameplayTagLibrary.GetTagName` InTag) bSuccess) true true (struct :`R` 1.0 :`G` 0.100098 :`A` 1.0)))

(event `Clear`
  (params (InTag :type "GameplayTag Structure"))
  (`KismetSystemLibrary.PrintText` (`|FormatText` "ActiveEventCleared: {a}" (`BlueprintGameplayTagLibrary.GetTagName` InTag)))
  (`KismetSystemLibrary.K2_ClearAndInvalidateTimerHandle` (`self.testTimer`)))

(event `Test`
  (bind _returnvalue (`GameplayStatics.GetActorOfClass` "/Game/Blueprints/SocialMedia/BP_SocialMediaManager.BP_SocialMediaManager_C"))
  (`/Game/Blueprints/SocialMedia/BP_SocialMediaManager.AddCounter` _returnvalue))

(fn `UserConstructionScript`)