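; Base actor for a location-based objective that a donator requests during the social media stream, with rewards and notifications on completion.
; The stream reporter enables or disables the area and resumes or pauses a running objective.
; A detect sphere toggles locator tracking, and a start sphere pushes the objective to the context manager and its view model.
; Leaving or losing tracking clears the context, pausing unfinished objectives; completion either resets or destroys the actor.
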(event `self.ReceiveBeginPlay`
  (bind _returnvalue (`GameplayStatics.GetActorOfClass` "/Game/Blueprints/SocialMedia/BP_SocialMediaManager.BP_SocialMediaManager_C"))
  (bind _output_get (set `self._manager` _returnvalue))
  (set `self.objectiveComponent` (`self.GetComponentByClass` _output_get "/Game/Blueprints/Core/Objective/Context/B_ObjectiveContextManager.B_ObjectiveContextManager_C"))
  (bind _returnvalue_2 (`|AddComponentByClass` (`self.ViewModel`)))
  (set `self.vm_dynamicObjective` _returnvalue_2)
  (`/Game/Blueprints/SocialMedia/Source/Reporters/B_Reporter_SocialMedia_Stream.Start` (`self.B_Reporter_SocialMedia_Stream`)) ; once all initializations take place then start, this runs the report to determine if the objective is enabled or disabled
)

(event `self.B_SocialMediaDonatorComponent.OnDonatorFound`
  (`/Game/Blueprints/SocialMedia/B_SocialMediaDonatorComponent.GenerateNotification` (`self.B_SocialMediaDonatorComponent`) (defaults `Object` (`self.Objective`)) (`/Game/Blueprints/SocialMedia/B_SocialMediaDonatorComponent.GetDonatorMessage` (`self.B_SocialMediaDonatorComponent`) (struct :`TagName` "Objective")) "/Game/Blueprints/SocialMedia/Channel/Banner/B_NotificationChannelMessage_SocialMediaBanner_Request_New.B_NotificationChannelMessage_SocialMediaBanner_Request_New_C" true))

(event `self.B_Reporter_SocialMedia_Stream.OnStreamUpdated`
  (params (bIsStreaming :type Boolean) (bIsPaused :type Boolean))
  (bind __objective (`self._objective`))
  (if (`self.bStarted`)
    (`/Engine/EditorBlueprintResources/StandardMacros.IsValid` (`self._objective`)
      (:`Is Valid`
        (if bIsStreaming
          (`/Game/Blueprints/Core/Objective/B_Objective_Base.Resume` __objective)
          (else
            (`/Game/Blueprints/Core/Objective/B_Objective_Base.Pause` __objective)))))
    (elif bIsStreaming
      (`self.EnableObjectiveArea`)
      (else
        (`self.DisableObjectiveArea`)))))

(event `self.StartRange.OnComponentBeginOverlap`
  (params (OverlappedComponent :type "PrimitiveComponent Object Reference") (OtherActor :type "Actor Object Reference") (OtherComp :type "PrimitiveComponent Object Reference") (OtherBodyIndex :type Integer) (bFromSweep :type Boolean) (SweepResult :type "HitResult Structure (by ref)"))
  ;[0.07292 0.05984 0 1 32] OVERLAP EVENT: START
  (`self.VALIDATE_LOCAL_PLAYER` OtherActor)
  (`self.RequestPushContext`))

(event `self.DetectRange.OnComponentBeginOverlap`
  (params (OverlappedComponent :type "PrimitiveComponent Object Reference") (OtherActor :type "Actor Object Reference") (OtherComp :type "PrimitiveComponent Object Reference") (OtherBodyIndex :type Integer) (bFromSweep :type Boolean) (SweepResult :type "HitResult Structure (by ref)"))
  ;[0.07292 0.05984 0 1 32] OVERLAP EVENT: DETECT
  (`self.VALIDATE_LOCAL_PLAYER` OtherActor)
  (`self.OnPlayerRangeValid`))

(event `self.StartRange.OnComponentEndOverlap`
  (params (OverlappedComponent :type "PrimitiveComponent Object Reference") (OtherActor :type "Actor Object Reference") (OtherComp :type "PrimitiveComponent Object Reference") (OtherBodyIndex :type Integer))
  ;[0.07292 0.05984 0 1 32] OVERLAP EVENT: START
  (`self.VALIDATE_LOCAL_PLAYER` OtherActor)
  (`self.RequestClearInactiveContext`))

(event `self.DetectRange.OnComponentEndOverlap`
  (params (OverlappedComponent :type "PrimitiveComponent Object Reference") (OtherActor :type "Actor Object Reference") (OtherComp :type "PrimitiveComponent Object Reference") (OtherBodyIndex :type Integer))
  ;[0.07292 0.05984 0 1 32] OVERLAP EVENT: DETECT
  (`self.VALIDATE_LOCAL_PLAYER` OtherActor)
  (`self.OnPlayerRangeInvalid`))

(event `self.B_SceneTracker_InteractableLocator.OnTrackingEnabled`
  ;[0.07292 0.05984 0 1 32] ENABLE / DISABLE TRACKING EVENTS
  (`PrimitiveComponent.SetCollisionEnabled` (`self.StartRange`) "QueryOnly"))

(event `Complete`
  (params (InTag :type "GameplayTag Structure") (bSuccess :type Boolean))
  ;[0.07292 0.05984 0 1 32] Clearing Active, Inactive or Completed Contexts
  (`self.VALIDATE_OBJECTIVE_TAG` InTag)
  (`self.ProcessCompletion`))

(event `/Game/Blueprints/Core/Rewards/BPI_Rewarder.GiveRewards`
  (params (InGameState :type "GameStateBase Object Reference"))
  ;[0.07292 0.05984 0 1 32] Clearing Active, Inactive or Completed Contexts
  (`/Game/Blueprints/Core/Objective/Utilities/B_Utilities_Objective_Rewards.DistributeReward` (`self.Rewards`) self))

(event `self.B_SceneTracker_InteractableLocator.OnTrackingDisabled`
  ;[0.07292 0.05984 0 1 32] ENABLE / DISABLE TRACKING EVENTS
  (if (`self.bStarted`)
    (`self.RequestClearActiveContext`)
    (else
      (`self.RequestClearInactiveContext`))))

(event `Clear`
  (params (InTag :type "GameplayTag Structure"))
  ;[0.07292 0.05984 0 1 32] Clearing Active, Inactive or Completed Contexts
  (`self.VALIDATE_OBJECTIVE_TAG` InTag)
  (`self.ProcessCleanup`))

(event `self.B_SceneTracker_InteractableLocator.OnRangeDetected`
  (params (player :type "Pawn Object Reference"))
  (bind _viewmodel (`/Game/Blueprints/Interactables/Locator/B_SceneTracker_InteractableLocator.GetViewModel` (`self.B_SceneTracker_InteractableLocator`)))
  ;[1 0 0.832 1 32] VIEW/HIDE OBJECTIVE LOCATION
  (`/Game/Blueprints/Interactables/Locator/ViewModel/B_VM_InteractableLocator.VM_SetShouldDisplayLocator` _viewmodel true)
  (`/Game/Blueprints/Interactables/Locator/ViewModel/B_VM_InteractableLocator.VM_SetInRange` _viewmodel true))

(event `self.B_SceneTracker_InteractableLocator.OnRangeExceeded`
  (params (player :type "Pawn Object Reference") (inMaxRange :type Boolean))
  (bind _viewmodel (`/Game/Blueprints/Interactables/Locator/B_SceneTracker_InteractableLocator.GetViewModel` (`self.B_SceneTracker_InteractableLocator`)))
  ;[1 0 0.832 1 32] VIEW/HIDE OBJECTIVE LOCATION
  (if inMaxRange
    (`/Game/Blueprints/Interactables/Locator/ViewModel/B_VM_InteractableLocator.VM_SetShouldDisplayLocator` _viewmodel true)
    (`/Game/Blueprints/Interactables/Locator/ViewModel/B_VM_InteractableLocator.VM_SetInRange` _viewmodel false)
    (else
      (`/Game/Blueprints/Interactables/Locator/ViewModel/B_VM_InteractableLocator.VM_SetShouldDisplayLocator` _viewmodel false))))

(fn `CheckPlayerInRange`
  (returns (InDetectRange :type Boolean) (InStartRange :type Boolean))
  (locals (squareDistance :type "Float (double-precision)" :default 0.0) (squareDetectDistance :type "Float (double-precision)") (squareStartDistance :type "Float (double-precision)"))
  (bind _b_scenetracker_interactablelocator (`self.B_SceneTracker_InteractableLocator`))
  (`|ExecutionSequence`
    (:`then_0`
      (set `local.squareDistance` (`KismetMathLibrary.Vector_Distance2DSquared` (`self.K2_GetActorLocation` (`GameplayStatics.GetPlayerPawn` 0)) (`self.K2_GetActorLocation`)))
      (set `local.squareStartDistance` (`KismetMathLibrary.Square` (`/ActorTracker/Blueprints/B_SceneTracker_Base.radius` _b_scenetracker_interactablelocator)))
      (set `local.squareDetectDistance` (`KismetMathLibrary.Square` (+ (`/ActorTracker/Blueprints/B_SceneTracker_Base.maxRadius` _b_scenetracker_interactablelocator) 200.0))))
    (:`then_1`
      (if (not (< (`local.squareDistance`) (`local.squareDetectDistance`)))
        (return false false)))
    (:`then_2`
      (if (< (`local.squareDistance`) (`local.squareStartDistance`))
        (return true true)
        (else
          (return true false))))))

(fn `DisableObjectiveArea`
  (`/ActorTracker/Blueprints/B_SceneTracker_Base.SetTrackingEnabled` (`self.B_SceneTracker_InteractableLocator`) false)
  (`PrimitiveComponent.SetCollisionEnabled` (`self.DetectRange`) "NoCollision")
  (`PrimitiveComponent.SetCollisionEnabled` (`self.StartRange`) "NoCollision"))

(fn `EnableObjectiveArea`
  (`PrimitiveComponent.SetCollisionEnabled` (`self.DetectRange`) "QueryOnly") ; sets tracking enabled upon overlay, if set tracking enabled is called manually, 2 instances of widget shows up - so dont do it
  (bind (_indetectrange _instartrange) (`self.CheckPlayerInRange`))
  (if _instartrange
    (`self.RequestPushContext`)))

(fn `GetScope`
  (returns (OutScope :type "Object Object Reference"))
  (return (`self._scope`)))

(fn `Invalidate`
  (`|ExecutionSequence`
    (:`then_0`
      (if (`self.bStarted`)
        (`self.RequestClearActiveContext`)
        (else
          (`self.RequestClearInactiveContext`))))
    (:`then_1`
      (`self.OnInvalidated` (defaults `Object` (`self.Objective`)))
      (`self.K2_DestroyActor`))))

(fn `LockObjectiveStatus`
  (`/Game/Blueprints/Core/Objective/ViewModel/B_VM_DynamicObjective.VM_SetSuccess` (`self.vm_dynamicObjective`) (`/Game/Blueprints/Core/Objective/B_Objective_Base.IsObjectiveSuccess` (`self._objective`)))
  (`self.Invalidate`))

(fn `OnPlayerRangeInvalid`
  (if (`/Game/Blueprints/SocialMedia/Source/Reporters/B_Reporter_SocialMedia_Stream.IsStreaming` (`self.B_Reporter_SocialMedia_Stream`))
    (`/ActorTracker/Blueprints/B_SceneTracker_Base.SetTrackingEnabled` (`self.B_SceneTracker_InteractableLocator`) false)
    (else
      (`self.DisableObjectiveArea`))))

(fn `OnPlayerRangeValid`
  (`/ActorTracker/Blueprints/B_SceneTracker_Base.SetTrackingEnabled` (`self.B_SceneTracker_InteractableLocator`) true))

(fn `ProcessCleanup`)

(fn `ProcessCompletion`
  (set `self.bCompleted` true)
  (`/Game/Blueprints/Core/Objective/ViewModel/B_VM_DynamicObjective.VM_SetSuccess` (`self.vm_dynamicObjective`) true)
  (`/ActorTracker/Blueprints/B_SceneTracker_Base.SetTrackingEnabled` (`self.B_SceneTracker_InteractableLocator`) false)
  (`/Game/Blueprints/SocialMedia/B_SocialMediaDonatorComponent.GenerateRewardNotification` (`self.B_SocialMediaDonatorComponent`) (defaults `Object` (`self.Objective`)) (`/Game/Blueprints/SocialMedia/B_SocialMediaDonatorComponent.GetDonatorMessage` (`self.B_SocialMediaDonatorComponent`) (struct :`TagName` "Objective.State.Complete")) "/Game/Blueprints/SocialMedia/Channel/Banner/B_NotificationChannelMessage_SocialMediaBanner_Request_Complete.B_NotificationChannelMessage_SocialMediaBanner_Request_Complete_C" (`self.Rewards`) false)
  (`/Game/Blueprints/Core/Rewards/BPI_Rewarder.GiveRewards` (`GameplayStatics.GetGameState`))
  (`self.OnComplete` (defaults `Object` (`self.Objective`)))
  (if (`self.bInvalidateOnComplete`)
    (`self.Invalidate`)
    (else
      (`self.Reset`))))

(fn `RequestClearActiveContext`
  (returns (bSuccess :type Boolean))
  (bind __objective (`self._objective`))
  (bind _vm_dynamicobjective (`self.vm_dynamicObjective`))
  (`|ExecutionSequence`
    (:`then_0`
      (`/Engine/EditorBlueprintResources/StandardMacros.IsValid` (`self.objectiveComponent`)
        (:`Is Not Valid`
          (return false))))
    (:`then_1`
      (if (not (`self.bStarted`))
        (return false)))
    (:`then_2`
      (`PrimitiveComponent.SetCollisionEnabled` (`self.StartRange`) "NoCollision")
      (`/Game/Blueprints/Core/Objective/Context/B_ObjectiveContextManager.ClearContext` (`self.objectiveComponent`) (`self.Objective`) (`self.GetScope`))
      (`self.Stop`)
      (`/Game/Blueprints/Core/Objective/ViewModel/B_VM_DynamicObjectiveList.VM_RemoveObjective` (`/Game/Blueprints/SocialMedia/BP_SocialMediaManager.GetViewModelObjective` (`self._manager`)) _vm_dynamicobjective)
      (`/Game/Blueprints/Core/Objective/ViewModel/B_VM_DynamicObjective.VM_ClearObjective` _vm_dynamicobjective))
    (:`then_3`
      (if (`self.bCompleted`)
        (set `self._objective` null)
        (return true) ; simplest case, when completed just flush all info
      ))
    (:`then_4`
      (`/Engine/EditorBlueprintResources/StandardMacros.IsValid` __objective
        (:`Is Valid`
          (if (`/Game/Blueprints/Core/Objective/B_Objective_Base.IsPaused` __objective)
            (return true) ; objective not completed yet and stream was disabled mid-way, no need to pause again as disabling stream pauses the objective automatically
            (else
              (`/Game/Blueprints/Core/Objective/B_Objective_Base.Pause` (`self._objective`))
              (return true) ; objective incomplete while stream is active this means objective needs to be paused when clearing this objective, eg. moving out of objective range
            )))
        (:`Is Not Valid`
          (return true) ; in case objective was removed for any reason
        )))))

(fn `RequestClearInactiveContext`
  (returns (bSuccess :type Boolean))
  (bind _vm_dynamicobjective (`self.vm_dynamicObjective`))
  (`|ExecutionSequence`
    (:`then_0`
      (`/Engine/EditorBlueprintResources/StandardMacros.IsValid` (`self.objectiveComponent`)
        (:`Is Not Valid`
          (return false))))
    (:`then_1`
      (if (`self.bStarted`)
        (return false)))
    (:`then_2`
      (`/Game/Blueprints/Core/Objective/Context/B_ObjectiveContextManager.ClearContext` (`self.objectiveComponent`) (`self.Objective`) (`self.GetScope`))
      (`/Game/Blueprints/Core/Objective/ViewModel/B_VM_DynamicObjectiveList.VM_RemoveObjective` (`/Game/Blueprints/SocialMedia/BP_SocialMediaManager.GetViewModelObjective` (`self._manager`)) _vm_dynamicobjective)
      (`/Game/Blueprints/Core/Objective/ViewModel/B_VM_DynamicObjective.VM_ClearObjective` _vm_dynamicobjective)
      (set `self._objective` null)
      (return true))))

(fn `RequestPushContext`
  (returns (bSuccess :type Boolean))
  (`|ExecutionSequence`
    (:`then_0`
      (if (`self.bStarted`)
        (return false)))
    (:`then_1`
      (`self.RetrieveScope`)
      (`/Game/Blueprints/SocialMedia/B_SocialMediaDonatorComponent.GenerateDonation` (`self.B_SocialMediaDonatorComponent`) false))
    (:`then_2`
      (`/Game/Blueprints/Core/Objective/Context/B_ObjectiveContextManager.PushContext` (`self.objectiveComponent`) (`self.Objective`))
      (`/Engine/EditorBlueprintResources/StandardMacros.IsValid` (`self._objective`) ; Valid if the objective was paused mid-way\nNot valid  means objective is new or previously completed
        (:`Is Valid`
          (bind _outsuccess (`/Game/Blueprints/Core/Objective/Context/B_ObjectiveContextManager.ResumeObjective` (`self.objectiveComponent`) (`self._objective`)))
          (if (not _outsuccess)
            (return false)))
        (:`Is Not Valid`
          (bind (_outobjective _outsuccess_2) (`/Game/Blueprints/Core/Objective/Context/B_ObjectiveContextManager.AddObjectiveByTag` (`self.objectiveComponent`) (defaults `Object` (`self.Objective`)) (`self.GetScope`)))
          (if _outsuccess_2
            (set `self._objective` _outobjective)
            (else
              (return false))))))
    (:`then_3`
      (`/Game/Blueprints/Core/Objective/ViewModel/B_VM_DynamicObjective.VM_SetObjective` (`self.vm_dynamicObjective`) (`KismetTextLibrary.Conv_NameToText` (defaults `Object` (`self.Objective`))) (`/Game/Blueprints/SocialMedia/B_SocialMediaDonatorComponent.GetDonator` (`self.B_SocialMediaDonatorComponent`)))
      (`/Game/Blueprints/Core/Objective/ViewModel/B_VM_DynamicObjective.VM_SetConditions` (`self.vm_dynamicObjective`) (`/Game/Blueprints/Core/Objective/B_Objective_Base.GetConditions` (`self._objective`)))
      (`/Game/Blueprints/Core/Objective/ViewModel/B_VM_DynamicObjective.VM_SetRewards` (`self.vm_dynamicObjective`) (`self.Rewards`))
      (`self.Start`)
      (`/Game/Blueprints/Core/Objective/ViewModel/B_VM_DynamicObjectiveList.VM_AddObjective` (`/Game/Blueprints/SocialMedia/BP_SocialMediaManager.GetViewModelObjective` (`self._manager`)) (`self.vm_dynamicObjective`))
      (return true))))

(fn `Reset`
  (`/Game/Blueprints/SocialMedia/B_SocialMediaDonatorComponent.Reset` (`self.B_SocialMediaDonatorComponent`))
  (set `self.bCompleted` false)
  (`self.OnReset` (defaults `Object` (`self.Objective`))))

(fn `RetrieveScope`
  (if (`KismetSystemLibrary.IsValid` (`self._scope`))
    (return)
    (else
      (`/Engine/EditorBlueprintResources/StandardMacros.IsValid` (`self.Scope`)
        (:`Is Valid`
          (`self.SetScope` (`self.Scope`)))
        (:`Is Not Valid`
          (`self.SetScope` self))))))

(fn `SetScope`
  (params (InScope :type "Object Object Reference"))
  (set `self._scope` InScope))

(fn `Start`
  (set `self.bStarted` true)
  (add `/Game/Blueprints/Core/Objective/Context/B_ObjectiveContextManager.OnObjectiveContextCleared` (`self.objectiveComponent`) (`|CreateDelegate` :!event `Clear`))
  (add `/Game/Blueprints/Core/Objective/Context/B_ObjectiveContextManager.OnObjectiveContextCompleted` (`self.objectiveComponent`) (`|CreateDelegate` :!event `Complete`)))

(fn `Stop`
  (set `self.bStarted` false)
  (remove `/Game/Blueprints/Core/Objective/Context/B_ObjectiveContextManager.OnObjectiveContextCleared` (`self.objectiveComponent`) (`|CreateDelegate` :!event `Clear`))
  (remove `/Game/Blueprints/Core/Objective/Context/B_ObjectiveContextManager.OnObjectiveContextCompleted` (`self.objectiveComponent`) (`|CreateDelegate` :!event `Complete`)))

(fn `UserConstructionScript`
  (`SphereComponent.SetSphereRadius` (`self.DetectRange`) (+ (`/ActorTracker/Blueprints/B_SceneTracker_Base.maxRadius` (`self.B_SceneTracker_InteractableLocator`)) 200.0) false)
  (`SphereComponent.SetSphereRadius` (`self.StartRange`) (`/ActorTracker/Blueprints/B_SceneTracker_Base.radius` (`self.B_SceneTracker_InteractableLocator`)) false)
  (`PrimitiveComponent.SetCollisionEnabled` (`self.StartRange`) "NoCollision"))