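; Gameflow view model registry that keeps UI view models in a fixed order and tracks an Initialized flag.
; RegisterViewModel slots each instance by its class position in VmFlow, and GetViewModel retrieves one by exact class.
; BeginPlay calls Reset, which clears the flag and starts a FlowDelay timer.
; InitializeViewModels only sets the flag; its loop chaining SafeInitialize with each previous view model is disconnected.
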(event `self.ReceiveBeginPlay`
  (`self.Reset`))

(fn `Clear`
  (`KismetArrayLibrary.Array_Clear` (`self.registeredViewModels`))
  (set `self.bInitialized` false))

(fn `GetOrderIndex`
  (params (viewModel :type "/Game/Blueprints/Core/ViewModel/B_VM_BaseComponent Object Reference"))
  (returns (orderIndex :type Integer))
  (for (_array_element _array_index) (`self.vm_flow`)
    (if (`GameplayStatics.ObjectIsA` (`local.viewModel`) _array_element)
      (return _array_index)))
  (return -1))

(fn `GetViewModel`
  (params (InClass :type "/Game/Blueprints/Core/ViewModel/B_VM_BaseComponent Class Reference"))
  (returns (OutViewModel :type "/Game/Blueprints/Core/ViewModel/B_VM_BaseComponent Object Reference"))
  (for _array_element (`self.registeredViewModels`)
    (if (== (`GameplayStatics.GetObjectClass` _array_element) (`local.InClass`))
      (return _array_element)))
  (return null))

(fn `Initialize View Models`
  (locals (currentViewModel :type "/Game/Blueprints/Core/ViewModel/B_VM_BaseComponent Object Reference") (previousViewModel :type "/Game/Blueprints/Core/ViewModel/B_VM_BaseComponent Object Reference") (localController :type "Controller Object Reference"))
  (set `self.bInitialized` true))

(fn `RegisterViewModel`
  (params (viewModel :type "/Game/Blueprints/Core/ViewModel/B_VM_BaseComponent Object Reference"))
  (locals (indexToAdd :type Integer :default 0))
  (set `local.indexToAdd` (`self.GetOrderIndex` (`local.viewModel`)))
  (if (!= (`local.indexToAdd`) -1)
    (`KismetArrayLibrary.Array_Set` (`self.registeredViewModels`) (`local.indexToAdd`) (`local.viewModel`) true)
    (`self.OnRegisterViewModel`)))

(fn `Reset`
  (set `self.bInitialized` false)
  (`KismetSystemLibrary.K2_SetTimerDelegate` (`|CreateDelegate` :!event `Initialize View Models`) (`self.flowDelay`))
  (`self.OnReset`))

(fn `UserConstructionScript`)

(fn `ValidateInitialization`
  (returns (OutValidated :type Boolean))
  (return (`self.bInitialized`)))