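; Context entry for a "Back" option, used to return from the current window.
; On initialization it sets the display name on its view model.
; On execution it gets the controller from its B_ContextItem_Return item, has that player state's window tracker collapse the top window, then runs the parent execute logic.
; The parent logic sits on a separate sequence branch, so it still runs if a cast fails.
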(fn `ExecuteContext`
  (`|ExecutionSequence`
    (:`then_0`
      (bind _asb_context_item_return (cast `/Game/Blueprints/Core/Contexts/Entries/B_ContextItem_Return` (`self.GetContextInfo`)))
      (bind _outcontroller (`/Game/Blueprints/Core/Contexts/Entries/B_ContextItem_Return.GetController` _asb_context_item_return))
      (bind _asbp_pawn_controller_custom (cast `/Game/Blueprints/Pawn/BP_PawnControllerCustom` _outcontroller))
      (bind _asbp_player_state_custom (cast `/Game/Blueprints/Player/BP_PlayerStateCustom` (`Controller.PlayerState` _asbp_pawn_controller_custom)))
      (`/Game/Blueprints/Core/Contexts/B_ContextWindowTracker.CollapseTopWindow` (`/Game/Blueprints/Player/BP_PlayerStateCustom.GetWindowTracker` _asbp_player_state_custom) _outcontroller))
    (:`then_1`
      (`parent.ExecuteContext`))))

(fn `GetDisplayName`
  (returns (name :type Text))
  (return "Back"))

(fn `InitializeContext`
  (`parent.InitializeContext`)
  (`/Game/Blueprints/Core/Contexts/ViewModel/B_VM_ContextEntry_Base.VM_SetDisplayName` (`self.GetViewModel`) (`self.GetDisplayName`)))

(fn `UserConstructionScript`
  (`parent.UserConstructionScript`))