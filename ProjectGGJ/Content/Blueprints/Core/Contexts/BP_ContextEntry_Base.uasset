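; Base actor for a context entry, holding a context item, its owner and its context component, with a placeholder display name.
; InitializeContext loads a soft view model class, adds it as a component, binds its notify event and registers the entry with it.
; SetupContextItem constructs the item from a soft class and binds its verified event.
; Received notifications switch on an identifier to execute the context, which fires OnExecute.
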(event `OnNotifyReceived`
  (params (identifier :type Name))
  (switch `name` identifier
    (:`contextExecute`
      (`self.ExecuteContext`))))

(fn `ExecuteContext`
  (`self.OnExecute` self))

(fn `GetContextInfo`
  (returns (item :type "/Game/Blueprints/Core/Contexts/B_ContextItem_Base Object Reference") (owner :type "Object Object Reference") (contextComponent :type "/Game/Blueprints/Core/Contexts/B_ContextComponent Object Reference"))
  (return (`self.contextItem`) (`self.contextOwner`) (`self.contextComponent`)))

(fn `GetDisplayName`
  (returns (name :type Text))
  (return "default"))

(fn `GetViewModel`
  (returns (viewModel :type "/Game/Blueprints/Core/Contexts/ViewModel/B_VM_ContextEntry_Base Object Reference"))
  (return (`self.vm_contextEntry`)))

(fn `InitializeContext`
  (if (`KismetSystemLibrary.IsValidSoftClassReference` (`self.viewModelClass`))
    (bind _returnvalue (`KismetSystemLibrary.LoadClassAsset_Blocking` (`self.viewModelClass`)))
    (bind _returnvalue_2 (`|AddComponentByClass` (castclass `/Game/Blueprints/Core/Contexts/ViewModel/B_VM_ContextEntry_Base` _returnvalue :!pure true)))
    (bind _output_get (set `self.vm_contextEntry` _returnvalue_2))
    (add `/Game/Blueprints/Core/ViewModel/B_VM_BaseComponent.OnNotifyVariable` _output_get (`|CreateDelegate` :!event `OnNotifyReceived`))
    (`/Game/Blueprints/Core/Contexts/ViewModel/B_VM_ContextEntry_Base.VM_SetEntry` (`self.GetViewModel`) self)))

(fn `SetContextComponent`
  (params (contextComponent :type "/Game/Blueprints/Core/Contexts/B_ContextComponent Object Reference"))
  (set `self.contextComponent` contextComponent))

(fn `SetContextOwner`
  (params (owner :type "Object Object Reference"))
  (set `self.contextOwner` owner))

(fn `SetupContextItem`
  (if (`KismetSystemLibrary.IsValidSoftClassReference` (`self.contextItemClass`))
    (bind _returnvalue (`KismetSystemLibrary.LoadClassAsset_Blocking` (`self.contextItemClass`)))
    (bind _returnvalue_2 (`|GenericCreateObject` (castclass `/Game/Blueprints/Core/Contexts/B_ContextItem_Base` _returnvalue :!pure true)))
    (bind _output_get (set `self.contextItem` _returnvalue_2))
    (add `/Game/Blueprints/Core/Contexts/B_ContextItem_Base.OnContextVerified` _output_get (`|CreateDelegate` :!event `InitializeContext`))))

(fn `UserConstructionScript`)