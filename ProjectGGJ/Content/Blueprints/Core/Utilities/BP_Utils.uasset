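; BP_Utils is a shared helper library for the GGJ2024 game, offering static-style functions for common lookups and math.
; It returns the cast game mode and game state, and samples or tests values against float ranges.
; CreateStat builds and initializes a B_Stat from the DT_StatDefs row matching the enum name, using a default definition when none exists.
; ClampAxisToRadius projects out-of-circle 2D coordinates onto the circle's edge and reports whether they were inside.
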(fn `ClampAxisToRadius`
  (params (coordinates :type "Vector2D Structure") (radius :type "Float (double-precision)"))
  (returns (clampedAxis :type "Vector2D Structure") (inRadius :type Boolean))
  (locals (eqn_X :type "Float (double-precision)") (eqn_Y :type "Float (double-precision)") (radiusSquared :type "Float (double-precision)") (modifiedY :type "Float (double-precision)") (modifiedX :type "Float (double-precision)"))
  (bind (_coordinates_x _coordinates_y) (`KismetMathLibrary.BreakVector2D` (`local.coordinates`)))
  (bind (_coordinates_x_2 _coordinates_y_2) (`KismetMathLibrary.BreakVector2D` (`local.coordinates`)))
  (bind (_coordinates_x_3 _coordinates_y_3) (`KismetMathLibrary.BreakVector2D` (`local.coordinates`)))
  (bind _returnvalue (/ (`local.radiusSquared`) (+ 1.0 (`KismetMathLibrary.Square` (/ _coordinates_y_2 _coordinates_x_2)))))
  (`|ExecutionSequence`
    (:`then_1`
      (set `local.eqn_X` (`KismetMathLibrary.Square` _coordinates_x))
      (set `local.eqn_Y` (`KismetMathLibrary.Square` _coordinates_y))
      (set `local.radiusSquared` (`KismetMathLibrary.Square` (`local.radius`))))
    (:`then_2`
      (if (<= (+ (`local.eqn_X`) (`local.eqn_Y`)) (`local.radiusSquared`))
        (return (`local.coordinates`) true) ; inCircle
        (else
          (set `local.modifiedX` (* (`KismetMathLibrary.Sqrt` _returnvalue) (`KismetMathLibrary.SignOfFloat` _coordinates_x_3)))
          (set `local.modifiedY` (* (`KismetMathLibrary.SignOfFloat` _coordinates_y_3) (`KismetMathLibrary.Sqrt` (- (`local.radiusSquared`) _returnvalue)))))))
    (:`then_3`
      (return (`KismetMathLibrary.MakeVector2D` (`local.modifiedX`) (`local.modifiedY`)) false))))

(fn `Create Stat`
  (params (Stat :type "/Game/Blueprints/Core/Stats/E_Stat Enum" :default "NewEnumerator5") (Owner :type "Object Object Reference"))
  (returns (`Created Stat` :type "/Game/Blueprints/Core/Stats/B_Stat Object Reference"))
  (bind _owner (`local.Owner`))
  (bind _returnvalue (`KismetStringLibrary.Conv_StringToName` (`|GetEnumeratorNameAsString` Stat)))
  (bind _returnvalue_2 (`|GetDataTableRow` "/Game/Blueprints/Core/Stats/DT_StatDefs.DT_StatDefs" _returnvalue)
    (:`then`
      (bind _returnvalue_3 (`|GenericCreateObject` _owner "/Game/Blueprints/Core/Stats/B_Stat.B_Stat_C"))
      (`/Game/Blueprints/Core/Stats/B_Stat.Initialize` _returnvalue_3 _returnvalue _returnvalue_2)
      (return _returnvalue_3))
    (:`RowNotFound`
      ;[1 1 1] Default Stat if not defined in data table
      (bind _returnvalue_4 (`|GenericCreateObject` _owner "/Game/Blueprints/Core/Stats/B_Stat.B_Stat_C"))
      (`/Game/Blueprints/Core/Stats/B_Stat.Initialize` _returnvalue_4 _returnvalue (make `/Game/Blueprints/Core/Stats/STR_StatDef`))
      (return _returnvalue_4))))

(fn `Game Mode`
  (returns (`Game Mode` :type "/Game/Blueprints/Gameflow/GM_GGJ2024_Base Object Reference"))
  (bind _asgm_ggj2024_base (cast `/Game/Blueprints/Gameflow/GM_GGJ2024_Base` (`GameplayStatics.GetGameMode` (`local.__WorldContext`))))
  (return _asgm_ggj2024_base))

(fn `Game State`
  (returns (`Game State` :type "/Game/Blueprints/Gameflow/GS_GameStateCustom Object Reference"))
  (bind _asgs_game_state_custom (cast `/Game/Blueprints/Gameflow/GS_GameStateCustom` (`GameplayStatics.GetGameState` (`local.__WorldContext`))))
  (return _asgs_game_state_custom))

(fn `Is Within Range`
  (params (Range :type "FloatRange Structure") (Value :type "Float (double-precision)"))
  (returns (`Is In Range` :type Boolean))
  (locals (NewLocalVar :type "Float (double-precision)"))
  (bind (_lowerbound _upperbound) (break `FloatRange` Range))
  (return (and (>= Value (`.Value` (break `FloatRangeBound` _lowerbound))) (<= Value (`.Value` (break `FloatRangeBound` _upperbound))))))

(fn `Random from Range`
  (params (Range :type "FloatRange Structure"))
  (returns (Value :type "Float (double-precision)"))
  (bind (_lowerbound _upperbound) (break `FloatRange` Range))
  (return (`KismetMathLibrary.RandomFloatInRange` (`.Value` (break `FloatRangeBound` _lowerbound)) (`.Value` (break `FloatRangeBound` _upperbound)))))