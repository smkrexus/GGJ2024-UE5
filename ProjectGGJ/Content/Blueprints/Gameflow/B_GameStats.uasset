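; Game stats Blueprint that tracks the score and running counts of adjustments and complaints.
; On BeginPlay it creates an owned Score stat, then signals that stats are initialized.
; CountRating converts each rating tier into a fixed delta, applies it to Score and broadcasts the rating with the Score stat.
; The conversion also returns a signed intensity, which CountRating leaves unused.
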(event `self.ReceiveBeginPlay`
  (`|ExecutionSequence`
    (:`then_0`
      (bind _created_stat (`/Game/Blueprints/Core/Utilities/BP_Utils.Create Stat` "NewEnumerator1" self))
      (set `self.Score` _created_stat))
    (:`then_1`
      (`self.OnStatsInitialized`))))

(fn `ConvertRatingToScore`
  (params (rating :type "/Game/Blueprints/Gameflow/MiniGame/Scoring/E_MiniGame_Rating Enum" :default "NewEnumerator0"))
  (returns (Delta :type "Float (double-precision)") (Intensity :type Integer))
  (return (select `/Game/Blueprints/Gameflow/MiniGame/Scoring/E_MiniGame_Rating` rating :`NewEnumerator0` -0.25 :`NewEnumerator1` 0.15 :`NewEnumerator2` 0.25) (select `/Game/Blueprints/Gameflow/MiniGame/Scoring/E_MiniGame_Rating` rating :`NewEnumerator0` -2 :`NewEnumerator1` 1 :`NewEnumerator2` 2)))

(fn `CountAdjustment`
  (bind _result (`/Engine/EditorBlueprintResources/StandardMacros.IncrementInt` (`self.NumAdjustments`))
    (:`  `
      (set `self.NumAdjustments` _result))))

(fn `CountComplaint`
  (bind _result (`/Engine/EditorBlueprintResources/StandardMacros.IncrementInt` (`self.NumComplaints`))
    (:`  `
      (set `self.NumComplaints` _result))))

(fn `CountRating`
  (params (data :type "/Game/Blueprints/Gameflow/MiniGame/STR_MiniGame_Attribute Structure") (rating :type "/Game/Blueprints/Gameflow/MiniGame/Scoring/E_MiniGame_Rating Enum" :default "NewEnumerator0"))
  (`/Game/Blueprints/Core/Stats/B_Stat.Change` (`self.Score`) (`self.ConvertRatingToScore` rating))
  (`self.OnCountRating` (`local.rating`) (`self.Score`)))