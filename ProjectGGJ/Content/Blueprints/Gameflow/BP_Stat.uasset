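; BP_Stat is a named numeric stat that holds a current value within the Min, Max and Initial of its StatDef.
; It supports clamped changes, reset, percent of max and runtime limit edits, and can double as a timer.
; While ticking is enabled, its Tick function applies scaled delta time in the current direction.
; Reaching a limit applies GetBouncedLimitValue, which can flip direction, and fires OnTimerInterval.
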(fn `Begin Tick`
  (params (`Tick Direction` :type "ETimelineDirection Enum" :default "Forward"))
  (set `self.Tick Direction` `Tick Direction`)
  (`self.Reset`)
  (set `self.Should Tick` true))

(fn `Change`
  (params (Delta :type "Float (double-precision)"))
  (returns (`New Value` :type "Float (double-precision)") (`Raw Value` :type "Float (double-precision)") (`Is Clamped` :type Boolean))
  (bind ((`Min_12_8F45C98F4BABC71E0416F39725F4D52D` _min) (`Max_13_8A895D624DE880DAA7CAD194D3205837` _max)) (break `/Game/Blueprints/Gameflow/BP_StatDef` (`self.Stat Def`)))
  (bind _returnvalue (+ (`local.Delta`) (`self.Current`)))
  (bind _output_get (set `self.Current` (`KismetMathLibrary.FClamp` _returnvalue _min _max)))
  (return _output_get _returnvalue (not (`KismetMathLibrary.InRange_FloatFloat` _returnvalue _min _max false false))))

(fn `Change Max`
  (params (`New Max` :type "Float (double-precision)"))
  (setmembers `/Game/Blueprints/Gameflow/BP_StatDef` :`StructRef` (`self.Stat Def`) :`Max` `New Max`))

(fn `Change Min`
  (params (`New Min` :type "Float (double-precision)"))
  (setmembers `/Game/Blueprints/Gameflow/BP_StatDef` :`StructRef` (`self.Stat Def`) :`Min` `New Min`))

(fn `Current as Int`
  (returns (`Current (Int)` :type Integer))
  (return (`KismetMathLibrary.FTrunc` (`self.Current`))))

(fn `End Tick`
  (set `self.Should Tick` false))

(fn `Initialize`
  (params (`Stat Name` :type Name) (`Stat Def` :type "/Game/Blueprints/Gameflow/BP_StatDef Structure"))
  (set `self.Stat Name` `Stat Name`)
  (set `self.Stat Def` `Stat Def`)
  (`self.Reset`))

(fn `Percent`
  (returns (Percent :type "Float (double-precision)"))
  (return (`KismetMathLibrary.SafeDivide` (`self.Current`) (`.Max_13_8A895D624DE880DAA7CAD194D3205837` (break `/Game/Blueprints/Gameflow/BP_StatDef` (`self.Stat Def`))))))

(fn `Reset`
  (set `self.Current` (`.Initial_11_C524B33C4230C8DF5B8A40B9CC9BA4F8` (break `/Game/Blueprints/Gameflow/BP_StatDef` (`self.Stat Def`)))))

(fn `SetDeltaMultiplier`
  (params (newMultiplier :type "Float (double-precision)"))
  (set `self.timeMultiplier` (`KismetMathLibrary.Abs` newMultiplier)))

(fn `Tick`
  (params (`Delta Time` :type "Float (double-precision)"))
  (returns (`New Value` :type "Float (double-precision)") (`Delta Percent` :type "Float (double-precision)"))
  (bind _delta_time (`local.Delta Time`))
  (bind ((`Min_12_8F45C98F4BABC71E0416F39725F4D52D` _min) (`Max_13_8A895D624DE880DAA7CAD194D3205837` _max) (`DoesTickFlip_16_AABE89DE47B63AA48DDDBAAE27C339AF` _doestickflip)) (break `/Game/Blueprints/Gameflow/BP_StatDef` (`self.Stat Def`)))
  (if (`self.Should Tick`)
    (bind (_new_value _raw_value _is_clamped) (`self.Change` (* (select `ETimelineDirection` (`self.Tick Direction`) :`Forward` _delta_time :`Backward` (* _delta_time -1.0)) (`self.timeMultiplier`))))
    (if _is_clamped
      (set `self.Current` (`KismetMathLibrary.SelectFloat` (- (* (select `ETimelineDirection` (`self.Tick Direction`) :`Forward` _max :`Backward` _min) 2.0) _raw_value) (- _raw_value _max) _doestickflip))
      (if _doestickflip
        (set `self.Tick Direction` (select `ETimelineDirection` (`self.Tick Direction`) :`Forward` "Backward" :`Backward` "Forward" :!type "ETimelineDirection Enum")))
      (`self.OnTimerInterval`))
    (return (`self.Current`) (`KismetMathLibrary.SafeDivide` (`local.Delta Time`) (`.Max_13_8A895D624DE880DAA7CAD194D3205837` (break `/Game/Blueprints/Gameflow/BP_StatDef` (`self.Stat Def`)))))))