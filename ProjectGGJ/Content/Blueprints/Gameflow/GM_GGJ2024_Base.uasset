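; Base game mode for the GGJ2024 game, handling scenario startup, respawn points, save requests and session end.
; BeginPlay starts a debug scenario when no scenario save exists, and FindPlayerStart maps the lives component's respawn tag to base or checkpoint starts.
; EndSession disables input mapping, clears the HUD and shows a timed win/lose overlay before signalling completion.
; DEV functions set gameplay-tag cheat flags, including a custom time scale broadcast instead of global dilation.
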(event `self.ReceiveBeginPlay`
  (`self.SafeStartScenario`))

(event `/Game/Blueprints/Core/Debug/BPI_CheatInterface.DEV_DisableJointRequirement`
  (params (enabled :type Boolean))
  (if enabled
    (bind _outinfo (`/Game/Blueprints/Core/Debug/B_CheatFlags.AddCheatFlag` (`self.CheatFlagsComponent`) (struct :`TagName` "Interaction.Cheats.DisableJointRequirement")))
    (`KismetSystemLibrary.PrintText` _outinfo)
    (else
      (bind _outinfo_2 (`/Game/Blueprints/Core/Debug/B_CheatFlags.RemoveCheatFlag` (`self.CheatFlagsComponent`) (struct :`TagName` "Interaction.Cheats.DisableJointRequirement")))
      (`KismetSystemLibrary.PrintText` _outinfo_2))))

(event `/Game/Blueprints/Gameflow/Save/BPI_SaveGame.Save`
  (`self.OnGlobalSaveRequest`)
  (message `/Game/Blueprints/Gameflow/Save/BPI_SaveGame.Save` (`GameplayStatics.GetGameInstance`)))

(event `OnEndSession`
  (params (winCondition :type Boolean))
  (set `self.winCondition` winCondition)
  (set `PlayerController.bShowMouseCursor` true (`GameplayStatics.GetPlayerController` 0))
  (bind _asbp_pawn_controller_custom (cast `/Game/Blueprints/Pawn/BP_PawnControllerCustom` (`GameplayStatics.GetPlayerController` 0)))
  (`/Game/Blueprints/Pawn/BP_PawnControllerCustom.DisableMappingContext` _asbp_pawn_controller_custom "/Game/Blueprints/Core/Inputs/Maps/IM_CustomInputMap.IM_CustomInputMap" true))

(event `OnEndSessionCleanup`
  (bind _foundwidgets (`WidgetBlueprintLibrary.GetAllWidgetsOfClass` "/Game/Blueprints/HUD/WBP_Player_MasterUI.WBP_Player_MasterUI_C")) ; remove base HUD
  (for _array_element _foundwidgets
    (`Widget.RemoveFromParent` _array_element))
  (`self.OnPostEndSessionCleanup`))

(event `OnPostEndSessionCleanup`
  (if (`self.winCondition`)
    (bind _returnvalue (`|GenericCreateObject` "/Game/Blueprints/HUD/GameState/WBP_GameState_Overlay_Win.WBP_GameState_Overlay_Win_C")) ; transition HUD
    (`UserWidget.AddToViewport` _returnvalue 1)
    (`KismetSystemLibrary.Delay` 2.0)
    (bind _foundwidgets (`WidgetBlueprintLibrary.GetAllWidgetsOfClass` (`GameplayStatics.GetObjectClass` _returnvalue)))
    (for _array_element _foundwidgets
      (`Widget.RemoveFromParent` _array_element))
    (`self.OnCompleteEndSession`)
    (else
      (bind _returnvalue_2 (`|GenericCreateObject` "/Game/Blueprints/HUD/GameState/WBP_GameState_Overlay_Lose.WBP_GameState_Overlay_Lose_C")) ; transition HUD
      (`UserWidget.AddToViewport` _returnvalue_2 1)
      (`KismetSystemLibrary.Delay` 2.0)
      (bind _foundwidgets_2 (`WidgetBlueprintLibrary.GetAllWidgetsOfClass` (`GameplayStatics.GetObjectClass` _returnvalue_2)))
      (for _array_element_2 _foundwidgets_2
        (`Widget.RemoveFromParent` _array_element_2))
      (`self.OnCompleteEndSession`))))

(event `OnCompleteEndSession`
  (`self.OnGameModeComplete`) ; should also change player state
)

(fn `DEV_LockMiniGameRating`
  (params (Type :type Integer))
  (bind _cheatflagscomponent (`self.CheatFlagsComponent`))
  (bind _cheatflagscomponent_2 (`self.CheatFlagsComponent`))
  (bind _cheatflagscomponent_3 (`self.CheatFlagsComponent`))
  (if (`KismetMathLibrary.InRange_IntInt` Type 0 2)
    (bind _outinfo (`/Game/Blueprints/Core/Debug/B_CheatFlags.AddCheatFlag` (`self.CheatFlagsComponent`) (struct :`TagName` "MiniGame.Cheats.LockRating")))
    (`KismetSystemLibrary.PrintText` _outinfo)
    (switch `int` (`local.Type`)
      (:`0`
        (bind _outinfo_2 (`/Game/Blueprints/Core/Debug/B_CheatFlags.AddCheatFlag` _cheatflagscomponent_2 (struct :`TagName` "MiniGame.Shared.Rating.Bad")))
        (`KismetSystemLibrary.PrintText` _outinfo_2)
        (`/Game/Blueprints/Core/Debug/B_CheatFlags.RemoveCheatFlag` _cheatflagscomponent_2 (struct :`TagName` "MiniGame.Shared.Rating.Good"))
        (`/Game/Blueprints/Core/Debug/B_CheatFlags.RemoveCheatFlag` _cheatflagscomponent_2 (struct :`TagName` "MiniGame.Shared.Rating.Excellent")))
      (:`1`
        (bind _outinfo_3 (`/Game/Blueprints/Core/Debug/B_CheatFlags.AddCheatFlag` _cheatflagscomponent_3 (struct :`TagName` "MiniGame.Shared.Rating.Good")))
        (`KismetSystemLibrary.PrintText` _outinfo_3)
        (`/Game/Blueprints/Core/Debug/B_CheatFlags.RemoveCheatFlag` _cheatflagscomponent_3 (struct :`TagName` "MiniGame.Shared.Rating.Bad"))
        (`/Game/Blueprints/Core/Debug/B_CheatFlags.RemoveCheatFlag` _cheatflagscomponent_3 (struct :`TagName` "MiniGame.Shared.Rating.Excellent")))
      (:`2`
        (bind _outinfo_4 (`/Game/Blueprints/Core/Debug/B_CheatFlags.AddCheatFlag` _cheatflagscomponent (struct :`TagName` "MiniGame.Shared.Rating.Excellent")))
        (`KismetSystemLibrary.PrintText` _outinfo_4)
        (`/Game/Blueprints/Core/Debug/B_CheatFlags.RemoveCheatFlag` _cheatflagscomponent (struct :`TagName` "MiniGame.Shared.Rating.Bad"))
        (`/Game/Blueprints/Core/Debug/B_CheatFlags.RemoveCheatFlag` _cheatflagscomponent (struct :`TagName` "MiniGame.Shared.Rating.Good"))))
    (else
      (return))))

(fn `DEV_SetTimeScale`
  (params (InScale :type Integer))
  (locals (initialScale :type "Float (double-precision)" :default 0.0))
  (set `local.initialScale` (`self._gameTimeScale`))
  (`|ExecutionSequence`
    (:`then_0`
      (if (<= (`local.InScale`) 0)
        (set `self._gameTimeScale` 1.0)
        (bind _outinfo (`/Game/Blueprints/Core/Debug/B_CheatFlags.RemoveCheatFlag` (`self.CheatFlagsComponent`) (struct :`TagName` "GameMode.Cheats.TimeScale")))
        (`KismetSystemLibrary.PrintText` _outinfo)
        (else
          (set `self._gameTimeScale` (`KismetMathLibrary.Conv_IntToDouble` (`KismetMathLibrary.Abs_Int` (`local.InScale`))))
          (bind _outinfo_2 (`/Game/Blueprints/Core/Debug/B_CheatFlags.AddCheatFlag` (`self.CheatFlagsComponent`) (struct :`TagName` "GameMode.Cheats.TimeScale")))
          (`KismetSystemLibrary.PrintText` (`|FormatText` "{Cheat} -Value {v}" _outinfo_2 (`self._gameTimeScale`))))))
    (:`then_1`
      (`self.OnModifyTimeScale` (/ (`local.initialScale`) (`self._gameTimeScale`))))))

(fn `DEV_UnlockMiniGameRating`
  (bind _cheatflagscomponent (`self.CheatFlagsComponent`))
  (`/Game/Blueprints/Core/Debug/B_CheatFlags.RemoveCheatFlag` _cheatflagscomponent (struct :`TagName` "MiniGame.Shared.Rating.Bad"))
  (`/Game/Blueprints/Core/Debug/B_CheatFlags.RemoveCheatFlag` _cheatflagscomponent (struct :`TagName` "MiniGame.Shared.Rating.Good"))
  (`/Game/Blueprints/Core/Debug/B_CheatFlags.RemoveCheatFlag` _cheatflagscomponent (struct :`TagName` "MiniGame.Shared.Rating.Excellent"))
  (bind _outinfo (`/Game/Blueprints/Core/Debug/B_CheatFlags.RemoveCheatFlag` _cheatflagscomponent (struct :`TagName` "MiniGame.Cheats.LockRating")))
  (`KismetSystemLibrary.PrintText` _outinfo))

(fn `EndSession`
  (params (winCondition :type Boolean :default true))
  (`self.OnEndSession` winCondition)
  (`self.OnEndSessionCleanup`))

(fn `FindPlayerStart`
  (params (Player :type "Controller Object Reference") (IncomingName :type String))
  (returns (ReturnValue :type "Actor Object Reference"))
  (locals (playerLives :type "/Game/Blueprints/Player/B_PlayerLivesComponent Object Reference") (checkpointName :type String))
  (`|ExecutionSequence`
    (:`then_0`
      (bind _output_get (set `local.playerLives` (`self.GetComponentByClass` (`Controller.PlayerState` (`local.Player`)) "/Game/Blueprints/Player/B_PlayerLivesComponent.B_PlayerLivesComponent_C")))
      (`/Engine/EditorBlueprintResources/StandardMacros.IsValid` _output_get
        (:`Is Valid`
          (`|SwitchGameplayTag` (`/Game/Blueprints/Player/B_PlayerLivesComponent.GetRespawnTag` (`local.playerLives`))
            (:`GameMode.RespawnTypes.Start`
              (set `local.checkpointName` "base"))
            (:`GameMode.RespawnTypes.Checkpoint`
              (set `local.checkpointName` "checkpoint"))))
        (:`Is Not Valid`
          (bind _returnvalue (`parent.FindPlayerStart` (`local.Player`) (`local.IncomingName`)))
          (return _returnvalue))))
    (:`then_1`
      (bind _returnvalue_2 (`parent.FindPlayerStart` (`local.Player`) (`local.checkpointName`)))
      (return _returnvalue_2))))

(fn `GetTimeScale`
  (returns (OutTime :type "Float (double-precision)"))
  (return (`self._gameTimeScale`)))

(fn `IsCheatEnabled`
  (params (tag :type "GameplayTag Structure"))
  (returns (valid :type Boolean))
  (bind _cheatflagscomponent (`self.CheatFlagsComponent`))
  (if (`ActorComponent.bIsEditorOnly` _cheatflagscomponent)
    (return (`/Game/Blueprints/Core/Debug/B_CheatFlags.HasCheatTag` _cheatflagscomponent (`local.tag`)))
    (else
      (return false))))

(fn `SafeStartScenario`
  (locals (gameInstance :type "/Game/Blueprints/Gameflow/GI_Uncertified Object Reference") (debugScenario :type "DataTableRowHandle Structure" :default (struct :`DataTable` "/Script/Engine.DataTable'/Game/Blueprints/GameScenario/DT_ScenarioDefinition.DT_ScenarioDefinition'" :`RowName` "DEV-1A")))
  (bind (_datatable _rowname) (break `DataTableRowHandle` (`local.debugScenario`)))
  (`|ExecutionSequence`
    (:`then_0`
      (bind _asgi_uncertified (cast `/Game/Blueprints/Gameflow/GI_Uncertified` (`GameplayStatics.GetGameInstance`)))
      (set `local.gameInstance` _asgi_uncertified))
    (:`then_1`
      ;[1 1 1] Scenario saves should be valid if run from menu, this is a safe start when loading directly into map as developer
      (`/Engine/EditorBlueprintResources/StandardMacros.IsValid` (`/Game/Blueprints/Gameflow/GI_Uncertified.ScenarioSave` (`local.gameInstance`))
        (:`Is Valid`
          (return))
        (:`Is Not Valid`
          (`/Game/Blueprints/Gameflow/GI_Uncertified.ClearScenario` (`local.gameInstance`)))))
    (:`then_2`
      (bind _returnvalue (`|GetDataTableRow` _datatable _rowname)
        (:`then`
          (`/Game/Blueprints/Gameflow/GI_Uncertified.StartScenario` (`local.gameInstance`) (`.RowName` (break `DataTableRowHandle` (`local.debugScenario`))) _returnvalue 0.0))))))

(fn `SetInteractFocusMode`
  (params (focus :type Boolean) (enableMap :type "InputMappingContext Object Reference") (disableMap :type "InputMappingContext Object Reference"))
  (bind _asbp_pawn_controller_custom (cast `/Game/Blueprints/Pawn/BP_PawnControllerCustom` (`GameplayStatics.GetPlayerController` 0) :!pure true))
  (`|ExecutionSequence`
    (:`then_0`
      (bind _enablemap (`local.enableMap`)
        (:`then`
          (`/Game/Blueprints/Pawn/BP_PawnControllerCustom.SetMappingContext` _asbp_pawn_controller_custom _enablemap true 0))
        (:`else`)))
    (:`then_1`
      (bind _disablemap (`local.disableMap`)
        (:`then`
          (`/Game/Blueprints/Pawn/BP_PawnControllerCustom.DisableMappingContext` _asbp_pawn_controller_custom _disablemap true))
        (:`else`)))))

(fn `UserConstructionScript`)