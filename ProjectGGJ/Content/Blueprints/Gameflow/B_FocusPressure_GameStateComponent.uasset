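; Game state component running the focus pressure minigame, where a patient joint is twisted toward randomized targets within its safe limit.
; A timer slows inside random pressure windows and runs at a compensating rate outside, toggling Steps 0 and 1.
; Step 2 requires on-target twist to enter; twisting then builds score, faster inside windows, against decay that steepens outside or above a random target.
; Twist-direction detection is unconnected debug code.
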(event `self.ReceiveBeginPlay`)

(event `self.ReceiveTick`
  (params (DeltaSeconds :type "Float (single-precision)"))
  (bind (_pressuretimemultiplier_x _pressuretimemultiplier_y) (`KismetMathLibrary.BreakVector2D` (`self.pressureTimeMultiplier`)))
  (bind _timer (`self.timer`))
  (bind _returnvalue (select `bool` (`self.IsInPressureRange`) :`false` (* DeltaSeconds 5.0) :`true` DeltaSeconds :!type "Float (double-precision)"))
  (bind _joint (`self.joint`)
    (:`then`
      (`self.UpdateTwistCurrent` _joint)
      (`|ExecutionSequence`
        (:`then_0`
          (`/Game/Blueprints/Gameflow/BP_Stat.Tick` (`self.timer`) DeltaSeconds)
          (if (`self.IsInPressureRange`)
            (`/Game/Blueprints/Gameflow/BP_Stat.SetDeltaMultiplier` _timer _pressuretimemultiplier_x)
            (switch `int` (`self.step`)
              (:`0`
                (`self.ChangeStep` 1)))
            (else
              (`/Game/Blueprints/Gameflow/BP_Stat.SetDeltaMultiplier` _timer _pressuretimemultiplier_y)
              (switch `int` (`self.step`)
                (:`1`
                  (`self.ChangeStep` 0))))))
        (:`then_1`
          (switch `int` (`self.step`)
            (:`2`
              (bind _output_get (set `self.tempPressureScoreRaw` (`KismetMathLibrary.FClamp` (- (`self.tempPressureScoreRaw`) (select `bool` (> (`self.tempPressureScoreRaw`) (`self.tempPressureScoreTarget`)) :`false` _returnvalue :`true` (* _returnvalue 5.0))) 0.0 (`self.tempPressureScoreMax`))))
              (set `self.tempPressureScore` (`KismetMathLibrary.FTrunc` _output_get)))))))
    (:`else`)))

(event `OnChangedStep`
  (switch `int` (`self.step`)
    (:`1`
      (`self.RandomizeTwistTarget` (`self.twistTarget`)))
    (:`2`
      (set `self.twistSaved` (`self.twistTarget`))
      (`self.RandomizeTwistTarget` (`self.twistTarget`)))))

(event `OnFailStep`
  (params (failedStep :type Integer))
  (`self.OnFailStepEvent` failedStep))

(fn `ChangeStep`
  (params (tryChangeToStep :type Integer))
  (if (!= tryChangeToStep (`self.step`))
    (if (== (`local.tryChangeToStep`) 2)
      (if (`self.IsInTwistRange`)
        (set `self.step` (`local.tryChangeToStep`) :!label _label)
        (`self.OnChangedStep`)
        (else
          (`self.OnFailStep` (`local.tryChangeToStep`))))
      (else
        (goto _label)))))

(fn `GetLimit`
  (returns (safeLimit :type "Vector2D Structure") (dangerLimit :type "Vector2D Structure"))
  (bind _joint (`self.joint`)
    (:`then`
      (bind (_limits_bonename _limits_safelimit _limits_dangerlimit) (break `/Game/Blueprints/Patient/STR_RotateBoneLimits` (`/Game/Blueprints/Patient/B_PatientJointComponent.limits` (`/Game/Blueprints/Interactables/BP_ChiropractorPoint.PatientJointComponent` _joint))))
      (return _limits_safelimit _limits_dangerlimit))
    (:`else`
      (return (0.0 0.0) (0.0 0.0)))))

(fn `HasJointIssue`
  (returns (hasIssue :type Boolean))
  (bind _joint (`self.joint`)
    (:`then`
      (return (`/Game/Blueprints/Interactables/BP_ChiropractorPoint.hasJointIssue` _joint)))
    (:`else`
      (return false))))

(fn `InPressureRange`
  (params (compareValue :type "Float (double-precision)"))
  (returns (inRange :type Boolean))
  (for _array_element (`self.pressureRange`)
    (bind (_x _y) (`KismetMathLibrary.BreakVector2D` _array_element))
    (if (<= _y 1.0)
      (if (`KismetMathLibrary.InRange_FloatFloat` (`local.compareValue`) _x _y)
        (return true))))
  (return false))

(fn `IsInPressureRange`
  (returns (inRange :type Boolean))
  (return (`self.InPressureRange` (`/Game/Blueprints/Gameflow/BP_Stat.Percent` (`self.timer`)))))

(fn `IsInTwistRange`
  (returns (inRange :type Boolean))
  (bind (_twisttarget_x _twisttarget_y) (`KismetMathLibrary.BreakVector2D` (`self.twistTarget`)))
  (bind (_twistcurrent_x _twistcurrent_y) (`KismetMathLibrary.BreakVector2D` (`self.twistCurrent`)))
  (bind _returnvalue (select `int` (`self.step`) :`0` 1.0 :`1` 1.0 :`2` 10.0))
  (return (and (< (`KismetMathLibrary.Abs` (- _twisttarget_x _twistcurrent_x)) _returnvalue) (< (`KismetMathLibrary.Abs` (- _twisttarget_y _twistcurrent_y)) _returnvalue))))

(fn `RandomizePressureRange`
  (locals (rangePoints :type Integer :default 2) (randomValue :type "Float (double-precision)") (fixedAngle :type Boolean :default true) (angleBetweenPoint :type "Float (double-precision)" :default 135.0) (angleBetweenPointNomalized :type "Float (double-precision)") (pressureArea :type "Float (double-precision)" :default 0.05) (slowMultiplier :type "Float (double-precision)" :default 0.25) (baseMultiplier :type "Float (double-precision)"))
  (bind _randomvalue (`local.randomValue`))
  (bind _randomvalue_2 (`local.randomValue`))
  (bind _returnvalue (* (`local.pressureArea`) 0.5))
  (bind _returnvalue_2 (* (`local.pressureArea`) (`local.rangePoints`)))
  (bind _returnvalue_3 (/ 1.0 (`KismetMathLibrary.Conv_IntToDouble` (`local.rangePoints`))))
  (bind _returnvalue_4 (`KismetSystemLibrary.MakeLiteralDouble` (`.Max_13_8A895D624DE880DAA7CAD194D3205837` (break `/Game/Blueprints/Gameflow/BP_StatDef` (`/Game/Blueprints/Gameflow/BP_Stat.Stat Def` (`self.timer`))))))
  (`|ExecutionSequence`
    (:`then_0`
      (if (`local.fixedAngle`)
        (`|ExecutionSequence`
          (:`then_0`
            (set `local.angleBetweenPointNomalized` (/ (`local.angleBetweenPoint`) 360.0)))
          (:`then_1`
            (for _index (range (`local.rangePoints`))
              (set `local.randomValue` (select `bool` (== _index 0) :`false` (+ (`local.angleBetweenPointNomalized`) (`local.randomValue`)) :`true` (`KismetMathLibrary.RandomFloatInRange` 0.0 (`local.angleBetweenPointNomalized`))))
              (`KismetArrayLibrary.Array_Add` (`self.pressureRange`) (`KismetMathLibrary.MakeVector2D` (- _randomvalue_2 _returnvalue) (+ _randomvalue_2 _returnvalue))))))
        (else
          (for _index_2 (range (`local.rangePoints`))
            (set `local.randomValue` (`KismetMathLibrary.RandomFloatInRange` (* _index_2 _returnvalue_3) (* (+ _index_2 1) _returnvalue_3)))
            (`KismetArrayLibrary.Array_Add` (`self.pressureRange`) (`KismetMathLibrary.MakeVector2D` _randomvalue (+ _randomvalue (`local.pressureArea`))))))))
    (:`then_1`
      (set `local.baseMultiplier` (/ _returnvalue_4 (/ (- _returnvalue_4 (/ _returnvalue_4 (/ 1.0 _returnvalue_2) (`local.slowMultiplier`))) (- 1.0 _returnvalue_2))))
      (set `self.pressureTimeMultiplier` (`KismetMathLibrary.MakeVector2D` (`local.slowMultiplier`) (`local.baseMultiplier`))))))

(fn `RandomizeTwistTarget`
  (params (targetToRandomize :type "Vector2D Structure (by ref)"))
  (bind _safelimit (`self.GetLimit`))
  (`|VariableSetRef` targetToRandomize (`/Game/Blueprints/Gameflow/BP_Utils.ClampAxisToRadius` (`KismetMathLibrary.MakeVector2D` (`KismetMathLibrary.RandomFloatInRange` (`KismetMathLibrary.BreakVector2D` _safelimit) (`.Y` (`KismetMathLibrary.BreakVector2D` _safelimit))) (`KismetMathLibrary.RandomFloatInRange` (`KismetMathLibrary.BreakVector2D` _safelimit) (`.Y` (`KismetMathLibrary.BreakVector2D` _safelimit)))) (`KismetMathLibrary.BreakVector2D` _safelimit))))

(fn `ScoreByTwist`
  (params (twist :type "Vector2D Structure"))
  (locals (preScore :type Integer))
  (switch `int` (`self.step`)
    (:`2`
      (if (`self.IsInTwistRange`)
        (bind _output_get (set `self.tempPressureScoreRaw` (`KismetMathLibrary.FClamp` (+ (* (`KismetMathLibrary.VSize2D` twist) (`GameplayStatics.GetWorldDeltaSeconds`) (select `bool` (`self.IsInPressureRange`) :`false` 10.0 :`true` 100.0)) (`self.tempPressureScoreRaw`)) 0.0 (`self.tempPressureScoreMax`))))
        (set `self.tempPressureScore` (`KismetMathLibrary.FTrunc` _output_get))))))

(fn `StartMode`
  (params (joint :type "/Game/Blueprints/Interactables/BP_ChiropractorPoint Object Reference"))
  (bind _temppressurescoremax (`self.tempPressureScoreMax`))
  (`|ExecutionSequence`
    (:`then_0`
      (set `self.joint` joint)
      (`/Game/Blueprints/Gameflow/BP_Stat.Change Max` (`self.timer`) (`/Game/Blueprints/Gameflow/BP_Utils.Random from Range` (`self.pressureDuration`))))
    (:`then_1`
      (`self.RandomizeTwistTarget` (`self.twistTarget`))
      (`self.RandomizePressureRange`)
      (set `self.step` 0)
      (set `self.tempPressureScoreRaw` 0.0)
      (set `self.tempPressureScoreTarget` (`KismetMathLibrary.RandomFloatInRange` (* _temppressurescoremax 0.5) _temppressurescoremax))
      (set `self.tempPressureScore` 0))
    (:`then_2`
      (`self.UpdateTwistCurrent` (`self.joint`)) ; reset to current joint twist
    )))

(fn `StopMode`
  (set `self.joint` null) ; remove references
  (`KismetArrayLibrary.Array_Clear` (`self.pressureRange`)))

(fn `TempCheckBeyondQuadrantThreshold`
  (params (currentQuadrant :type Integer) (prevQuadrant :type Integer))
  (returns (isClockwise :type Boolean))
  (`|ExecutionSequence`
    (:`then_0`
      (if (== (`local.currentQuadrant`) 1)
        (return true)))
    (:`then_1`
      (if (== (`local.currentQuadrant`) 4)
        (return false)))))

(fn `TempCheckTwistDirection`
  (locals (anchorDirection :type "Vector2D Structure" :default (0.0 20.0)) (currentToCenterDirection :type "Vector2D Structure") (prevToCenterDirection :type "Vector2D Structure") (angleThisFrame :type "Float (double-precision)") (quadrantThisFrame :type Integer))
  (bind _twistcurrent (`self.twistCurrent`))
  (bind _quadrantthisframe (`local.quadrantThisFrame`))
  (bind _quadrantpreviousframe (`self.quadrantPreviousFrame`))
  (bind _returnvalue (`KismetMathLibrary.Normal2D` _twistcurrent))
  (bind _returnvalue_2 (`KismetMathLibrary.DegAcos` (`KismetMathLibrary.DotProduct2D` (`KismetMathLibrary.Normal2D` (`local.anchorDirection`)) _returnvalue)))
  (`|ExecutionSequence`
    (:`then_1`
      (if (> (`KismetMathLibrary.VSize2DSquared` _twistcurrent) (`KismetMathLibrary.Square` 15.0))
        (bind _output_get (set `local.angleThisFrame` (select `bool` (> (`KismetMathLibrary.BreakVector2D` _returnvalue) 0.0) :`false` (- 360.0 _returnvalue_2) :`true` _returnvalue_2)))
        (set `local.quadrantThisFrame` (`self.TempConvertAngleToQuadrant` _output_get))
        (if (> (`KismetMathLibrary.Abs` (- (`local.angleThisFrame`) (`self.anglePreviousFrame`))) 0.3)
          (if (and (!= (`local.quadrantThisFrame`) (`self.quadrantPreviousFrame`)) (or (== _quadrantthisframe 1) (== _quadrantthisframe 4)) (or (== _quadrantpreviousframe 1) (== _quadrantpreviousframe 4)))
            (`KismetSystemLibrary.PrintString` (select `bool` (`self.TempCheckBeyondQuadrantThreshold` (`local.quadrantThisFrame`) (`self.quadrantPreviousFrame`)) :`false` "anticlockwise past threshold" :`true` "clockwise past threshold"))
            (else
              (`KismetSystemLibrary.PrintString` (select `bool` (> (`local.angleThisFrame`) (`self.anglePreviousFrame`)) :`false` "anticlockwise" :`true` "clockwise")))))
        (set `self.anglePreviousFrame` (`local.angleThisFrame`))
        (set `self.quadrantPreviousFrame` (`local.quadrantThisFrame`))))))

(fn `TempConvertAngleToQuadrant`
  (params (angle :type "Float (double-precision)"))
  (returns (quadrant :type Integer))
  (`|ExecutionSequence`
    (:`then_0`
      (if (`KismetMathLibrary.InRange_FloatFloat` (`local.angle`) 0.0 90.0 true false)
        (return 1)))
    (:`then_1`
      (if (`KismetMathLibrary.InRange_FloatFloat` (`local.angle`) 90.0 180.0 true false)
        (return 2)))
    (:`then_2`
      (if (`KismetMathLibrary.InRange_FloatFloat` (`local.angle`) 180.0 270.0 true false)
        (return 3)))
    (:`then_3`
      (if (`KismetMathLibrary.InRange_FloatFloat` (`local.angle`) 270.0 360.0 true false)
        (return 4)))))