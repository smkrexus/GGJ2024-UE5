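; Game phase notification component that puts on-screen notification widgets in the viewport for a given tag.
; AddScreenNotification looks up the tag in the ScreenNotifications map and passes any matching widget class to LoadScreenNotification.
; That event async-loads the class, constructs it and adds it to the viewport as a UserWidget, so widget classes load only on demand.
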(event `LoadScreenNotification`
  (params (InWidget :type "Widget Soft Class Reference"))
  (bind _class (`|LoadAssetClass` InWidget)
    (:`Completed`
      (bind _returnvalue (`|GenericCreateObject` _class))
      (bind _asuser_widget (cast `UserWidget` _returnvalue))
      (`UserWidget.AddToViewport` _asuser_widget 0))))

(fn `AddScreenNotification`
  (params (InTag :type "GameplayTag Structure"))
  (locals (selectedWidget :type "UserWidget Soft Class Reference"))
  (bind (_value _returnvalue) (`BlueprintMapLibrary.Map_Find` (`self.ScreenNotifications`) (`local.InTag`)))
  (`|ExecutionSequence`
    (:`then_0`
      (if (`BlueprintMapLibrary.Map_IsEmpty` (`self.ScreenNotifications`))
        (return)))
    (:`then_1`
      (if _returnvalue
        (bind _output_get (set `local.selectedWidget` _value))
        (`self.LoadScreenNotification` _output_get)))))