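; Bone-twister minigame Blueprint in which the player moves a patient joint and applies pressure to earn a rating.
; Joint input is scaled per axis by the joint's safe limit, while pressure input drives the BoneTwister state component.
; Once pressure execution is confirmed, release plays a rating-based finisher, whose end stops and clears the minigame.
; It also feeds the end screen, commits the rating to game state and provides camera shakes.
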(event `self.OnDisplayEndScreen`
  (params (screen :type "UserWidget Object Reference"))
  (bind _aswbp_pressure_mode_end_screen (cast `/Game/Blueprints/HUD/Game_PressureMode/WBP_PressureMode_EndScreen` screen))
  (`/Game/Blueprints/HUD/Game_PressureMode/WBP_PressureMode_EndScreen.Initialize` _aswbp_pressure_mode_end_screen (`self.GetJoint`) (`/Game/Blueprints/Gameflow/MiniGame/B_MiniGameStateComponent.GetRating` (`self.minigameState`))))

(event `self.FinisherHandlerComponent.OnFinisherEnd`
  (`self.Stop`)
  (`KismetSystemLibrary.Delay` 0.1)
  (`self.ClearByTransition` 0.75))

(event `ApplyPressure`
  (`/Game/Blueprints/Gameflow/MiniGame/B_MiniGameStateComponent_BoneTwister.AddPressure` (`self.minigameState`) false))

(event `HoldPressure`
  (if (not (`self.bGameEndConfirmation`))
    (bind _success (`/Game/Blueprints/Gameflow/MiniGame/B_MiniGameStateComponent_BoneTwister.ExecutePressure` (`self.minigameState`)))
    (if _success
      (set `self.bGameEndConfirmation` true)
      (`/Game/Blueprints/Gameflow/MiniGame/B_MiniGameStateComponent_BoneTwister.ReadyPressure` (`self.minigameState`)))))

(event `ReleasePressure`
  (if (`self.bGameEndConfirmation`)
    (`/Game/Assets/VFX/Finisher/B_FinisherHandlerComponent.StartFinisherSequence` (`self.FinisherHandlerComponent`) (`self.GetRatingTag`))
    (else
      (`/Game/Blueprints/Gameflow/MiniGame/B_MiniGameStateComponent_BoneTwister.ReleasePressure` (`self.minigameState`)))))

(event `ApplyJointMovement`
  (params (InDirection :type "Vector2D Structure"))
  (if (`self.IsGameActive`)
    (`/Game/Blueprints/Interactables/BP_ChiropractorPoint.MoveJoint` (`self.GetJoint`) InDirection (`KismetMathLibrary.GetAbs2D` (/ (`.safeLimit_3_EF976C614C11A2F94B65DE85F5B0B9C1` (break `/Game/Blueprints/Patient/STR_RotateBoneLimits` (`/Game/Blueprints/Patient/B_PatientJointComponent.limits` (`/Game/Blueprints/Interactables/BP_ChiropractorPoint.PatientJointComponent` (`self.GetJoint`))))) (`self.InputLimit`))))))

(fn `SendRating`
  (`|ExecutionSequence`
    (:`then_0`
      (`/Game/Blueprints/Gameflow/B_GameStats.CountRating` (`/Game/Blueprints/Gameflow/GS_GameStateCustom.stats` (`/Game/Blueprints/Core/Utilities/BP_Utils.Game State`)) (`/Game/Blueprints/Gameflow/MiniGame/B_MiniGameStateComponent.GetRating` (`self.minigameState`))))
    (:`then_1`
      (`/Game/Blueprints/Gameflow/GS_GameStateCustom.CommitFlow` (`/Game/Blueprints/Core/Utilities/BP_Utils.Game State`) self))))

(fn `Start`
  (params (joint :type "/Game/Blueprints/Interactables/BP_ChiropractorPoint Object Reference") (controller :type "Controller Object Reference"))
  (returns (success :type Boolean))
  (`|ExecutionSequence`
    (:`then_0`
      (bind _success (`parent.Start` (`local.joint`) (`local.controller`)))
      (if (not _success)
        (return false)))
    (:`then_1`
      (bind _asminigamestate_bonetwister (cast `/Game/Blueprints/Gameflow/MiniGame/B_MiniGameStateComponent_BoneTwister` (`self.GetState`))
        (:`then`
          (set `self.minigameState` _asminigamestate_bonetwister))
        (:`CastFailed`
          (return false))))
    (:`then_2`
      (return true))))

(fn `UserConstructionScript`
  (`parent.UserConstructionScript`))