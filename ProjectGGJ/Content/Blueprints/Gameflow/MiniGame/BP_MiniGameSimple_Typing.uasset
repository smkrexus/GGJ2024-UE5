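; Simple typing minigame that has the player press a randomized key sequence within a timed round.
; Start builds key pools from the input mapping, then picks keys with a capped number of digits.
; SendInput checks each press in order, while a typing view model receives inputs, timer progress and results.
; Any miss or unfinished sequence fails; a flawless one gets a random choice of two ratings.
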(event `self.ReceiveTick`
  (params (DeltaSeconds :type "Float (single-precision)"))
  (bind __roundtimer (`self._roundTimer`))
  (if (`self.IS_ROUND_ACTIVE`)
    (`/Game/Blueprints/Gameflow/MiniGame/ViewModel/B_VM_MiniGameSimple_Typing.VM_SetRoundProgress` (`self.vm_typing`) (- 1.0 (`/Game/Blueprints/Core/Utilities/BP_Utils.GetTimerInfo` __roundtimer)) (`KismetSystemLibrary.K2_GetTimerRemainingTimeHandle` __roundtimer))))

(event `OnCompleted`
  (`self.CompletedSummary`)
  (`self.Stop`))

(event `OnCompletedFail`
  (`self.SetRating` "NewEnumerator4")
  (`/Game/Blueprints/Gameflow/MiniGame/ViewModel/B_VM_MiniGameSimple_Typing.VM_SetRoundSuccess` (`self.vm_typing`) false)
  (`self.Stop`))

(event `OnInputPressed`
  (params (Index :type Integer) (bSuccess :type Boolean))
  (`/Game/Blueprints/Gameflow/MiniGame/ViewModel/B_VM_MiniGameSimple_Typing.VM_RegisterInput` (`self.vm_typing`) Index bSuccess))

(event `self.OnNotifyReceivedEvent_ViewModel`
  (params (tag :type "GameplayTag Structure"))
  (`|SwitchGameplayTag` tag
    (:`ViewModel.Common.Remove`
      (`self.Clear`))))

(fn `ClearLatestInput`
  (bind __keyssuccess (`self._keysSuccess`))
  (`KismetArrayLibrary.Array_Remove` __keyssuccess (`KismetArrayLibrary.Array_LastIndex` __keyssuccess))
  (`/Engine/EditorBlueprintResources/StandardMacros.DecrementInt` (`self._inputIndex`)
    (:`  `
      (`/Game/Blueprints/Gameflow/MiniGame/ViewModel/B_VM_MiniGameSimple_Typing.VM_ClearLastInput` (`self.vm_typing`)))))

(fn `CompletedSummary`
  (for _array_element (`self._keysSuccess`)
    (if (not _array_element)
      (`/Game/Blueprints/Gameflow/MiniGame/ViewModel/B_VM_MiniGameSimple_Typing.VM_SetRoundSuccess` (`self.vm_typing`) false)
      (`self.SetRating` "NewEnumerator4")
      (return)))
  (`self.SetRating` (`KismetArrayLibrary.Array_Random` (`|MakeArray` "NewEnumerator1" "NewEnumerator2" :!type "/Game/Blueprints/Gameflow/MiniGame/Scoring/E_MiniGame_Rating Enum")))
  (`/Game/Blueprints/Gameflow/MiniGame/ViewModel/B_VM_MiniGameSimple_Typing.VM_SetRoundSuccess` (`self.vm_typing`) true))

(fn `EndRound`
  (`KismetSystemLibrary.K2_ClearAndInvalidateTimerHandle` (`self._roundTimer`))
  (`self.SetActorTickEnabled` false)
  (if (> (`self._inputIndex`) (`KismetArrayLibrary.Array_LastIndex` (`self._keysRandomized`)))
    (`self.OnCompleted`)
    (else
      (`self.OnCompletedFail`))))

(fn `RandomizeKeys`
  (params (InputCount :type Integer))
  (locals (selectedKey :type "Key Structure" :default "None") (keyNumberCount :type Integer) (keyDisplayNames :type Text) (inputs :type "Array of Text"))
  (set `self._inputIndex` 0)
  (`KismetArrayLibrary.Array_Clear` (`self._keysSuccess`))
  (`KismetArrayLibrary.Array_Clear` (`self._keysRandomized`))
  (for _ (range (`local.InputCount`))
    (`|ExecutionSequence`
      (:`then_0`
        ;[1 1 1] Random if should choose number
        (if (`KismetMathLibrary.RandomBool`)
          (if (< (`local.keyNumberCount`) (`self.NumberLimit`))
            (set `local.selectedKey` (`KismetArrayLibrary.Array_Random` (`self._keysNumbersAvailable`)))
            (`/Engine/EditorBlueprintResources/StandardMacros.IncrementInt` (`local.keyNumberCount`))
            (else
              (set `local.selectedKey` (`KismetArrayLibrary.Array_Random` (`self._keysAvailable`)) :!label _label)))
          (else
            (goto _label))))
      (:`then_1`
        (`KismetArrayLibrary.Array_Add` (`self._keysRandomized`) (`local.selectedKey`))
        (`KismetArrayLibrary.Array_Add` (`local.inputs`) (`KismetInputLibrary.Key_GetDisplayName` (`local.selectedKey`))))))
  (`/Game/Blueprints/Gameflow/MiniGame/ViewModel/B_VM_MiniGameSimple_Typing.VM_SetInputs` (`self.vm_typing`) (`local.inputs`))
  (`self.StartRound`))

(fn `SendInput`
  (params (InKey :type "Key Structure" :default "None"))
  (returns (OutSuccess :type Boolean))
  (locals (success :type Boolean :default false))
  (`|ExecutionSequence`
    (:`then_0`
      (if (not (`self.IS_ROUND_ACTIVE`))
        (return false)))
    (:`then_1`
      (if (not (`KismetArrayLibrary.Array_IsValidIndex` (`self._keysRandomized`) (`self._inputIndex`)))
        (return false)))
    (:`then_2`
      (bind _output_get (set `local.success` (== (`KismetInputLibrary.Key_GetDisplayName` (`local.InKey`)) (`KismetInputLibrary.Key_GetDisplayName` (`|GetArrayItem` (`self._keysRandomized`) (`self._inputIndex`))))))
      (bind _returnvalue (`KismetArrayLibrary.Array_Add` (`self._keysSuccess`) _output_get))
      (`self.OnInputPressed` _returnvalue (`local.success`)))
    (:`then_3`
      (`/Engine/EditorBlueprintResources/StandardMacros.IncrementInt` (`self._inputIndex`)
        (:`  `
          (if (> (`self._inputIndex`) (`KismetArrayLibrary.Array_LastIndex` (`self._keysRandomized`)))
            (`self.EndRound`)))))
    (:`then_4`
      (return (`local.success`)))))

(fn `Start`
  (params (InController :type "PlayerController Object Reference"))
  (locals (numberDescription :type Text :default "NSLOCTEXT(\"[05A8860A8AA8557A623418760897D245]\", \"990DD1464DC695191ED58B956DB73182\", \"number\")"))
  (`parent.Start` InController)
  (`|ExecutionSequence`
    (:`then_0`
      ;[1 1 1] changing input mapping can result in different keys
      (for _array_element (`.Mappings` (break `InputMappingContextMappingData` (`InputMappingContext.DefaultKeyMappings` (`|GetArrayItem` (`/Game/Blueprints/Core/Inputs/B_InputController_Base.InputMaps` (`self.GetInputController`))))))
        (bind ((`Action` _action) (`Key` _key)) (break `EnhancedActionKeyMapping` _array_element))
        (if (== (`InputAction.ActionDescription` _action) (`local.numberDescription`))
          (`KismetArrayLibrary.Array_Add` (`self._keysNumbersAvailable`) _key)
          (else
            (`KismetArrayLibrary.Array_Add` (`self._keysAvailable`) _key)))))
    (:`then_1`
      (bind _asb_vm_mini_game_simple_typing (cast `/Game/Blueprints/Gameflow/MiniGame/ViewModel/B_VM_MiniGameSimple_Typing` (`self.GetViewModel`)))
      (set `self.vm_typing` _asb_vm_mini_game_simple_typing))
    (:`then_2`
      (`self.RandomizeKeys` (`self.KeyCount`)))))

(fn `StartRound`
  (bind _returnvalue (`KismetSystemLibrary.K2_SetTimerDelegate` (`|CreateDelegate` :!event `EndRound`) (`self.RoundTime`)))
  (set `self._roundTimer` _returnvalue)
  (`self.SetActorTickEnabled` true)
  (`/Game/Blueprints/Core/ViewModel/B_VM_BaseComponent.ForceRefresh` (`self.vm_typing`)))

(fn `UserConstructionScript`
  (`parent.UserConstructionScript`))