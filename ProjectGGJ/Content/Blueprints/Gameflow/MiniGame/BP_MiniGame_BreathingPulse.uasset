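; Breathing pulse minigame Blueprint, in which mouse input moves a patient's joint and a press releases it and stops the game.
; Start runs the parent setup and caches the BreathingPulse state component, failing if either step fails.
; SendRating logs the adjustment and rating to game stats, changes patient pain by rating plus the profile's bone modifier, then commits the game flow.
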(event `/Game/Blueprints/Pawn/BPI_ExternalInputHandler.MiniGameBeginPress`
  (`/Game/Blueprints/Interactables/BP_ChiropractorPoint.ReleaseJoint` (`self.GetJoint`))
  (`self.Stop`))

(event `/Game/Blueprints/Pawn/BPI_ExternalInputHandler.OnReceiveMouseInput`
  (params (lookDirection :type "Vector2D Structure"))
  (`/Game/Blueprints/Interactables/BP_ChiropractorPoint.MoveJoint` (`self.GetJoint`) lookDirection))

(fn `SendRating`
  (bind _rating (`/Game/Blueprints/Gameflow/MiniGame/B_MiniGameStateComponent.GetRating` (`self.minigameState`)))
  (bind _patient (`/Game/Blueprints/Interactables/BP_ChiropractorPoint.GetOwningPatient` (`self.GetJoint`)))
  (bind _stats (`/Game/Blueprints/Gameflow/GS_GameStateCustom.stats` (`/Game/Blueprints/Core/Utilities/BP_Utils.Game State`)))
  (`|ExecutionSequence`
    (:`then_0`
      (`/Game/Blueprints/Gameflow/B_GameStats.CountAdjustment` _stats))
    (:`then_1`
      (`/Game/Blueprints/Gameflow/B_GameStats.CountRating` :`self` _stats :`rating` _rating))
    (:`then_2`
      (`/Game/Blueprints/Core/Stats/B_Stat.Change` (`/Game/Blueprints/Patient/BP_Patient.Pain` _patient) (+ (select `/Game/Blueprints/Gameflow/MiniGame/Scoring/E_MiniGame_Rating` _rating :`NewEnumerator0` 1.0 :`NewEnumerator1` -0.25 :`NewEnumerator2` -1.0) (`/Game/Blueprints/Patient/BP_PatientProfile.GetPainModifierFromBone` (`/Game/Blueprints/Patient/BP_Patient.GetPatientProfile` _patient) (`/Game/Blueprints/Interactables/BP_ChiropractorPoint.boneName` (`self.GetJoint`))))) ; make as funciton
    )
    (:`then_3`
      (`/Game/Blueprints/Gameflow/GS_GameStateCustom.CommitFlow` (`/Game/Blueprints/Core/Utilities/BP_Utils.Game State`) self))))

(fn `Start`
  (params (joint :type "/Game/Blueprints/Interactables/BP_ChiropractorPoint Object Reference") (controller :type "Controller Object Reference"))
  (returns (success :type Boolean))
  (`|ExecutionSequence`
    (:`then_0`
      (bind _success (`parent.Start` (`local.joint`) (`local.controller`)))
      (if (not _success)
        (return false)))
    (:`then_1`
      (bind _asminigamestate_breathingpulse (cast `/Game/Blueprints/Gameflow/MiniGame/B_MiniGameStateComponent_BreathingPulse` (`self.GetState`))
        (:`then`
          (set `self.minigameState` _asminigamestate_breathingpulse))
        (:`CastFailed`
          (return false))))
    (:`then_2`
      (return true))))

(fn `UserConstructionScript`
  (`parent.UserConstructionScript`))