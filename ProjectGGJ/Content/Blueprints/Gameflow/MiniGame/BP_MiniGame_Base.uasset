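; Base actor for a mini-game played on a patient's joint, from start through rating.
; Start sets player mode, focuses the joint, adds input plus class-loaded view model and state components, then blends to a camera randomly placed in a cone toward the player.
; Finisher events bind the patient and switch to cinematic mode.
; Stop shows the end screen; clearing restores mode and input, applies the rating to patient stats and social interest, then destroys the actor.
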(event `ClearByTransition`
  (params (BlendTime :type "Float (single-precision)"))
  (bind _returnvalue (`GameplayStatics.GetPlayerController` 0))
  (`PlayerController.SetViewTargetWithBlend` _returnvalue (`Controller.K2_GetPawn` _returnvalue) BlendTime "VTBlend_EaseInOut" 5.0 false)
  (`KismetSystemLibrary.K2_SetTimerDelegate` (`|CreateDelegate` :!event `ClearOnTransitionEnd`) BlendTime))

(event `ClearOnTransitionEnd`
  (`self.K2_DestroyActor` (`self.GameCamera`))
  (`self.Clear`))

(event `OnDisplayEndScreen`
  (params (screen :type "UserWidget Object Reference")))

(event `self.FinisherHandlerComponent.OnDisplayFinisherEffect`
  (bind _controller (`self.GetOwningController`))
  (bind (_returnvalue_location _returnvalue_rotation) (`KismetMathLibrary.BreakTransform` (`SceneComponent.K2_GetComponentToWorld` (`self.GetComponentByClass` (`Controller.K2_GetPawn` _controller) "/Script/Engine.CameraComponent"))))
  (`/Game/Blueprints/Core/ViewModel/B_VM_BaseComponent.SetWidgetVisible` (`self.GetViewModel`) false)
  (`/Game/Blueprints/Player/ViewModel/B_VM_PlayerState.VM_SetCurrentMode` (`self.vm_playerState`) (struct :`TagName` "ViewModel.PlayerState.Modes.Cinematic"))
  (`/Game/Blueprints/Patient/B_PatientJointComponent.EnableAnimation` (`/Game/Blueprints/Interactables/BP_ChiropractorPoint.PatientJointComponent` (`self.GetJoint`)) (`self.GetOwningController`))
  (`/Game/Blueprints/Gameflow/MiniGame/B_MiniGameStateComponent.AttemptUnloadState` (`self.state`))
  (`PlayerController.SetAudioListenerOverride` (cast `PlayerController` _controller :!pure true) null _returnvalue_location _returnvalue_rotation) ; force location before camera animation takes over
)

(event `self.FinisherHandlerComponent.OnModifyFinisherSequenceInfo`
  (bind _outproxy (`/Game/Blueprints/Patient/BP_Patient.SetCinematicProxySettings` (`/Game/Blueprints/Interactables/BP_ChiropractorPoint.GetOwningPatient` (`self.targetJoint`)) (`.customTags_7_19B5CF194D880B98AFDB24B379D0C240` (break `/Game/Assets/VFX/Finisher/STR_FinisherSettings` (`/Game/Assets/VFX/Finisher/B_FinisherHandlerComponent.GetFinisherSettings` (`self.FinisherHandlerComponent`))))))
  (`/Game/Assets/VFX/Finisher/B_FinisherHandlerComponent.ModifyFinisherBindings` (`self.FinisherHandlerComponent`) "Target" (`|MakeArray` _outproxy :!type "Actor Object Reference"))
  (`/Game/Assets/VFX/Finisher/B_FinisherHandlerComponent.ModifyFinisherTransform` (`self.FinisherHandlerComponent`) (`self.GetTransform` (`/Game/Blueprints/Interactables/BP_ChiropractorPoint.GetOwningPatient` (`self.targetJoint`)))) ; subject is patient, so use patient as the origin\nonly works for finishers with non fixed origin
)

(fn `Assign State`
  (params (Class :type "Object Class Reference"))
  (returns (bSuccess :type Boolean))
  (bind _asactor_component (castclass `ActorComponent` Class)
    (:`then`
      (bind _returnvalue (`|AddComponentByClass` _asactor_component))
      (bind _asminigamestate_base (cast `/Game/Blueprints/Gameflow/MiniGame/B_MiniGameStateComponent` _returnvalue)
        (:`then`
          (set `self.state` _asminigamestate_base)
          (return true))
        (:`CastFailed`
          (return false))))
    (:`CastFailed`
      (return false))))

(fn `Clear`
  (`|ExecutionSequence`
    (:`then_0`
      (if (`/Game/Blueprints/HUD/Utilities/BP_Utilities_Widget.IsTrailerMode`)
        (`/Game/Blueprints/Player/ViewModel/B_VM_PlayerState.VM_SetCurrentMode` (`self.vm_playerState`) (struct :`TagName` "ViewModel.PlayerState.Modes.Cinematic"))
        (else
          (`/Game/Blueprints/Player/ViewModel/B_VM_PlayerState.VM_SetCurrentMode` (`self.vm_playerState`) (struct :`TagName` "ViewModel.PlayerState.Modes.Game"))))
      (`/Game/Blueprints/Core/Inputs/B_InputController_Base.RemoveInputs` (`self.input`) true)
      (`self.SendRating`))
    (:`then_1`
      (`/Engine/EditorBlueprintResources/ActorMacros.Switch Has Authority`
        (:`Authority`
          (`self.K2_DestroyActor`) ; temp
        )))))

(fn `DisplayEndScreen`
  (`|ExecutionSequence`
    (:`then_0`
      ;[1 1 1] don't display if trailer mode is active
      (if (`/Game/Blueprints/HUD/Utilities/BP_Utilities_Widget.IsTrailerMode`)
        (return)))
    (:`then_1`
      (bind _endscreenwidget (`self.endScreenWidget`)
        (:`then`
          (bind _returnvalue (`KismetSystemLibrary.LoadClassAsset_Blocking` _endscreenwidget))
          (bind _returnvalue_2 (`|GenericCreateObject` _returnvalue))
          (bind _asuser_widget (cast `UserWidget` _returnvalue_2))
          (`UserWidget.AddToViewport` _asuser_widget 0)
          (`self.OnDisplayEndScreen` _asuser_widget))
        (:`else`)))))

(fn `GetInputController`
  (returns (OutController :type "/Game/Blueprints/Core/Inputs/B_InputController_Base Object Reference"))
  (return (`self.input`)))

(fn `GetJoint`
  (returns (targetJoint :type "/Game/Blueprints/Interactables/BP_ChiropractorPoint Object Reference"))
  (return (`self.targetJoint`)))

(fn `GetOwningController`
  (returns (controller :type "Controller Object Reference"))
  (return (`self.owningController`)))

(fn `GetRatingTag`
  (returns (OutRatingTag :type "GameplayTag Structure"))
  (return (select `/Game/Blueprints/Gameflow/MiniGame/Scoring/E_MiniGame_Rating` (`/Game/Blueprints/Gameflow/MiniGame/B_MiniGameStateComponent.GetRating` (`self.state`)) :`NewEnumerator0` (struct :`TagName` "MiniGame.Shared.Rating.Bad") :`NewEnumerator1` (struct :`TagName` "MiniGame.Shared.Rating.Good") :`NewEnumerator2` (struct :`TagName` "MiniGame.Shared.Rating.Excellent") :!type "GameplayTag Structure")))

(fn `GetState`
  (returns (state :type "/Game/Blueprints/Gameflow/MiniGame/B_MiniGameStateComponent Object Reference"))
  (return (`self.state`)))

(fn `GetViewModel`
  (returns (viewModel :type "/Game/Blueprints/Core/ViewModel/B_VM_BaseComponent Object Reference"))
  (return (`self.loadedViewModel`)))

(fn `IsGameActive`
  (returns (IsActive :type Boolean))
  (return (not (`self.bIsEnded`))))

(fn `IsGameEnded`
  (returns (IsEnded :type Boolean))
  (return (`self.bIsEnded`)))

(fn `SendRating`
  (`|ExecutionSequence`
    (:`then_0`
      (if (`|EnumEquality` (`/Game/Blueprints/Gameflow/MiniGame/B_MiniGameStateComponent.GetRating` (`self.state`)) "NewEnumerator0")
        (`/Game/Blueprints/Core/Stats/B_StatComponent.ChangeStatFromTag` (`/Game/Blueprints/Patient/BP_Patient.PatientStatComponent` (`/Game/Blueprints/Interactables/BP_ChiropractorPoint.GetOwningPatient` (`self.GetJoint`))) -35.0 (struct :`TagName` "Stats.Patient.Comfort"))))
    (:`then_1`
      (`/Game/Blueprints/Patient/Stats/B_CounterComponent_Patient.CountAdjustment` (`/Game/Blueprints/Patient/BP_Patient.PatientCounterComponent` (`/Game/Blueprints/Interactables/BP_ChiropractorPoint.GetOwningPatient` (`self.GetJoint`))) (`/Game/Blueprints/Gameflow/MiniGame/B_MiniGameStateComponent.GetRating` (`self.state`))))
    (:`then_2`
      (`/Game/Blueprints/Core/Utilities/BP_UtilsMacro.AddSocialMediaInterest` 20))))

(fn `Start`
  (params (joint :type "/Game/Blueprints/Interactables/BP_ChiropractorPoint Object Reference") (controller :type "Controller Object Reference"))
  (returns (success :type Boolean))
  (locals (pawnController :type "/Game/Blueprints/Pawn/BP_PawnControllerCustom Object Reference"))
  (bind _returnvalue (`self.K2_GetActorLocation` (`self.GetJoint`)))
  (bind (_returnvalue_x _returnvalue_y _returnvalue_z) (`KismetMathLibrary.BreakVector` (`KismetMathLibrary.RandomUnitVectorInConeInDegrees` (- (`SceneComponent.K2_GetComponentLocation` (`self.GetComponentByClass` (`Controller.K2_GetPawn` (`self.GetOwningController`)) "/Script/Engine.CameraComponent")) (`self.K2_GetActorLocation` (`self.GetJoint`))) 30.0)))
  (bind _returnvalue_2 (+ _returnvalue (* (`KismetMathLibrary.MakeVector` _returnvalue_x _returnvalue_y (`KismetMathLibrary.Abs` _returnvalue_z)) 50.0)))
  (bind _output_get (set `self.owningController` (`local.controller`)))
  (bind _output_get_2 (set `self.vm_playerState` (`/Game/Blueprints/Core/Utilities/BP_Utils.GetPlayerStateViewFromController` _output_get)))
  (`/Game/Blueprints/Player/ViewModel/B_VM_PlayerState.VM_SetCurrentMode` _output_get_2 (struct :`TagName` "ViewModel.PlayerState.Modes.MiniGame"))
  (`|ExecutionSequence`
    (:`then_0`
      (set `self.targetJoint` (`local.joint`))
      (`/Game/Blueprints/Patient/B_PatientJointComponent.EnableFocus` (`/Game/Blueprints/Interactables/BP_ChiropractorPoint.PatientJointComponent` (`local.joint`)) (`self.GetOwningController`)))
    (:`then_1`
      (if (`KismetSystemLibrary.IsValidClass` (`self.InputController`))
        (bind _outinputcontroller (`/Game/Blueprints/Core/Utilities/BP_Utils.AddInputController` (`self.GetOwningController`) (`self.InputController`) self))
        (set `self.input` _outinputcontroller)
        (else
          (`KismetSystemLibrary.PrintString` "error, no input map specified" true true (struct :`R` 1.0 :`B` 0.025572 :`A` 1.0))
          (return false))))
    (:`then_2`
      (bind _viewmodelclass (`self.viewModelClass`)
        (:`then`
          (bind _returnvalue_3 (`KismetSystemLibrary.LoadClassAsset_Blocking` _viewmodelclass))
          (bind _returnvalue_4 (`|AddComponentByClass` (castclass `ActorComponent` _returnvalue_3 :!pure true)))
          (bind _asviewmodel_base (cast `/Game/Blueprints/Core/ViewModel/B_VM_BaseComponent` _returnvalue_4))
          (set `self.loadedViewModel` _asviewmodel_base))
        (:`else`)))
    (:`then_3`
      (bind _stateclass (`self.stateClass`)
        (:`then`
          (bind _returnvalue_5 (`KismetSystemLibrary.LoadClassAsset_Blocking` _stateclass))
          (bind _bsuccess (`self.Assign State` _returnvalue_5))
          (if _bsuccess
            (`/Game/Blueprints/Gameflow/MiniGame/B_MiniGameStateComponent.InitializeState` (`self.state`) self)
            (else
              (return false))))
        (:`else`
          (return false))))
    (:`then_4`
      (bind _returnvalue_6 (`|SpawnActorFromClass` "/Game/Assets/VFX/Camera/BP_Camera_Joint.BP_Camera_Joint_C" (`KismetMathLibrary.MakeTransform` _returnvalue_2 (`KismetMathLibrary.FindLookAtRotation` _returnvalue_2 _returnvalue)) "Undefined" "MultiplyWithRoot" null null))
      (bind _output_get_3 (set `self.GameCamera` _returnvalue_6))
      (`PlayerController.SetViewTargetWithBlend` (`GameplayStatics.GetPlayerController` 0) _output_get_3 0.5 "VTBlend_EaseInOut" 5.0 false)
      (return true))))

(fn `Stop`
  (bind _controller (`self.GetOwningController`))
  (bind _controller_2 (`self.GetOwningController`))
  (bind _patientjointcomponent (`/Game/Blueprints/Interactables/BP_ChiropractorPoint.PatientJointComponent` (`self.GetJoint`)))
  (`|ExecutionSequence`
    (:`then_0`
      (set `self.bIsEnded` true)
      (`/Game/Blueprints/Gameflow/MiniGame/B_MiniGameStateComponent.AttemptUnloadState` (`self.state`))
      (`PlayerController.SetAudioListenerOverride` :`self` (cast `PlayerController` _controller :!pure true) :`AttachToComponent` (`self.GetComponentByClass` (`Controller.K2_GetPawn` _controller) "/Script/Engine.CameraComponent")) ; set back to itself
    )
    (:`then_1`
      (`self.DisplayEndScreen`))
    (:`then_2`
      (`/Game/Blueprints/Gameflow/MiniGame/B_MiniGameStateComponent.RemoveState` (`self.state`)) ; clean up
      (`/Game/Blueprints/Patient/B_PatientJointComponent.DisableAnimation` _patientjointcomponent _controller_2)
      (`/Game/Blueprints/Patient/B_PatientJointComponent.DisableFocus` _patientjointcomponent _controller_2))))

(fn `UserConstructionScript`)