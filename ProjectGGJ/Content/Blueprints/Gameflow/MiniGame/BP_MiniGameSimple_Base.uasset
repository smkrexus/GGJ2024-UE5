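; Base actor for simple minigames, managing their input, UI and lifecycle, with a stored rating and auto-clear flag.
; Start adds a configurable input component to the player controller and a view-model component to itself, shows its widget, binds notify events and sets MiniGame mode.
; Stop restores Game mode, removes inputs and calls the stop callback, while Clear removes the view and destroys the actor.
; The view-model notify handlers are empty stubs.
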(event `OnNotifyReceivedEvent_ViewModel`
  (params (tag :type "GameplayTag Structure")))

(event `OnNotifyReceived_ViewModel`
  (params (identifier :type Name)))

(fn `Clear`
  (`/Game/Blueprints/Core/ViewModel/B_VM_BaseComponent.RemoveView` (`self.GetViewModel`))
  (`self.K2_DestroyActor`))

(fn `GetController`
  (returns (OutController :type "PlayerController Object Reference"))
  (return (`self._playerController`)))

(fn `GetInputController`
  (returns (OutController :type "/Game/Blueprints/Core/Inputs/B_InputController_Base Object Reference"))
  (return (`self._inputController`)))

(fn `GetRating`
  (returns (OutRating :type "/Game/Blueprints/Gameflow/MiniGame/Scoring/E_MiniGame_Rating Enum"))
  (return (`self._rating`)))

(fn `GetViewModel`
  (returns (OutViewModel :type "/Game/Blueprints/Core/ViewModel/B_VM_BaseComponent Object Reference"))
  (return (`self._viewModel`)))

(fn `IsAutoClear`
  (returns (OutValid :type Boolean))
  (return (`self.bAutoClear`)))

(fn `SetRating`
  (params (InRating :type "/Game/Blueprints/Gameflow/MiniGame/Scoring/E_MiniGame_Rating Enum" :default "NewEnumerator0"))
  (set `self._rating` InRating))

(fn `Start`
  (params (InController :type "PlayerController Object Reference"))
  (bind _outviewmodel (`self.GetViewModel`))
  (set `self._playerController` InController)
  (`|ExecutionSequence`
    (:`then_0`
      (if (`KismetSystemLibrary.IsValidClass` (`self.InputClass`))
        (bind _returnvalue (`|AddComponentByClass` (`local.InController`) (`self.InputClass`)))
        (bind _output_get (set `self._inputController` _returnvalue))
        (`/Game/Blueprints/Core/Inputs/B_InputController_Base.ActivateInputs` _output_get (`local.InController`))
        (`/Game/Blueprints/Core/Inputs/B_InputController_Base.RegisterTargetForInput` _output_get self)))
    (:`then_1`
      (if (`KismetSystemLibrary.IsValidClass` (`self.ViewModelClass`))
        (bind _returnvalue_2 (`|AddComponentByClass` (`self.ViewModelClass`)))
        (bind _output_get_2 (set `self._viewModel` _returnvalue_2))
        (bind _view (`/Game/Blueprints/Core/ViewModel/B_VM_BaseComponent.CreateView` _output_get_2 (`/Game/Blueprints/Core/ViewModel/B_VM_BaseComponent.GetDefaultWidget` _output_get_2)))
        (`UserWidget.AddToViewport` _view 0)
        (message `/Game/Blueprints/Core/ViewModel/BPI_Widget_ViewModel.AddViewModel` _view (`self._viewModel`))
        (add `/Game/Blueprints/Core/ViewModel/B_VM_BaseComponent.OnNotifyEvent` _outviewmodel (`|CreateDelegate` :!event `OnNotifyReceivedEvent_ViewModel`))
        (add `/Game/Blueprints/Core/ViewModel/B_VM_BaseComponent.OnNotifyVariable` _outviewmodel (`|CreateDelegate` :!event `OnNotifyReceived_ViewModel`))))
    (:`then_2`
      (set `self.vm_playerState` (`/Game/Blueprints/Core/Utilities/BP_Utils.GetPlayerStateViewFromController` (`local.InController`)))
      (`/Game/Blueprints/Player/ViewModel/B_VM_PlayerState.VM_SetCurrentMode` (`self.vm_playerState`) (struct :`TagName` "ViewModel.PlayerState.Modes.MiniGame")))))

(fn `Stop`
  (`/Game/Blueprints/Player/ViewModel/B_VM_PlayerState.VM_SetCurrentMode` (`self.vm_playerState`) (struct :`TagName` "ViewModel.PlayerState.Modes.Game"))
  (`/Game/Blueprints/Core/Inputs/B_InputController_Base.RemoveInputs` (`self.GetInputController`) true)
  (`self.OnStop`))

(fn `UserConstructionScript`)