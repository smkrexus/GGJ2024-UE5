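; Custom game state for a chiropractic game, tracking the current patient, activated treatment points and gameflow stats.
; Construction creates attention, intensity and complaint stats; Tick advances the attention and complaint timers, while intensity ticking is disconnected.
; The attention interval handler flags a random chiropractic point, up to a fixed cap, skipping any already needing attention.
; It also exposes point removal, a player state getter and a CommitFlow dispatcher call for minigames.
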(event `self.ReceiveTick`
  (params (DeltaSeconds :type "Float (single-precision)"))
  (`|ExecutionSequence`
    (:`then_0`
      (`/Game/Blueprints/Gameflow/BP_Stat.Tick` (`self.attentionTimer`) DeltaSeconds))
    (:`then_2`
      (`/Game/Blueprints/Gameflow/BP_Stat.Tick` (`self.complaintTimer`) DeltaSeconds))))

(fn `CommitFlow`
  (params (miniGame :type "/Game/Blueprints/Gameflow/MiniGame/BP_MiniGame_Base Object Reference"))
  (`self.OnCommitFlow` miniGame))

(fn `Current Player State`
  (returns (`Player State` :type "/Game/Blueprints/BP_PlayerStateCustom Object Reference"))
  (bind _asbp_player_state_custom (cast `/Game/Blueprints/BP_PlayerStateCustom` (`GameplayStatics.GetPlayerState` 0)))
  (return _asbp_player_state_custom))

(fn `OnAttentionTimerInterval`
  (locals (selectedPoint :type "/Game/Blueprints/Interactables/BP_ChiropractorPoint Object Reference"))
  (if (<= (`KismetArrayLibrary.Array_Length` (`self.activatedPoints`)) 3)
    (bind _output_get (set `local.selectedPoint` (`KismetArrayLibrary.Array_Random` (`self.chiropracticPoints`))))
    (if (not (`/Game/Blueprints/Interactables/BP_ChiropractorPoint.IsRequiringAttention` (`local.selectedPoint`)))
      (`/Game/Blueprints/Interactables/BP_ChiropractorPoint.CreateAttention` _output_get)
      (`KismetArrayLibrary.Array_Add` (`self.activatedPoints`) (`local.selectedPoint`)))))

(fn `RemoveActivatedPoint`
  (params (pointToRemove :type "/Game/Blueprints/Interactables/BP_ChiropractorPoint Object Reference"))
  (bind _activatedpoints (`self.activatedPoints`))
  (if (`KismetArrayLibrary.Array_IsNotEmpty` _activatedpoints)
    (`KismetArrayLibrary.Array_RemoveItem` _activatedpoints (`local.pointToRemove`))))

(fn `Set Patient`
  (params (`New Patient` :type "/Game/Blueprints/BP_Patient Object Reference"))
  (set `self.currentPatient` `New Patient`))

(fn `UserConstructionScript`
  (`|ExecutionSequence`
    (:`then_0`
      (bind _created_stat (`/Game/Blueprints/Gameflow/BP_Utils.Create Stat` "NewEnumerator2" self))
      (bind _output_get (set `self.attentionTimer` _created_stat))
      (`/Game/Blueprints/Gameflow/BP_Stat.Begin Tick` _output_get "Forward")
      (add `/Game/Blueprints/Gameflow/BP_Stat.OnTimerInterval` _output_get (`|CreateDelegate` :!event `OnAttentionTimerInterval`)))
    (:`then_1`
      (bind _created_stat_2 (`/Game/Blueprints/Gameflow/BP_Utils.Create Stat` "NewEnumerator4" self))
      (set `self.intensity` _created_stat_2))
    (:`then_2`
      (bind _created_stat_3 (`/Game/Blueprints/Gameflow/BP_Utils.Create Stat` "NewEnumerator8" self))
      (set `self.complaintTimer` _created_stat_3))))