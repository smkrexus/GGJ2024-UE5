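; BP_Stats tracks gameflow statistics: a score, an adjustment count and a complaint count.
; On BeginPlay it constructs a BP_PatientStats object and creates a stat owned by itself to serve as the Score.
; CountAdjustment and CountComplaint increment their counters, while CountRating maps a rating to a point value and applies it to Score.
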(event `self.ReceiveBeginPlay`
  (`|ExecutionSequence`
    (:`then_0`
      (bind _returnvalue (`|GenericCreateObject` "/Game/Blueprints/Gameflow/BP_PatientStats.BP_PatientStats_C"))
      (set `self.Patient Stats` _returnvalue))
    (:`then_1`
      (bind _created_stat (`/Game/Blueprints/Gameflow/BP_Utils.Create Stat` "NewEnumerator1" self))
      (set `self.Score` _created_stat))))

(fn `CountAdjustment`
  (bind _result (`/Engine/EditorBlueprintResources/StandardMacros.IncrementInt` (`self.NumAdjustments`))
    (:`  `
      (set `self.NumAdjustments` _result))))

(fn `CountComplaint`
  (bind _result (`/Engine/EditorBlueprintResources/StandardMacros.IncrementInt` (`self.Num Complaints`))
    (:`  `
      (set `self.Num Complaints` _result))))

(fn `CountRating`
  (params (data :type "/Game/Blueprints/Gameflow/MiniGame/STR_MiniGame_Attribute Structure") (rating :type "/Game/Blueprints/Gameflow/MiniGame/Scoring/E_MiniGame_Rating Enum" :default "NewEnumerator0"))
  (`/Game/Blueprints/Gameflow/BP_Stat.Change` (`self.Score`) (select `/Game/Blueprints/Gameflow/MiniGame/Scoring/E_MiniGame_Rating` rating :`NewEnumerator0` 1.0 :`NewEnumerator1` 5.0 :`NewEnumerator2` 10.0)))