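; Custom GameState that runs a scenario workday with streaming and social-media influence, tracking time, missions, game events and noise.
; Components report through events: time of day drives the scenario manager, event and follower changes raise notifications, and excess noise triggers a restart.
; A game-state view model relays state and responds to gameplay-tagged pause, passive and end notifications.
; Day end compiles component saves and builds a summary, overwriting the save only on the final day.
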(event `self.ReceiveBeginPlay`
  (bind _returnvalue (`GameplayStatics.GetPlayerController` 0))
  (bind _gamescenariomanager (`self.GameScenarioManager`))
  (bind (_outstart _outend) (`/Game/Blueprints/Gameflow/Components/B_GameTimeOfDay.GetTimeOfDayRange` (`self.GameTimeOfDay`)))
  (add `/Game/Blueprints/Gameflow/GM_GGJ2024_Base.OnGameModeComplete` (`/Game/Blueprints/Core/Utilities/BP_Utils.Game Mode`) (`|CreateDelegate` :!event `OnDisplayEndSummary`))
  (`/Engine/EditorBlueprintResources/StandardMacros.IsValid` (`self.GetComponentByClass` _returnvalue "/Game/Blueprints/Player/ViewModel/B_VM_Player.B_VM_Player_C")
    (:`Is Valid`
      _)
    (:`Is Not Valid`
      (bind _asbp_pawn_controller_custom (cast `/Game/Blueprints/Pawn/BP_PawnControllerCustom` _returnvalue))
      (add `/Game/Blueprints/Pawn/BP_PawnControllerCustom.OnPlayerViewLoaded` _asbp_pawn_controller_custom (`|CreateDelegate` :!event `OnPlayerViewReady`)) ; controller has not initialized fully, so bind to that, should use component for loading issues in future\nOnLoaded (GameplayTag) seems better
    ))
  (`/Game/Blueprints/Gameflow/ViewModel/B_VM_GameState.VM_SetWorkRange` (`self.ViewModel_GameState`) _outstart _outend)
  (`/Game/Blueprints/Gameflow/ViewModel/B_VM_GameState.VM_SetCurrentDay` (`self.ViewModel_GameState`) (`/Game/Blueprints/Gameflow/Components/B_GameScenarioManager.GetCurrentDay` _gamescenariomanager) (`/Game/Blueprints/GameScenario/PDA_ScenarioDefinition.Days` (`/Game/Blueprints/Gameflow/Components/B_GameScenarioManager.GetScenarioDefinition` _gamescenariomanager))))

(event `OnPlayerViewReady`
  (`/Game/Blueprints/Core/ViewModel/B_VM_BaseComponent.ForceRefresh` (`self.ViewModel_GameState`))
  ;[1 1 1] Track score in display in-game
  (bind _asgi_uncertified (cast `/Game/Blueprints/Gameflow/GI_Uncertified` (`GameplayStatics.GetGameInstance`)))
  (bind _output_get (set `self._gameInstance` _asgi_uncertified))
  (bind _outmission (`/Game/Blueprints/Gameflow/Save/B_SaveGame_Scenario_Base.GetMission` (`/Game/Blueprints/Gameflow/GI_Uncertified.ScenarioSave` _output_get)))
  (`/Engine/EditorBlueprintResources/StandardMacros.IsValid` _outmission
    (:`Is Valid`
      (`/Game/Blueprints/Core/Objective/B_Objective_Base.Start` _outmission self)
      (`/Game/Blueprints/Gameflow/ViewModel/B_VM_GameState.VM_AddMission` (`self.GetViewModel`) _outmission))))

(event `self.ViewModel_GameState.OnNotifyEvent`
  (params (tag :type "GameplayTag Structure"))
  (bind _gametimeofday (`self.GameTimeOfDay`))
  ;[1 1 1 1 60] GAMESTATE EVENTS
  (`|SwitchGameplayTag` tag
    (:`GameMode.Pause`
      (`GameplayStatics.SetGlobalTimeDilation` (select `bool` (`/Game/Blueprints/Gameflow/ViewModel/B_VM_GameState.VM_GetGamePaused` (`self.ViewModel_GameState`)) :`false` 1.0 :!type "Float (single-precision)")))
    (:`GameMode.End`
      (`/Game/Blueprints/Gameflow/Components/B_GameTimeOfDay.Stop` (`self.GameTimeOfDay`)))
    (:`GameMode.Passive`
      (if (`/Game/Blueprints/Gameflow/ViewModel/B_VM_GameState.VM_GetGamePassive` (`self.ViewModel_GameState`))
        (`/Game/Blueprints/Gameflow/Components/B_GameTimeOfDay.Pause` _gametimeofday)
        (else
          (`/Game/Blueprints/Gameflow/Components/B_GameTimeOfDay.Resume` _gametimeofday))))))

(event `self.B_SocialMediaInfluenceComponent.OnFollowersUpdated`
  (`/Game/Blueprints/SocialMedia/B_SocialMediaNotificationComponent.DisplayNotification` (`self.B_SocialMediaNotificationComponent`) "" 0.0 (struct :`TagName` "GameMode.Notification.SocialMedia.Follower") "/Game/Blueprints/SocialMedia/Channel/B_NotificationChannelMessage_SocialMedia_Follower.B_NotificationChannelMessage_SocialMedia_Follower_C" true null))

(event `self.GameEventAttributes.OnStatsInitialized`
  ;[1 0.8206 0 1 36] GLOBAL EVENTS
  (`/Game/Blueprints/Gameflow/Components/B_GameEvents.CreateEvents` (`self.GameEvents`) (`self.GameEventAttributes`) (`/Game/Blueprints/Gameflow/Components/B_GameScenarioManager.GetScenarioDefinition` (`self.GameScenarioManager`))))

(event `self.GameEvents.OnEventReminder`
  (params (InTag :type "GameplayTag Structure"))
  ;[1 0.8206 0 1 36] GLOBAL EVENTS
  (`|SwitchGameplayTag` InTag
    (:`Scenario.GameEvents.Latency`
      (`/Game/Blueprints/SocialMedia/B_SocialMediaNotificationComponent.DisplayNotification` (`self.B_SocialMediaNotificationComponent`) "" 0.0 (struct :`TagName` "Scenario.GameEvents.Latency") "/Game/Blueprints/SocialMedia/Channel/B_NotificationChannelMessage_SocialMedia_Admin.B_NotificationChannelMessage_SocialMedia_Admin_C" true null))))

(event `OnDisplayEndSummary`
  (bind _vm_summary (`self.vm_summary`))
  (bind _view (`/Game/Blueprints/Core/ViewModel/B_VM_BaseComponent.CreateView` _vm_summary (`/Game/Blueprints/Core/ViewModel/B_VM_BaseComponent.GetDefaultWidget` _vm_summary)))
  (`WidgetBlueprintLibrary.SetInputMode_UIOnlyEx` (`GameplayStatics.GetPlayerController` 0) _view)
  (`UserWidget.AddToViewport` _view 0)
  (`/Game/Blueprints/Core/ViewModel/B_VM_BaseComponent.ForceRefresh` (`self.vm_summary`)))

(event `self.GameEvents.OnEventActive`
  (params (InTag :type "GameplayTag Structure"))
  ;[1 0.8206 0 1 36] GLOBAL EVENTS
  (`|SwitchGameplayTag` InTag
    (:`Scenario.GameEvents.Latency`
      (`/Game/Blueprints/SocialMedia/B_SocialMediaNotificationComponent.DisplayNotification` (`self.B_SocialMediaNotificationComponent`) "" 0.0 (struct :`TagName` "Scenario.GameEvents.Latency") "/Game/Blueprints/SocialMedia/Channel/B_NotificationChannelMessage_SocialMedia_Admin.B_NotificationChannelMessage_SocialMedia_Admin_C" true null))))

(event `self.GameEvents.OnEventLevelChanged`
  (params (InTag :type "GameplayTag Structure") (InLevel :type Integer))
  ;[1 0.8206 0 1 36] GLOBAL EVENTS
)

(event `self.GameEvents.OnEventInactive`
  (params (InTag :type "GameplayTag Structure"))
  ;[1 0.8206 0 1 36] GLOBAL EVENTS
  (`|SwitchGameplayTag` InTag
    (:`Scenario.GameEvents.Latency`
      (`/Game/Blueprints/SocialMedia/B_SocialMediaNotificationComponent.DisplayNotification` (`self.B_SocialMediaNotificationComponent`) "" 0.0 (struct :`TagName` "Scenario.GameEvents.Latency.End") "/Game/Blueprints/SocialMedia/Channel/B_NotificationChannelMessage_SocialMedia_Admin.B_NotificationChannelMessage_SocialMedia_Admin_C" true null))))

(event `self.GameDecibels.OnReachedThreshold`
  (`/Game/Blueprints/Gameflow/Components/B_GameRestarter.Restart` (`self.GameRestarter`) "Too much noise"))

(event `self.GameRestarter.OnRestartSuccess`
  (`/Game/Blueprints/Core/ViewModel/BP_Gameflow_ViewModel.Clear` (`/Game/Blueprints/HUD/Utilities/BP_Utilities_Widget.GlobalViewModelSystem`)))

(event `self.GameRestarter.OnRestartComplete`
  (`/Game/Blueprints/Gameflow/Components/B_GameDecibels.ResetDecibels` (`self.GameDecibels`))
  (`/Game/Blueprints/Core/ViewModel/BP_Gameflow_ViewModel.Reset` (`/Game/Blueprints/HUD/Utilities/BP_Utilities_Widget.GlobalViewModelSystem`)))

(event `self.B_SocialMediaInfluenceComponent.OnStreamStateChanged`
  (params (bIsStreaming :type Boolean))
  (bind _gamestateview (`self.GetViewModel`))
  ;[0.07292 0.05984 0] Stream On/Off - Add Blackboard to track multiple states
  (if bIsStreaming
    (`/Game/Blueprints/Gameflow/ViewModel/B_VM_GameState.VM_AddBlackboardState` _gamestateview (struct :`TagName` "Stream.Flow"))
    (else
      (`/Game/Blueprints/Gameflow/ViewModel/B_VM_GameState.VM_RemoveBlackboardState` _gamestateview (struct :`TagName` "Stream.Flow")))))

(event `self.GameTimeOfDay.OnDayProgressTick`
  (params (InHour :type Integer) (InMinutes :type Integer))
  (`/Game/Blueprints/Gameflow/ViewModel/B_VM_GameState.VM_SetWorkTime` (`self.ViewModel_GameState`) InHour InMinutes))

(event `self.GameTimeOfDay.OnDayComplete`
  (`/Game/Blueprints/Gameflow/Components/B_GameScenarioManager.EndWork` (`self.GameScenarioManager`)))

(event `self.GameScenarioManager.OnWorkEnd`
  (`/Game/Blueprints/Gameflow/ViewModel/B_VM_GameState.VM_SetScenarioClosure` (`self.ViewModel_GameState`) (`/Game/Blueprints/Gameflow/Components/B_GameScenarioManager.CloseScenarioDuration` (`self.GameScenarioManager`)))
  (`/Game/Blueprints/SocialMedia/B_SocialMediaInfluenceComponent.EndStream` (`self.B_SocialMediaInfluenceComponent`))
  (bind _returnvalue (`|AddComponentByClass` "/Game/Blueprints/GameScenario/Summary/B_VM_ScenarioSummary.B_VM_ScenarioSummary_C"))
  (set `self.vm_summary` _returnvalue)
  (`/Game/Blueprints/Gameflow/ViewModel/B_VM_GameState.VM_SetGameEnded` (`self.ViewModel_GameState`)))

(event `self.GameScenarioManager.OnRequestCompileSave`
  (`self.CompileSaveData`) ; calls save on all related components, this updates scenario saves for any object to reference its data\nthis does not override save data until end session is called below
)

(event `self.GameScenarioManager.OnScenarioEnd`
  (params (InRemainingDays :type Integer))
  (bind _vm_summary (`self.vm_summary`))
  (`|ExecutionSequence`
    (:`then_0`
      (`/Game/Blueprints/GameScenario/Summary/B_VM_ScenarioSummary.VM_SetProgressScore` _vm_summary (`self.GameScenarioCounter`))
      (`/Game/Blueprints/GameScenario/Summary/B_VM_ScenarioSummary.VM_SetProgressScenario` _vm_summary (`self.GameScenarioManager`)))
    (:`then_1`
      (`/Game/Blueprints/Core/Objective/B_Objective_Base.Cleanup` (`/Game/Blueprints/Gameflow/Save/B_SaveGame_Scenario_Base.GetMission` (`/Game/Blueprints/Gameflow/GI_Uncertified.ScenarioSave` (`self._gameInstance`))))
      (`/Game/Blueprints/Gameflow/GM_GGJ2024_Base.EndSession` (`/Game/Blueprints/Core/Utilities/BP_Utils.Game Mode`) true))
    (:`then_2`
      ;[1 1 1] Overwrite save file only if final day
      (if (<= InRemainingDays 0)
        (message `/Game/Blueprints/Gameflow/Save/BPI_SaveGame.Save` (`GameplayStatics.GetGameInstance`))))))

(fn `CompileSaveData`
  (`/Game/Blueprints/Gameflow/Save/BPI_SaveGame.Save` (`self.B_SocialMediaInfluenceComponent`))
  (`/Game/Blueprints/Gameflow/Save/BPI_SaveGame.Save` (`self.GameScenarioManager`))
  (`/Game/Blueprints/Gameflow/Save/BPI_SaveGame.Save` (`self.GameScenarioCounter`)))

(fn `GetGameEvents`
  (returns (OutGameEvents :type "/Game/Blueprints/Gameflow/Components/B_GameEvents Object Reference") (OutGameEventStats :type "/Game/Blueprints/Core/Stats/B_StatComponent Object Reference"))
  (return (`self.GameEvents`) (`self.GameEventAttributes`)))

(fn `GetInfluenceComponent`
  (returns (OutComponent :type "/Game/Blueprints/SocialMedia/B_SocialMediaInfluenceComponent Object Reference"))
  (return (`self.B_SocialMediaInfluenceComponent`)))

(fn `GetScenarioComponents`
  (returns (OutManager :type "/Game/Blueprints/Gameflow/Components/B_GameScenarioManager Object Reference") (OutCounter :type "/Game/Blueprints/Gameflow/Components/B_GameScenarioCounter Object Reference"))
  (return (`self.GameScenarioManager`) (`self.GameScenarioCounter`)))

(fn `GetSocialMediaFeedComponent`
  (returns (OutComponent :type "/Game/Blueprints/SocialMedia/B_SocialMediaFeedComponent Object Reference"))
  (return (`self.B_SocialMediaFeedComponent`)))

(fn `GetTimeOfDayComponent`
  (returns (OutComponent :type "/Game/Blueprints/Gameflow/Components/B_GameTimeOfDay Object Reference"))
  (return (`self.GameTimeOfDay`)))

(fn `GetViewModel`
  (returns (GameStateView :type "/Game/Blueprints/Gameflow/ViewModel/B_VM_GameState Object Reference"))
  (return (`self.ViewModel_GameState`)))

(fn `UserConstructionScript`)