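; Game instance that owns the game's two save objects, one global and one for the scenario.
; On Init it loads both from the slot names in their class defaults, or deletes and recreates them when ResetSaveOnStart is set.
; A failed load has no fallback to create a new save object.
; StartScenario deletes and recreates only the scenario save, leaving the global save untouched.
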(event `self.ReceiveInit`
  (`self.Load`))

(event `/Game/Blueprints/Gameflow/Save/BPI_SaveGame.Load`
  (bind (_dayspassed _subcribersgained _adjustments _objectivecompleteday _objectivecompleteobjectives _objectiveperfectobjectives _slotname) (defaults `Object` (`self.ScenarioSaveClass`)))
  (bind (_socialmedia _slotname_2) (defaults `Object` (`self.GlobalSaveClass`)))
  (`|ExecutionSequence`
    (:`then_0`
      (if (`self.bResetSaveOnStart`)
        (`GameplayStatics.DeleteGameInSlot` _slotname_2)
        (bind _returnvalue (`GameplayStatics.CreateSaveGameObject` (`self.GlobalSaveClass`)))
        (set `self.GlobalSave` _returnvalue)
        (else
          (bind _returnvalue_2 (`GameplayStatics.LoadGameFromSlot` _slotname_2))
          (bind _asb_save_game_global (cast `/Game/Blueprints/Gameflow/Save/B_SaveGame_Global` _returnvalue_2))
          (set `self.GlobalSave` _asb_save_game_global))))
    (:`then_1`
      (if (`self.bResetSaveOnStart`)
        (`GameplayStatics.DeleteGameInSlot` _slotname)
        (bind _returnvalue_3 (`GameplayStatics.CreateSaveGameObject` (`self.ScenarioSaveClass`)))
        (set `self.ScenarioSave` _returnvalue_3)
        (else
          (bind _returnvalue_4 (`GameplayStatics.LoadGameFromSlot` _slotname))
          (bind _asb_save_game_scenario_base (cast `/Game/Blueprints/Gameflow/Save/B_SaveGame_Scenario_Base` _returnvalue_4))
          (set `self.ScenarioSave` _asb_save_game_scenario_base))))))

(fn `StartScenario`
  (`GameplayStatics.DeleteGameInSlot` (defaults `Object` (`self.ScenarioSaveClass`)))
  (bind _returnvalue (`GameplayStatics.CreateSaveGameObject` (`self.ScenarioSaveClass`)))
  (set `self.ScenarioSave` _returnvalue))