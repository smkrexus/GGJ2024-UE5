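; Cooldown component that tracks whether a timed cooldown is active on its owner.
; SetCooldown starts a one-shot timer and sets the IsCooldown flag, and OnCooldownEnd clears both the flag and the timer handle.
; GetStatus returns the flag, and GetCooldownTime reports elapsed and remaining time, or zeros when the timer handle is invalid.
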(event `OnCooldownEnd`
  (set `self.isCooldown` false)
  (`KismetSystemLibrary.K2_ClearAndInvalidateTimerHandle` (`self.timer`)))

(fn `GetCooldownTime`
  (returns (elapsed :type "Float (double-precision)") (remaining :type "Float (double-precision)"))
  (bind _timer (`self.timer`))
  (if (`KismetSystemLibrary.K2_IsValidTimerHandle` _timer)
    (return (`KismetSystemLibrary.K2_GetTimerElapsedTimeHandle` _timer) (`KismetSystemLibrary.K2_GetTimerRemainingTimeHandle` _timer))
    (else
      (return 0.0 0.0))))

(fn `GetStatus`
  (returns (isCooldown :type Boolean))
  (return (`self.isCooldown`)))

(fn `SetCooldown`
  (params (Time :type "Float (single-precision)"))
  (bind _returnvalue (`KismetSystemLibrary.K2_SetTimerDelegate` (`|CreateDelegate` :!event `OnCooldownEnd`) Time))
  (set `self.timer` _returnvalue)
  (set `self.isCooldown` true))