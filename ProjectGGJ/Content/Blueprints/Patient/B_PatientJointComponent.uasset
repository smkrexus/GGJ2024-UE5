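; Patient joint component that keeps a bone's accumulated rotation within a safe limit.
; LimitBoneRotation adds the input to the current rotation and clamps the result to a radius taken from the X value of the safe limit.
; It returns the previous rotation minus the clamped one, intended to be zero once the joint is at its limit.
; The event graph is unused.
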(fn `LimitBoneRotation`
  (params (input :type "Vector2D Structure"))
  (returns (boneRotation :type "Vector2D Structure"))
  (locals (initialRotation :type "Vector2D Structure") (tempRotation :type "Vector2D Structure"))
  (`|ExecutionSequence`
    (:`then_0`
      (set `local.initialRotation` (`self.currentRotation`)))
    (:`then_1`
      (set `self.currentRotation` (`/Game/Blueprints/Gameflow/BP_Utils.ClampAxisToRadius` (+ (`local.input`) (`self.currentRotation`)) (`KismetMathLibrary.BreakVector2D` (`.safeLimit_3_EF976C614C11A2F94B65DE85F5B0B9C1` (break `/Game/Blueprints/Patient/STR_RotateBoneLimits` (`self.limits`)))))))
    (:`then_2`
      (return (- (`local.initialRotation`) (`self.currentRotation`))))))