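; BP_PatientProfile generates and holds a randomized patient health profile that maps issue types to affected bones.
; CreateRandomProfile builds three HealthSummary entries with random rates, then uses each rate to size random picks from the supplied bones.
; Picks use AddUnique, so repeats can leave fewer issues than the rate implies.
; Lookups return a summary by issue type and translate bone names to basic names through the HealthNames data table.
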(fn `CreateRandomProfile`
  (params (availableBones :type "Array of Name"))
  (locals (bonesToChoose :type Integer))
  (bind _healthsummary (`self.healthSummary`))
  (`self.DefineHealthSummary`)
  (for (_array_element _array_index) _healthsummary
    (bind _output_get (set `local.bonesToChoose` (`KismetMathLibrary.FTrunc` (* (`KismetArrayLibrary.Array_Length` (`local.availableBones`)) (`.rate_7_BC590F0548EDB8C01C3E4CBC8E1F6218` (break `/Game/Blueprints/Patient/STR_PatientHealthSummary` _array_element))))))
    (if (> _output_get 0)
      (for _ (range (`local.bonesToChoose`))
        (bind (_output_type _output_rate _output_issues) (break `/Game/Blueprints/Patient/STR_PatientHealthSummary` (`|GetArrayItem` _healthsummary _array_index)))
        (`KismetArrayLibrary.Array_AddUnique` _output_issues (`KismetArrayLibrary.Array_Random` (`local.availableBones`)))))))

(fn `DefineHealthSummary`
  (`KismetArrayLibrary.Array_Add` (`self.healthSummary`) (make `/Game/Blueprints/Patient/STR_PatientHealthSummary` "NewEnumerator0" (`KismetMathLibrary.RandomFloatInRange` 0.4 0.7) (`|MakeArray`)))
  (`KismetArrayLibrary.Array_Add` (`self.healthSummary`) (make `/Game/Blueprints/Patient/STR_PatientHealthSummary` "NewEnumerator1" (`KismetMathLibrary.RandomFloatInRange` 0.4 0.7) (`|MakeArray`)))
  (`KismetArrayLibrary.Array_Add` (`self.healthSummary`) (make `/Game/Blueprints/Patient/STR_PatientHealthSummary` "NewEnumerator2" (`KismetMathLibrary.RandomFloatInRange` 0.4 0.7) (`|MakeArray`))))

(fn `GetBasicName`
  (params (boneName :type Name))
  (returns (basicName :type String))
  (locals (healthNames :type "DataTable Object Reference" :default "/Script/Engine.DataTable'/Game/Blueprints/Patient/DT_HealthNames.DT_HealthNames'") (rowData :type "/Game/Blueprints/Patient/STR_HealthBasicNames Structure"))
  (bind _healthnames (`local.healthNames`))
  (bind _outrownames (`DataTableFunctionLibrary.GetDataTableRowNames` _healthnames))
  (for _array_element _outrownames
    (bind _returnvalue (`|GetDataTableRow` _healthnames _array_element)
      (:`then`
        (bind _output_get (set `local.rowData` _returnvalue))
        (if (== (break `/Game/Blueprints/Patient/STR_HealthBasicNames` _output_get) (`local.boneName`))
          (return (`.basicName_6_7379D97F4B87453D71F11C9C577E762D` (break `/Game/Blueprints/Patient/STR_HealthBasicNames` _output_get))))))))

(fn `GetHealthIssue`
  (params (issueType :type "/Game/Blueprints/Patient/Enum_PatientIssueType Enum" :default "NewEnumerator0"))
  (returns (issueSummary :type "/Game/Blueprints/Patient/STR_PatientHealthSummary Structure") (valid :type Boolean))
  (locals (element :type Integer))
  (bind _healthsummary (`self.healthSummary`))
  (bind _element (`local.element`))
  (for (_array_element _array_index) _healthsummary
    (if (`|EnumEquality` (break `/Game/Blueprints/Patient/STR_PatientHealthSummary` _array_element) (`local.issueType`))
      (set `local.element` _array_index)))
  (if (`KismetArrayLibrary.Array_IsValidIndex` _healthsummary _element)
    (return (`|GetArrayItem` _healthsummary _element) true)
    (else
      (return (struct) false))))