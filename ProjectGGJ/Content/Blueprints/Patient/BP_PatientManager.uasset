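; BP_PatientManager is the patient manager, owning a view model that backs the local player's "info_tag" UI slot.
; On BeginPlay it polls the local player controller on a timer until initialization validates, then creates the view model and adds it to the player's view model component.
; RegisterPatient only initializes the patient, while UnregisterPatient removes it from the view model.
; Getters expose the view model and the initialized flag.
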(event `self.ReceiveBeginPlay`
  (if (`Controller.IsLocalController` (`GameplayStatics.GetPlayerController` 0))
    (`self.ValidateController`)))

(event `ValidateController`
  (bind _outvalidated (message `/Game/Blueprints/Gameflow/Components/BPI_Gameflow_Validator.ValidateInitialization` (`GameplayStatics.GetPlayerController` 0)))
  (if _outvalidated
    (`self.ValidateControllerSuccess`)
    (else
      (`KismetSystemLibrary.K2_SetTimerDelegate` (`|CreateDelegate` :!event `ValidateController`) 0.5))))

(event `ValidateControllerSuccess`
  (bind _returnvalue (`|AddComponentByClass` "/Game/Blueprints/Patient/ViewModel/B_VM_PatientManager.B_VM_PatientManager_C"))
  (set `self.vm_patientManager` _returnvalue)
  (`/Game/Blueprints/Player/ViewModel/B_VM_Player.VM_AddExtension` (`self.GetComponentByClass` (`GameplayStatics.GetPlayerController` 0) "/Game/Blueprints/Player/ViewModel/B_VM_Player.B_VM_Player_C") "info_tag" (`self.vm_patientManager`))
  (set `self.bHasInitialized` true))

(fn `GetViewModel`
  (returns (OutViewModel :type "/Game/Blueprints/Patient/ViewModel/B_VM_PatientManager Object Reference"))
  (return (`self.vm_patientManager`)))

(fn `RegisterPatient`
  (params (InPatient :type "/Game/Blueprints/Patient/BP_Patient Object Reference"))
  (`/Game/Blueprints/Patient/BP_Patient.Initialize` InPatient))

(fn `UnregisterPatient`
  (params (InPatient :type "/Game/Blueprints/Patient/BP_Patient Object Reference"))
  (`/Game/Blueprints/Patient/ViewModel/B_VM_PatientManager.VM_RemovePatient` (`self.vm_patientManager`) InPatient))

(fn `UserConstructionScript`)

(fn `ValidateInitialization`
  (returns (OutValidated :type Boolean))
  (return (`self.bHasInitialized`)))