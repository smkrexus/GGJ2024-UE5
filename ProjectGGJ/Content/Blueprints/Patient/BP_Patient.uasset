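; BP_Patient is a chiropractic patient actor that runs one treatment session from random injury-profile setup to review and cleanup.
; It polls dependency readiness before registering with PatientManager, then generates skeleton joints and moves through preparation, examination and adjustment flows.
; Components handle poses, proximity context options, stats, complaints, emotes and social-media objectives, updating a patient view model.
; Session end scores comfort, grants rewards, files a summary and posts a review while streaming.
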(event `self.PatientStatComponent.OnStatEmpty`
  (params (statTag :type "GameplayTag Structure"))
  (`|SwitchGameplayTag` statTag
    (:`Stats.Patient.Comfort`
      (`/Game/Blueprints/Patient/ViewModel/B_VM_Patient.VM_ObjectiveComplete` (`self.vm_patient`) false (`|MakeArray` "Patient lost patience!" :!type "Text")) ; see if can also disable objective completion at this point
      (`/Game/Blueprints/Patient/Session/B_PatientSessionManager.EndSession` (`self.PatientSessionManager`)))))

(event `self.PatientStatComponent.OnStatChanged`
  (params (statTag :type "GameplayTag Structure"))
  (`|SwitchGameplayTag` statTag
    (:`Stats.Patient.Comfort`
      (`self.UPDATE_STAT_COMFORT`))))

(event `/Game/Blueprints/Room/BPI_RoomItemSystem.AddRoom`
  (params (InRoom :type "/Game/Blueprints/Room/BP_Room_Base Object Reference"))
  (set `self._roomOwner` InRoom))

(event `RemovePatient`
  (bind (_outrating _outmax) (`/Game/Blueprints/Patient/Session/B_PatientSessionManager.GetReviewRating` (`self.PatientSessionManager`)))
  ;[0.07292 0.05984 0 1 36] FLOW: CLEANUP (Patient leaves)
  (`|ExecutionSequence`
    (:`then_0`
      (`/Game/Blueprints/Patient/BP_PatientManager.UnregisterPatient` (`self._patientManager`) self)
      (bind _currenttable (`self.CurrentTable`)
        (:`then`
          (`/Game/Blueprints/Interactables/Ingredients/AdjustmentTable/BP_ING_AdjustmentTable.RemoveUser` _currenttable))
        (:`else`)))
    (:`then_1`
      (`/Game/Blueprints/Patient/Session/B_PatientSessionManager.CalculateReviewRating` (`self.PatientSessionManager`) (`/Game/Blueprints/Core/Stats/B_StatComponent.GetStatFromTag` (`self.PatientStatComponent`) (struct :`TagName` "Stats.Patient.Comfort")))
      (`/Game/Blueprints/Patient/Stats/B_CounterComponent_Patient.CompileScores` (`self.PatientCounterComponent`))
      (`self.SetLifeSpan` 1.0)
      (`/Game/Blueprints/Patient/B_PatientJointManager.ClearGeneratedJoints` (`self.PatientJointManager`) 1.0) ; delay for other actors to de-reference eg. minigame
    )
    (:`then_2`
      (message `/Game/Blueprints/Core/Rewards/BPI_Rewarder.GiveRewards` (`self.ObjectiveComponent_Patient`) (`GameplayStatics.GetGameState`))
      (bind _outactors (`GameplayStatics.GetAllActorsOfClassWithTag` "/Game/Blueprints/Interactables/Ingredient_FileCabinet/BP_ING_FileCabinet_Base.BP_ING_FileCabinet_Base_C" "TempTag"))
      (bind _output (`|GetArrayItem` _outactors))
      (`/Engine/EditorBlueprintResources/StandardMacros.IsValid` _output
        (:`Is Valid`
          (bind _asbp_part_file_cabinet_drawer (cast `/Game/Blueprints/Interactables/Ingredient_FileCabinet/BP_Part_FileCabinet_Drawer` (`ChildActorComponent.ChildActor` (`/Game/Blueprints/Interactables/Ingredient_FileCabinet/BP_ING_FileCabinet_Base.Drawer_01` _output))))
          (bind _outactor (`/Game/Blueprints/Interactables/Ingredient_FileCabinet/BP_Part_FileCabinet_Drawer.Place` _asbp_part_file_cabinet_drawer "/Game/Blueprints/Patient/Session/5_Summary/BP_PatientSessionSummary.BP_PatientSessionSummary_C")) ; TEMP: drops a review into the cabinet
          (`/Game/Blueprints/Patient/Session/5_Summary/BP_PatientSessionSummary.DisplaySummary` (cast `/Game/Blueprints/Patient/Session/5_Summary/BP_PatientSessionSummary` _outactor :!pure true) self)
          ; Stream must be ongoing social media notification
          (if (`self.GET_STREAM_STATE`)
            (`|ExecutionSequence`
              (:`then_0`
                (bind _outinfo (`/Game/Blueprints/SocialMedia/B_SocialMediaNotificationComponent.AddCustomInfo` (`self.SocialMediaNotificationComponent`) "/Game/Blueprints/SocialMedia/Channel/B_NotificationChannelMessageInfo_SocialMedia_Review.B_NotificationChannelMessageInfo_SocialMedia_Review_C"))
                (bind _associalmediainforeview (cast `/Game/Blueprints/SocialMedia/Channel/B_NotificationChannelMessageInfo_SocialMedia_Review` _outinfo :!pure true))
                (`/Game/Blueprints/SocialMedia/Channel/B_NotificationChannelMessageInfo_SocialMedia_Review.SetReviewRating` _associalmediainforeview _outrating _outmax)
                (`/Game/Blueprints/SocialMedia/B_SocialMediaNotificationComponent.DisplayNotification` (`self.SocialMediaNotificationComponent`) "" 0.0 (`/Game/Blueprints/SocialMedia/Channel/B_NotificationChannelMessageInfo_SocialMedia_Review.GetReviewNotificationTag` _associalmediainforeview) "/Game/Blueprints/SocialMedia/Channel/B_NotificationChannelMessage_SocialMedia_Review.B_NotificationChannelMessage_SocialMedia_Review_C" true _outinfo)))))))))

(event `self.ReceiveBeginPlay`
  ;[1 0.8808 0.185 1 36] FLOW: SETUP & INITIALIZATION
  (bind _returnvalue (`|GenericCreateObject` "/Game/Blueprints/Patient/BP_PatientProfile.BP_PatientProfile_C"))
  (set `self._profile` _returnvalue)
  (bind _returnvalue_2 (`|AddComponentByClass` "/Game/Blueprints/Patient/ViewModel/B_VM_Patient.B_VM_Patient_C"))
  (set `self.vm_patient` _returnvalue_2)
  (`|ExecutionSequence`
    (:`then_0`
      (bind _returnvalue_3 (`GameplayStatics.GetActorOfClass` "/Game/Blueprints/Patient/BP_PatientManager.BP_PatientManager_C"))
      (set `self._patientManager` _returnvalue_3))
    (:`then_1`
      (`/Game/Blueprints/Patient/Dialogue/B_PatientDialogueComponent.AssignLocation` (`self.PatientDialogueComponent`) (+ (`self.GetBonePosition` "head") (0.0 0.0 25.0))) ; location of the speech bubble
      (`/Game/Blueprints/Interactables/B_InteractAreaComponent.AssignArea` (`self.InteractAreaComponent`) (`self.SkeletalMesh`)) ; Skeleton is an interactable but disabled at start
      (message `/Game/Blueprints/Core/Contexts/BPI_ContextSystemInterface.CreateContexts` (`self.PatientPoseManager`) (`self.Patient_ContextComponent`))
      (`/Game/Blueprints/Core/Stats/B_StatComponent.InitializeStats` (`self.PatientStatComponent`))
      (`self.UPDATE_STAT_COMFORT`)
      (`self.ValidateInitRequest`) ; this will call initialize once all references ready
    )))

(event `/Game/Blueprints/Room/BPI_RoomItemSystem.RemoveRoom`
  (params (InRoom :type "/Game/Blueprints/Room/BP_Room_Base Object Reference"))
  (if (== InRoom (`self._roomOwner`))
    (set `self._roomOwner` null)))

(event `Initialize`
  (bind ((`Min_12_8F45C98F4BABC71E0416F39725F4D52D` _min) (`Max_13_8A895D624DE880DAA7CAD194D3205837` _max)) (break `/Game/Blueprints/Core/Stats/STR_StatDef` (`/Game/Blueprints/Core/Stats/B_Stat.GetStatDefinition` (`/Game/Blueprints/Core/Stats/B_StatComponent.GetStatFromTag` (`self.PatientStatComponent`) (struct :`TagName` "Stats.Patient.Comfort")))))
  (bind _returnvalue (`KismetMathLibrary.RandomFloatInRange` _min _max))
  ;[1 0.8808 0.185 1 36] FLOW: SETUP & INITIALIZATION
  (`|ExecutionSequence`
    (:`then_0`
      (bind _outjointcollection (`/Game/Blueprints/Patient/B_PatientJointManager.GenerateJointsFromSkeleton` (`self.PatientJointManager`) (`self.SkeletalMesh`)))
      (`/Game/Blueprints/Patient/BP_PatientProfile.CreateRandomProfile` (`self._profile`) _outjointcollection)
      (`/Game/Blueprints/Patient/B_PatientJointManager.AssignJointProfile` (`self.PatientJointManager`) (`self._profile`)))
    (:`then_1`
      (`/Game/Blueprints/Patient/Poses/B_PatientPoseManager.Set New Pose` (`self.PatientPoseManager`) 0)
      (`self.RunPreparationFlow`)
      ;;[1 0.09896 0.09896] health chart is currently selected in scene, will need to re-think this later
      (bind _healthchart (`self.healthChart`)
        (:`then`
          (`/Game/Blueprints/Interactables/BP_PatientHealthChart.Initialize` _healthchart (`self._profile`)))
        (:`else`)))
    (:`then_2`
      (`/Game/Blueprints/Core/Objective/Component/B_ObjectiveComponent_Base.StartObjective` (`self.ObjectiveComponent_Patient`) self)
      (`/Game/Blueprints/Core/Objective/Component/B_ObjectiveComponent_Base.StartObjective` (`self.ObjectiveComponent_EndSession`) self)
      (`/Game/Blueprints/Core/Stats/B_Stat.SetStatValue` (`/Game/Blueprints/Core/Stats/B_StatComponent.GetStatFromTag` (`self.PatientStatComponent`) (struct :`TagName` "Stats.Patient.Comfort")) (- _returnvalue (`KismetMathLibrary.Fraction` _returnvalue)) true))))

(event `RunPreparationFlow`
  (`KismetSystemLibrary.K2_SetTimerDelegate` (`|CreateDelegate` :!event `RunStartFlow`) 5.0) ; wait awhile before starting
  (`/Game/Blueprints/Patient/Session/B_PatientTreatmentFlow_Base.RegisterForTreatment` (`self.TreatmentFlow_Examination`) (`/Game/Blueprints/Patient/B_PatientJointManager.GetInjuredJoints` (`self.PatientJointManager`)))
  (`/Game/Blueprints/Patient/ViewModel/B_VM_Patient.VM_SetPhase` (`self.vm_patient`) (struct :`TagName` "ViewModel.Patient.Phase.Preparation")))

(event `self.ObjectiveComponent_EndSession.OnPreComplete`
  (`/Game/Blueprints/Patient/Session/B_PatientSessionManager.ClearSession` (`self.PatientSessionManager`)))

(event `self.PatientPoseManager.OnPoseChanged`
  (params (oldPose :type "/Game/Blueprints/Patient/Poses/STR_PatientPoseHandle Structure") (newPose :type "/Game/Blueprints/Patient/Poses/STR_PatientPoseHandle Structure"))
  ;[1 1 1 1 24] Select New Pose
  (`/Game/Blueprints/Patient/B_PatientJointManager.RefreshJointsOnPose` (`self.PatientJointManager`) newPose)
  (`KismetSystemLibrary.DelayUntilNextTick`) ; anim update at end of frame
  (`/Game/Blueprints/Patient/Dialogue/B_PatientDialogueComponent.AssignLocation` (`self.PatientDialogueComponent`) (+ (`self.GetBonePosition` "head") (0.0 0.0 25.0))))

(event `RunStartFlow`
  (bind _currenttable (`self.CurrentTable`))
  (`/Game/Blueprints/Patient/ViewModel/B_VM_Patient.VM_SetObjective` (`self.vm_patient`) (`/Game/Blueprints/Core/Objective/Component/B_ObjectiveComponent_Base.GetObjective` (`self.ObjectiveComponent_EndSession`)))
  (`/Game/Blueprints/Patient/ViewModel/B_VM_Patient.VM_SetPhase` (`self.vm_patient`) (struct :`TagName` "ViewModel.Patient.Phase.Start"))
  (`/Game/Blueprints/Patient/Session/B_PatientSessionManager.StartSession` (`self.PatientSessionManager`)) ; prevents multiple end sessions\nfrom being called by setting a flag for start session
  (`/Engine/EditorBlueprintResources/StandardMacros.IsValid` _currenttable
    (:`Is Valid`
      (if (not (`/Game/Blueprints/Interactables/Ingredients/AdjustmentTable/BP_ING_AdjustmentTable.IsCleaned` _currenttable))
        (`/Game/Blueprints/Patient/Stats/B_CounterComponent_Patient.CountComplaint` (`self.PatientCounterComponent`))))))

(event `self.ObjectiveComponent_EndSession.OnObjectiveComplete`
  (params (InSuccess :type Boolean))
  (bind (_outsuccess _outfails) (`/Game/Blueprints/Core/Objective/B_Objective_Base.GetCompletionReasons` (`/Game/Blueprints/Core/Objective/Component/B_ObjectiveComponent_Base.GetObjective` (`self.ObjectiveComponent_EndSession`))))
  (`|ExecutionSequence`
    (:`then_0`
      (if (not InSuccess)
        (`/Game/Blueprints/Environment/Decibels/B_DecibelEmitterComponent.EmitSoundByData` (`self.DecibelEmitterComponent`) (`self._roomOwner`) "/Game/Blueprints/Environment/Decibels/Data/DA_Decibel_Patient_Leave_Angry.DA_Decibel_Patient_Leave_Angry")))
    (:`then_1`
      (`/Game/Blueprints/Patient/ViewModel/B_VM_Patient.VM_ObjectiveComplete` (`self.vm_patient`) InSuccess (select `bool` InSuccess :`false` _outfails :`true` _outsuccess))
      (`/Game/Blueprints/Patient/Session/B_PatientSessionManager.EndSession` (`self.PatientSessionManager`)))))

(event `self.TreatmentFlow_Examination.OnRegisterFlow`
  ;[1 0.8206 0 1 36] FLOW: EXAMINATION
  (`/Game/Blueprints/Patient/ViewModel/B_VM_Patient.VM_SetTreatmentPhase` (`self.vm_patient`) (struct :`TagName` "ViewModel.Patient.Phase.Examination")))

(event `self.PatientSessionManager.OnSessionStart`
  ;[0.07292 0.05984 0 1 36] FLOW: SESSION MAIN
  (`/Game/Blueprints/Core/Objective/Context/B_ObjectiveContextGenerator.GenerateObjective` (`self.B_ObjectiveGeneratorComponent_Base`) "/Game/Blueprints/SocialMedia/Objectives/B_Objective_SocialMedia.B_Objective_SocialMedia_C" (`self.PatientCounterComponent`) true))

(event `self.PatientSessionManager.OnSessionCleanup`
  ;[0.07292 0.05984 0 1 36] FLOW: SESSION MAIN
  (`/Game/Blueprints/Patient/Session/B_PatientTreatmentFlow_Base.ClearTreatment` (`self.TreatmentFlow_Adjustment`)))

(event `self.SceneTracker_PatientLocator.OnRangeDetected`
  (params (player :type "Pawn Object Reference"))
  (bind _patient_contextcomponent (`self.Patient_ContextComponent`))
  ;[1 1 1 1 24] Tracking & Proximity
  (if (not (`/Game/Blueprints/Core/Contexts/B_ContextComponent.IsContextActive` (`self.Patient_ContextComponent`)))
    (`/Game/Blueprints/Core/Contexts/B_ContextComponent.AddToScreen` _patient_contextcomponent (`self.GetController` player) "contextOptions")
    (`/Game/Blueprints/Core/Contexts/B_ContextComponent.SetContextActive` _patient_contextcomponent true)))

(event `self.TreatmentFlow_Examination.OnExaminationComplete`
  ;[1 0.8206 0 1 36] FLOW: EXAMINATION
  (`PrimitiveComponent.SetCollisionResponseToChannel` (`self.SkeletalMesh`) "ECC_GameTraceChannel1" "ECR_Block") ; temporarily use character as collision for interaction
)

(event `self.PatientSessionManager.OnSessionEnd`
  ;[0.07292 0.05984 0 1 36] FLOW: SESSION MAIN
  (`/Game/Blueprints/Core/Objective/Context/B_ObjectiveContextGenerator.ClearAllObjectives` (`self.B_ObjectiveGeneratorComponent_Base`))
  (`/Game/Blueprints/Patient/B_PatientJointManager.CleanupGeneratedJoints` (`self.PatientJointManager`))
  (message `/Game/Blueprints/Core/Contexts/BPI_ContextSystemInterface.ClearContexts` (`self.PatientPoseManager`) (`self.Patient_ContextComponent`))
  (`/Game/Blueprints/Core/Contexts/B_ContextComponent.SetContextActive` (`self.Patient_ContextComponent`) false)
  (`/ActorTracker/Blueprints/B_SceneTracker_Base.SetTrackingEnabled` (`self.SceneTracker_PatientLocator`) false)
  (`PrimitiveComponent.SetCollisionResponseToChannel` (`self.SkeletalMesh`) "ECC_GameTraceChannel1" "ECR_Ignore") ; this may not have been disabled if chiro session not begun but examination completed
  (`self.RemovePatient`))

(event `self.SceneTracker_PatientLocator.OnTrackingDisabled`
  ;[1 1 1 1 24] Tracking & Proximity
  (if (`/Game/Blueprints/Core/Contexts/B_ContextComponent.IsContextActive` (`self.Patient_ContextComponent`)) :!label _label
    (`/Game/Blueprints/Core/Contexts/B_ContextComponent.SetContextActive` (`self.Patient_ContextComponent`) false)))

(event `self.SceneTracker_PatientLocator.OnRangeExceeded`
  (params (player :type "Pawn Object Reference") (inMaxRange :type Boolean))
  ;[1 1 1 1 24] Tracking & Proximity
  (goto _label))

(event `self.InteractAreaComponent.OnInteracted`
  (params (controller :type "Controller Object Reference"))
  ;[1 0.8206 0 1 36] FLOW: EXAMINATION
  (`/Game/Blueprints/Patient/Session/B_PatientTreatmentFlow_Base.ClearTreatment` (`self.TreatmentFlow_Examination`))
  (`PrimitiveComponent.SetCollisionResponseToChannel` (`self.SkeletalMesh`) "ECC_GameTraceChannel1" "ECR_Ignore") ; then disable it after to prevent blocking other interaction on patient
)

(event `self.TreatmentFlow_Examination.OnExaminationCleared`
  ;[1 0.8206 0 1 36] FLOW: EXAMINATION
  (`/Game/Blueprints/Patient/Session/B_PatientTreatmentFlow_Base.RegisterForTreatment` (`self.TreatmentFlow_Adjustment`) (`/Game/Blueprints/Patient/B_PatientJointManager.GetGeneratedJoints` (`self.PatientJointManager`))))

(event `self.PatientCounterComponent.OnUpdate`
  (params (InRating :type Integer))
  ;[1 1 1] EMOTES based on action score
  (switch `int` InRating
    (:`-1`
      (`/Game/Blueprints/Environment/Decibels/B_DecibelEmitterComponent.EmitSoundByData` (`self.DecibelEmitterComponent`) (`self._roomOwner`) "/Game/Blueprints/Environment/Decibels/Data/DA_Decibel_Patient_Complaint.DA_Decibel_Patient_Complaint")
      (if (> (`/Game/Blueprints/Core/Stats/B_Stat.Current as Int` (`/Game/Blueprints/Core/Stats/B_StatComponent.GetStatFromTag` (`self.PatientStatComponent`) (struct :`TagName` "Stats.Patient.Comfort"))) 50)
        (`/Game/Blueprints/HUD/Emotes/B_EmoteHandlerComponent.DisplayEmote` (`self.EmoteHandlerComponent`) (struct :`TagName` "MiniGame.Shared.Rating.Bad"))
        (else
          (`/Game/Blueprints/Patient/Stats/B_CounterComponent_Patient.CountComplaint` (`self.PatientCounterComponent`)))))
    (:`0`
      (`/Game/Blueprints/HUD/Emotes/B_EmoteHandlerComponent.DisplayEmote` (`self.EmoteHandlerComponent`) (struct :`TagName` "MiniGame.Shared.Rating.Good")))
    (:`1`
      (`/Game/Blueprints/HUD/Emotes/B_EmoteHandlerComponent.DisplayEmote` (`self.EmoteHandlerComponent`) (struct :`TagName` "MiniGame.Shared.Rating.Excellent")))))

(event `self.TreatmentFlow_Adjustment.OnRegisterFlow`
  ;[1 0.8206 0 1 36] FLOW: ADJUSTMENT
  (`/Game/Blueprints/Patient/Session/B_PatientTreatmentFlow_Adjustment.StartTreatment` (`self.TreatmentFlow_Adjustment`) (`.Max_13_8A895D624DE880DAA7CAD194D3205837` (break `/Game/Blueprints/Core/Stats/STR_StatDef` (`/Game/Blueprints/Core/Stats/B_Stat.Stat Def` (`/Game/Blueprints/Core/Stats/B_StatComponent.GetStatFromTag` (`self.PatientStatComponent`) (struct :`TagName` "Stats.Patient.Joint.Attention"))))))
  (`/Game/Blueprints/Patient/Session/B_PatientSessionManager.DisplaySessionNotification` (`self.PatientSessionManager`) (struct :`TagName` "GameMode.Phase.SessionStart")) ; show the banner
  (`/ActorTracker/Blueprints/B_SceneTracker_Base.SetTrackingEnabled` (`self.SceneTracker_PatientLocator`) true)
  (`/Game/Blueprints/Patient/ViewModel/B_VM_Patient.VM_SetTreatmentPhase` (`self.vm_patient`) (struct :`TagName` "ViewModel.Patient.Phase.Adjustment"))
  (`/Game/Blueprints/Core/Utilities/BP_UtilsMacro.AddSocialMediaInterest` 50)
  (`/Game/Blueprints/Core/Objective/Context/B_ObjectiveContextGenerator.GenerateObjective` (`self.B_ObjectiveGeneratorComponent_Base`) "/Game/Blueprints/SocialMedia/Objectives/B_Objective_SocialMedia_Tag2.B_Objective_SocialMedia_Tag2_C" (`self.PatientCounterComponent`) true))

(event `self.TreatmentFlow_Adjustment.OnTreatmentCleared`
  (`/Game/Blueprints/Core/Objective/Context/B_ObjectiveContextGenerator.ClearObjective` (`self.B_ObjectiveGeneratorComponent_Base`) (struct :`TagName` "Test.StateTree.Tag2")))

(event `self.PatientCounterComponent.OnComplaint`
  ;[1 1 1] EMOTES based on action score
  (`/Game/Blueprints/HUD/Emotes/B_EmoteHandlerComponent.DisplayEmote` (`self.EmoteHandlerComponent`) (struct :`TagName` "MiniGame.Shared.Rating.Bad")))

(event `self.PatientJointManager.OnRequestSocialMedia`
  (params (RequestTag :type "GameplayTag Structure"))
  (`/Game/Blueprints/SocialMedia/B_SocialMediaNotificationComponent.DisplayNotification` (`self.SocialMediaNotificationComponent`) "" 0.0 RequestTag "/Game/Blueprints/SocialMedia/Channel/B_NotificationChannelMessage_SocialMedia_Base.B_NotificationChannelMessage_SocialMedia_Base_C" true null)
  (`/Game/Blueprints/Core/Utilities/BP_UtilsMacro.AddSocialMediaInterest` 10))

(event `self.PatientJointManager.OnRequestDeniedSocialMedia`
  (`/Game/Blueprints/Core/Notification/Channels/B_NotificationChannelManager.AddMessageToChannel` (`/Game/Blueprints/Gameflow/GS_GameStateCustom.NotificationChannelManager` (`/Game/Blueprints/Core/Utilities/BP_Utils.Game State`)) "/Game/Blueprints/Core/Notification/Channels/Dynamic/B_NotificationChannel_Dynamic.B_NotificationChannel_Dynamic_C" "Broadcast Offline" "Remember to stream to entertain your viewers!" 0.0 "/Game/Blueprints/HUD/Notification/Reminder/B_NotificationChannelMessage_Common_Reminder.B_NotificationChannelMessage_Common_Reminder_C" null))

(fn `GetBonePosition`
  (params (boneName :type Name))
  (returns (position :type "Vector Structure"))
  (bind _returnvalue_location (`KismetMathLibrary.BreakTransform` (`SkinnedMeshComponent.GetBoneTransform` (`self.SkeletalMesh`) boneName "RTS_World")))
  (return _returnvalue_location))

(fn `GetManager`
  (returns (manager :type "/Game/Blueprints/Patient/B_PatientJointManager Object Reference"))
  (return (`self.PatientJointManager`)))

(fn `SetAdjustmentTable`
  (params (InTable :type "/Game/Blueprints/Interactables/Ingredients/AdjustmentTable/BP_ING_AdjustmentTable Object Reference"))
  (bind _output_get (set `self.CurrentTable` InTable))
  (`/Engine/EditorBlueprintResources/StandardMacros.IsValid` _output_get
    (:`Is Valid`
      (`/Game/Blueprints/Interactables/Ingredients/AdjustmentTable/BP_ING_AdjustmentTable.AddUser` (`self.CurrentTable`) self))))

(fn `SetCinematicProxySettings`
  (params (ProxyTag :type "GameplayTagContainer Structure"))
  (returns (OutProxy :type "/Game/Assets/VFX/Camera/Example/BP_Camera_Target_Example Object Reference"))
  (bind _asbp_camera_target_example (cast `/Game/Assets/VFX/Camera/Example/BP_Camera_Target_Example` (`ChildActorComponent.ChildActor` (`self.CinematicProxy`))))
  (`/Game/Assets/VFX/Camera/Example/BP_Camera_Target_Example.SetProxy` _asbp_camera_target_example (`local.ProxyTag`) (`SkeletalMeshComponent.GetSkeletalMeshAsset` (`self.SkeletalMesh`)) (`self.FinisherProxyTable`))
  (return _asbp_camera_target_example))

(fn `UserConstructionScript`
  (bind _currenttable (`self.CurrentTable`))
  (`/Engine/EditorBlueprintResources/StandardMacros.IsValid` _currenttable
    (:`Is Valid`
      (`/Game/Blueprints/Interactables/Ingredients/AdjustmentTable/BP_ING_AdjustmentTable.AddUserDefault` _currenttable self))))

(fn `ValidateInitRequest`
  (bind __patientmanager (`self._patientManager`))
  (bind _currenttable (`self.CurrentTable`))
  (`|ExecutionSequence`
    (:`then_0`
      (`/Engine/EditorBlueprintResources/StandardMacros.IsValid` __patientmanager
        (:`Is Valid`
          (bind _outvalidated (message `/Game/Blueprints/Gameflow/Components/BPI_Gameflow_Validator.ValidateInitialization` __patientmanager))
          (if (not _outvalidated)
            (`self.REVALIDATE_INIT_REQUEST`)
            (return)))
        (:`Is Not Valid`
          (`KismetSystemLibrary.PrintString` "PATIENT MANAGER NOT FOUND - PLEASE ADD PATIENT MANAGER TO SCENE" true true (struct :`R` 1.0 :`B` 0.008162 :`A` 1.0))
          (return))))
    (:`then_1`
      (`/Engine/EditorBlueprintResources/StandardMacros.IsValid` _currenttable
        (:`Is Valid`
          (bind _outvalidated_2 (message `/Game/Blueprints/Gameflow/Components/BPI_Gameflow_Validator.ValidateInitialization` _currenttable))
          (if (not _outvalidated_2)
            (`self.REVALIDATE_INIT_REQUEST`)
            (return)))))
    (:`then_2`
      (bind _outvalidated_3 (message `/Game/Blueprints/Gameflow/Components/BPI_Gameflow_Validator.ValidateInitialization` (`self.PatientCounterComponent`)))
      (if (not _outvalidated_3)
        (`self.REVALIDATE_INIT_REQUEST`)
        (return)))
    (:`then_3`
      (bind _outvalidated_4 (message `/Game/Blueprints/Gameflow/Components/BPI_Gameflow_Validator.ValidateInitialization` (`self.EmoteHandlerComponent`)))
      (if (not _outvalidated_4)
        (`self.REVALIDATE_INIT_REQUEST`)
        (return)))
    (:`then_4`
      (`/Game/Blueprints/Patient/BP_PatientManager.RegisterPatient` (`self._patientManager`) self))))