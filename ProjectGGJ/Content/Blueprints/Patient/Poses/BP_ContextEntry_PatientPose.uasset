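; Context menu entry Blueprint that lets the player switch a patient to a specific pose.
; On initialization it reads pose info from its patient pose context item, caches the owning patient pose manager and sets the view model's display name from the pose ID.
; Executing the entry passes that pose ID to the manager's SetNewPose, provided the manager is valid.
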(fn `ExecuteContext`
  (bind _posemanager (`self.poseManager`)
    (:`then`
      (`/Game/Blueprints/Patient/Poses/B_PatientPoseManager.Set New Pose` _posemanager (`.ID_5_BCC065B74DDC85A0FA4013805A219D3B` (break `/Game/Blueprints/Patient/Poses/STR_PatientPoseHandle` (`self.Pose`)))))
    (:`else`)))

(fn `GetDisplayName`
  (returns (name :type Text))
  (return (`|FormatText` "Patient Pose {id}" (`.ID_5_BCC065B74DDC85A0FA4013805A219D3B` (break `/Game/Blueprints/Patient/Poses/STR_PatientPoseHandle` (`self.Pose`))))))

(fn `InitializeContext`
  (bind (_item _owner) (`self.GetContextInfo`))
  (`parent.InitializeContext`)
  (`|ExecutionSequence`
    (:`then_0`
      (bind _asb_context_item_patient_pose (cast `/Game/Blueprints/Patient/Poses/B_ContextItem_PatientPose` _item))
      (bind _output_get (set `self.Pose` (`/Game/Blueprints/Patient/Poses/B_ContextItem_PatientPose.GetPoseInfo` _asb_context_item_patient_pose))))
    (:`then_1`
      (bind _asb_patient_pose_manager (cast `/Game/Blueprints/Patient/Poses/B_PatientPoseManager` _owner))
      (set `self.poseManager` _asb_patient_pose_manager))
    (:`then_2`
      (`/Game/Blueprints/Core/Contexts/ViewModel/B_VM_ContextEntry_Base.VM_SetDisplayName` (`self.GetViewModel`) (`self.GetDisplayName`)))))

(fn `UserConstructionScript`
  (`parent.UserConstructionScript`))