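; Patient component that manages the chiropractic joint points on a patient and relays social media notification requests.
; It spawns point actors at non-excluded skeleton bones using JointData classes, then tracks injured joints from a profile and restricts joints disabled by the pose.
; Notification requests become randomly sized, timer-spaced bursts that pass only while the GameState influence component is streaming, with denials throttled by a cooldown.
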(event `self.ReceiveBeginPlay`
  (`|ExecutionSequence`
    (:`then_0`
      (bind _asbp_patient (cast `/Game/Blueprints/Patient/BP_Patient` (`self.GetOwner`)))
      (set `self._patient` _asbp_patient))
    (:`then_1`
      (set `self.socialMediaComponent` (`/Game/Blueprints/Gameflow/GS_GameStateCustom.GetInfluenceComponent` (`/Game/Blueprints/Core/Utilities/BP_Utils.Game State`))))))

(event `ClearSocialMediaNotificationQueue`
  (bind __notificationrequestqueue (`self._notificationRequestQueue`))
  (if (`KismetArrayLibrary.Array_IsEmpty` (`self._notificationRequestQueue`))
    (`KismetSystemLibrary.K2_ClearAndInvalidateTimerHandle` (`self._notificationRequestQueueTimer`))
    (else
      (`self.VerifyNotificationRequest` (`|GetArrayItem` __notificationrequestqueue))
      (`KismetArrayLibrary.Array_Remove` __notificationrequestqueue))))

(event `VerifyNotificationRequest`
  (params (InTag :type "GameplayTag Structure"))
  ; Validate if notification request should go through
  (if (`/Game/Blueprints/SocialMedia/B_SocialMediaInfluenceComponent.IsStreaming` (`self.socialMediaComponent`))
    (`self.OnRequestSocialMedia` InTag)
    (else
      (`self.VerifyNotifcationRequestDenied`))))

(event `VerifyNotifcationRequestDenied`
  ; Deny Notification Request (On Cooldown or Not Streaming)
  (if (not (`KismetSystemLibrary.K2_IsValidTimerHandle` (`self._notificationDeniedCooldownTimer`)))
    (`self.OnRequestDeniedSocialMedia`)
    (bind _returnvalue (`KismetSystemLibrary.K2_SetTimerDelegate` (`|CreateDelegate` :!event `ResetNotificationDeniedCooldown`) 10.0))
    (set `self._notificationDeniedCooldownTimer` _returnvalue)))

(event `ResetNotificationDeniedCooldown`
  ; Deny Notification Request (On Cooldown or Not Streaming)
  (`KismetSystemLibrary.K2_ClearAndInvalidateTimerHandle` (`self._notificationDeniedCooldownTimer`)))

(fn `AssignJointProfile`
  (params (InProfile :type "/Game/Blueprints/Patient/BP_PatientProfile Object Reference"))
  (locals (currentJoint :type "/Game/Blueprints/Interactables/BP_ChiropractorPoint Object Reference"))
  (for _array_element (`self.GetGeneratedJoints`)
    (set `local.currentJoint` _array_element)
    (bind _hasissue (`/Game/Blueprints/Patient/BP_PatientProfile.HasJointIssue` (`local.InProfile`) (`/Game/Blueprints/Interactables/BP_ChiropractorPoint.boneName` _array_element) "NewEnumerator0"))
    (`/Game/Blueprints/Interactables/BP_ChiropractorPoint.RegisterJointIssue` (`local.currentJoint`) _hasissue)
    (if _hasissue
      (`KismetArrayLibrary.Array_Add` (`self._injuredJoints`) (`local.currentJoint`)))))

(fn `CleanupGeneratedJoints`
  (for _array_element (`self._allJoints`)
    (`/Game/Blueprints/Interactables/BP_ChiropractorPoint.Cleanup` _array_element)))

(fn `ClearGeneratedJoints`
  (params (InClearDelay :type "Float (single-precision)"))
  (for _array_element (`self.GetGeneratedJoints`)
    (if (> (`local.InClearDelay`) 0.0)
      (`Actor.SetLifeSpan` _array_element (`local.InClearDelay`))
      (else
        (`Actor.K2_DestroyActor` _array_element)))))

(fn `GenerateJointsFromSkeleton`
  (params (InSkeleton :type "SkeletalMeshComponent Object Reference"))
  (returns (OutJointCollection :type "Array of Name"))
  (locals (currentBone :type Name :default "None") (spawnedJoint :type "/Game/Blueprints/Interactables/BP_ChiropractorPoint Object Reference") (jointNameCollection :type "Array of Name"))
  (for _index (range (`SkinnedMeshComponent.GetNumBones` (`local.InSkeleton`)))
    (bind _output_get (set `local.currentBone` (`SkinnedMeshComponent.GetBoneName` (`local.InSkeleton`) _index)))
    (if (`self.HasBoneControl` _output_get)
      (bind _outrownames (`DataTableFunctionLibrary.GetDataTableRowNames` (`self.JointData`)))
      (for _array_element _outrownames
        (bind _returnvalue (`|GetDataTableRow` (`self.JointData`) _array_element)
          (:`then`
            (bind (_bonename _spawnclass) (break `/Game/Blueprints/Patient/Data/STR_PatientJointSetting` _returnvalue))
            (if (== _bonename (`local.currentBone`))
              (bind _returnvalue_2 (`KismetSystemLibrary.LoadClassAsset_Blocking` _spawnclass))
              (bind _returnvalue_3 (`|SpawnActorFromClass` (castclass `/Game/Blueprints/Interactables/BP_ChiropractorPoint` _returnvalue_2 :!pure true) (`SkinnedMeshComponent.GetBoneTransform` (`local.InSkeleton`) (`local.currentBone`) "RTS_World") "Undefined" "MultiplyWithRoot" null null))
              (set `local.spawnedJoint` _returnvalue_3)
              (break)))))
      (`local.spawnedJoint`
        (:`then`
          (`/Game/Blueprints/Interactables/BP_ChiropractorPoint.DefineJointProperties` (`local.spawnedJoint`) (`local.currentBone`) (make `/Game/Blueprints/Patient/STR_RotateBoneLimits` (`local.currentBone`) (-30.0 30.0) (-30.0 30.0)))
          (`self.RegisterNewJoint` (`local.spawnedJoint`))
          (`KismetArrayLibrary.Array_AddUnique` (`local.jointNameCollection`) (`local.currentBone`)))
        (:`else`))))
  (return (`local.jointNameCollection`)))

(fn `GetGeneratedJoints`
  (returns (OutJoints :type "Array of /Game/Blueprints/Interactables/BP_ChiropractorPoint Object Reference"))
  (return (`self._allJoints`)))

(fn `GetInjuredJoints`
  (returns (OutJoints :type "Array of /Game/Blueprints/Interactables/BP_ChiropractorPoint Object Reference"))
  (return (`self._injuredJoints`)))

(fn `GetPatient`
  (returns (patient :type "/Game/Blueprints/Patient/BP_Patient Object Reference"))
  (return (`self._patient`)))

(fn `HasBoneControl`
  (params (boneName :type Name))
  (returns (hasControl :type Boolean))
  (locals (excludeBones :type "Array of String") (isAvailable :type Boolean :default true))
  (for _array_element (`local.excludeBones`)
    (if (`KismetStringLibrary.Contains` (`KismetStringLibrary.Conv_NameToString` (`local.boneName`)) _array_element)
      (set `local.isAvailable` false)
      (break)))
  (return (`local.isAvailable`)))

(fn `RefreshJointsOnPose`
  (params (InPose :type "/Game/Blueprints/Patient/Poses/STR_PatientPoseHandle Structure"))
  (`|ExecutionSequence`
    (:`then_0`
      (if (`KismetArrayLibrary.Array_IsEmpty` (`.disableJoints_12_C28EE33F4B36007FC6C172B126FF19FD` (break `/Game/Blueprints/Patient/Poses/STR_PatientPoseHandle` (`local.InPose`))))
        (return)))
    (:`then_1`
      (for _array_element (`self.GetGeneratedJoints`)
        (if (`KismetArrayLibrary.Array_Contains` (`.disableJoints_12_C28EE33F4B36007FC6C172B126FF19FD` (break `/Game/Blueprints/Patient/Poses/STR_PatientPoseHandle` (`local.InPose`))) (`/Game/Blueprints/Interactables/BP_ChiropractorPoint.boneName` _array_element))
          (`/Game/Blueprints/Interactables/BP_ChiropractorPoint.DisableAttention` _array_element)
          (set `/Game/Blueprints/Interactables/BP_ChiropractorPoint.bPoseRestriction` true _array_element)
          (else
            (set `/Game/Blueprints/Interactables/BP_ChiropractorPoint.bPoseRestriction` false _array_element)))))))

(fn `RegisterNewJoint`
  (params (newJoint :type "/Game/Blueprints/Interactables/BP_ChiropractorPoint Object Reference"))
  (`KismetArrayLibrary.Array_Add` (`self._allJoints`) newJoint)
  (`/Game/Blueprints/Patient/B_PatientJointComponent.SetManager` (`/Game/Blueprints/Interactables/BP_ChiropractorPoint.PatientJointComponent` (`local.newJoint`)) self)
  (`/Game/Blueprints/Interactables/BP_ChiropractorPoint.SetOwningPatient` (`local.newJoint`) (`self.GetPatient`)))

(fn `RequestSocialMediaNotification`
  (params (InMaxCount :type Integer :default 1) (InRequestTag :type "GameplayTag Structure"))
  (locals (maxNotifications :type Integer :default 0) (remainingNotifications :type Integer))
  (set `local.maxNotifications` (`KismetMathLibrary.RandomIntegerInRange` 1 (`KismetMathLibrary.Clamp` InMaxCount 1 5)))
  (`self.VerifyNotificationRequest` (`local.InRequestTag`))
  (set `local.remainingNotifications` (- (`local.maxNotifications`) 1))
  (if (> (`local.remainingNotifications`) 0)
    (for _ (range 1 (+ (`local.remainingNotifications`) 1))
      (`KismetArrayLibrary.Array_Add` (`self._notificationRequestQueue`) (`local.InRequestTag`)))
    (bind _returnvalue (`KismetSystemLibrary.K2_SetTimerDelegate` (`|CreateDelegate` :!event `ClearSocialMediaNotificationQueue`) 1.5 true))
    (set `self._notificationRequestQueueTimer` _returnvalue)))