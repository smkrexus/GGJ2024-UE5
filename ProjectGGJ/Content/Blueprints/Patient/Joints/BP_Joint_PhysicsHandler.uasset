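; Helper actor that grabs a component's bone with a physics handle to drive its position and rotation, apparently for patient joints.
; BonePositionReflector stores the grab rotation, accumulates local rotation deltas and passes its world rotation to the handle as the target.
; Location updates go directly to the handle, and Release drops the component and destroys the actor.
; Includes optional debug boxes and an unused random-rotation test.
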(event `self.ReceiveTick`
  (params (DeltaSeconds :type "Float (single-precision)")))

(event `RandomPositionHandle`
  (bind _bonepositionreflector (`self.BonePositionReflector`))
  (bind (_targetlocation _targetrotation) (`PhysicsHandleComponent.GetTargetLocationAndRotation` (`self.PhysicsHandle`)))
  (`SceneComponent.K2_AddLocalRotation` _bonepositionreflector (select `bool` (`KismetMathLibrary.RandomBool`) :`false` (struct :`Yaw` -15.0) :`true` (struct :`Yaw` 15.0) :!type "Rotator Structure") false false)
  (`PhysicsHandleComponent.SetTargetRotation` (`self.PhysicsHandle`) (`SceneComponent.K2_GetComponentRotation` _bonepositionreflector))
  (if (`self.bEnableDebug`)
    (`KismetSystemLibrary.DrawDebugBox` _targetlocation (10.0 10.0 10.0) (struct :`R` 1.0 :`B` 0.041794 :`A` 1.0) _targetrotation 0.5 1.0)))

(fn `Grab`
  (params (Component :type "PrimitiveComponent Object Reference") (InBoneName :type Name) (Location :type "Vector Structure") (Rotation :type "Rotator Structure"))
  (`PhysicsHandleComponent.GrabComponentAtLocationWithRotation` (`self.PhysicsHandle`) Component InBoneName Location Rotation)
  (`SceneComponent.K2_SetWorldRotation` (`self.BonePositionReflector`) Rotation false false))

(fn `Release`
  (`PhysicsHandleComponent.ReleaseComponent` (`self.PhysicsHandle`))
  (`self.K2_DestroyActor`))

(fn `UpdateHandlerLocation`
  (params (NewLocation :type "Vector Structure"))
  (`PhysicsHandleComponent.SetTargetLocation` (`self.PhysicsHandle`) NewLocation))

(fn `UpdateHandlerRotation`
  (params (NewRotation :type "Rotator Structure"))
  (bind _bonepositionreflector (`self.BonePositionReflector`))
  (bind (_targetlocation _targetrotation) (`PhysicsHandleComponent.GetTargetLocationAndRotation` (`self.PhysicsHandle`)))
  (`SceneComponent.K2_AddLocalRotation` _bonepositionreflector NewRotation false false)
  (`PhysicsHandleComponent.SetTargetRotation` (`self.PhysicsHandle`) (`SceneComponent.K2_GetComponentRotation` _bonepositionreflector))
  (if (`self.bEnableDebug`)
    (`KismetSystemLibrary.DrawDebugBox` _targetlocation (10.0 10.0 10.0) (struct :`R` 0.332467 :`G` 1.0 :`B` 0.004949 :`A` 1.0) _targetrotation 0.1 0.1)))

(fn `UserConstructionScript`)