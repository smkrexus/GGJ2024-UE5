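; Context menu entry labelled "Select Table", used when assigning a table in a patient session.
; On initialization it caches its select-table view model, reads the table from the context item and sets availability from that table's state.
; It binds to the table's user added and removed events, with handlers that toggle availability.
; Execution only calls the parent; logic to collapse the player's top window is left disconnected.
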(event `OnUserAdded`
  (params (NewUser :type "Actor Object Reference"))
  (`/Game/Blueprints/Patient/Session/2_AssignTable/B_VM_ContextEntry_SelectTable.VM_SetAvailability` (`self.vm_customContextEntry`) false))

(event `OnUserRemoved`
  (`/Game/Blueprints/Patient/Session/2_AssignTable/B_VM_ContextEntry_SelectTable.VM_SetAvailability` (`self.vm_customContextEntry`) true))

(fn `ExecuteContext`
  (`|ExecutionSequence`
    (:`then_1`
      (`parent.ExecuteContext`))))

(fn `GetDisplayName`
  (returns (name :type Text))
  (return "Select Table"))

(fn `InitializeContext`
  (bind _viewmodel (`self.GetViewModel`))
  (`parent.InitializeContext`)
  (`|ExecutionSequence`
    (:`then_0`
      (`/Game/Blueprints/Core/Contexts/ViewModel/B_VM_ContextEntry_Base.VM_SetDisplayName` _viewmodel (`self.GetDisplayName`))
      (bind _asb_vm_context_entry_select_table (cast `/Game/Blueprints/Patient/Session/2_AssignTable/B_VM_ContextEntry_SelectTable` _viewmodel))
      (set `self.vm_customContextEntry` _asb_vm_context_entry_select_table))
    (:`then_1`
      (bind _asb_context_item_patient_select_table (cast `/Game/Blueprints/Patient/Session/2_AssignTable/B_ContextItem_Patient_SelectTable` (`self.GetContextInfo`)))
      (bind _output_get (set `self._option` _asb_context_item_patient_select_table))
      (bind _table (`/Game/Blueprints/Patient/Session/2_AssignTable/B_ContextItem_Patient_SelectTable.GetTable` _output_get))
      (add `/Game/Blueprints/Interactables/Ingredients/AdjustmentTable/BP_ING_AdjustmentTable.OnUserAdded` _table (`|CreateDelegate` :!event `OnUserAdded`))
      (add `/Game/Blueprints/Interactables/Ingredients/AdjustmentTable/BP_ING_AdjustmentTable.OnUserRemoved` _table (`|CreateDelegate` :!event `OnUserRemoved`))
      (`/Game/Blueprints/Patient/Session/2_AssignTable/B_VM_ContextEntry_SelectTable.VM_SetAvailability` (`self.vm_customContextEntry`) (`/Game/Blueprints/Interactables/Ingredients/AdjustmentTable/BP_ING_AdjustmentTable.IsAvailable` _table)))))

(fn `UserConstructionScript`
  (`parent.UserConstructionScript`))