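; BP_ContextEntry_PatientSessionEnd is a context menu entry labelled "End Patient Session" that ends a session on a patient actor.
; On initialization it pushes that display name to its view model.
; On execution it casts the context owner to BP_Patient, calls RemovePatient and removes itself from the owning context component, then runs the parent execute logic.
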(fn `ExecuteContext`
  (bind (_item _owner _contextcomponent) (`self.GetContextInfo`))
  (`|ExecutionSequence`
    (:`then_0`
      (bind _asbp_patient (cast `/Game/Blueprints/Patient/BP_Patient` _owner))
      (`/Game/Blueprints/Patient/BP_Patient.RemovePatient` _asbp_patient)
      (`/Game/Blueprints/Core/Contexts/B_ContextComponent.RemoveContext` _contextcomponent self))
    (:`then_1`
      (`parent.ExecuteContext`))))

(fn `GetDisplayName`
  (returns (name :type Text))
  (return "End Patient Session"))

(fn `InitializeContext`
  (`parent.InitializeContext`)
  (`/Game/Blueprints/Core/Contexts/ViewModel/B_VM_ContextEntry_Base.VM_SetDisplayName` (`self.GetViewModel`) (`self.GetDisplayName`)))

(fn `UserConstructionScript`
  (`parent.UserConstructionScript`))