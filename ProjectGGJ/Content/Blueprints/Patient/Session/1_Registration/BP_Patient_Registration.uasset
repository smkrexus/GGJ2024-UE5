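; BP_Patient_Registration is a patient awaiting registration that the player interacts with to open a registration context menu.
; InteractAreaComponent captures the interacting controller, and ContextComponent handles the option window's focus and collapse.
; Register spawns a BP_Patient at the assigned table, copies over the mesh materials and links the table.
; RegistrationCompleted then releases window tracking, disables interaction, cleans up tags and sets a short timer for safe destruction.
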(event `self.ReceiveBeginPlay`
  (bind _contextcomponent (`self.ContextComponent`))
  (`/Game/Blueprints/Interactables/B_InteractAreaComponent.AssignArea` (`self.InteractAreaComponent`) (`self.SkeletalMesh`))
  ;[1 1 1] Registration context button
  (bind _context (`/Game/Blueprints/Core/Contexts/B_ContextComponent.SetupContext` _contextcomponent "/Game/Blueprints/Patient/Session/1_Registration/BP_ContextEntry_Patient_Registration.BP_ContextEntry_Patient_Registration_C" self))
  (`/Game/Blueprints/Core/Contexts/B_ContextComponent.AddContext` _contextcomponent _context)
  (`/Game/Blueprints/Interactables/Extensions/Tag/B_TagComponent.Initialize` (`self.B_TagComponent`)))

(event `self.ContextComponent.OnCollapseContexts`
  ;[1 0.6989 0] CONTEXT WINDOW FOCUS
  (`/Game/Blueprints/Interactables/B_InteractAreaComponent.ShowInteraction` (`self.InteractAreaComponent`)) ; revert to original
  (`/Game/Blueprints/Core/Contexts/B_ContextComponent.SetContextActive` (`self.ContextComponent`) false)
  (set `self._currentController` null) ; no controller in focus
  (`/Game/Blueprints/Core/Contexts/B_ContextComponent.RemoveReturnContext` (`self.ContextComponent`)))

(event `self.InteractAreaComponent.OnInteracted`
  (params (controller :type "Controller Object Reference"))
  (if (not (`/Game/Blueprints/Core/Contexts/B_ContextComponent.IsContextActive` (`self.ContextComponent`)))
    ;[1 1 1] Enable Interaction Focus
    (set `self._currentController` controller)
    (`/Game/Blueprints/Interactables/B_InteractAreaComponent.HideInteraction` (`self.InteractAreaComponent`)) ; focus on the options available
    (`/Game/Blueprints/Core/Contexts/B_ContextComponent.AddReturnContext` (`self.ContextComponent`) self (`self._currentController`))
    (`/Game/Blueprints/Core/Contexts/B_ContextComponent.AddWindowTracking` (`self.ContextComponent`) (`self._currentController`))))

(event `self.ContextComponent.OnFocusContexts`
  ;[1 0.6989 0] CONTEXT WINDOW FOCUS
  (`/Game/Blueprints/Core/Contexts/B_ContextComponent.AddToScreen` (`self.ContextComponent`) (`self._currentController`) "contextOptions")
  (`/Game/Blueprints/Core/Contexts/B_ContextComponent.SetContextActive` (`self.ContextComponent`) true))

(event `self.ContextComponent.OnUnfocusContexts`
  ;[1 0.6989 0] CONTEXT WINDOW FOCUS
  (`/Game/Blueprints/Core/Contexts/B_ContextComponent.SetContextActive` (`self.ContextComponent`) false))

(event `RegistrationCompleted`
  (bind __currentcontroller (`self._currentController`) ; this should be valid since you need to be in menu to complete registration
    (:`then`
      (`/Game/Blueprints/Core/Contexts/B_ContextComponent.RemoveWindowTracking` (`self.ContextComponent`) __currentcontroller)
      (`/Game/Blueprints/Interactables/B_InteractAreaComponent.DisableInteraction` (`self.InteractAreaComponent`)) ; cannot be interacted now since it is going to destroy
      (`KismetSystemLibrary.K2_SetTimerDelegate` (`|CreateDelegate` :!event `K2_DestroyActor`) 0.5) ; safe destroy
      (`/Game/Blueprints/Interactables/Extensions/Tag/B_TagComponent.Cleanup` (`self.B_TagComponent`)))
    (:`else`)))

(fn `AssignTable`
  (params (InTable :type "/Game/Blueprints/Interactables/Ingredients/AdjustmentTable/BP_ING_AdjustmentTable Object Reference"))
  (set `self._assignedTable` InTable))

(fn `Register`
  (locals (newPatient :type "/Game/Blueprints/Patient/BP_Patient Object Reference"))
  (bind __assignedtable (`self._assignedTable`)
    (:`then`
      (bind (_returnvalue_location _returnvalue_rotation) (`KismetMathLibrary.BreakTransform` (`self.GetTransform` __assignedtable)))
      (bind _returnvalue (`|SpawnActorFromClass` "/Game/Blueprints/Patient/BP_Patient.BP_Patient_C" (`KismetMathLibrary.MakeTransform` _returnvalue_location (`KismetMathLibrary.MakeRotator` (.roll _returnvalue_rotation) (.pitch _returnvalue_rotation) (+ (.yaw _returnvalue_rotation) -90.0))) "AlwaysSpawn" "MultiplyWithRoot" null null))
      (set `local.newPatient` _returnvalue)
      (for (_array_element _array_index) (`MeshComponent.GetMaterials` (`self.SkeletalMesh`))
        (`PrimitiveComponent.SetMaterial` (`/Game/Blueprints/Patient/BP_Patient.SkeletalMesh` (`local.newPatient`)) _array_index _array_element))
      (`/Game/Blueprints/Patient/BP_Patient.SetAdjustmentTable` (`local.newPatient`) (`self._assignedTable`))
      (`self.RegistrationCompleted`))
    (:`else`)))

(fn `UserConstructionScript`)