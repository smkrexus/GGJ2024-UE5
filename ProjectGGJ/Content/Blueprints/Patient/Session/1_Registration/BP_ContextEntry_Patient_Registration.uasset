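; Context menu entry "Register Patient" that lets the player pick an adjustment table and spawns a new patient there.
; Executing it builds a SelectTable sub-option for every adjustment table in the level and tracks that submenu through the player state's window tracker.
; Picking one collapses the window, spawns BP_Patient at the table with a yaw offset, assigns the table, completes registration and removes this entry.
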(event `self.ContextOptions_SelectTable.OnCollapseContexts`
  (bind _contextoptions_selecttable (`self.ContextOptions_SelectTable`))
  (bind _viewmodel (`/Game/Blueprints/Core/Contexts/B_ContextComponent.GetViewModel` _contextoptions_selecttable))
  (for _array_element (`/Game/Blueprints/Core/Contexts/B_ContextComponent.GetContexts` _contextoptions_selecttable)
    (`/Game/Blueprints/Core/Contexts/B_ContextComponent.RemoveContext` _contextoptions_selecttable _array_element))
  (`/Game/Blueprints/Core/Contexts/ViewModel/B_VM_Contexts.VM_ShouldUpdateContext` _viewmodel)
  (`/Game/Blueprints/Core/Contexts/ViewModel/B_VM_Contexts.VM_SetRemoveContext` _viewmodel true))

(event `self.ContextOptions_SelectTable.OnFocusContexts`
  (bind _viewmodel (`/Game/Blueprints/Core/Contexts/B_ContextComponent.GetViewModel` (`self.ContextOptions_SelectTable`)))
  (bind _view (`/Game/Blueprints/Core/ViewModel/B_VM_BaseComponent.CreateView` _viewmodel (`/Game/Blueprints/Core/ViewModel/B_VM_BaseComponent.defaultWidget` _viewmodel)))
  (`UserWidget.AddToViewport` _view 0)
  (`/Game/Blueprints/Core/Contexts/ViewModel/B_VM_Contexts.VM_ShouldUpdateContext` _viewmodel))

(fn `ExecuteContext`
  (locals (selectedTable :type "/Game/Blueprints/Interactables/Ingredients/AdjustmentTable/BP_ING_AdjustmentTable Object Reference"))
  (`parent.ExecuteContext`)
  (bind _outactors (`GameplayStatics.GetAllActorsOfClass` "/Game/Blueprints/Interactables/Ingredients/AdjustmentTable/BP_ING_AdjustmentTable.BP_ING_AdjustmentTable_C"))
  (for _array_element _outactors
    (bind _context (`/Game/Blueprints/Core/Contexts/B_ContextComponent.SetupContext` (`self.ContextOptions_SelectTable`) "/Game/Blueprints/Patient/Session/2_AssignTable/BP_ContextEntry_Patient_SelectTable.BP_ContextEntry_Patient_SelectTable_C" (`.owner` (`self.GetContextInfo`))))
    (bind _asb_context_item_patient_select_table (cast `/Game/Blueprints/Patient/Session/2_AssignTable/B_ContextItem_Patient_SelectTable` (`self.GetContextInfo` _context)))
    (`/Game/Blueprints/Patient/Session/2_AssignTable/B_ContextItem_Patient_SelectTable.SetTable` _asb_context_item_patient_select_table _array_element)
    (`/Game/Blueprints/Core/Contexts/B_ContextComponent.AddContext` (`self.ContextOptions_SelectTable`) _context)
    (add `self.OnExecute` _context (`|CreateDelegate` :!event `OnExecuteContextOption`)))
  (bind _asbp_patient_registration (cast `/Game/Blueprints/Patient/Session/1_Registration/BP_Patient_Registration` (`.owner` (`self.GetContextInfo`))))
  (bind _asbp_player_state_custom (cast `/Game/Blueprints/Player/BP_PlayerStateCustom` (`Controller.PlayerState` (`/Game/Blueprints/Patient/Session/1_Registration/BP_Patient_Registration._currentController` _asbp_patient_registration))))
  (`/Game/Blueprints/Core/Contexts/B_ContextWindowTracker.TrackWindow` (`/Game/Blueprints/Player/BP_PlayerStateCustom.GetWindowTracker` _asbp_player_state_custom) (`self.ContextOptions_SelectTable`)))

(fn `GetDisplayName`
  (returns (name :type Text))
  (return "Register Patient"))

(fn `InitializeContext`
  (`parent.InitializeContext`)
  (`/Game/Blueprints/Core/Contexts/ViewModel/B_VM_ContextEntry_Base.VM_SetDisplayName` (`self.GetViewModel`) (`self.GetDisplayName`)))

(fn `OnExecuteContextOption`
  (params (contextEntry :type "/Game/Blueprints/Core/Contexts/BP_ContextEntry_Base Object Reference"))
  (locals (selectedTable :type "/Game/Blueprints/Interactables/Ingredients/AdjustmentTable/BP_ING_AdjustmentTable Object Reference"))
  (bind (_item _owner _contextcomponent) (`self.GetContextInfo`))
  (`|ExecutionSequence`
    (:`then_0`
      (bind _asbp_context_entry_patient_select_table (cast `/Game/Blueprints/Patient/Session/2_AssignTable/BP_ContextEntry_Patient_SelectTable` contextEntry))
      (bind _asb_context_item_patient_select_table (cast `/Game/Blueprints/Patient/Session/2_AssignTable/B_ContextItem_Patient_SelectTable` (`self.GetContextInfo` _asbp_context_entry_patient_select_table)))
      (set `local.selectedTable` (`/Game/Blueprints/Patient/Session/2_AssignTable/B_ContextItem_Patient_SelectTable.GetTable` _asb_context_item_patient_select_table)))
    (:`then_1`
      (bind _asbp_patient_registration (cast `/Game/Blueprints/Patient/Session/1_Registration/BP_Patient_Registration` (`.owner` (`self.GetContextInfo`))))
      (bind _asbp_player_state_custom (cast `/Game/Blueprints/Player/BP_PlayerStateCustom` (`Controller.PlayerState` (`/Game/Blueprints/Patient/Session/1_Registration/BP_Patient_Registration._currentController` _asbp_patient_registration))))
      (`/Game/Blueprints/Core/Contexts/B_ContextWindowTracker.CollapseTopWindow` (`/Game/Blueprints/Player/BP_PlayerStateCustom.GetWindowTracker` _asbp_player_state_custom)))
    (:`then_2`
      (bind _selectedtable (`local.selectedTable`)
        (:`then`
          (bind (_returnvalue_location _returnvalue_rotation) (`KismetMathLibrary.BreakTransform` (`self.GetTransform` _selectedtable)))
          (bind _returnvalue (`|SpawnActorFromClass` "/Game/Blueprints/Patient/BP_Patient.BP_Patient_C" (`KismetMathLibrary.MakeTransform` _returnvalue_location (`KismetMathLibrary.MakeRotator` (.roll _returnvalue_rotation) (.pitch _returnvalue_rotation) (+ (.yaw _returnvalue_rotation) -90.0))) "AlwaysSpawn" "MultiplyWithRoot" null null))
          (`/Game/Blueprints/Patient/BP_Patient.SetAdjustmentTable` _returnvalue (`local.selectedTable`))
          (bind _asbp_patient_registration_2 (cast `/Game/Blueprints/Patient/Session/1_Registration/BP_Patient_Registration` _owner))
          (`/Game/Blueprints/Patient/Session/1_Registration/BP_Patient_Registration.RegistrationCompleted` _asbp_patient_registration_2)
          (`/Game/Blueprints/Core/Contexts/B_ContextComponent.RemoveContext` _contextcomponent self))
        (:`else`)))))

(fn `UserConstructionScript`
  (`parent.UserConstructionScript`))