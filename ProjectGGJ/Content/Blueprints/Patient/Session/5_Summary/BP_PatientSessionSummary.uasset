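; Interactable actor that presents the end-of-session summary for a patient.
; DisplaySummary fills a view model with session scores, mission, adjustment scores and a random feedback row from a review DataTable, then adds a prompt.
; Interacting or using the input shortcut clears the prompt and opens the summary popup through the player state's popup manager.
; The view model refreshes when the popup shows, and the actor destroys itself when it hides.
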(event `self.ReceiveBeginPlay`
  (`/Game/Blueprints/Interactables/B_InteractAreaComponent.AssignArea` (`self.B_InteractAreaComponent`) (`self.Interact_Area`)))

(event `OnDisplayPopup`
  (params (InDisplayEnabled :type Boolean))
  (if InDisplayEnabled
    (`/Game/Blueprints/Core/ViewModel/B_VM_BaseComponent.ForceRefresh` (`self.B_VM_PatientSessionSummary`))
    (else
      (`self.K2_DestroyActor`))))

(event `self.B_InteractAreaComponent.OnInteracted`
  (params (controller :type "Controller Object Reference"))
  (`self.DisplayPopup` controller))

(event `/Game/Blueprints/Core/Inputs/BPI_InputShortcutAction.OnInputShortcutActivated`
  (params (InController :type "Controller Object Reference"))
  (`self.DisplayPopup` InController))

(fn `DisplayPopup`
  (params (InController :type "Controller Object Reference"))
  (`|ExecutionSequence`
    (:`then_0`
      (`/Game/Blueprints/Core/Notification/Prompt/B_PromptTarget.ClearPrompt` (`self.B_PromptTarget`)))
    (:`then_1`
      (bind _output_get (set `self._popupManager` (`self.GetComponentByClass` (`GameplayStatics.GetPlayerState` 0) "/Game/Blueprints/HUD/Popup/B_PopupManager.B_PopupManager_C")))
      (add `/Game/Blueprints/HUD/Popup/B_PopupManager.OnPopupDisplay` _output_get (`|CreateDelegate` :!event `OnDisplayPopup`))
      (`/Game/Blueprints/HUD/Popup/B_PopupManager.CreatePopup` (`self._popupManager`) "/Game/Blueprints/Patient/Session/5_Summary/BP_Popup_SessionSummary.BP_Popup_SessionSummary_C" (`local.InController`) (`self.B_VM_PatientSessionSummary`)))))

(fn `DisplaySummary`
  (params (InPatient :type "/Game/Blueprints/Patient/BP_Patient Object Reference"))
  (locals (rowName :type Name))
  (bind _b_vm_patientsessionsummary (`self.B_VM_PatientSessionSummary`))
  (set `self._patient` InPatient)
  (`|ExecutionSequence`
    (:`then_0`
      (bind _outscores (`/Game/Blueprints/Patient/Session/B_PatientSessionManager.GetScores` (`/Game/Blueprints/Patient/BP_Patient.PatientSessionManager` (`local.InPatient`))))
      (`/Game/Blueprints/Patient/Session/5_Summary/B_VM_PatientSessionSummary.VM_SetReviewScores` _b_vm_patientsessionsummary _outscores)
      (`/Game/Blueprints/Patient/Session/5_Summary/B_VM_PatientSessionSummary.VM_SetMission` (`self.B_VM_PatientSessionSummary`) (`/Game/Blueprints/Core/Objective/Component/B_ObjectiveComponent_Patient.GetObjectivePatient` (`/Game/Blueprints/Patient/BP_Patient.ObjectiveComponent_Patient` (`local.InPatient`)))))
    (:`then_1`
      (bind _outscores_2 (`/Game/Blueprints/Patient/Stats/B_CounterComponent_Patient.GetScores` (`/Game/Blueprints/Patient/BP_Patient.PatientCounterComponent` (`local.InPatient`))))
      (`/Game/Blueprints/Patient/Session/5_Summary/B_VM_PatientSessionSummary.VM_SetAdjustmentScores` _b_vm_patientsessionsummary _outscores_2))
    (:`then_2`
      (bind _output_get (set `self._reviewData` (select `int` (- (`.OutScore` (`/Game/Blueprints/Patient/Session/Scoring/B_SessionScore_Base.GetScores` (`/Game/Blueprints/Patient/Session/5_Summary/B_VM_PatientSessionSummary.VM_GetReviewScore` (`self.B_VM_PatientSessionSummary`) (struct :`TagName` "Score.Session.Review")))) 1) :`0` "/Game/Blueprints/Patient/Session/5_Summary/DT_PatientReview_Bad.DT_PatientReview_Bad" :`1` "/Game/Blueprints/Patient/Session/5_Summary/DT_PatientReview_Bad.DT_PatientReview_Bad" :`2` "/Game/Blueprints/Patient/Session/5_Summary/DT_PatientReview_Good.DT_PatientReview_Good" :`3` "/Game/Blueprints/Patient/Session/5_Summary/DT_PatientReview_Excellent.DT_PatientReview_Excellent" :`4` "/Game/Blueprints/Patient/Session/5_Summary/DT_PatientReview_Excellent.DT_PatientReview_Excellent" :!type "DataTable Object Reference")))
      (bind _outrownames (`DataTableFunctionLibrary.GetDataTableRowNames` _output_get))
      (bind _output_get_2 (set `local.rowName` (`KismetArrayLibrary.Array_Random` _outrownames)))
      (bind _returnvalue (`|GetDataTableRow` (`self._reviewData`) _output_get_2)
        (:`then`
          (`/Game/Blueprints/Patient/Session/5_Summary/B_VM_PatientSessionSummary.VM_SetReviewFeedback` (`self.B_VM_PatientSessionSummary`) _returnvalue))))
    (:`then_3`
      (`/Game/Blueprints/Core/Notification/Prompt/B_PromptTarget.AddPrompt` (`self.B_PromptTarget`)))))

(fn `UserConstructionScript`)