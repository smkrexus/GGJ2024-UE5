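; Context menu entry that lets the player directly get a new request from a patient, or a reminder of the one already started.
; On initialization it caches the request context item and the owner's request component, and stores the patient's current room.
; First execution adds a random-in-room request, relabels the entry and makes the patient voice it; later executions voice a reminder.
; Completing the request removes the entry from its context component.
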(event `OnRequestCompleted`
  (params (request :type "/Game/Blueprints/Patient/Requests/BP_Request_Base Object Reference"))
  (`KismetSystemLibrary.PrintString` "completed in context entry, removing context")
  (`/Game/Blueprints/Core/Contexts/B_ContextComponent.RemoveContext` (`.contextComponent` (`self.GetContextInfo`)) self))

(fn `ExecuteContext`
  (bind _request (`/Game/Blueprints/Patient/Requests/Contexts/B_ContextItem_Request.request` (`self.requestContext`)))
  (bind _request_2 (`/Game/Blueprints/Patient/Requests/Contexts/B_ContextItem_Request.request` (`self.requestContext`)))
  (bind _returnvalue (`self.GetComponentByClass` (`/Game/Blueprints/Patient/Requests/BP_Request_Base.GetRequestor` _request_2) "/Game/Blueprints/Patient/Dialogue/B_PatientDialogueComponent.B_PatientDialogueComponent_C"))
  (bind _returnvalue_2 (`self.GetComponentByClass` (`/Game/Blueprints/Patient/Requests/BP_Request_Base.GetRequestor` _request) "/Game/Blueprints/Patient/Dialogue/B_PatientDialogueComponent.B_PatientDialogueComponent_C"))
  (`|ExecutionSequence`
    (:`then_0`
      (if (`/Game/Blueprints/Patient/Requests/Contexts/B_ContextItem_Request.bRequestStarted` (`self.requestContext`))
        (`/Engine/EditorBlueprintResources/StandardMacros.IsValid` _returnvalue_2
          (:`Is Valid`
            (`/Game/Blueprints/Patient/Dialogue/B_PatientDialogueComponent.AddDialogue` _returnvalue_2 (`|FormatText` "Maybe you forgot {action} {subject}? If not, it's alright really!" (`KismetTextLibrary.TextToLower` (`.name` (`/Game/Blueprints/Patient/Requests/BP_Request_Base.GetFeedbackAction` _request))) (`.name` (`/Game/Blueprints/Patient/Requests/BP_Request_Base.GetFeedbackSubject` _request))))))
        (else
          (`KismetSystemLibrary.PrintString` "adding a new request!")
          (set `/Game/Blueprints/Patient/Requests/Contexts/B_ContextItem_Request.bRequestStarted` true (`self.requestContext`))
          (bind _addedrequest (`/Game/Blueprints/Patient/Requests/B_RequestComponent.AddRequest` (`self.requestComponent`) (`/Game/Blueprints/Patient/Requests/Contexts/B_ContextItem_Request.room` (`self.requestContext`)) "/Game/Blueprints/Patient/Requests/Options/B_RequestOption_RandomInRoom.B_RequestOption_RandomInRoom_C"))
          (bind _output_get (set `/Game/Blueprints/Patient/Requests/Contexts/B_ContextItem_Request.request` _addedrequest (`self.requestContext`)))
          (add `/Game/Blueprints/Patient/Requests/BP_Request_Base.OnCompleteRequest` _output_get (`|CreateDelegate` :!event `OnRequestCompleted`))
          (`/Game/Blueprints/Core/Contexts/ViewModel/B_VM_ContextEntry_Base.VM_SetDisplayName` (`self.GetViewModel`) "Remind Request")
          (`/Engine/EditorBlueprintResources/StandardMacros.IsValid` _returnvalue
            (:`Is Valid`
              (`/Game/Blueprints/Patient/Dialogue/B_PatientDialogueComponent.AddDialogue` _returnvalue (`|FormatText` "Could you {action} the {subject}?" (`KismetTextLibrary.TextToLower` (`.name` (`/Game/Blueprints/Patient/Requests/BP_Request_Base.GetFeedbackAction` _request_2))) (`.name` (`/Game/Blueprints/Patient/Requests/BP_Request_Base.GetFeedbackSubject` _request_2)))))))))
    (:`then_1`
      (`parent.ExecuteContext`))))

(fn `GetDisplayName`
  (returns (name :type Text))
  (return "New Request"))

(fn `InitializeContext`
  (bind (_item _owner) (`self.GetContextInfo`))
  (`parent.InitializeContext`)
  (`|ExecutionSequence`
    (:`then_0`
      (bind _asb_context_item_request (cast `/Game/Blueprints/Patient/Requests/Contexts/B_ContextItem_Request` _item))
      (set `self.requestContext` _asb_context_item_request))
    (:`then_1`
      (bind _asb_request_component (cast `/Game/Blueprints/Patient/Requests/B_RequestComponent` _owner))
      (bind _output_get (set `self.requestComponent` _asb_request_component))
      (bind _asbp_patient (cast `/Game/Blueprints/BP_Patient` (`ActorComponent.GetOwner` _output_get)))
      (set `/Game/Blueprints/Patient/Requests/Contexts/B_ContextItem_Request.room` (`/Game/Blueprints/BP_Patient.currentRoom` _asbp_patient) (`self.requestContext`)))
    (:`then_2`
      (`/Game/Blueprints/Core/Contexts/ViewModel/B_VM_ContextEntry_Base.VM_SetDisplayName` (`self.GetViewModel`) (`self.GetDisplayName`)))))

(fn `UserConstructionScript`
  (`parent.UserConstructionScript`))