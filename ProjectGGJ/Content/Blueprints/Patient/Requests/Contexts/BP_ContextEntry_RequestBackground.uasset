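; Context entry that represents an in-progress patient request, shown under the display name "Request InProgress".
; On initialization it marks the request context item as started, links it to the owning request, binds to its completion and sets the view model name.
; Executing it makes the requestor's dialogue component ask for the action on the subject, built from the request's feedback data.
; When the request completes, the entry removes itself from its context component.
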(event `OnRequestCompleted`
  (params (request :type "/Game/Blueprints/Patient/Requests/BP_Request_Base Object Reference"))
  (`/Game/Blueprints/Core/Contexts/B_ContextComponent.RemoveContext` (`.contextComponent` (`self.GetContextInfo`)) self))

(fn `ExecuteContext`
  (bind _request (`/Game/Blueprints/Patient/Requests/Contexts/B_ContextItem_Request.request` (`self.requestContext`)))
  (bind _returnvalue (`self.GetComponentByClass` (`/Game/Blueprints/Patient/Requests/BP_Request_Base.GetRequestor` _request) "/Game/Blueprints/Patient/Dialogue/B_PatientDialogueComponent.B_PatientDialogueComponent_C"))
  (if (`/Game/Blueprints/Patient/Requests/Contexts/B_ContextItem_Request.bRequestStarted` (`self.requestContext`))
    (`/Engine/EditorBlueprintResources/StandardMacros.IsValid` _returnvalue
      (:`Is Valid`
        (`/Game/Blueprints/Patient/Dialogue/B_PatientDialogueComponent.AddDialogue` _returnvalue (`|FormatText` "Could you {action} the {subject}?" (`.name` (`/Game/Blueprints/Patient/Requests/BP_Request_Base.GetFeedbackSubject` _request)) (`KismetTextLibrary.TextToLower` (`.name` (`/Game/Blueprints/Patient/Requests/BP_Request_Base.GetFeedbackAction` _request)))))))))

(fn `GetDisplayName`
  (returns (name :type Text))
  (return "Request InProgress"))

(fn `InitializeContext`
  (bind (_item _owner) (`self.GetContextInfo`))
  (`parent.InitializeContext`)
  (`|ExecutionSequence`
    (:`then_0`
      (bind _asb_context_item_request (cast `/Game/Blueprints/Patient/Requests/Contexts/B_ContextItem_Request` _item))
      (bind _output_get (set `self.requestContext` _asb_context_item_request))
      (set `/Game/Blueprints/Patient/Requests/Contexts/B_ContextItem_Request.bRequestStarted` true _output_get))
    (:`then_1`
      (bind _asbp_request_base (cast `/Game/Blueprints/Patient/Requests/BP_Request_Base` _owner))
      (bind _output_get_2 (set `/Game/Blueprints/Patient/Requests/Contexts/B_ContextItem_Request.request` _asbp_request_base _output_get))
      (add `/Game/Blueprints/Patient/Requests/BP_Request_Base.OnCompleteRequest` _output_get_2 (`|CreateDelegate` :!event `OnRequestCompleted`)))
    (:`then_2`
      (`/Game/Blueprints/Core/Contexts/ViewModel/B_VM_ContextEntry_Base.VM_SetDisplayName` (`self.GetViewModel`) (`self.GetDisplayName`)))))

(fn `UserConstructionScript`
  (`parent.UserConstructionScript`))