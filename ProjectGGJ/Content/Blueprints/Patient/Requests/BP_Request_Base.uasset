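; BP_Request_Base is the base Blueprint for patient requests, storing a requestor plus a requirement tag and target.
; Validate routes CanValidate, which always passes here, to accept or deny handlers that print the EndValidation result.
; A successful EndValidation calls OnCompleteRequest, while failure only formats a message.
; Feedback getters expose the target as subject and the tag as action, with placeholder names.
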(fn `CanValidate`
  (params (info :type "/Game/Blueprints/Core/Notification/STR_NotifyHandle_Basic Structure"))
  (returns (valid :type Boolean) (OutMessage :type Text))
  (return true ""))

(fn `EndValidation`
  (params (success :type Boolean) (message :type Text))
  (returns (OutMessage :type Text))
  (if success
    (`self.OnCompleteRequest` self)
    (return (`|FormatText` "Success: {message}" (`local.message`)))
    (else
      (return (`|FormatText` "Failed: {message}" (`local.message`))))))

(fn `GetConditions`
  (returns (requirementTag :type "GameplayTag Structure") (requirementTarget :type "Object Object Reference"))
  (return (`self.requirementTag`) (`self.requirementTarget`)))

(fn `GetFeedbackAction`
  (returns (action :type "GameplayTag Structure") (name :type Text))
  (return (`self.requirementTag`) "Default Action Name"))

(fn `GetFeedbackSubject`
  (returns (subject :type "Object Object Reference") (name :type Text))
  (return (`self.requirementTarget`) "Default Subject Name"))

(fn `GetRequestor`
  (returns (requestor :type "Actor Object Reference"))
  (return (`self.requestor`)))

(fn `OnValidateAccept`
  (params (info :type "/Game/Blueprints/Core/Notification/STR_NotifyHandle_Basic Structure"))
  (bind _outmessage (`self.EndValidation` true "Base validate accept"))
  (`KismetSystemLibrary.PrintText` _outmessage))

(fn `OnValidateDenied`
  (params (info :type "/Game/Blueprints/Core/Notification/STR_NotifyHandle_Basic Structure") (message :type Text))
  (bind _outmessage (`self.EndValidation` false message))
  (`KismetSystemLibrary.PrintText` _outmessage))

(fn `SetRequestConditions`
  (params (requirementTag :type "GameplayTag Structure") (requirementTarget :type "Object Object Reference"))
  (set `self.requirementTag` requirementTag)
  (set `self.requirementTarget` requirementTarget))

(fn `SetRequestor`
  (params (requestor :type "Actor Object Reference"))
  (set `self.requestor` requestor))

(fn `UserConstructionScript`)

(fn `Validate`
  (params (info :type "/Game/Blueprints/Core/Notification/STR_NotifyHandle_Basic Structure"))
  (bind (_valid _outmessage) (`self.CanValidate` info))
  (bind _info (`local.info`))
  (if _valid
    (`self.OnValidateAccept` _info)
    (else
      (`self.OnValidateDenied` _info _outmessage))))