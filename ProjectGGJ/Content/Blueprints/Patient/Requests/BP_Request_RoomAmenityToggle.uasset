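; Patient request Blueprint that checks whether a room amenity has been toggled to the required state.
; It validates only events in the Environment.Amenity category from the required target on a matching channel.
; The event key is compared to the requirement tag's name, avoiding casts, to end validation as success or failure with a message.
; Feedback names for action and subject come from the target's descriptor interface and the parent's subject.
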(fn `CanValidate`
  (params (info :type "/Game/Blueprints/Core/Notification/STR_NotifyHandle_Basic Structure"))
  (returns (valid :type Boolean) (OutMessage :type Text))
  (bind ((`category_2_07B5DF2948628D11FE7D1FA9ACAFB0A5` _category) (`instigator_5_BFFEB6B64822060984F65EB65E5D6305` _instigator)) (break `/Game/Blueprints/Core/Notification/STR_NotifyHandle_Basic` info))
  (bind _returnvalue (`BlueprintGameplayTagLibrary.MakeLiteralGameplayTag` (struct :`TagName` "Environment.Amenity")))
  (if (`BlueprintGameplayTagLibrary.MatchesTag` _category _returnvalue)
    (return true "")
    (else
      (return false (`|FormatText` "Incorrect Category: {item} is not {name}" _instigator (`BlueprintGameplayTagLibrary.GetTagName` _returnvalue))))))

(fn `GetFeedbackAction`
  (returns (action :type "GameplayTag Structure") (name :type Text))
  (bind (_requirementtag _requirementtarget) (`self.GetConditions`))
  (bind (_action _name) (`parent.GetFeedbackAction`))
  (if (`KismetSystemLibrary.DoesImplementInterface` (`.requirementTarget` (`self.GetConditions`)) "/Game/Blueprints/Core/Descriptors/BPI_DescriptorSystemInterface.BPI_DescriptorSystemInterface_C")
    (bind _description (message `/Game/Blueprints/Core/Descriptors/BPI_DescriptorSystemInterface.TranslateOption` _requirementtarget _requirementtag))
    (return _requirementtag _description)
    (else
      (return _action _name))))

(fn `GetFeedbackSubject`
  (returns (subject :type "Object Object Reference") (name :type Text))
  (bind _subject (`parent.GetFeedbackSubject`))
  (bind _description (message `/Game/Blueprints/Core/Descriptors/BPI_DescriptorSystemInterface.GetDescription` _subject))
  (return _subject _description))

(fn `OnValidateAccept`
  (params (info :type "/Game/Blueprints/Core/Notification/STR_NotifyHandle_Basic Structure"))
  (bind (_requirementtag _requirementtarget) (`self.GetConditions`))
  (bind ((`key_10_444AA8D442F1047C215320B16095F6C5` _key)) (break `/Game/Blueprints/Core/Notification/STR_NotifyHandle_Basic` (`local.info`)))
  (bind _returnvalue (`KismetStringLibrary.Conv_StringToName` _key))
  (`|ExecutionSequence`
    (:`then_0`
      (if (not (== (`.instigator_5_BFFEB6B64822060984F65EB65E5D6305` (break `/Game/Blueprints/Core/Notification/STR_NotifyHandle_Basic` (`local.info`))) _requirementtarget))
        (return)))
    (:`then_1`
      (if (not (`BlueprintGameplayTagLibrary.MatchesTag` _requirementtag (`.channel_13_5DCDBF0C42B3BE5076C51295589D0D2E` (break `/Game/Blueprints/Core/Notification/STR_NotifyHandle_Basic` (`local.info`)))))
        (return)))
    (:`then_2`
      ;[1 1 1] Use keys to differentiate states, so no casting needed (in this case)
      (if (== _key (`KismetStringLibrary.Conv_NameToString` (`BlueprintGameplayTagLibrary.GetTagName` (`self.GetConditions`))))
        (bind _outmessage (`self.EndValidation` true (`|FormatText` "Correct Amenity State {state}" _returnvalue)))
        (`KismetSystemLibrary.PrintText` _outmessage)
        (else
          (bind _outmessage_2 (`self.EndValidation` false (`|FormatText` "Wrong Amenity State {state}" _returnvalue)))
          (`KismetSystemLibrary.PrintText` _outmessage_2))))))

(fn `UserConstructionScript`
  (`parent.UserConstructionScript`))