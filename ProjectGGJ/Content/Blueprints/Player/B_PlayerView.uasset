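; B_PlayerView is the player's HUD view layer, owned by the player controller, creating the interaction-info and custom HUD widgets at BeginPlay.
; It also acts as a view model, storing interaction object, descriptions, display and requirement component.
; Setters raise named variable-change notifications, while getters expose the current interaction state.
; A placeholder equipment setter passes the equipment component's view model to the interaction widget.
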(event `self.ReceiveBeginPlay`
  (`|ExecutionSequence`
    (:`then_0`
      (bind _view (`self.CreateView` "/Game/Blueprints/HUD/BP_Widget_HUDInteractInfo.BP_Widget_HUDInteractInfo_C"))
      (bind _output_get (set `self.view_interact` _view))
      (`UserWidget.AddToViewport` _output_get 0))
    (:`then_1`
      (bind _view_2 (`self.CreateView` "/Game/Blueprints/HUD/BP_Widget_HUDCustom.BP_Widget_HUDCustom_C"))
      (`UserWidget.AddToViewport` _view_2 0))))

(fn `CreateHUD`
  (params (hudClass :type "UserWidget Class Reference"))
  (returns (widget :type "UserWidget Object Reference"))
  (if (`KismetSystemLibrary.IsValidClass` hudClass)
    (bind _returnvalue (`|CreateWidget` (`local.hudClass`) (cast `PlayerController` (`self.GetOwner`) :!pure true)))
    (`UserWidget.AddToViewport` _returnvalue 0)
    (return _returnvalue)))

(fn `VM_GetInteractionData`
  (returns (object :type "Object Object Reference") (info :type "/Game/Blueprints/Interactables/InteractableInfoData Object Reference") (display :type "/Game/Blueprints/HUD/DisplayHandlers/STR_DisplayHandler_Interactable Structure"))
  (return (`KismetSystemLibrary.Conv_InterfaceToObject` (`self.interactionObject`)) (`self.interactionInfo`) (`self.interactionDisplay`)))

(fn `VM_GetInteractRequirement`
  (returns (requirement :type "/Game/Blueprints/Interactables/B_InteractRequirementComponent Object Reference"))
  (return (`self.interactRequirementComponent`)))

(fn `VM_HasInteraction`
  (returns (valid :type Boolean))
  (return (`KismetSystemLibrary.IsValid` (`KismetSystemLibrary.Conv_InterfaceToObject` (`self.interactionObject`)))))

(fn `VM_SetEquipmentComponent`
  (params (input :type "/Game/Blueprints/Pawn/B_PawnEquipmentComponent Object Reference"))
  (bind _output_get (set `self.equipmentComponent` input))
  (message `/Game/Blueprints/HUD/ViewModel/BPI_Widget_ViewModel.AddViewModel` (`self.view_interact`) (`/Game/Blueprints/Pawn/B_PawnEquipmentComponent.viewModel` _output_get)))

(fn `VM_SetInteractionDescription`
  (params (info :type "/Game/Blueprints/Interactables/InteractableInfoData Object Reference") (subInfo :type "/Game/Blueprints/HUD/DisplayHandlers/STR_DisplayHandler_Interactable Structure") (notify :type "/Game/Blueprints/Player/ViewModel/E_VM_Direction Enum" :default "NewEnumerator0"))
  (set `self.interactionInfo` info)
  (set `self.interactionDisplay` subInfo)
  (`self.OnNotifyVariable` "interactionDescription"))

(fn `VM_SetInteractionDisplay`
  (params (interactionDisplay :type "/Game/Blueprints/HUD/DisplayHandlers/STR_DisplayHandler_Interactable Structure") (Setting :type "/Game/Blueprints/Player/ViewModel/E_VM_Direction Enum" :default "NewEnumerator0"))
  (set `self.interactionDisplay` interactionDisplay)
  (`self.OnNotifyVariable` "interactionDisplay"))

(fn `VM_SetInteractionObject`
  (params (object :type "/Game/Blueprints/Interactables/BPI_Interactable Interface"))
  (set `self.interactionObject` object)
  (`self.OnNotifyVariable` "interactionObject"))

(fn `VM_SetInteractRequirement`
  (params (requirement :type "/Game/Blueprints/Interactables/B_InteractRequirementComponent Object Reference"))
  (set `self.interactRequirementComponent` requirement)
  (`self.OnNotifyVariable` "interactRequirement"))