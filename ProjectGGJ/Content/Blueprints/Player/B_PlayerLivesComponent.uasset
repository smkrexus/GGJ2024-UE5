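; Player lives component on the PlayerState that handles the respawn and final-death flows.
; Respawn and Kill both spawn a transition handler showing the fail/respawn widget, fed by stat and GameState view models, then wait for input.
; On input, respawn clears the transition and teleports the existing pawn to a GameMode-selected PlayerStart rather than restarting it, while death opens the main menu.
; Respawn also sets a Checkpoint respawn tag, exposed through a getter.
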(event `InputRespawn`
  (`/Game/Blueprints/Core/UI/Transition/BP_TransitionHandler_Base.Clear` (`self._transitionHandler`))
  (`self.MoveToPlayerStart`)
  (`self.OnRespawnComplete`))

(event `InputDeath`
  (`self.OnKillComplete`)
  (`GameplayStatics.OpenLevelBySoftObjectPtr` "/Game/Levels/MainMenu.MainMenu"))

(fn `GetRespawnTag`
  (returns (OutTag :type "GameplayTag Structure"))
  (return (`self._respawnTag`)))

(fn `Kill`
  (`self.FADE_TO_BLACK`)
  (add `/Game/Blueprints/Core/UI/Transition/BP_TransitionHandler_Base.OnInputReceived` (`self._transitionHandler`) (`|CreateDelegate` :!event `InputDeath`)))

(fn `MoveToPlayerStart`
  (locals (controller :type "PlayerController Object Reference") (pawn :type "Pawn Object Reference"))
  (bind _returnvalue (`GameplayStatics.GetPlayerPawn` 0))
  (bind _rotation (.rotation (`Actor.GetTransform` (`GameModeBase.K2_FindPlayerStart` (`GameplayStatics.GetGameMode`) (`local.controller`) ""))))
  (bind _asplayer_state (cast `PlayerState` (`self.GetOwner`)))
  (set `local.controller` (`PlayerState.GetPlayerController` _asplayer_state))
  (`Actor.K2_TeleportTo` _returnvalue (.location (`Actor.GetTransform` (`GameModeBase.K2_FindPlayerStart` (`GameplayStatics.GetGameMode`) (`local.controller`) ""))) _rotation)
  (`Controller.SetControlRotation` (`Pawn.GetController` _returnvalue) _rotation))

(fn `Respawn`
  (`self.FADE_TO_BLACK`)
  (add `/Game/Blueprints/Core/UI/Transition/BP_TransitionHandler_Base.OnInputReceived` (`self._transitionHandler`) (`|CreateDelegate` :!event `InputRespawn`))
  (set `self._respawnTag` (struct :`TagName` "GameMode.RespawnTypes.Checkpoint")))