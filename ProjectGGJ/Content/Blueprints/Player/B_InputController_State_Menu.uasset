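; Menu-state input controller that lets the player close open UI windows.
; RegisterTargetForInput casts the supplied target to BP_PlayerStateCustom and caches it as PlayerState.
; When IA_LockInteract starts, it tells that player state's window tracker to collapse the top window for the owning player controller.
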(event `EnhancedInput|/Game/Blueprints/Core/Inputs/Actions/IA_LockInteract`
  (params (ActionValue :type Boolean) (ElapsedSeconds :type "Float (double-precision)") (TriggeredSeconds :type "Float (double-precision)") (InputAction :type "InputAction Object Reference" :default "/Game/Blueprints/Core/Inputs/Actions/IA_LockInteract.IA_LockInteract"))
  (bind __playerstate (`self._playerState`))
  (:`Started`
    (`/Game/Blueprints/Core/Contexts/B_ContextWindowTracker.CollapseTopWindow` (`/Game/Blueprints/Player/BP_PlayerStateCustom.GetWindowTracker` __playerstate) (`PlayerState.GetPlayerController` __playerstate))))

(fn `RegisterTargetForInput`
  (params (InTarget :type "Actor Object Reference"))
  (bind _asbp_player_state_custom (cast `/Game/Blueprints/Player/BP_PlayerStateCustom` InTarget))
  (set `self._playerState` _asbp_player_state_custom))