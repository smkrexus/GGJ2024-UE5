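; Custom player state that drives the player's mode (game, menu, popup, mini game, cinematic, respawn) through a tag-based view model.
; Popups, context menus and stat changes set the mode, which swaps input controllers and toggles a passive state mirrored to the game state view model.
; Pausing lowers game audio and shows an overlay.
; A restart notify costs health, and health changes trigger respawn, which validates the game restart on completion.
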(event `self.ReceiveBeginPlay`
  (`|ExecutionSequence`
    (:`then_0`
      (set `self._inputCache` (`self.GetComponentByClass` (`self.GetPlayerController`) "/Game/Blueprints/Core/Inputs/B_InputCacheComponent.B_InputCacheComponent_C"))
      (bind _output_get (set `self._gameState` (`/Game/Blueprints/Core/Utilities/BP_Utils.Game State`)))
      (bind _output_get_2 (set `self.vm_gameState` (`/Game/Blueprints/Gameflow/GS_GameStateCustom.GetViewModel` _output_get)))
      (add `/Game/Blueprints/Core/ViewModel/B_VM_BaseComponent.OnNotifyEvent` _output_get_2 (`|CreateDelegate` :!event `OnNotifyEventReceived_GameState`)))
    (:`then_1`
      (`self.Initialize`))))

(event `Initialize`
  (bind _outvalidated (message `/Game/Blueprints/Gameflow/Components/BPI_Gameflow_Validator.ValidateInitialization` (`GameplayStatics.GetPlayerController` 0)))
  (if _outvalidated
    (`/Game/Blueprints/Core/Stats/B_StatComponent.InitializeStats` (`self.PlayerStats`))
    (bind _view (`/Game/Blueprints/Core/ViewModel/B_VM_BaseComponent.CreateView` (`/Game/Blueprints/Core/Stats/B_StatComponent.GetViewModel` (`self.PlayerStats`)) "/Game/Blueprints/HUD/Player/WBP_PlayerStat_Lives.WBP_PlayerStat_Lives_C"))
    (`/Game/Blueprints/Player/ViewModel/B_VM_Player.VM_AddExtensionManual` (`self.GetComponentByClass` (`GameplayStatics.GetPlayerController` 0) "/Game/Blueprints/Player/ViewModel/B_VM_Player.B_VM_Player_C") "stat_lives" _view)
    (`/Game/Blueprints/Core/ViewModel/B_VM_BaseComponent.ForceRefresh` (`/Game/Blueprints/Core/Stats/B_StatComponent.GetViewModel` (`self.PlayerStats`)))
    (else
      (`KismetSystemLibrary.K2_SetTimerDelegate` (`|CreateDelegate` :!event `Initialize`) 0.5))))

(event `self.B_PopupManager.OnPopupDisplay`
  (params (InDisplayEnabled :type Boolean))
  ;[1 1 1] Display Menu Modes
  (`/Game/Blueprints/Player/ViewModel/B_VM_PlayerState.VM_SetCurrentMode` (`self.B_VM_PlayerState`) (select `bool` InDisplayEnabled :`false` (struct :`TagName` "ViewModel.PlayerState.Modes.Game") :`true` (struct :`TagName` "ViewModel.PlayerState.Modes.Menu.Popup") :!type "GameplayTag Structure"))
  (`/Game/Blueprints/Gameflow/ViewModel/B_VM_GameState.VM_SetGamePaused` (`self.GetGameStateViewModel`) InDisplayEnabled))

(event `self.B_ContextWindowTracker.OnContextMenuStateChanged`
  (params (menuEnabled :type Boolean))
  ;[1 1 1] Display Menu Modes
  (if menuEnabled
    (`/Game/Blueprints/Player/ViewModel/B_VM_PlayerState.VM_SetCurrentMode` (`self.B_VM_PlayerState`) (struct :`TagName` "ViewModel.PlayerState.Modes.Menu"))
    (else
      (`/Game/Blueprints/Player/ViewModel/B_VM_PlayerState.VM_SetCurrentMode` (`self.B_VM_PlayerState`) (struct :`TagName` "ViewModel.PlayerState.Modes.Game")) ; may need to be driven from the menu flow instead, implement when encounter this issue
    )))

(event `self.B_VM_PlayerState.OnNotifyEvent`
  (params (tag :type "GameplayTag Structure"))
  (`|SwitchGameplayTag` tag
    (:`ViewModel.PlayerState.StateHasChanged`
      ;[0.02732 0.06771 0.01199] PLAYER STATE GRAPH
      (`self.ManagePlayerStates`))
    (:`ViewModel.PlayerState.Pause`
      (`self.ManagePauseState`))
    (:`ViewModel.PlayerState.Passive`
      (`/Game/Blueprints/Gameflow/ViewModel/B_VM_GameState.VM_SetGamePassive` (`self.GetGameStateViewModel`) (`/Game/Blueprints/Player/ViewModel/B_VM_PlayerState.VM_GetPassiveState` (`self.B_VM_PlayerState`))))))

(event `OnNotifyEventReceived_GameState`
  (params (tag :type "GameplayTag Structure"))
  (`|SwitchGameplayTag` tag
    (:`GameMode.End.Restart`
      (`/Game/Blueprints/Core/Stats/B_StatComponent.ChangeStatFromTag` (`self.PlayerStats`) -1.0 (struct :`TagName` "Stats.Common.Health")))))

(event `self.B_PromptManager.OnPromptRegistered`
  (params (InTarget :type "/Game/Blueprints/Core/Notification/Prompt/B_PromptTarget Object Reference") (InPreviousTarget :type "/Game/Blueprints/Core/Notification/Prompt/B_PromptTarget Object Reference"))
  (bind _outviewmodel (`/Game/Blueprints/Core/Notification/Prompt/B_PromptTarget.GetViewModel` InTarget))
  (`/Engine/EditorBlueprintResources/StandardMacros.IsValid` InPreviousTarget
    (:`Is Valid`
      (`/Game/Blueprints/Core/Notification/Prompt/B_PromptTarget.OnRequestHandoverViewModel` InTarget (`/Game/Blueprints/Core/Notification/Prompt/B_PromptTarget.GetViewModel` InPreviousTarget)))
    (:`Is Not Valid`
      (`/Game/Blueprints/Core/Notification/Prompt/B_PromptTarget.OnRequestAddViewModel` InTarget self)
      (`/Game/Blueprints/Player/ViewModel/B_VM_Player.VM_AddExtension` (`self.GET_PLAYER_VIEWMODEL`) (`/Game/Blueprints/Core/Notification/Prompt/B_VM_PromptHandler_Base.SlotName` _outviewmodel) _outviewmodel)))
  (`/Game/Blueprints/Core/Notification/Prompt/B_VM_PromptHandler_Base.VM_DisplayPrompt` _outviewmodel))

(event `self.PlayerStats.OnStatChanged`
  (params (statTag :type "GameplayTag Structure"))
  (`|SwitchGameplayTag` statTag
    (:`Stats.Common.Health`
      (if (> (`/Game/Blueprints/Core/Stats/B_Stat.Current as Int` (`/Game/Blueprints/Core/Stats/B_StatComponent.GetStatFromTag` (`self.PlayerStats`) statTag)) 0)
        (add `/Game/Blueprints/Gameflow/Components/B_GameRestarter.OnRestartSuccess` (`/Game/Blueprints/Gameflow/GS_GameStateCustom.GameRestarter` (`self._gameState`)) (`|CreateDelegate` (`self.B_PlayerLives`) :!event `Respawn`))
        (`/Game/Blueprints/Player/ViewModel/B_VM_PlayerState.VM_SetCurrentMode` (`self.GetViewModel`) (struct :`TagName` "ViewModel.PlayerState.Modes.Respawn"))))))

(event `self.PlayerStats.OnStatEmpty`
  (params (statTag :type "GameplayTag Structure"))
  (`|SwitchGameplayTag` statTag
    (:`Stats.Common.Health`
      (add `/Game/Blueprints/Gameflow/Components/B_GameRestarter.OnRestartSuccess` (`/Game/Blueprints/Gameflow/GS_GameStateCustom.GameRestarter` (`self._gameState`)) (`|CreateDelegate` (`self.B_PlayerLives`) :!event `Kill`))
      (`/Game/Blueprints/Player/ViewModel/B_VM_PlayerState.VM_SetCurrentMode` (`self.GetViewModel`) (struct :`TagName` "ViewModel.PlayerState.Modes.Respawn")))))

(event `self.B_PlayerLives.OnRespawnComplete`
  (`/Game/Blueprints/Gameflow/Components/B_GameRestarter.ValidateRestart` (`/Game/Blueprints/Gameflow/GS_GameStateCustom.GameRestarter` (`self._gameState`)))
  (remove `/Game/Blueprints/Gameflow/Components/B_GameRestarter.OnRestartSuccess` (`/Game/Blueprints/Gameflow/GS_GameStateCustom.GameRestarter` (`self._gameState`)) (`|CreateDelegate` (`self.B_PlayerLives`) :!event `Respawn`)))

(event `ManagePlayerStates`
  (`|SwitchGameplayTag` (`/Game/Blueprints/Player/ViewModel/B_VM_PlayerState.VM_GetCurrentMode` (`self.B_VM_PlayerState`))
    (:`ViewModel.PlayerState.Modes.Game`
      (`self.DISABLE_PASSIVE_STATE`)
      (`self.ActivateInputController` (`self._globalGameInput`) "/Game/Blueprints/Player/B_InputController_State_Game.B_InputController_State_Game_C")
      (`self.DeactivateInputController` (`self._globalMenuInput`))
      (bind __inputcache (`self._inputCache`)
        (:`then`
          (`/Game/Blueprints/Core/Inputs/B_InputCacheComponent.ActivateInputs` __inputcache))
        (:`else`)))
    (:`ViewModel.PlayerState.Modes.Menu`
      (`self.ENABLE_PASSIVE_STATE`)
      (`self.ActivateInputController` (`self._globalMenuInput`) "/Game/Blueprints/Player/B_InputController_State_Menu.B_InputController_State_Menu_C")
      (`self.DeactivateInputController` (`self._globalGameInput`))
      (`/Game/Blueprints/Core/Inputs/B_InputCacheComponent.RemoveInputs` (`self._inputCache`)))
    (:`ViewModel.PlayerState.Modes.MiniGame`
      (`self.ENABLE_PASSIVE_STATE`)
      (`self.DeactivateInputController` (`self._globalGameInput`))
      (`/Game/Blueprints/Core/Inputs/B_InputCacheComponent.RemoveInputs` (`self._inputCache`)))
    (:`ViewModel.PlayerState.Modes.Cinematic`
      (`self.ENABLE_PASSIVE_STATE`)
      (`self.DeactivateInputController` (`self._globalGameInput`))
      (`/Game/Blueprints/Core/Inputs/B_InputCacheComponent.RemoveInputs` (`self._inputCache`)))
    (:`ViewModel.PlayerState.Modes.Menu.Popup`
      (`self.ENABLE_PASSIVE_STATE`)
      (`self.DeactivateInputController` (`self._globalGameInput`))
      (`/Game/Blueprints/Core/Inputs/B_InputCacheComponent.RemoveInputs` (`self._inputCache`)))
    (:`ViewModel.PlayerState.Modes.Respawn`
      (`self.ENABLE_PASSIVE_STATE`)
      (`self.DeactivateInputController` (`self._globalGameInput`))
      (`/Game/Blueprints/Core/Inputs/B_InputCacheComponent.RemoveInputs` (`self._inputCache`)))))

(event `ManagePauseState`
  (bind _loadedwidget (`/Game/Blueprints/Core/ViewModel/B_VM_BaseComponent.GetWidgetObject` (`self.vm_pause`)))
  (if (`/Game/Blueprints/Player/ViewModel/B_VM_PlayerState.VM_GetPauseState` (`self.B_VM_PlayerState`))
    (`/Game/Blueprints/Core/Inputs/B_InputCacheComponent.RemoveInputs` (`self._inputCache`))
    (`GameplayStatics.SetSoundMixClassOverride` "/Game/Assets/Audio/Mixer/AudioChannelMix_Group_Game.AudioChannelMix_Group_Game" "/Game/Assets/Audio/Mixer/AudioChannel_Group_Game.AudioChannel_Group_Game" 0.1)
    (`GameplayStatics.PushSoundMixModifier` "/Game/Assets/Audio/Mixer/AudioChannelMix_Group_Game.AudioChannelMix_Group_Game")
    (`|ExecutionSequence`
      (:`then_0`
        (`self.vm_pause`
          (:`then`
            (`/Engine/EditorBlueprintResources/StandardMacros.IsValid` _loadedwidget
              (:`Is Valid`
                (`UserWidget.AddToViewport` _loadedwidget 0))
              (:`Is Not Valid`
                (bind _view (`/Game/Blueprints/Core/ViewModel/B_VM_BaseComponent.CreateView` (stale _output_get) (`/Game/Blueprints/Core/ViewModel/B_VM_BaseComponent.GetDefaultWidget` (`self.vm_pause`)) :!label _label))
                (`/Game/Blueprints/HUD/GameState/B_VM_GameState_Pause.VM_AssignPlayerState` (`self.vm_pause`) (`self.B_VM_PlayerState`))
                (`UserWidget.AddToViewport` _view 0))))
          (:`else`
            (bind _returnvalue (`|AddComponentByClass` "/Game/Blueprints/HUD/GameState/B_VM_GameState_Pause.B_VM_GameState_Pause_C"))
            (bind _output_get (set `self.vm_pause` _returnvalue))
            (goto _label))))
      (:`then_1`
        (`/Game/Blueprints/Core/Utilities/BP_Utils.EnableMenuInteraction` (`self.GetPlayerController`))
        (`self.ENABLE_PASSIVE_STATE`)
        (`/Game/Blueprints/Gameflow/ViewModel/B_VM_GameState.VM_SetGamePaused` (`self.GetGameStateViewModel`) true)))
    (else
      (`GameplayStatics.SetSoundMixClassOverride` "/Game/Assets/Audio/Mixer/AudioChannelMix_Group_Game.AudioChannelMix_Group_Game" "/Game/Assets/Audio/Mixer/AudioChannel_Group_Game.AudioChannel_Group_Game")
      (`GameplayStatics.PushSoundMixModifier` "/Game/Assets/Audio/Mixer/AudioChannelMix_Group_Game.AudioChannelMix_Group_Game")
      (`/Game/Blueprints/Core/ViewModel/B_VM_BaseComponent.RemoveView` (`self.vm_pause`))
      (`/Game/Blueprints/Core/Utilities/BP_Utils.DisableMenuInteraction` (`self.GetPlayerController`))
      (`/Game/Blueprints/Gameflow/ViewModel/B_VM_GameState.VM_SetGamePaused` (`self.GetGameStateViewModel`) false))))

(fn `GetGameStateViewModel`
  (returns (OutViewModel :type "/Game/Blueprints/Gameflow/ViewModel/B_VM_GameState Object Reference"))
  (`/Engine/EditorBlueprintResources/StandardMacros.IsValid` (`self._gameState`)
    (:`Is Valid`
      (return (`/Game/Blueprints/Gameflow/GS_GameStateCustom.GetViewModel` (`self._gameState`))))
    (:`Is Not Valid`
      (return (`/Game/Blueprints/Gameflow/GS_GameStateCustom.GetViewModel` (`/Game/Blueprints/Core/Utilities/BP_Utils.Game State`))))))

(fn `GetPopupManager`
  (returns (OutComponent :type "/Game/Blueprints/HUD/Popup/B_PopupManager Object Reference"))
  (return (`self.B_PopupManager`)))

(fn `GetViewModel`
  (returns (viewModel :type "/Game/Blueprints/Player/ViewModel/B_VM_PlayerState Object Reference"))
  (return (`self.B_VM_PlayerState`)))

(fn `GetWindowTracker`
  (returns (ScreenTracker :type "/Game/Blueprints/Core/Contexts/B_ContextWindowTracker Object Reference"))
  (return (`self.B_ContextWindowTracker`)))

(fn `UserConstructionScript`)