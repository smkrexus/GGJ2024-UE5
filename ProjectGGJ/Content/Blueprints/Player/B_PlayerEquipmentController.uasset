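; Player equipment controller that turns Enhanced Input actions into commands on the player's equipment component.
; Initialize casts the controller to BP_PawnControllerCustom, sets the equipment mapping context on it and stores the equipment component.
; The drop action drops one of the active item, while the use action only prints a debug string.
; An unconnected debug snippet for listing the drop action's mapped keys never runs.
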(event `self.ReceiveBeginPlay`)

(event `EnhancedInput|/Game/Inputs/IA_EquipmentUse`
  (params (ActionValue :type Boolean) (ElapsedSeconds :type "Float (double-precision)") (TriggeredSeconds :type "Float (double-precision)") (InputAction :type "InputAction Object Reference" :default "/Game/Inputs/IA_EquipmentUse.IA_EquipmentUse"))
  (:`Started`
    (`KismetSystemLibrary.PrintString` "Equipment Use")))

(event `EnhancedInput|/Game/Inputs/IA_EquipmentDrop`
  (params (ActionValue :type Boolean) (ElapsedSeconds :type "Float (double-precision)") (TriggeredSeconds :type "Float (double-precision)") (InputAction :type "InputAction Object Reference" :default "/Game/Inputs/IA_EquipmentDrop.IA_EquipmentDrop"))
  (bind _equipmentcomponent (`self.equipmentComponent`))
  (:`Started`
    (`/Game/Blueprints/Pawn/B_PawnEquipmentComponent.DropItem` _equipmentcomponent (`/Game/Blueprints/Pawn/B_PawnEquipmentComponent.GetActiveItem` _equipmentcomponent) 1)))

(fn `Initialize`
  (params (equipment :type "/Game/Blueprints/Pawn/B_PawnEquipmentComponent Object Reference") (controller :type "Controller Object Reference"))
  (`|ExecutionSequence`
    (:`then_0`
      (bind _asbp_pawn_controller_custom (cast `/Game/Blueprints/BP_PawnControllerCustom` (`local.controller`)))
      (bind _output_get (set `self.playerController` _asbp_pawn_controller_custom))
      (`/Game/Blueprints/BP_PawnControllerCustom.SetMappingContext` _output_get "/Game/Inputs/IM_EquipmentMap.IM_EquipmentMap"))
    (:`then_1`
      (set `self.equipmentComponent` (`local.equipment`)))))