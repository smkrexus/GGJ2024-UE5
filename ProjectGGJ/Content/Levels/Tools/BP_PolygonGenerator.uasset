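; BP_PolygonGenerator is a level tool actor that builds an extruded polygon mesh from the shape of its spline.
; The construction script resets the dynamic mesh, flattens each spline point's local position to 2D, and extrudes the resulting polygon by Height using Geometry Script.
; Only the spline points define the outline, so curvature between them is not sampled, and point Z is discarded.
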(fn `MakePolygonFromSpline`
  (locals (DynamicMesh :type "DynamicMesh Object Reference"))
  (bind _returnvalue (`BaseDynamicMeshComponent.GetDynamicMesh` (`self.DynamicMeshComponent`)))
  (bind _returnvalue_2 (`DynamicMesh.Reset` _returnvalue))
  (set `local.DynamicMesh` _returnvalue_2)
  (`KismetArrayLibrary.Array_Clear` (`self.Vertices`))
  (for _index (range (`SplineComponent.GetNumberOfSplinePoints` (`self.Spline`)))
    (`KismetArrayLibrary.Array_Add` (`self.Vertices`) (`KismetMathLibrary.Conv_VectorToVector2D` (`SplineComponent.GetLocationAtSplinePoint` (`self.Spline`) _index "Local"))))
  (`GeometryScriptLibrary_MeshPrimitiveFunctions.AppendSimpleExtrudePolygon` (`local.DynamicMesh`) (struct) (struct) (`self.Vertices`) (`self.Height`) 0 true "Base" null)
  (`self.ReleaseAllComputeMeshes`))

(fn `UserConstructionScript`
  (locals (DynamicMesh :type "DynamicMesh Object Reference"))
  (`self.MakePolygonFromSpline`))