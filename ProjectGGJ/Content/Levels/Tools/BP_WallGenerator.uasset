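; BP_WallGenerator is a Geometry Script level tool that procedurally builds a wall with window cutouts.
; On mesh rebuild, it makes one straight box along X, sized by the spline's length plus Thickness and Height, without following the spline's curve.
; It appends a box per Windows entry to a pooled temporary mesh, subtracts that from the wall with a single boolean, then releases the compute meshes.
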(event `self.OnRebuildGeneratedMesh`
  (params (TargetMesh :type "DynamicMesh Object Reference"))
  (bind _returnvalue (`SplineComponent.GetSplineLength` (`self.Spline`)))
  (`DynamicMesh.Reset` TargetMesh)
  (bind _returnvalue_2 (`GeometryScriptLibrary_MeshPrimitiveFunctions.AppendBox` TargetMesh (struct) (`KismetMathLibrary.MakeTransform` (`KismetMathLibrary.MakeVector` (/ _returnvalue 2.0))) _returnvalue (`self.thickness`) (`self.height`) 0 0 0 "Base" null))
  (set `self.mainWall` _returnvalue_2)
  (bind _returnvalue_3 (`GeometryScriptLibrary_SceneUtilityFunctions.CreateDynamicMeshPool`))
  (bind _returnvalue_4 (`DynamicMeshPool.RequestMesh` _returnvalue_3))
  (set `self.windowMesh` _returnvalue_4)
  (for _array_element (`self.windows`)
    (`GeometryScriptLibrary_MeshPrimitiveFunctions.AppendBox` (`self.windowMesh`) (struct) (`KismetMathLibrary.MakeTransform` (break `/Game/Levels/Tools/STR_WallBoolean` _array_element)) (.x (`.size_5_6AB1E7F844B2F7EE4EFED08882BC2EC3` (break `/Game/Levels/Tools/STR_WallBoolean` _array_element))) (.y (`.size_5_6AB1E7F844B2F7EE4EFED08882BC2EC3` (break `/Game/Levels/Tools/STR_WallBoolean` _array_element))) (.z (`.size_5_6AB1E7F844B2F7EE4EFED08882BC2EC3` (break `/Game/Levels/Tools/STR_WallBoolean` _array_element))) 0 0 0 "Base" null))
  (`GeometryScriptLibrary_MeshBooleanFunctions.ApplyMeshBoolean` (`self.mainWall`) (struct) (`self.windowMesh`) (struct) "Subtract" (struct) null)
  (`self.ReleaseAllComputeMeshes`))

(fn `UserConstructionScript`)