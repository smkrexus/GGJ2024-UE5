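; Level tool actor that visualises a cone angle as a flat fan outline with a configurable angle, segment count and display distance.
; The construction script calls DisplayAngle to compute arc points, closed at both ends, and draw a debug line along each segment ray.
; Those points become a linear spline, along which Geometry Script sweeps a narrow strip into the dynamic mesh with the cone material.
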(event `self.ReceiveBeginPlay`)

(event `self.ReceiveTick`
  (params (DeltaSeconds :type "Float (single-precision)")))

(fn `DisplayAngle`
  (returns (OutPoints :type "Array of Vector Structure"))
  (locals (startAngle :type "Float (double-precision)" :default 0.0) (displayDistance :type "Float (single-precision)" :default 200.0) (anglePerSegment :type "Float (double-precision)") (segmentX :type "Float (double-precision)") (segmentY :type "Float (double-precision)") (localVectorSegment :type "Vector Structure") (conePoints :type "Array of Vector Structure"))
  (bind _returnvalue (`self.K2_GetActorLocation`))
  (set `local.startAngle` (* (- 180.0 (`KismetMathLibrary.FClamp` (`self.ConeAngle`) 0.1 360.0)) 0.5))
  (`KismetArrayLibrary.Array_Add` (`local.conePoints`))
  (set `local.anglePerSegment` (/ (`KismetMathLibrary.FClamp` (`self.ConeAngle`) 0.1 360.0) (`self.ConeSegments`)))
  (for _index (range (+ (`self.ConeSegments`) 1))
    (bind _returnvalue_2 (+ (`local.startAngle`) (* (`local.anglePerSegment`) _index)))
    (set `local.segmentX` (`KismetMathLibrary.DegSin` _returnvalue_2))
    (set `local.segmentY` (`KismetMathLibrary.DegCos` _returnvalue_2))
    (set `local.localVectorSegment` (`KismetMathLibrary.Normal` (+ (* (`self.GetActorForwardVector`) (`local.segmentX`)) (* (`self.GetActorRightVector`) (`local.segmentY`)))))
    (`KismetSystemLibrary.DrawDebugLine` _returnvalue (+ _returnvalue (* (`local.localVectorSegment`) (`local.displayDistance`))) (struct :`R` 1.0 :`G` 1.0 :`B` 1.0 :`A` 1.0) 0.0 0.0 "Foreground")
    (`KismetArrayLibrary.Array_Add` (`local.conePoints`) (`KismetMathLibrary.MakeVector` (* (`local.segmentX`) (`local.displayDistance`)) (* (`local.segmentY`) (`local.displayDistance`)))))
  (`KismetArrayLibrary.Array_Add` (`local.conePoints`))
  (return (`local.conePoints`)))

(fn `GenerateConeAngle`
  (params (Angle :type "Float (double-precision)")))

(fn `UserConstructionScript`
  (bind _spline (`self.Spline`))
  (bind _returnvalue (`SplineComponent.GetNumberOfSplinePoints` _spline))
  (bind _outpoints (`self.DisplayAngle`))
  (`SplineComponent.SetSplinePoints` _spline _outpoints "Local" true)
  (for _index (range _returnvalue)
    (`SplineComponent.SetSplinePointType` (`self.Spline`) _index "Linear" true))
  (`SplineComponent.UpdateSpline` (`self.Spline`))
  (bind _returnvalue_2 (`BaseDynamicMeshComponent.GetDynamicMesh` (`self.DynamicMeshComponent`)))
  (bind _returnvalue_3 (`DynamicMesh.Reset` _returnvalue_2))
  (bind _frames (`GeometryScriptLibrary_PolyPathFunctions.SampleSplineToTransforms` (`self.Spline`) (make `GeometryScriptSplineSamplingOptions` _returnvalue 1.0 "UniformTime")))
  (`GeometryScriptLibrary_MeshPrimitiveFunctions.AppendSweepPolyline` :`TargetMesh` _returnvalue_3 :`PrimitiveOptions` (make `GeometryScriptPrimitiveOptions` "PerFace" false) :`PolylineVertices` (`|MakeArray` (2.0 0.0) (-2.0 0.0) :!type "Vector2D Structure") :`SweepPath` _frames :`MiterLimit` 1.1)
  (`DynamicMeshComponent.ConfigureMaterialSet` (`self.DynamicMeshComponent`) (`self.ConeMaterial`) true)
  (`self.ReleaseAllComputeMeshes`))