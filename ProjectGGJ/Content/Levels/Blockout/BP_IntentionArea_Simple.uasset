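; Blockout helper actor that marks an intention area in a level with a scaled visualiser and a text description.
; The construction script scales the AreaVisualiser in X and Y from AreaSize while keeping its Z scale, and writes AreaDescription to the TextRender.
; It applies VisualiserMaterial when valid, otherwise falling back to the MI_ProcGrid material.
; The event graph has no active logic.
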(fn `UserConstructionScript`
  (bind _areavisualiser (`self.AreaVisualiser`))
  (bind _areavisualiser_2 (`self.AreaVisualiser`))
  (bind (_returnvalue_x _returnvalue_y _returnvalue_z) (`KismetMathLibrary.BreakVector` (`SceneComponent.K2_GetComponentScale` _areavisualiser)))
  (bind (_x _y) (`KismetMathLibrary.BreakVector2D` (`self.AreaSize`)))
  (`SceneComponent.SetWorldScale3D` _areavisualiser (`KismetMathLibrary.MakeVector` _x _y _returnvalue_z))
  (`TextRenderComponent.K2_SetText` (`self.TextRender`) (`self.AreaDescription`))
  (`self.VisualiserMaterial`
    (:`then`
      (`PrimitiveComponent.SetMaterial` _areavisualiser_2 0 (`self.VisualiserMaterial`)))
    (:`else`
      (`PrimitiveComponent.SetMaterial` _areavisualiser_2 0 "/Engine/OpenWorldTemplate/LandscapeMaterial/MI_ProcGrid.MI_ProcGrid"))))