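; Post-process Blueprint that applies a configurable material to its PostProcess component, named as an editor variant.
; The construction script passes the soft-referenced material to SetPostProcessMaterial, which loads it with a blocking load and appends it as a full-weight blendable without clearing existing entries.
; An invalid reference clears the blendable array instead, and the event graph has no active logic.
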(fn `SetPostProcessMaterial`
  (params (material :type "MaterialInstance Soft Object Reference"))
  (bind _array (break `WeightedBlendables` (`.WeightedBlendables` (break `PostProcessSettings` (`PostProcessComponent.Settings` (`self.PostProcess`))))))
  (if (`KismetSystemLibrary.IsValidSoftObjectReference` material)
    (bind _returnvalue (`KismetSystemLibrary.LoadAsset_Blocking` (`local.material`)))
    (`KismetArrayLibrary.Array_Add` _array (make `WeightedBlendable` 1.0 _returnvalue))
    (else
      (`KismetArrayLibrary.Array_Clear` _array))))

(fn `UserConstructionScript`
  (`self.SetPostProcessMaterial` (`self.PostProcessMaterial`)))