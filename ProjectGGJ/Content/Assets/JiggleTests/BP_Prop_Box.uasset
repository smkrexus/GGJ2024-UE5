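; BP_Prop_Box is an interactable box prop whose top turns to look at the player and dips when interacted with.
; It drives TopRotation and TopOffset on its ABP_Prop_Box anim instance.
; Each tick it tracks the player within a 60-degree angle of world +X, otherwise resetting rotation and slowing its tick interval.
; The interact area component triggers the brief downward offset, with a short timer set afterward.
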(event `self.ReceiveBeginPlay`
  (bind _asabp_prop_box (cast `/Game/Assets/JiggleTests/ABP_Prop_Box` (`SkeletalMeshComponent.GetAnimInstance` (`self.SkeletalMesh`))))
  (set `self._boxAnim` _asabp_prop_box)
  (`/Game/Blueprints/Interactables/B_InteractAreaComponent.AssignArea` (`self.B_InteractAreaComponent`) (`self.InteractArea`)))

(event `self.ReceiveTick`
  (params (DeltaSeconds :type "Float (single-precision)"))
  (`self.Pop`))

(event `Pop`
  (bind _returnvalue (`self.K2_GetActorLocation`))
  (bind __boxanim (`self._boxAnim`))
  (bind _returnvalue_2 (`self.K2_GetActorLocation` (`GameplayStatics.GetPlayerCharacter` 0)))
  (if (<= (`KismetMathLibrary.DegAcos` (.x (`KismetMathLibrary.Vector_Normal2D` (- _returnvalue_2 _returnvalue)))) 60.0)
    (set `/Game/Assets/JiggleTests/ABP_Prop_Box.TopRotation` (`KismetMathLibrary.FindLookAtRotation` _returnvalue _returnvalue_2) __boxanim)
    (`self.SetActorTickInterval` 0.0)
    (else
      (set `/Game/Assets/JiggleTests/ABP_Prop_Box.TopRotation` (struct) __boxanim)
      (`self.SetActorTickInterval` 0.25))))

(event `self.B_InteractAreaComponent.OnInteracted`
  (params (controller :type "Controller Object Reference"))
  (set `/Game/Assets/JiggleTests/ABP_Prop_Box.TopOffset` (0.0 0.0 -5.0) (`self._boxAnim`))
  (`KismetSystemLibrary.K2_SetTimerDelegate` (`|CreateDelegate` :!event `ReturnToNormal`) 0.1))

(event `ReturnToNormal`
  (set `/Game/Assets/JiggleTests/ABP_Prop_Box.TopOffset` (0.0 0.0 0.0) (`self._boxAnim`)))

(fn `UserConstructionScript`)