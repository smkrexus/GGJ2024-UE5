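; Test character Blueprint for trying finisher animations and bone physics through debug keys, with input enabled on BeginPlay.
; G randomly picks the SelfHug or Stretch finisher tag and passes it with the female finisher proxy table to the skeletal mesh's AnimBP.
; Holding H simulates physics below a bone and spawns a joint physics handler that grabs it and targets a random sideways rotation.
; Releasing H lets go and resets body simulation.
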(event EventBeginPlay
  (Input|EnableInput (Game|GetPlayerController 0))
  (bind _asbpa_finisher_female_standard (Utilities|Casting|CastToBPA_Finisher_Female_Standard (Components|SkeletalMesh|GetAnimInstance (Variables|Default|GetSkeletalMesh))))
  (Variables|Default|SetanimBP _asbpa_finisher_female_standard))

(event EventTick
  (params (DeltaSeconds :type Float%20%28single-precision%29)))

(event Input|KeyboardEvents|DebugKeyG
  (params (Key :type Key%20Structure :default "None") (ActionValue :type Input%20Action%20Value%20Structure))
  (:Pressed
    (bind _asbpa_finisher_female_standard (Utilities|Casting|CastToBPA_Finisher_Female_Standard (Components|SkeletalMesh|GetAnimInstance (Variables|Default|GetSkeletalMesh))))
    (Variables|/Game/Assets/VFX/Finisher/BPA_Finisher_Female_Standard.BPA_Finisher_Female_Standard_C|SetFinisherTag _asbpa_finisher_female_standard (select (Math|Random|RandomBool) "(GameplayTags=((TagName=\"Finisher.Reserved.SelfHug\")))" "(GameplayTags=((TagName=\"Finisher.Loud.Stretch\")))"))
    (Variables|/Game/Assets/VFX/Finisher/BPA_Finisher_Female_Standard.BPA_Finisher_Female_Standard_C|SetProxy%20Table _asbpa_finisher_female_standard "/Game/Assets/VFX/Finisher/PT_Finisher_Female.PT_Finisher_Female")))

(event Input|KeyboardEvents|DebugKeyH
  (params (Key :type Key%20Structure :default "None") (ActionValue :type Input%20Action%20Value%20Structure))
  (bind _skeletalmesh (Variables|Default|GetSkeletalMesh))
  (bind _in_bone_name (Variables|Default|GetIn%20Bone%20Name))
  (bind _skeletalmesh_2 (Variables|Default|GetSkeletalMesh))
  (bind _returnvalue (Transformation|GetBoneTransform _skeletalmesh_2 _in_bone_name "RTS_World"))
  (bind (_location _rotation) (Math|Transform|BreakTransform _returnvalue))
  (:Pressed
    (Class|SkeletalMeshComponent|SetAllBodiesBelowSimulatePhysics (Variables|Default|GetSkeletalMesh) (Variables|Default|GetIn%20Bone%20Name) true true)
    (bind _returnvalue_2 (Game|SpawnActorfromClass "/Game/Blueprints/Patient/Joints/BP_Joint_PhysicsHandler.BP_Joint_PhysicsHandler_C" _returnvalue "Undefined" "MultiplyWithRoot" 0 0))
    (Variables|Default|Sethandle _returnvalue_2)
    (Transformation|AddLocalRotation (Variables|/Game/Blueprints/Patient/Joints/BP_Joint_PhysicsHandler.BP_Joint_PhysicsHandler_C|GetBonePositionReflector (Variables|Default|Gethandle)) (select (Math|Random|RandomBool) "0.000000,60.000000,0.000000" "0.000000,-60.000000,0.000000") false false)
    (Default|Grab (Variables|Default|Gethandle) (Variables|Default|GetSkeletalMesh) (Variables|Default|GetIn%20Bone%20Name) _location _rotation)
    (Class|PhysicsHandleComponent|SetTargetRotation (Variables|/Game/Blueprints/Patient/Joints/BP_Joint_PhysicsHandler.BP_Joint_PhysicsHandler_C|GetPhysicsHandle (Variables|Default|Gethandle)) (Transformation|GetWorldRotation (Variables|/Game/Blueprints/Patient/Joints/BP_Joint_PhysicsHandler.BP_Joint_PhysicsHandler_C|GetBonePositionReflector (Variables|Default|Gethandle)))))
  (:Released
    (Default|Release (Variables|Default|Gethandle))
    (Class|SkeletalMeshComponent|SetAllBodiesBelowSimulatePhysics _skeletalmesh (Variables|Default|GetIn%20Bone%20Name) false false)
    (Class|SkeletalMeshComponent|ResetAllBodiesSimulatePhysics _skeletalmesh)))

(fn ConstructionScript)